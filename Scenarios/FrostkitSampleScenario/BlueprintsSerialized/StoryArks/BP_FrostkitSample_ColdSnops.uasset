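; Frostkit sample story ark that raises a Cold-problem event between the Shelter and PrepareForWhiteout quests, offering a promise to warm the city.
; The first choice starts a timed side quest, capped at whiteout arrival, to lower Cold, with optional Warmth and Shelter objectives.
; Success or failure opens a dialog and applies a trust modifier; any unlock change fails the quest silently, flagged as ended by whiteout.
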(event `self.OnStarted`
  (bind _trait_level_to_solve (`self.Trait Level to solve`))
  (bind _duration (`self.Duration`))
  (bind _returnvalue (`PXTimeUtils.Subtract` (`/Game/Scenarios/Main/Configs/Constants/BP_S1_Constants_BaseClass.Get Nomads Whiteout Arrive Time` (`/Game/Scenarios/Main/BlueprintsNonSerialized/ScenarioFunctionLibrary/BPFL_S1_ScenarioStorage.Get S1 Constants Storage`)) (`PXTimeUtils.GetCurrentGameTime`)))
  ;[1 1 1] Check conditions still valid
  (bind _ispresent (`/Game/Scenarios/Shared/BlueprintsNonSerialized/SocietyUtils/BPFL_CanBeStarted_Utils.Stat Problem Exists` "/Game/Scenarios/Shared/Configs/Statistics/Entries/DA_Cold.DA_Cold" (`PXTraitType.SeverityLevel` (`/Game/Scenarios/Shared/BlueprintsNonSerialized/SocietyUtils/BPFL_CanBeStarted_Utils.Get Stat Trait from Int` (`PXNationUtils.GetPlayerMainCity`) "/Game/Scenarios/Shared/Configs/Statistics/Entries/DA_Cold.DA_Cold" (`self.Required Cold to Trigger`)))))
  (if _ispresent
    (bind _decision (`/Game/Scenarios/Shared/BlueprintsNonSerialized/SocietyUtils/BPFL_Communication_Utils.Send Config Message` "/Game/Scenarios/FrostkitSampleScenario/Configs/Messages/Lenses/DA_FrostkitSample_ColdSnops_Lens.DA_FrostkitSample_ColdSnops_Lens" null (`PXCityUtils.GetRandomCommunityFromCity` (`PXNationUtils.GetPlayerMainCity`)) null (`|MakeMap` "" :!valuetype "Text") null null (struct) true))
    (bind _choice (`PXAsyncWaitForChoice.AsyncAction_WaitForChoice` _decision)
      (:`Completed`
        (bind _output_get (set `self.Choice` _choice))
        (switch `int` _output_get
          (:`0`
            (if (`PXTimeUtils.GreaterEqual` _returnvalue _duration)
              (set `self.Duration` _duration)
              (else
                (set `self.Duration` _returnvalue)))
            (bind _returnvalue_2 (`PXQuestUtils.StartQuestInPlace` "Keep people warm" "Access more oil to keep people warm" (`self.Duration`) "SideQuest" "DebugQuestName" true))
            (bind _output_get_2 (set `self.Quest` _returnvalue_2))
            (`PXQuestUtils.AddStatisticQuestObjective` :`quest` _output_get_2 :`objectiveName` (`|FormatText` "Reduce Cold to {TRAIT}" (`PXTraitType.IngameName` _trait_level_to_solve)) :`objectiveDescription` "Reduce Cold" :`city` (`PXNationUtils.GetPlayerMainCity`) :`trait` _trait_level_to_solve :`questType` "LessThanOrEqualTo" :`optionalIcon` null)
            (`self.Add Warmth Need Optional Objective`)
            (`self.Add Shelter Need Optional Objective`)))))))

(event `self.OnFinished`
  (`/Engine/EditorBlueprintResources/StandardMacros.IsValid` (`self.Quest`)
    (:`Is Valid`
      (`|ExecutionSequence`
        (:`then_0`
          (bind _succeeded (`PXAsyncWaitForQuest.AsyncAction_WaitForQuest` (`self.Quest`))
            (:`Completed`
              (if _succeeded
                (`PXAsyncOpenPredefinedDialog.AsyncAction_OpenPredefinedDialog` "/Game/Scenarios/Main/Configs/Messages/Dialogs/Nomads/DA_S1_NMD_ColdSnops_Success.DA_S1_NMD_ColdSnops_Success"
                  (:`Completed`
                    (`PXPredefinedModifierUtils.SetPredefinedModifierActive` (`PXNationUtils.GetPlayerNation`) "/Game/Scenarios/Shared/BlueprintsSerialized/Quests/Demands/DA_PromiseKept_AllCommunitiesTrust.DA_PromiseKept_AllCommunitiesTrust" true)))
                (elif (not (`self.Quest finished by whiteout`))
                  (`PXAsyncOpenPredefinedDialog.AsyncAction_OpenPredefinedDialog` "/Game/Scenarios/Main/Configs/Messages/Dialogs/Nomads/DA_S1_NMD_ColdSnops_Fail.DA_S1_NMD_ColdSnops_Fail"
                    (:`Completed`
                      (`PXPredefinedModifierUtils.SetPredefinedModifierActive` (`PXNationUtils.GetPlayerNation`) "/Game/Scenarios/Shared/BlueprintsSerialized/Quests/Demands/DA_PromiseBroken_AllCommunitiesTrust.DA_PromiseBroken_AllCommunitiesTrust" true))))))))
        (:`then_1`
          (add `PXUnlockSubsystem.UnlockChangedEvent` (`|Subsystem`) (delegate `CustomEvent`)))))))

(event `CustomEvent`
  (params (unlockComponent :type "PXUnlockComponent Object Reference") (Unlock :type "PXUnlockType Object Reference") (Unlocked :type Boolean))
  (`/Engine/EditorBlueprintResources/StandardMacros.IsValid` (`self.Quest`)
    (:`Is Valid`
      (set `self.Quest finished by whiteout` true)
      (`PXQuestUtils.FinishQuest` (`self.Quest`))
      (remove `PXUnlockSubsystem.UnlockChangedEvent` (`|Subsystem`) (delegate `CustomEvent`)))))

(fn `Add Shelter Need Optional Objective`
  (returns (ReturnValue :type "PXQuestObjective Object Reference"))
  (bind _returnvalue (`PXQuestUtils.AddNeedQuestObjective` (make `PXObjectiveParameters` (`|FormatText` "Build enough Housing Districts to meet shelter demand") "" true 1 null (`self.Quest`)) (make `PXNeedObjectiveParameters` "GreaterThanOrEqualTo" (`PXNationUtils.GetPlayerMainCity`) (`self.Shelter`) 1.0)))
  (return _returnvalue))

(fn `Add Warmth Need Optional Objective`
  (returns (ReturnValue :type "PXQuestObjective Object Reference"))
  (bind _returnvalue (`PXQuestUtils.AddNeedQuestObjective` (make `PXObjectiveParameters` (`|FormatText` "Extract enough oil to satisfy power demand") "" true 1 null (`self.Quest`)) (make `PXNeedObjectiveParameters` "GreaterThanOrEqualTo" (`PXNationUtils.GetPlayerMainCity`) (`self.Warmth`) 1.0)))
  (return _returnvalue))

(fn `CanBeStarted`
  (returns (ReturnValue :type Boolean))
  ;[1 1 1] Furnace must be on
  (if (`PXQuestUtils.IsAnyQuestOfTypeFinished` "/Game/Scenarios/Main/BlueprintsSerialized/Quests/NomadsQuests/BP_Shelter_NLScenario.BP_Shelter_NLScenario_C")
    (if (not (`PXQuestUtils.IsAnyQuestOfTypeFinished` "/Game/Scenarios/Main/BlueprintsSerialized/Quests/NomadsQuests/BP_PrepareForWhiteout_NLScenario.BP_PrepareForWhiteout_NLScenario_C"))
      (if (>= (`PXStatisticUtils.GetCurrentStatisticValue` (`PXNationUtils.GetPlayerMainCity`) "/Game/Scenarios/Shared/Configs/Statistics/Entries/DA_Cold.DA_Cold") (`self.Required Cold to Trigger`))
        (bind _ispresent (`/Game/Scenarios/Shared/BlueprintsNonSerialized/SocietyUtils/BPFL_CanBeStarted_Utils.Stat Problem Exists` "/Game/Scenarios/Shared/Configs/Statistics/Entries/DA_Cold.DA_Cold" (`PXTraitType.SeverityLevel` (`/Game/Scenarios/Shared/BlueprintsNonSerialized/SocietyUtils/BPFL_CanBeStarted_Utils.Get Stat Trait from Int` (`PXNationUtils.GetPlayerMainCity`) "/Game/Scenarios/Shared/Configs/Statistics/Entries/DA_Cold.DA_Cold" (`self.Required Cold to Trigger`)))))
        (if _ispresent
          (return true))))))