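; BP_LOG_QuarterHUB is a quarter hub Blueprint that plays a visual effect when the Exile the Weak trigger fires.
; On BeginPlay it binds to a subsystem's effect trigger event, then activates NPSExcileVFX and resets reserved Niagara GPU emission points on that trigger.
; Affinity-driven scaling of MeltBuildingsQuad with mask recapture is present, but its binding and initialization are disconnected, so it never runs.
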(event `self.ReceiveBeginPlay`
  (bind _returnvalue (`|Subsystem`)
    (:`then`
      (add `PXEffectsSupportSubsystem.EffectTriggerEvent` _returnvalue (delegate `Exile`)))))

(event `Exile`
  (params (triggerType :type "PXEffectTriggerType Object Reference") (caller :type "Object Object Reference"))
  (if (== triggerType "/Game/Scenarios/Shared/Configs/VisualEffectsTriggers/DA_ExileTheWeakTrigger.DA_ExileTheWeakTrigger")
    (`ActorComponent.Activate` (`self.NPS_ExcileVFX`) false)
    (bind _returnvalue (`|Subsystem`)
      (:`then`
        (`PXNiagaraGPUEmissionPointRootSubsystem.ResetReservedPoints` _returnvalue (`self.PXNiagaraGPUEmissionPointRoot`))))))

(event `CustomEvent`
  (params (holder :type "PXAffinityHolderComponent Object Reference") (affinityPermutation :type "PXAffinityPermutation Structure (by ref)"))
  (`SceneComponent.SetWorldScale3D` (`self.MeltBuildingsQuad`) (`KismetMathLibrary.VLerp` (`self.BaseScale`) (`self.MinScale`) (`/Game/Scenarios/Shared/BlueprintsNonSerialized/FactionEmergence/BPFL_Affinity_Support_Utils.GetValueFromAffinityEntry` (struct :`Name` "Symbiosis"))))
  (bind _returnvalue (`|Subsystem`)
    (:`then`
      (`PXLandscapeMaskSubsystem.CaptureMasks` _returnvalue))))

(fn `UserConstructionScript`)