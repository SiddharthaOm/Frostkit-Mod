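; Small generator addon for the main district hub, handling its smoke and three positional random spawn components.
; On BeginPlay it sets the smoke material on its Smoke component.
; When PXState reports a change for a matching state, it enables or disables the three ANIM spawn components inversely to that state's activation, so they switch off while the state is active.
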(event `self.ReceiveBeginPlay`
  (`parent.ReceiveBeginPlay`)
  (`self.SetSmokeMaterial` (`self.Smoke`)))

(event `self.PXState.ChangedStateEvent`
  (params (StateComponent :type "PXStateComponent Object Reference") (Entry :type "PXStateEntry Structure (by ref)") (Activate :type Boolean))
  (if (`PXStateUtils.AreStatesEqual` Entry (struct :`StateGuid` "9AD8B03B4C6AAFC3C2859C96A6402D87"))
    (for _array_element (`|MakeArray` (`self.PXPositionalRandomSpawn_ANIM_B`) (`self.PXPositionalRandomSpawn_ANIM_C`) (`self.PXPositionalRandomSpawn_ANIM_A`))
      (`PXComponentUtils.SetComponentEnabled` _array_element (not Activate)))))

(fn `UserConstructionScript`)