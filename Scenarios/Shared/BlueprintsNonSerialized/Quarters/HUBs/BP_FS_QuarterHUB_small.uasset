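; Small quarter HUB Blueprint that resizes its MeltBuildingsQuad according to an affinity value.
; Its custom event lerps the quad's world scale from BaseScale toward MinScale by the affinity entry value, then has a valid subsystem recapture masks.
; The setup that binds this event to affinity changes and caches BaseScale is disconnected, and the state-change event is empty.
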(event `CustomEvent`
  (params (holder :type "PXAffinityHolderComponent Object Reference") (affinityPermutation :type "PXAffinityPermutation Structure (by ref)"))
  (`SceneComponent.SetWorldScale3D` (`self.MeltBuildingsQuad`) (`KismetMathLibrary.VLerp` (`self.BaseScale`) (`self.MinScale`) (`/Game/Scenarios/Shared/BlueprintsNonSerialized/FactionEmergence/BPFL_Affinity_Support_Utils.GetValueFromAffinityEntry` (struct :`Name` "Symbiosis"))))
  (bind _returnvalue (`|Subsystem`)
    (:`then`
      (`PXLandscapeMaskSubsystem.CaptureMasks` _returnvalue))))

(event `self.PXState.ChangedStateEvent`
  (params (StateComponent :type "PXStateComponent Object Reference") (Entry :type "PXStateEntry Structure (by ref)") (Activate :type Boolean)))

(fn `UserConstructionScript`)