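; City sticky fog actor that blends the material on its fog cube between a city look and a weather look as camera weather changes.
; It binds to the weather subsystem's camera weather event and keeps a dynamic material instance of the cube's material.
; A weather change enables Tick, which interpolates between the two source instances using the global parameter collection's weather lerp.
; Tick switches itself off once that lerp equals the new weather level.
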(event `self.ReceiveActorStarted`
  (add `PXWeatherSubsystem.CameraWeatherChangedEvent` (subsystem `PXWeatherSubsystem`) (delegate `WeatgerChanged`))
  (bind _asmaterial_instance_dynamic (cast `MaterialInstanceDynamic` (`PrimitiveComponent.GetMaterial` (`self.FogCube`) 0)))
  (bind _returnvalue (`PrimitiveComponent.CreateDynamicMaterialInstance` (`self.FogCube`) 0 _asmaterial_instance_dynamic "None"))
  (set `self.StickyFogMID` _returnvalue))

(event `WeatgerChanged`
  (params (newWeatherLevel :type "PXWeatherLevel Object Reference"))
  (set `self.New Weather Level` newWeatherLevel)
  (`self.SetActorTickEnabled` true))

(event `self.ReceiveTick`
  (params (DeltaSeconds :type "Float (single-precision)"))
  (bind _returnvalue (`KismetMaterialLibrary.GetScalarParameterValue` "/Game/Scenarios/Shared/Materials/MaterialParameterCollection/MPC_GlobalMaterialParameters.MPC_GlobalMaterialParameters" "OnCameraWeatherLightLerp"))
  (bind _returnvalue_2 (`KismetMathLibrary.FClamp` _returnvalue))
  (`MaterialInstanceDynamic.K2_InterpolateMaterialInstanceParams` (`self.StickyFogMID`) (`self.CityStickyFogMI`) (`self.WeatherStickiFogMI`) _returnvalue_2)
  (if (== _returnvalue_2 (`PXWeatherLevel.Level` (`self.New Weather Level`)))
    (`self.SetActorTickEnabled` false)))

(fn `UserConstructionScript`)