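; BP_Windshield_A1 is a windshield Blueprint that feeds the placement of three sockets into its mesh's material.
; On ActorStarted, after a zero-length delay, it creates a dynamic material instance on the windshield mesh's first slot and fills the socket array.
; Each socket's relative location and rotation up vector are written to numbered Socket_N and Socket_N_R vector parameters, handing the shader a position and direction per socket.
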(event `self.ReceiveActorStarted`
  (bind _socketsarray (`self.socketsarray`))
  (bind _mid (`self.MID`))
  (bind _sm_cit_unq_windshield_a (`self.SM_CIT_UNQ_WindShield_A`))
  (`KismetSystemLibrary.Delay` 0.0)
  (bind _returnvalue (`PrimitiveComponent.CreateDynamicMaterialInstance` _sm_cit_unq_windshield_a 0 (`PrimitiveComponent.GetMaterial` _sm_cit_unq_windshield_a 0) "None"))
  (bind _output_get (set `self.MID` _returnvalue))
  (`PrimitiveComponent.SetMaterial` _sm_cit_unq_windshield_a 0 _output_get)
  (`KismetArrayLibrary.Array_Set` _socketsarray 0 (`self.Socket_1`) true)
  (`KismetArrayLibrary.Array_Set` _socketsarray 1 (`self.Socket_2`) true)
  (`KismetArrayLibrary.Array_Set` _socketsarray 2 (`self.Socket_3`) true)
  (for (_array_element _array_index) _socketsarray
    (bind _returnvalue_2 (`KismetStringLibrary.Concat_StrStr` "Socket_" (`KismetStringLibrary.Conv_IntToString` (+ _array_index 1))))
    ;[1 1 1] loc
    (`MaterialInstanceDynamic.SetVectorParameterValue` _mid (`KismetStringLibrary.Conv_StringToName` _returnvalue_2) (`KismetMathLibrary.Conv_VectorToLinearColor` (.location (`SceneComponent.GetRelativeTransform` _array_element))))
    ;[1 1 1] rot
    (`MaterialInstanceDynamic.SetVectorParameterValue` _mid (`KismetStringLibrary.Conv_StringToName` (`KismetStringLibrary.Concat_StrStr` _returnvalue_2 "_R")) (`KismetMathLibrary.Conv_VectorToLinearColor` (`KismetMathLibrary.GetUpVector` (.rotation (`SceneComponent.GetRelativeTransform` _array_element)))))))

(fn `UserConstructionScript`)