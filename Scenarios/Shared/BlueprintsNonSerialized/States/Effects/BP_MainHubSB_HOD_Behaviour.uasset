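; State behaviour for the MainHub SB HOD actor that switches its effect and lights on or off.
; Activation and deactivation share one function, which acts only when the FromConstruction argument matches the actor's state-by-entry result.
; It then activates or deactivates the "nps1" component and enables or disables children of "Lights" per the Activate argument, using the state's enablement reason.
; A separate visibility-setting BehaviorFunction is not called by these events.
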(event `self.OnActivate`
  (params (owner :type "Actor Object Reference") (gameInstance :type "PXGameInstance Object Reference") (arguments :type "PXStateBehaviourArguments Object Reference") (stateEntry :type "PXStateEntry Structure"))
  (`self.BehaviorFunction Multiple Arguments` arguments owner stateEntry))

(event `self.OnDeactivate`
  (params (owner :type "Actor Object Reference") (gameInstance :type "PXGameInstance Object Reference") (arguments :type "PXStateBehaviourArguments Object Reference") (stateEntry :type "PXStateEntry Structure"))
  (`self.BehaviorFunction Multiple Arguments` arguments owner stateEntry))

(fn `BehaviorFunction`
  (params (Arguments :type "PXStateBehaviourArguments Object Reference") (Actor :type "Actor Object Reference"))
  (bind _returnvalue (`self.GetComponentArgument` Arguments (`KismetStringLibrary.Conv_StringToName` "SceneComponent") Actor))
  (bind _returnvalue_2 (`self.GetBoolArgument` Arguments (`KismetStringLibrary.Conv_StringToName` "Visible")))
  (bind _asscene_component (cast `SceneComponent` _returnvalue)
    (:`then`
      (`SceneComponent.SetVisibility` _asscene_component _returnvalue_2 false))
    (:`CastFailed`
      (`KismetSystemLibrary.PrintString` (`KismetStringLibrary.Concat_StrStr` "The component: " (`KismetSystemLibrary.GetDisplayName` _returnvalue) "is not a SceneComponent")))))

(fn `BehaviorFunction Multiple Arguments`
  (params (Arguments :type "PXStateBehaviourArguments Object Reference") (Actor :type "Actor Object Reference") (stateEntry :type "PXStateEntry Structure"))
  (bind _returnvalue (`self.GetBoolArgument` Arguments (`KismetStringLibrary.Conv_StringToName` "FromConstruction")))
  (if _returnvalue
    (bind _returnvalue_2 (`PXStateUtils.GetActorStateByEntry` (`local.Actor`) (struct :`StateGuid` "5D0FDB9648B726EE7644089FB2AFB31D")))
    (if _returnvalue_2
      (`|ExecutionSequence` :!label _label
        (:`then_0`
          (bind _returnvalue_3 (`self.GetComponentArgument` (`local.Arguments`) (`KismetStringLibrary.Conv_StringToName` "nps1") (`local.Actor`)))
          (bind _returnvalue_4 (`self.GetBoolArgument` (`local.Arguments`) (`KismetStringLibrary.Conv_StringToName` "Activate")))
          (if _returnvalue_4
            (`ActorComponent.Activate` _returnvalue_3 true)
            (else
              (`ActorComponent.Deactivate` _returnvalue_3))))
        (:`then_1`
          (bind _returnvalue_5 (`self.GetComponentArgument` (`local.Arguments`) (`KismetStringLibrary.Conv_StringToName` "Lights") (`local.Actor`)))
          (bind _aspxtransform (cast `PXTransformComponent` _returnvalue_5))
          (for _array_element (`SceneComponent.GetChildrenComponents` _aspxtransform false)
            (bind _returnvalue_6 (`self.GetBoolArgument` (`local.Arguments`) (`KismetStringLibrary.Conv_StringToName` "Activate")))
            (bind _returnvalue_7 (`PXEnablementUtils.GetEnablementReasonForState` (`local.stateEntry`)))
            (`PXComponentUtils.SetComponentEnabled` _array_element _returnvalue_6 _returnvalue_7)))))
    (else
      (bind _returnvalue_8 (`PXStateUtils.GetActorStateByEntry` (`local.Actor`) (struct :`StateGuid` "9AD8B03B4C6AAFC3C2859C96A6402D87")))
      (if (not _returnvalue_8)
        (goto _label)))))