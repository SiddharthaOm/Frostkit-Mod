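; State effect behaviour that tints a point light according to the city mask at the owning actor's location, apparently to show tension.
; On activation it takes the point light from the "SceneComponent" argument and samples the first channel of the PXCityMask subsystem.
; That value selects the tension or no-tension color argument for the light.
; The color is set only on activation, with no update or revert on deactivation.
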(event `self.OnActivate`
  (params (owner :type "Actor Object Reference") (gameInstance :type "PXGameInstance Object Reference") (arguments :type "PXStateBehaviourArguments Object Reference") (stateEntry :type "PXStateEntry Structure"))
  (bind _returnvalue (`self.GetComponentArgument` arguments "SceneComponent" owner false))
  (bind _aspoint_light_component (cast `PointLightComponent` _returnvalue))
  (set `self.PointLight` _aspoint_light_component)
  (`/Engine/EditorBlueprintResources/StandardMacros.IsValid` (`self.PointLight`)
    (:`Is Valid`
      (bind _returnvalue_2 (`PXCityMaskSubsystem.GetCityMaskValueAtPosition` (subsystem `PXCityMaskSubsystem`) (`KismetMathLibrary.Conv_VectorToVector2D` (`Actor.K2_GetActorLocation` owner)) 0))
      (if (`|GetArrayItem` (`.MaskValuesPerChannel` (break `PXCityMaskCPUGridEntry` _returnvalue_2)))
        (bind _returnvalue_3 (`self.GetColorArgument` arguments (`KismetStringLibrary.Conv_StringToName` "LightColorTension")))
        (`LightComponent.SetLightColor` (`self.PointLight`) _returnvalue_3 true)
        (else
          (bind _returnvalue_4 (`self.GetColorArgument` arguments (`KismetStringLibrary.Conv_StringToName` "LightColorNoTension")))
          (`LightComponent.SetLightColor` (`self.PointLight`) _returnvalue_4 true))))))

(event `self.OnDeactivate`
  (params (owner :type "Actor Object Reference") (gameInstance :type "PXGameInstance Object Reference") (arguments :type "PXStateBehaviourArguments Object Reference") (stateEntry :type "PXStateEntry Structure")))

(event `self.OnUpdate`
  (params (owner :type "Actor Object Reference") (gameInstance :type "PXGameInstance Object Reference") (arguments :type "PXStateBehaviourArguments Object Reference") (stateEntry :type "PXStateEntry Structure")))