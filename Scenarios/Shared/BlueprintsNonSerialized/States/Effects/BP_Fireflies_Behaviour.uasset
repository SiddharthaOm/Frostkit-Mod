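; Fireflies behaviour state effect that applies a tension level to its owner's materials when the state activates.
; On activation it reads the TensionAmount float argument and writes it to the same-named scalar parameter on every mesh component's materials.
; It only affects existing dynamic material instances and creates none.
; Deactivation does not reset the value, and a duplicate copy of the update logic is left unconnected.
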(event `self.OnActivate`
  (params (owner :type "Actor Object Reference") (gameInstance :type "PXGameInstance Object Reference") (arguments :type "PXStateBehaviourArguments Object Reference") (stateEntry :type "PXStateEntry Structure"))
  (`/Engine/EditorBlueprintResources/StandardMacros.IsValid` owner
    (:`Is Valid`
      (for _array_element (`Actor.K2_GetComponentsByClass` owner "/Script/Engine.MeshComponent")
        (for _array_element_2 (`MeshComponent.GetMaterials` _array_element)
          (bind _asmaterial_instance_dynamic (cast `MaterialInstanceDynamic` _array_element_2))
          (bind _returnvalue (`self.GetFloatArgument` arguments (`KismetStringLibrary.Conv_StringToName` "TensionAmount")))
          (`MaterialInstanceDynamic.SetScalarParameterValue` _asmaterial_instance_dynamic "TensionAmount" _returnvalue))))))

(event `self.OnDeactivate`
  (params (owner :type "Actor Object Reference") (gameInstance :type "PXGameInstance Object Reference") (arguments :type "PXStateBehaviourArguments Object Reference") (stateEntry :type "PXStateEntry Structure")))