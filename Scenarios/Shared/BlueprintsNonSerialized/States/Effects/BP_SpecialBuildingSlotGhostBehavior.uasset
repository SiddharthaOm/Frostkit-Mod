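; State behavior for special building slot ghosts that tints their meshes to show active or inactive state.
; On activate and deactivate, it finds the owner's static mesh components from the state arguments and sets EmissiveColor to ActiveColor or InActiveColor.
; If a mesh's first material is not yet dynamic, it creates a dynamic instance in place, then applies the color.
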(event `self.OnActivate`
  (params (owner :type "Actor Object Reference") (gameInstance :type "PXGameInstance Object Reference") (arguments :type "PXStateBehaviourArguments Object Reference") (stateEntry :type "PXStateEntry Structure"))
  (bind _returnvalue (`self.GetComponentArguments` arguments owner false))
  (for _array_element _returnvalue
    (bind _asstatic_mesh_component (cast `StaticMeshComponent` _array_element))
    (bind _returnvalue_2 (`PrimitiveComponent.GetMaterial` _asstatic_mesh_component 0))
    (bind _asmaterial_instance_dynamic (cast `MaterialInstanceDynamic` _returnvalue_2 :!label _label)
      (:`then`
        (`MaterialInstanceDynamic.SetVectorParameterValue` _asmaterial_instance_dynamic "EmissiveColor" (`self.ActiveColor`)))
      (:`CastFailed`
        (`PrimitiveComponent.CreateDynamicMaterialInstance` _asstatic_mesh_component 0 _returnvalue_2 "None")
        (goto _label)))))

(event `self.OnDeactivate`
  (params (owner :type "Actor Object Reference") (gameInstance :type "PXGameInstance Object Reference") (arguments :type "PXStateBehaviourArguments Object Reference") (stateEntry :type "PXStateEntry Structure"))
  (bind _returnvalue (`self.GetComponentArguments` arguments owner false))
  (for _array_element _returnvalue
    (bind _asstatic_mesh_component (cast `StaticMeshComponent` _array_element))
    (bind _returnvalue_2 (`PrimitiveComponent.GetMaterial` _asstatic_mesh_component 0))
    (bind _asmaterial_instance_dynamic (cast `MaterialInstanceDynamic` _returnvalue_2 :!label _label_2)
      (:`then`
        (`MaterialInstanceDynamic.SetVectorParameterValue` _asmaterial_instance_dynamic "EmissiveColor" (`self.InActiveColor`)))
      (:`CastFailed`
        (`PrimitiveComponent.CreateDynamicMaterialInstance` _asstatic_mesh_component 0 _returnvalue_2 "None")
        (goto _label_2)))))