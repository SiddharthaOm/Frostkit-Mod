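; A state effect behaviour, named for the big boss, that switches Niagara visual effects on its owning actor on or off.
; Activate and deactivate events both call BehaviorFunction, so the "Activate" bool argument sets the direction rather than the event itself.
; It enables or disables the "emission" PX Niagara emission point component, then activates (with reset) or deactivates Niagara components passed as component arguments.
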(event `self.OnActivate`
  (params (owner :type "Actor Object Reference") (gameInstance :type "PXGameInstance Object Reference") (arguments :type "PXStateBehaviourArguments Object Reference") (stateEntry :type "PXStateEntry Structure"))
  (`self.BehaviorFunction` arguments owner))

(event `self.OnDeactivate`
  (params (owner :type "Actor Object Reference") (gameInstance :type "PXGameInstance Object Reference") (arguments :type "PXStateBehaviourArguments Object Reference") (stateEntry :type "PXStateEntry Structure"))
  (`self.BehaviorFunction` arguments owner))

(fn `BehaviorFunction`
  (params (Arguments :type "PXStateBehaviourArguments Object Reference") (Actor :type "Actor Object Reference"))
  (locals (Activate :type Boolean :default false))
  (bind _returnvalue (`self.GetBoolArgument` (`local.Arguments`) (`KismetStringLibrary.Conv_StringToName` "Activate")))
  (set `local.Activate` _returnvalue)
  (`|ExecutionSequence`
    (:`then_0`
      (bind _returnvalue_2 (`self.GetComponentArgument` (`local.Arguments`) (`KismetStringLibrary.Conv_StringToName` "emission") (`local.Actor`)))
      (bind _aspxniagara_emission_point_component (cast `PXNiagaraEmissionPointComponent` _returnvalue_2))
      (`PXComponentUtils.SetComponentEnabled` _aspxniagara_emission_point_component (`local.Activate`)))
    (:`then_1`
      (bind _returnvalue_3 (`self.GetComponentArguments` (`local.Arguments`) (`local.Actor`)))
      (for _array_element _returnvalue_3
        (bind _asniagara_particle_system_component (cast `NiagaraComponent` _array_element))
        (if (`local.Activate`)
          (`ActorComponent.Activate` _asniagara_particle_system_component true)
          (else
            (`ActorComponent.Deactivate` _asniagara_particle_system_component)))))))