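; State effect behaviour that recolours every light component on its owner actor according to tension.
; On activation it checks whether tension is high by OR-ing two actor state lookups on the owner.
; Each light then takes either the LightColorTension or LightColorNoTension colour from the behaviour's arguments.
; A city mask lookup at the light's position is left unconnected and never runs.
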(event `self.OnActivate`
  (params (owner :type "Actor Object Reference") (gameInstance :type "PXGameInstance Object Reference") (arguments :type "PXStateBehaviourArguments Object Reference") (stateEntry :type "PXStateEntry Structure"))
  (set `self.PointLightsArray` (`Actor.K2_GetComponentsByClass` owner "/Script/Engine.LightComponent"))
  (for _array_element (`self.PointLightsArray`)
    (bind _output_get (set `self.Light` _array_element))
    (if (`self.TensionHigh` owner)
      (bind _returnvalue (`self.GetColorArgument` arguments (`KismetStringLibrary.Conv_StringToName` "LightColorTension")))
      (`LightComponent.SetLightColor` (`self.Light`) _returnvalue true)
      (else
        (bind _returnvalue_2 (`self.GetColorArgument` arguments (`KismetStringLibrary.Conv_StringToName` "LightColorNoTension")))
        (`LightComponent.SetLightColor` (`self.Light`) _returnvalue_2 true)))))

(fn `TensionHigh`
  (params (InputPin :type "Actor Object Reference"))
  (returns (ReturnValue :type Boolean))
  (bind _returnvalue (`PXStateUtils.GetActorStateByEntry` InputPin (struct :`StateGuid` "BD330C5C41D1FBFEB581608A9A34F29B")))
  (bind _returnvalue_2 (`PXStateUtils.GetActorStateByEntry` InputPin (struct :`StateGuid` "BED5067B481B4978712C78B93BF8B621")))
  (return (or _returnvalue_2 _returnvalue)))