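; State behaviour for main hub lights that recolours all spot light components on the owning actor when activated.
; For each light, an actor state lookup on the owner picks either the LightColorTension or LightColorNoTension colour from the state's arguments.
; Only spot lights are affected, despite the PointLightsArray name, and the TensionHigh function is an unused stub.
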(event `self.OnActivate`
  (params (owner :type "Actor Object Reference") (gameInstance :type "PXGameInstance Object Reference") (arguments :type "PXStateBehaviourArguments Object Reference") (stateEntry :type "PXStateEntry Structure"))
  (set `self.PointLightsArray` (`Actor.K2_GetComponentsByClass` owner "/Script/Engine.SpotLightComponent"))
  (for _array_element (`self.PointLightsArray`)
    (set `self.Light` _array_element)
    (bind _returnvalue (`PXStateUtils.GetActorStateByEntry` owner (struct :`StateGuid` "BED5067B481B4978712C78B93BF8B621")))
    (if _returnvalue
      (bind _returnvalue_2 (`self.GetColorArgument` arguments (`KismetStringLibrary.Conv_StringToName` "LightColorTension")))
      (`LightComponent.SetLightColor` (`self.Light`) _returnvalue_2 true)
      (else
        (bind _returnvalue_3 (`self.GetColorArgument` arguments (`KismetStringLibrary.Conv_StringToName` "LightColorNoTension")))
        (`LightComponent.SetLightColor` (`self.Light`) _returnvalue_3 true)))))

(fn `TensionHigh`
  (params (InputPin :type "Actor Object Reference"))
  (returns (ReturnValue :type Boolean)))