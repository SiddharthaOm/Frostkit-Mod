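; State behaviour that switches a tension blob's protest effects on or off from its arguments.
; Activate and deactivate run the same function, which reads the Active flag to toggle Niagara emission points, with an extra pass when CheckProtestVFX is set.
; It also scales the mask mesh and sets the mask drawer's CPU radius, zeroing both when inactive, then updates the city mask CPU grid.
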(event `self.OnActivate`
  (params (owner :type "Actor Object Reference") (gameInstance :type "PXGameInstance Object Reference") (arguments :type "PXStateBehaviourArguments Object Reference") (stateEntry :type "PXStateEntry Structure"))
  (`self.BehaviorFunction Multiple Arguments` arguments owner))

(event `self.OnDeactivate`
  (params (owner :type "Actor Object Reference") (gameInstance :type "PXGameInstance Object Reference") (arguments :type "PXStateBehaviourArguments Object Reference") (stateEntry :type "PXStateEntry Structure"))
  (`self.BehaviorFunction Multiple Arguments` arguments owner))

(fn `BehaviorFunction`
  (params (Arguments :type "PXStateBehaviourArguments Object Reference") (Actor :type "Actor Object Reference"))
  (bind _returnvalue (`self.GetComponentArgument` Arguments (`KismetStringLibrary.Conv_StringToName` "SceneComponent") Actor))
  (bind _returnvalue_2 (`self.GetBoolArgument` Arguments (`KismetStringLibrary.Conv_StringToName` "Visible")))
  (bind _asscene_component (cast `SceneComponent` _returnvalue)
    (:`then`
      (`SceneComponent.SetVisibility` _asscene_component _returnvalue_2 false))
    (:`CastFailed`
      (`KismetSystemLibrary.PrintString` (`KismetStringLibrary.Concat_StrStr` "The component: " (`KismetSystemLibrary.GetDisplayName` _returnvalue) "is not a SceneComponent")))))

(fn `BehaviorFunction Multiple Arguments`
  (params (Arguments :type "PXStateBehaviourArguments Object Reference") (Actor :type "Actor Object Reference"))
  (bind _returnvalue (`self.GetBoolArgument` (`local.Arguments`) "CheckProtestVFX"))
  (if _returnvalue
    (bind _returnvalue_2 (`self.GetComponentArguments` (`local.Arguments`) (`local.Actor`) false))
    (for _array_element _returnvalue_2
      (bind _aspxniagara_emission_point_component (cast `PXNiagaraEmissionPointComponent` _array_element))
      (bind _returnvalue_3 (`self.GetBoolArgument` (`local.Arguments`) "Active"))
      (`PXComponentUtils.SetComponentEnabled` _aspxniagara_emission_point_component _returnvalue_3)))
  (`|ExecutionSequence`
    (:`then_0`
      (bind _returnvalue_4 (`self.GetComponentArgument` (`local.Arguments`) (`KismetStringLibrary.Conv_StringToName` "Mask") (`local.Actor`)))
      (bind _asstatic_mesh_component (cast `StaticMeshComponent` _returnvalue_4))
      (bind _returnvalue_5 (`self.GetBoolArgument` (`local.Arguments`) "Active"))
      (bind _returnvalue_6 (`self.GetFloatArgument` (`local.Arguments`) "MaskScale"))
      (`SceneComponent.SetWorldScale3D` _asstatic_mesh_component (select `bool` _returnvalue_5 :`true` (* _returnvalue_6 (1.0 1.0 1.0)))))
    (:`then_1`
      (bind _returnvalue_7 (`self.GetComponentArgument` (`local.Arguments`) (`KismetStringLibrary.Conv_StringToName` "MaskDrawer") (`local.Actor`)))
      (bind _aspxcity_mask_drawer_component (cast `PXCityMaskDrawerComponent` _returnvalue_7))
      (bind _returnvalue_8 (`self.GetBoolArgument` (`local.Arguments`) "Active"))
      (bind _returnvalue_9 (`self.GetFloatArgument` (`local.Arguments`) "CPURadius"))
      (set `PXCityMaskDrawerComponent.CPUGridRadius` (select `bool` _returnvalue_8 :`true` _returnvalue_9) _aspxcity_mask_drawer_component)
      (`PXCityMaskSubsystem.UpdateCPUGrid` (subsystem `PXCityMaskSubsystem`) _aspxcity_mask_drawer_component _returnvalue_8))
    (:`then_2`
      (bind _returnvalue_10 (`self.GetComponentArguments` (`local.Arguments`) (`local.Actor`) false))
      (for _array_element_2 _returnvalue_10
        (bind _aspxniagara_emission_point_component_2 (cast `PXNiagaraEmissionPointComponent` _array_element_2))
        (bind _returnvalue_11 (`self.GetBoolArgument` (`local.Arguments`) "Active"))
        (`PXTransformComponent.SetComponentEnabled` _aspxniagara_emission_point_component_2 _returnvalue_11)))))

(fn `IsProtest?`
  (params (actor :type "Actor Object Reference"))
  (returns (True :type Boolean))
  (bind _returnvalue (`PXStateUtils.GetActorStateByEntry` actor (struct :`StateGuid` "8C517CB748C4DEF89E3E3787FCDA1830")))
  (return _returnvalue))

(fn `IsTensionHigh?`
  (params (actor :type "Actor Object Reference"))
  (returns (True :type Boolean))
  (bind _returnvalue (`PXStateUtils.GetActorStateByEntry` actor (struct :`StateGuid` "BED5067B481B4978712C78B93BF8B621")))
  (bind _returnvalue_2 (`PXStateUtils.GetActorStateByEntry` actor (struct :`StateGuid` "4954AEBD4E8A7060FC6CFDBD6CE0E386")))
  (return (or _returnvalue_2 _returnvalue)))