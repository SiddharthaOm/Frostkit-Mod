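; State behaviour for a main-quarter tension blob, applying the blob's scale and city mask from state arguments.
; Activate and deactivate both run one function that uniformly scales the named scene component.
; It also sets the actor's city mask drawer CPU grid radius and updates the mask subsystem's grid with an enable flag.
; A visibility function and tension/protest state queries are defined but not called here.
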(event `self.OnActivate`
  (params (owner :type "Actor Object Reference") (gameInstance :type "PXGameInstance Object Reference") (arguments :type "PXStateBehaviourArguments Object Reference") (stateEntry :type "PXStateEntry Structure"))
  (`self.BehaviorFunction Multiple Arguments` arguments owner))

(event `self.OnDeactivate`
  (params (owner :type "Actor Object Reference") (gameInstance :type "PXGameInstance Object Reference") (arguments :type "PXStateBehaviourArguments Object Reference") (stateEntry :type "PXStateEntry Structure"))
  (`self.BehaviorFunction Multiple Arguments` arguments owner))

(fn `BehaviorFunction`
  (params (Arguments :type "PXStateBehaviourArguments Object Reference") (Actor :type "Actor Object Reference"))
  (bind _returnvalue (`self.GetComponentArgument` Arguments (`KismetStringLibrary.Conv_StringToName` "SceneComponent") Actor))
  (bind _returnvalue_2 (`self.GetBoolArgument` Arguments (`KismetStringLibrary.Conv_StringToName` "Visible")))
  (bind _asscene_component (cast `SceneComponent` _returnvalue)
    (:`then`
      (`SceneComponent.SetVisibility` _asscene_component _returnvalue_2 false))
    (:`CastFailed`
      (`KismetSystemLibrary.PrintString` (`KismetStringLibrary.Concat_StrStr` "The component: " (`KismetSystemLibrary.GetDisplayName` _returnvalue) "is not a SceneComponent")))))

(fn `BehaviorFunction Multiple Arguments`
  (params (Arguments :type "PXStateBehaviourArguments Object Reference") (Actor :type "Actor Object Reference"))
  (bind _returnvalue (`Actor.GetComponentByClass` (`local.Actor`) "/Script/Frostpunk2.PXCityMaskDrawerComponent"))
  ;[1 1 1] Blob scale
  (bind _returnvalue_2 (`self.GetComponentArgument` (`local.Arguments`) "SceneComponent" (`local.Actor`)))
  (bind _returnvalue_3 (`self.GetFloatArgument` (`local.Arguments`) (`KismetStringLibrary.Conv_StringToName` "BlobScale")))
  (bind _asscene_component (cast `SceneComponent` _returnvalue_2)
    (:`then`
      (`SceneComponent.SetRelativeScale3D` _asscene_component (`KismetMathLibrary.Conv_DoubleToVector` _returnvalue_3)))
    (:`CastFailed`
      _))
  (if (`KismetSystemLibrary.IsValid` _returnvalue)
    (bind _returnvalue_4 (`self.GetFloatArgument` (`local.Arguments`) "TensionMaskRadius"))
    (set `PXCityMaskDrawerComponent.CPUGridRadius` _returnvalue_4 _returnvalue)
    (bind _returnvalue_5 (`self.GetBoolArgument` (`local.Arguments`) "EnableMask"))
    (`PXCityMaskSubsystem.UpdateCPUGrid` (subsystem `PXCityMaskSubsystem`) _returnvalue _returnvalue_5)))

(fn `IsProtest?`
  (params (actor :type "Actor Object Reference"))
  (returns (True :type Boolean))
  (bind _returnvalue (`PXStateUtils.GetActorStateByEntry` actor (struct :`StateGuid` "8C517CB748C4DEF89E3E3787FCDA1830")))
  (return _returnvalue))

(fn `IsTensionHigh?`
  (params (actor :type "Actor Object Reference"))
  (returns (True :type Boolean))
  (bind _returnvalue (`PXStateUtils.GetActorStateByEntry` actor (struct :`StateGuid` "BED5067B481B4978712C78B93BF8B621")))
  (return _returnvalue))