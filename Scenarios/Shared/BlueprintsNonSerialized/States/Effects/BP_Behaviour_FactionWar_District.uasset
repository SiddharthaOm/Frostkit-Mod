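; State behaviour that switches faction war effects on a district and mirrors the state onto its owning city.
; Activation and deactivation share one function, which sets the argument-listed components by an Enabled flag and finds the city through the parent actor's district visual component.
; Enabling activates the city's state if the actor's state check passes; disabling clears it only when no faction war action is ongoing.
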(event `self.OnActivate`
  (params (owner :type "Actor Object Reference") (gameInstance :type "PXGameInstance Object Reference") (arguments :type "PXStateBehaviourArguments Object Reference") (stateEntry :type "PXStateEntry Structure"))
  (`self.BehaviorFunction Multiple Arguments` arguments owner))

(event `self.OnDeactivate`
  (params (owner :type "Actor Object Reference") (gameInstance :type "PXGameInstance Object Reference") (arguments :type "PXStateBehaviourArguments Object Reference") (stateEntry :type "PXStateEntry Structure"))
  (`self.BehaviorFunction Multiple Arguments` arguments owner))

(fn `BehaviorFunction Multiple Arguments`
  (params (Arguments :type "PXStateBehaviourArguments Object Reference") (Actor :type "Actor Object Reference"))
  (bind _returnvalue (`self.GetBoolArgument` (`local.Arguments`) (`KismetStringLibrary.Conv_StringToName` "Enabled")))
  (set `self.Enabled` _returnvalue)
  (set `self.TheCityThisShouldBe` (`ActorComponent.GetOwner` (`PXDistrictVisualComponent.GetCity` (`Actor.GetComponentByClass` (`Actor.GetAttachParentActor` (`local.Actor`)) "/Script/Frostpunk2.PXDistrictVisualComponent"))))
  (bind _returnvalue_2 (`self.GetComponentArguments` (`local.Arguments`) (`local.Actor`)))
  (for _array_element _returnvalue_2
    (`PXComponentUtils.SetComponentEnabled` _array_element (`self.Enabled`)))
  (if (`self.Enabled`)
    (bind _returnvalue_3 (`PXStateUtils.GetActorStateByEntry` (`local.Actor`) (struct :`StateGuid` "BED5067B481B4978712C78B93BF8B621")))
    (if _returnvalue_3
      (`PXStateUtils.SetActorStateByEntry` (`self.TheCityThisShouldBe`) (struct :`StateGuid` "AB6FBA1B4CB03C33680F8487529AFF73")))
    (elif (not (`/Game/Scenarios/Shared/BlueprintsNonSerialized/OngoingEvents/BPFL_OngoingAction_Utils.Is Any Action of type Ongoing?` "/Game/Scenarios/Shared/Configs/OngoingActions/System_Started/DA_FactionWar.DA_FactionWar"))
      (`PXStateUtils.SetActorStateByEntry` (`self.TheCityThisShouldBe`) (struct :`StateGuid` "AB6FBA1B4CB03C33680F8487529AFF73") false))))