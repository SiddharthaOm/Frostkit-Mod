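; State behaviour for the Urbos main hub generator that enables or disables the owner's components named in the state arguments.
; Activation and deactivation run the same function, which branches on whether the state's enablement reason is Construction.
; Construction applies the inverted Enabled argument when the actor's state is true; other reasons apply it unchanged when false.
; Components are always set with an Undefined reason, not the looked-up one.
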(event `self.OnActivate`
  (params (owner :type "Actor Object Reference") (gameInstance :type "PXGameInstance Object Reference") (arguments :type "PXStateBehaviourArguments Object Reference") (stateEntry :type "PXStateEntry Structure"))
  (`self.BehaviorFunction Multiple Arguments` arguments owner stateEntry))

(event `self.OnDeactivate`
  (params (owner :type "Actor Object Reference") (gameInstance :type "PXGameInstance Object Reference") (arguments :type "PXStateBehaviourArguments Object Reference") (stateEntry :type "PXStateEntry Structure"))
  (`self.BehaviorFunction Multiple Arguments` arguments owner stateEntry))

(fn `BehaviorFunction Multiple Arguments`
  (params (Arguments :type "PXStateBehaviourArguments Object Reference") (Actor :type "Actor Object Reference") (`State Entry` :type "PXStateEntry Structure"))
  (locals (Reason :type "EPXEnablementSystemDisabledReason Enum" :default "Undefined") (Enable :type Boolean :default false))
  (bind _returnvalue (`PXEnablementUtils.GetEnablementReasonForState` `State Entry`))
  (set `local.Reason` _returnvalue)
  (if (`|EnumEquality` _returnvalue "Construction")
    (bind _returnvalue_2 (`self.GetBoolArgument` (`local.Arguments`) (`KismetStringLibrary.Conv_StringToName` "Enabled")))
    (set `local.Enable` (not _returnvalue_2))
    (bind _returnvalue_3 (`PXStateUtils.GetActorStateByEntry` (`local.Actor`) (struct :`StateGuid` "5D0FDB9648B726EE7644089FB2AFB31D")))
    (if _returnvalue_3
      (bind _returnvalue_4 (`self.GetComponentArguments` (`local.Arguments`) (`local.Actor`) :!label _label))
      (for _array_element _returnvalue_4
        (`PXComponentUtils.SetComponentEnabled` _array_element (`local.Enable`))))
    (else
      (bind _returnvalue_5 (`self.GetBoolArgument` (`local.Arguments`) (`KismetStringLibrary.Conv_StringToName` "Enabled")))
      (set `local.Enable` _returnvalue_5)
      (bind _returnvalue_6 (`PXStateUtils.GetActorStateByEntry` (`local.Actor`) (struct :`StateGuid` "9AD8B03B4C6AAFC3C2859C96A6402D87")))
      (if (not _returnvalue_6)
        (goto _label)))))