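; BP_Progress_Legs_Behaviour is a state behaviour for Urbos scenarios that switches an actor's components on or off.
; Activation and deactivation both run one shared function with the owner and arguments, without inverting the value.
; When the actor state lookup by entry comes back negative, it applies the "Enabled" bool argument to every component named in the arguments, logging an error for missing ones.
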(event `self.OnActivate`
  (params (owner :type "Actor Object Reference") (gameInstance :type "PXGameInstance Object Reference") (arguments :type "PXStateBehaviourArguments Object Reference") (stateEntry :type "PXStateEntry Structure"))
  (`self.BehaviorFunction Multiple Arguments` arguments owner))

(event `self.OnDeactivate`
  (params (owner :type "Actor Object Reference") (gameInstance :type "PXGameInstance Object Reference") (arguments :type "PXStateBehaviourArguments Object Reference") (stateEntry :type "PXStateEntry Structure"))
  (`self.BehaviorFunction Multiple Arguments` arguments owner))

(fn `BehaviorFunction Multiple Arguments`
  (params (Arguments :type "PXStateBehaviourArguments Object Reference") (Actor :type "Actor Object Reference"))
  (bind _returnvalue (`PXStateUtils.GetActorStateByEntry` (`local.Actor`) (struct :`StateGuid` "9AD8B03B4C6AAFC3C2859C96A6402D87")))
  (if (not _returnvalue)
    (bind _returnvalue_2 (`self.GetComponentArguments` Arguments Actor))
    (for _array_element _returnvalue_2
      (bind _returnvalue_3 (`self.GetBoolArgument` (`local.Arguments`) (`KismetStringLibrary.Conv_StringToName` "Enabled")))
      (`PXComponentUtils.SetComponentEnabled` _array_element _returnvalue_3))))