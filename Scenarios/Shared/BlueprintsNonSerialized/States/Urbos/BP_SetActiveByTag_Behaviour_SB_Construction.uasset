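; State behaviour that toggles an actor's tagged Niagara components, named for Urbos construction states.
; Activation and deactivation both run one shared function, which reads "Active" and "Tag" from the behaviour arguments.
; When Active is true, it enables matching components only if GetActorStateByEntry returns true, otherwise leaving them untouched.
; When Active is false, it disables them unconditionally; neither path resets the effects.
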(event `self.OnActivate`
  (params (owner :type "Actor Object Reference") (gameInstance :type "PXGameInstance Object Reference") (arguments :type "PXStateBehaviourArguments Object Reference") (stateEntry :type "PXStateEntry Structure"))
  (`self.BehaviorFunction Multiple Arguments` arguments owner))

(event `self.OnDeactivate`
  (params (owner :type "Actor Object Reference") (gameInstance :type "PXGameInstance Object Reference") (arguments :type "PXStateBehaviourArguments Object Reference") (stateEntry :type "PXStateEntry Structure"))
  (`self.BehaviorFunction Multiple Arguments` arguments owner))

(fn `BehaviorFunction Multiple Arguments`
  (params (Arguments :type "PXStateBehaviourArguments Object Reference") (Actor :type "Actor Object Reference"))
  (bind _returnvalue (`self.GetBoolArgument` (`local.Arguments`) (`KismetStringLibrary.Conv_StringToName` "Active")))
  (if _returnvalue
    (bind _returnvalue_2 (`PXStateUtils.GetActorStateByEntry` (`local.Actor`) (struct :`StateGuid` "8DCFC9E04F97E52D6521FFB25C802177")))
    (if _returnvalue_2
      (bind _returnvalue_3 (`PXStateUtils.GetActorStateByEntry` (`local.Actor`) (struct :`StateGuid` "E02E58F040BEC2DEAFE6F9BE30186FA0")))
      (bind _returnvalue_4 (`self.GetNameArgument` (`local.Arguments`) (`KismetStringLibrary.Conv_StringToName` "Tag")))
      (for _array_element (`Actor.GetComponentsByTag` (`local.Actor`) "/Script/Niagara.NiagaraComponent" _returnvalue_4)
        (`ActorComponent.SetActive` _array_element _returnvalue_3 false)))
    (else
      (bind _returnvalue_5 (`self.GetNameArgument` (`local.Arguments`) (`KismetStringLibrary.Conv_StringToName` "Tag")))
      (for _array_element_2 (`Actor.GetComponentsByTag` (`local.Actor`) "/Script/Niagara.NiagaraComponent" _returnvalue_5)
        (`ActorComponent.SetActive` _array_element_2 false false)))))