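; State behaviour for wood resource deposits that shows or hides tree meshes around district hubs and buildings while the deposit has stock.
; Activate and deactivate both dirty the instancing batch and set the Urbos volume from the Enabled argument.
; Enabled shows all child static meshes; otherwise meshes near the closest district's hub are disabled, and others are toggled per city building by distance, without early exit.
; Decal and city-mask logic is unconnected.
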(event `self.OnActivate`
  (params (owner :type "Actor Object Reference") (gameInstance :type "PXGameInstance Object Reference") (arguments :type "PXStateBehaviourArguments Object Reference") (stateEntry :type "PXStateEntry Structure"))
  (`self.mulitple args` owner arguments stateEntry))

(event `self.OnDeactivate`
  (params (owner :type "Actor Object Reference") (gameInstance :type "PXGameInstance Object Reference") (arguments :type "PXStateBehaviourArguments Object Reference") (stateEntry :type "PXStateEntry Structure"))
  (`self.mulitple args` owner arguments stateEntry))

(fn `BuildingsOverlap`
  (params (Mesh :type "SceneComponent Object Reference") (city :type "PXCityComponent Object Reference"))
  (for _array_element (`PXBuildingUtils.GetBuildingsFromCity` city)
    (`/Engine/EditorBlueprintResources/StandardMacros.CompareFloat` (`KismetMathLibrary.Vector_Distance` (`Actor.K2_GetActorLocation` (`ActorComponent.GetOwner` _array_element)) (`SceneComponent.K2_GetComponentLocation` Mesh)) (`self.AllowedDistance_Building`)
      (:`>`
        (`PXComponentUtils.SetComponentEnabled` Mesh true :!label _label))
      (:`==`
        (goto _label))
      (:`<`
        (`PXComponentUtils.SetComponentEnabled` Mesh)))))

(fn `GetClosestCity`
  (params (Target :type "SceneComponent Object Reference"))
  (returns (SavedClosestCity :type "PXCityComponent Object Reference"))
  (locals (SavedDistance :type "Float (double-precision)" :default 10000000000.0) (ClosestCity :type "PXCityComponent Object Reference"))
  (for _array_element (`PXNationUtils.GetAllPlayerCities`)
    (bind _returnvalue (`KismetMathLibrary.Vector_Distance` (`Actor.K2_GetActorLocation` (`ActorComponent.GetOwner` _array_element)) (`SceneComponent.K2_GetComponentLocation` Target)))
    (if (< _returnvalue (`local.SavedDistance`))
      (set `local.SavedDistance` _returnvalue)
      (set `local.ClosestCity` _array_element)))
  (return (`local.ClosestCity`)))

(fn `mulitple args`
  (params (actor :type "Actor Object Reference") (arguments :type "PXStateBehaviourArguments Object Reference") (stateEntry :type "PXStateEntry Structure"))
  (bind _returnvalue (`Actor.GetComponentByClass` (`local.actor`) "/Script/Frostpunk2.PXUrbosVolumeComponent"))
  (if (> (`PXDepositComponent.Amount` (`PXDepositVisualizationComponent.DepositComponent` (`Actor.GetComponentByClass` actor "/Script/Frostpunk2.PXDepositVisualizationComponent"))) 0)
    (`|ExecutionSequence`
      (:`then_0`
        (bind _returnvalue_2 (`self.GetComponentArgument` (`local.arguments`) "BatchComponent" (`local.actor`) false))
        (bind _aspxinstancing_batch_component (cast `PXInstancingBatchComponent` _returnvalue_2))
        (`PXInstancingBatchSubsystem.SetBatchComponentDirty` (subsystem `PXInstancingBatchSubsystem`) _aspxinstancing_batch_component))
      (:`then_1`
        (bind _returnvalue_3 (`self.GetBoolArgument` (`local.arguments`) (`KismetStringLibrary.Conv_StringToName` "Enabled")))
        (bind _returnvalue_4 (`self.GetComponentArgument` (`local.arguments`) "Scene_ForPXStateVisibility" (`local.actor`) false))
        (bind _asscene_component (cast `SceneComponent` _returnvalue_4))
        (for _array_element (`SceneComponent.GetChildrenComponents` _asscene_component true)
          (bind _asstatic_mesh_component (cast `StaticMeshComponent` _array_element))
          (if (not _returnvalue_3)
            (bind (_returnvalue_5 _closestcity) (`self.NewFunction` _asstatic_mesh_component))
            (`/Engine/EditorBlueprintResources/StandardMacros.CompareFloat` _returnvalue_5 (`self.AllowedDistance_DistrictHub`)
              (:`>`
                (`self.BuildingsOverlap` _asstatic_mesh_component _closestcity :!label _label))
              (:`==`
                (goto _label))
              (:`<`
                (`PXComponentUtils.SetComponentEnabled` _asstatic_mesh_component false "Activity")))
            (else
              (`PXComponentUtils.SetComponentEnabled` _asstatic_mesh_component true "Activity")))))
      (:`then_2`
        (bind _returnvalue_6 (`self.GetBoolArgument` (`local.arguments`) "Enabled"))
        (`/Engine/EditorBlueprintResources/StandardMacros.IsValid` _returnvalue
          (:`Is Valid`
            (`PXUrbosVolumeSubsystem.SetEnabled` (subsystem `PXUrbosVolumeSubsystem`) _returnvalue _returnvalue_6)))))))

(fn `NewFunction`
  (params (Target :type "SceneComponent Object Reference"))
  (returns (ReturnValue :type "Float (double-precision)") (ClosestCity :type "PXCityComponent Object Reference"))
  (locals (City :type "PXCityComponent Object Reference"))
  (set `local.City` (`self.GetClosestCity` Target))
  (bind _returnvalue (`PXDistrictUtils.GetHubFromDistrict` (`PXDistrictUtils.FindClosestDistrict` (`KismetMathLibrary.Conv_VectorToVector2D` (`SceneComponent.K2_GetComponentLocation` Target)) (`local.City`) null))
    (:`ComponentIsValid`
      (return (`KismetMathLibrary.Vector_Distance` (`Actor.K2_GetActorLocation` _returnvalue) (`SceneComponent.K2_GetComponentLocation` Target)) (`local.City`)))))