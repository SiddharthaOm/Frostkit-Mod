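; State behaviour for wood resource deposits that hides tree meshes overlapped by a nearby district.
; Activation and deactivation run the same refresh, only while the deposit has an amount left.
; It samples the city mask at each static mesh under the argument-named scene component, disabling masked meshes and enabling the rest.
; It then sets the Urbos volume from the Enabled argument and dirties the instancing batch.
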(event `self.OnActivate`
  (params (owner :type "Actor Object Reference") (gameInstance :type "PXGameInstance Object Reference") (arguments :type "PXStateBehaviourArguments Object Reference") (stateEntry :type "PXStateEntry Structure"))
  (`self.mulitple args` owner arguments))

(event `self.OnDeactivate`
  (params (owner :type "Actor Object Reference") (gameInstance :type "PXGameInstance Object Reference") (arguments :type "PXStateBehaviourArguments Object Reference") (stateEntry :type "PXStateEntry Structure"))
  (`self.mulitple args` owner arguments))

(fn `mulitple args`
  (params (actor :type "Actor Object Reference") (arguments :type "PXStateBehaviourArguments Object Reference"))
  (bind _returnvalue (`Actor.GetComponentByClass` (`local.actor`) "/Script/Frostpunk2.PXUrbosVolumeComponent"))
  (if (> (`PXDepositComponent.Amount` (`PXDepositVisualizationComponent.DepositComponent` (`Actor.GetComponentByClass` actor "/Script/Frostpunk2.PXDepositVisualizationComponent"))) 0)
    (bind _returnvalue_2 (`self.GetComponentArgument` (`local.arguments`) "Scene_ForPXStateVisibility" (`local.actor`) false))
    (bind _asscene_component (cast `SceneComponent` _returnvalue_2))
    (for _array_element (`SceneComponent.GetChildrenComponents` _asscene_component true)
      (bind _asstatic_mesh_component (cast `StaticMeshComponent` _array_element))
      (bind _returnvalue_3 (`PXCityMaskSubsystem.GetCityMaskValueAtPosition` (subsystem `PXCityMaskSubsystem`) (`KismetMathLibrary.Conv_VectorToVector2D` (`SceneComponent.K2_GetComponentLocation` _asstatic_mesh_component)) 4))
      (bind _maskvaluesperchannel (break `PXCityMaskCPUGridEntry` _returnvalue_3))
      (if (or (`|GetArrayItem` _maskvaluesperchannel) (`|GetArrayItem` _maskvaluesperchannel 1))
        (`PXComponentUtils.SetComponentEnabled` _asstatic_mesh_component)
        (else
          (`PXComponentUtils.SetComponentEnabled` _asstatic_mesh_component true))))
    (`|ExecutionSequence`
      (:`then_0`
        (bind _returnvalue_4 (`self.GetBoolArgument` (`local.arguments`) "Enabled"))
        (`/Engine/EditorBlueprintResources/StandardMacros.IsValid` _returnvalue
          (:`Is Valid`
            (`PXUrbosVolumeSubsystem.SetEnabled` (subsystem `PXUrbosVolumeSubsystem`) _returnvalue _returnvalue_4))))
      (:`then_1`
        (bind _returnvalue_5 (`self.GetComponentArgument` (`local.arguments`) "BatchComponent" (`local.actor`) false))
        (bind _aspxinstancing_batch_component (cast `PXInstancingBatchComponent` _returnvalue_5))
        (`PXInstancingBatchSubsystem.SetBatchComponentDirty` (subsystem `PXInstancingBatchSubsystem`) _aspxinstancing_batch_component)))))