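; A state behaviour that switches Niagara components on an actor on or off, driven by the state's arguments.
; Activation and deactivation both run one shared function, which resolves the target components and enables and activates, or disables and deactivates, each according to the Active argument.
; An optional flag also pushes float, int, vector and bool arguments into fixed PXState_ Niagara variables, and non-Niagara targets print an on-screen warning.
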(event `self.OnActivate`
  (params (owner :type "Actor Object Reference") (gameInstance :type "PXGameInstance Object Reference") (arguments :type "PXStateBehaviourArguments Object Reference") (stateEntry :type "PXStateEntry Structure"))
  (`self.BehaviorFunction Multiple Arguments` arguments owner))

(event `self.OnDeactivate`
  (params (owner :type "Actor Object Reference") (gameInstance :type "PXGameInstance Object Reference") (arguments :type "PXStateBehaviourArguments Object Reference") (stateEntry :type "PXStateEntry Structure"))
  (`self.BehaviorFunction Multiple Arguments` arguments owner))

(fn `BehaviorFunction Multiple Arguments`
  (params (Arguments :type "PXStateBehaviourArguments Object Reference") (Actor :type "Actor Object Reference"))
  (bind _arguments (`local.Arguments`))
  (bind _returnvalue (`self.GetComponentArguments` Arguments Actor false))
  (for _array_element _returnvalue
    (bind _asniagara_particle_system_component (cast `NiagaraComponent` _array_element)
      (:`then`
        (bind _returnvalue_2 (`self.GetBoolArgument` _arguments "Active"))
        (if _returnvalue_2
          (`PXComponentUtils.SetComponentEnabled` _asniagara_particle_system_component true)
          (`ActorComponent.Activate` _asniagara_particle_system_component false)
          (else
            (`PXComponentUtils.SetComponentEnabled` _asniagara_particle_system_component)
            (`ActorComponent.Deactivate` _asniagara_particle_system_component)))
        (bind _returnvalue_3 (`self.GetBoolArgument` _arguments "SetAdditionalValues"))
        (if _returnvalue_3
          (bind _returnvalue_4 (`self.GetFloatArgument` _arguments "FloatA"))
          (`NiagaraComponent.SetVariableFloat` _asniagara_particle_system_component "PXState_FloatA" _returnvalue_4)
          (bind _returnvalue_5 (`self.GetIntArgument` _arguments "IntA"))
          (`NiagaraComponent.SetVariableInt` _asniagara_particle_system_component "PXState_IntA" _returnvalue_5)
          (bind _returnvalue_6 (`self.GetVectorArgument` _arguments "VectorA"))
          (`NiagaraComponent.SetVariableVec3` _asniagara_particle_system_component "PXState_VectorA" _returnvalue_6)
          (bind _returnvalue_7 (`self.GetBoolArgument` _arguments "BoolA"))
          (`NiagaraComponent.SetVariableBool` _asniagara_particle_system_component "PXState_BoolA" _returnvalue_7)))
      (:`CastFailed`
        (`KismetSystemLibrary.PrintString` (`KismetStringLibrary.Concat_StrStr` "bruh " (`KismetSystemLibrary.GetDisplayName` _array_element) "is not Nagara Component fix it!!!") true true (struct :`R` 5.0 :`B` 0.09315 :`A` 1.0))))))