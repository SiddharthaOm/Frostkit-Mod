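; State behavior that cross-fades two groups of an actor's components on activate and deactivate, then toggles their enablement.
; A subsystem plays a linear "Fade" animation starting from the stored progress, driving a scalar parameter on slot 0 dynamic materials, created if missing.
; The Enable and Disable counts split the component list into groups that fade oppositely, directed by the Enabled argument.
; Enablement is applied with the state's reason when the fade finishes, and any instancing batch component is marked dirty.
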(event `self.OnActivate`
  (params (owner :type "Actor Object Reference") (gameInstance :type "PXGameInstance Object Reference") (arguments :type "PXStateBehaviourArguments Object Reference") (stateEntry :type "PXStateEntry Structure"))
  (`self.BehaviorFunction Multiple Arguments` arguments owner stateEntry))

(event `self.OnDeactivate`
  (params (owner :type "Actor Object Reference") (gameInstance :type "PXGameInstance Object Reference") (arguments :type "PXStateBehaviourArguments Object Reference") (stateEntry :type "PXStateEntry Structure"))
  (`self.BehaviorFunction Multiple Arguments` arguments owner stateEntry))

(event `InitFadeAnimation`
  (params (AnimationData :type "PXBlueprintAnimationData Object Reference"))
  (bind _returnvalue (`Actor.GetComponentByClass` (`PXBlueprintAnimationData.Owner` AnimationData) "/Script/Frostpunk2.PXInstancingBatchComponent"))
  (`BlueprintMapLibrary.Map_Add` (`PXBlueprintAnimationData.StartFloatValues` AnimationData) "Progress" (`self.FadeProgress`))
  (`/Engine/EditorBlueprintResources/StandardMacros.IsValid` _returnvalue
    (:`Is Valid`
      (`PXInstancingBatchComponent.SetDirty` _returnvalue))))

(event `UpdateFadeAnimation`
  (params (AnimationData :type "PXBlueprintAnimationData Object Reference"))
  (bind _statearguments (`self.StateArguments`))
  (bind _statearguments_2 (`self.StateArguments`))
  (set `self.FadeProgress` (`BlueprintMapLibrary.Map_Find` (`PXBlueprintAnimationData.CurrentFloatValues` AnimationData) "Progress"))
  (bind _returnvalue (`self.GetComponentArguments` _statearguments (`PXBlueprintAnimationData.Owner` AnimationData) false))
  (bind _returnvalue_2 (`self.GetBoolArgument` (`self.StateArguments`) (`KismetStringLibrary.Conv_StringToName` "Enabled")))
  (bind _returnvalue_3 (`self.GetNameArgument` _statearguments "MaterialFadeParam"))
  (`|ExecutionSequence`
    (:`then_0`
      (bind _returnvalue_4 (`self.GetIntArgument` _statearguments_2 "Enable"))
      (for _index (range _returnvalue_4)
        (if (`KismetArrayLibrary.Array_IsValidIndex` _returnvalue _index)
          (if _returnvalue_2
            (bind _output (`|GetArrayItem` _returnvalue _index))
            (`self.SetComponentOpacity` _output (`self.FadeProgress`) _returnvalue_3)
            (else
              (`self.SetComponentOpacity` _output (- 1.0 (`self.FadeProgress`)) _returnvalue_3))))))
    (:`then_1`
      (bind _returnvalue_5 (`self.GetIntArgument` _statearguments_2 "Disable"))
      (if (> _returnvalue_5 0)
        (for _index_2 (range _returnvalue_4 (+ (+ _returnvalue_4 (- _returnvalue_5 1)) 1))
          (if (`KismetArrayLibrary.Array_IsValidIndex` _returnvalue _index_2)
            (if (not _returnvalue_2)
              (bind _output_2 (`|GetArrayItem` _returnvalue _index_2))
              (`self.SetComponentOpacity` _output_2 (`self.FadeProgress`) _returnvalue_3)
              (else
                (`self.SetComponentOpacity` _output_2 (- 1.0 (`self.FadeProgress`)) _returnvalue_3)))))))))

(event `FinishFadeAnimation`
  (params (AnimationData :type "PXBlueprintAnimationData Object Reference"))
  (bind _statearguments (`self.StateArguments`))
  (bind _statearguments_2 (`self.StateArguments`))
  (bind _cachedstateentry (`self.CachedStateEntry`))
  (bind _returnvalue (`Actor.GetComponentByClass` (`PXBlueprintAnimationData.Owner` AnimationData) "/Script/Frostpunk2.PXInstancingBatchComponent"))
  (bind _returnvalue_2 (`self.GetComponentArguments` (`self.StateArguments`) (`PXBlueprintAnimationData.Owner` AnimationData) false))
  (`|ExecutionSequence`
    (:`then_0`
      (bind _returnvalue_3 (`self.GetIntArgument` _statearguments "Enable"))
      (for _index (range _returnvalue_3)
        (if (`KismetArrayLibrary.Array_IsValidIndex` _returnvalue_2 _index)
          (bind _returnvalue_4 (`self.GetBoolArgument` _statearguments_2 (`KismetStringLibrary.Conv_StringToName` "Enabled")))
          (bind _returnvalue_5 (`PXEnablementUtils.GetEnablementReasonForState` _cachedstateentry))
          (`PXComponentUtils.SetComponentEnabled` (`|GetArrayItem` _returnvalue_2 _index) _returnvalue_4 _returnvalue_5))))
    (:`then_1`
      (bind _returnvalue_6 (`self.GetIntArgument` _statearguments "Disable"))
      (if (> _returnvalue_6 0)
        (for _index_2 (range _returnvalue_3 (+ (+ _returnvalue_3 (- _returnvalue_6 1)) 1))
          (if (`KismetArrayLibrary.Array_IsValidIndex` _returnvalue_2 _index_2)
            (bind _returnvalue_7 (`self.GetBoolArgument` _statearguments_2 (`KismetStringLibrary.Conv_StringToName` "Enabled")))
            (bind _returnvalue_8 (`PXEnablementUtils.GetEnablementReasonForState` _cachedstateentry))
            (`PXComponentUtils.SetComponentEnabled` (`|GetArrayItem` _returnvalue_2 _index_2) (not _returnvalue_7) _returnvalue_8)))))
    (:`then_2`
      (`/Engine/EditorBlueprintResources/StandardMacros.IsValid` _returnvalue
        (:`Is Valid`
          (`PXInstancingBatchComponent.SetDirty` _returnvalue))))))

(fn `BehaviorFunction Multiple Arguments`
  (params (Arguments :type "PXStateBehaviourArguments Object Reference") (Actor :type "Actor Object Reference") (stateEntry :type "PXStateEntry Structure"))
  (locals (CurrentEnableName :type String :default "ComponentToEnable") (EnableAppend :type Integer :default 0) (HasComps :type Boolean :default false) (FadeTime :type "Float (double-precision)"))
  (set `self.CachedStateEntry` stateEntry)
  (set `self.StateArguments` Arguments)
  (bind _returnvalue (`self.GetFloatArgument` Arguments "FadeTime"))
  (set `local.FadeTime` _returnvalue)
  (bind _returnvalue_2 (`|Subsystem`)
    (:`then`
      (`PXBlueprintAnimationSubsystem.PlayAnimation` _returnvalue_2 (`local.Actor`) "/Game/Scenarios/Shared/Configs/BlueprintAnimation/Common/DA_LinearFadeIn.DA_LinearFadeIn" (`local.FadeTime`) "Fade" (`|CreateDelegate` :!event `InitFadeAnimation`) (`|CreateDelegate` :!event `UpdateFadeAnimation`) (`|CreateDelegate` :!event `FinishFadeAnimation`)))))

(fn `SetComponentOpacity`
  (params (Component :type "ActorComponent Object Reference") (Opacity :type "Float (double-precision)") (MaterialParamName :type Name))
  (bind _asprimitive_component (cast `PrimitiveComponent` Component))
  (bind _returnvalue (`PrimitiveComponent.GetMaterial` _asprimitive_component 0))
  (bind _asmaterial_instance_dynamic (cast `MaterialInstanceDynamic` _returnvalue :!label _label)
    (:`then`
      (`MaterialInstanceDynamic.SetScalarParameterValue` _asmaterial_instance_dynamic MaterialParamName (`local.Opacity`)))
    (:`CastFailed`
      (`PrimitiveComponent.CreateDynamicMaterialInstance` _asprimitive_component 0 _returnvalue "None")
      (goto _label))))