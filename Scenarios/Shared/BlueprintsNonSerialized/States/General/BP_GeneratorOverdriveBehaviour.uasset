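; State behaviour that switches a generator's visuals in and out of overdrive on activation and deactivation.
; Both events call one function that loops over the component arguments, setting the overdrive or normal generator material on static meshes, using slot names from arguments keyed by array index.
; It then sets the "Overdrive" boolean on the Niagara component argument.
; A separate visibility-setting function is present but not called here.
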(event `self.OnActivate`
  (params (owner :type "Actor Object Reference") (gameInstance :type "PXGameInstance Object Reference") (arguments :type "PXStateBehaviourArguments Object Reference") (stateEntry :type "PXStateEntry Structure"))
  (`self.BehaviorFunction Multiple Arguments` arguments owner true))

(event `self.OnDeactivate`
  (params (owner :type "Actor Object Reference") (gameInstance :type "PXGameInstance Object Reference") (arguments :type "PXStateBehaviourArguments Object Reference") (stateEntry :type "PXStateEntry Structure"))
  (`self.BehaviorFunction Multiple Arguments` arguments owner))

(fn `BehaviorFunction`
  (params (Arguments :type "PXStateBehaviourArguments Object Reference") (Actor :type "Actor Object Reference"))
  (bind _returnvalue (`self.GetComponentArgument` Arguments (`KismetStringLibrary.Conv_StringToName` "SceneComponent") Actor))
  (bind _returnvalue_2 (`self.GetBoolArgument` Arguments (`KismetStringLibrary.Conv_StringToName` "Visible")))
  (bind _asscene_component (cast `SceneComponent` _returnvalue)
    (:`then`
      (`SceneComponent.SetVisibility` _asscene_component _returnvalue_2 false))
    (:`CastFailed`
      (`KismetSystemLibrary.PrintString` (`KismetStringLibrary.Concat_StrStr` "The component: " (`KismetSystemLibrary.GetDisplayName` _returnvalue) "is not a SceneComponent")))))

(fn `BehaviorFunction Multiple Arguments`
  (params (Arguments :type "PXStateBehaviourArguments Object Reference") (Actor :type "Actor Object Reference") (Activate :type Boolean))
  (bind _returnvalue (`self.GetComponentArguments` (`local.Arguments`) (`local.Actor`)))
  (for (_array_element _array_index) _returnvalue
    (bind _asstatic_mesh_component (cast `StaticMeshComponent` _array_element))
    (bind _returnvalue_2 (`self.GetNameArgument` (`local.Arguments`) (`KismetStringLibrary.Conv_StringToName` (`KismetStringLibrary.Conv_IntToString` _array_index))))
    (if (`local.Activate`)
      (`PXParliamentUtils.SetMaterial` _asstatic_mesh_component _returnvalue_2 "/Game/Scenarios/Shared/Materials/CityLights/MI_CIT_Generators_B_Overdrive.MI_CIT_Generators_B_Overdrive")
      (else
        (`PXParliamentUtils.SetMaterial` _asstatic_mesh_component _returnvalue_2 "/Game/Scenarios/Shared/Materials/CityLights/MI_CIT_Generators_B.MI_CIT_Generators_B"))))
  (bind _returnvalue_3 (`self.GetComponentArgument` (`local.Arguments`) (`KismetStringLibrary.Conv_StringToName` "Niagara") (`local.Actor`)))
  (bind _asniagara_particle_system_component (cast `NiagaraComponent` _returnvalue_3))
  (`NiagaraComponent.SetVariableBool` _asniagara_particle_system_component "Overdrive" (`local.Activate`)))