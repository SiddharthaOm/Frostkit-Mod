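; State behaviour that enables or disables the owner actor's components carrying a given tag, using Tag and Enabled arguments.
; Activation and deactivation both run the same function with their own arguments, looping over the tagged components.
; Niagara components are activated or deactivated and lights toggle visibility, while static meshes and all other components go through SetComponentEnabled.
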(event `self.OnActivate`
  (params (owner :type "Actor Object Reference") (gameInstance :type "PXGameInstance Object Reference") (arguments :type "PXStateBehaviourArguments Object Reference") (stateEntry :type "PXStateEntry Structure"))
  (`self.BehaviorFunction Multiple Arguments` arguments owner))

(event `self.OnDeactivate`
  (params (owner :type "Actor Object Reference") (gameInstance :type "PXGameInstance Object Reference") (arguments :type "PXStateBehaviourArguments Object Reference") (stateEntry :type "PXStateEntry Structure"))
  (`self.BehaviorFunction Multiple Arguments` arguments owner))

(fn `BehaviorFunction Multiple Arguments`
  (params (Arguments :type "PXStateBehaviourArguments Object Reference") (Actor :type "Actor Object Reference"))
  (bind _returnvalue (`self.GetNameArgument` Arguments (`KismetStringLibrary.Conv_StringToName` "Tag")))
  (for _array_element (`Actor.GetComponentsByTag` Actor "/Script/Engine.ActorComponent" _returnvalue)
    (bind _returnvalue_2 (`self.GetBoolArgument` (`local.Arguments`) (`KismetStringLibrary.Conv_StringToName` "Enabled")))
    (bind _asniagara_particle_system_component (cast `NiagaraComponent` _array_element)
      (:`then`
        (if _returnvalue_2
          ;[0.05208 0.05208 0.05208 1 11] It actually activates, not enables.. :(
          (`ActorComponent.Activate` _asniagara_particle_system_component false)
          (else
            (`ActorComponent.Deactivate` _asniagara_particle_system_component))))
      (:`CastFailed`
        (bind _asstatic_mesh_component (cast `StaticMeshComponent` _array_element)
          (:`then`
            (`PXComponentUtils.SetComponentEnabled` _asstatic_mesh_component _returnvalue_2))
          (:`CastFailed`
            (bind _aslight_component (cast `LightComponent` _array_element)
              (:`then`
                (`SceneComponent.SetVisibility` _aslight_component _returnvalue_2 false))
              (:`CastFailed`
                (`PXComponentUtils.SetComponentEnabled` _array_element _returnvalue_2)))))))))