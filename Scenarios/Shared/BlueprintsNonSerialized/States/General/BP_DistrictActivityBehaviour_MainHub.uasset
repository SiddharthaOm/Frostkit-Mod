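; State behaviour that switches the main hub district's activity visuals according to its Enable argument, ignoring actors not attached to a main district.
; Activation and deactivation share one function that updates the city mask CPU grid and toggles the GPU inactivity and activity mask components.
; It also sets a state across the whole city rectangle as a workaround to switch road lights, then fades the activity mask through the weather subsystem for snow melting.
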(event `self.OnActivate`
  (params (owner :type "Actor Object Reference") (gameInstance :type "PXGameInstance Object Reference") (arguments :type "PXStateBehaviourArguments Object Reference") (stateEntry :type "PXStateEntry Structure"))
  (`self.BehaviorFunction Multiple Arguments` arguments owner))

(event `self.OnDeactivate`
  (params (owner :type "Actor Object Reference") (gameInstance :type "PXGameInstance Object Reference") (arguments :type "PXStateBehaviourArguments Object Reference") (stateEntry :type "PXStateEntry Structure"))
  (`self.BehaviorFunction Multiple Arguments` arguments owner))

(fn `BehaviorFunction Multiple Arguments`
  (params (Arguments :type "PXStateBehaviourArguments Object Reference") (Actor :type "Actor Object Reference") (`State Entry` :type "PXStateEntry Structure"))
  (locals (Drawer :type "PXCityMaskDrawerComponent Object Reference") (ShouldEnable :type Boolean :default false) (DistrictActivityMaskSC :type "SceneComponent Object Reference") (DistrictInactivityMask :type "ActorComponent Object Reference") (NewLocalVar :type Boolean) (MeltBuildings :type "ActorComponent Object Reference") (MeltBuildings2 :type "ActorComponent Object Reference") (MeltBuildings3 :type "ActorComponent Object Reference") (MeltBuildings4 :type "ActorComponent Object Reference") (MeltBuildings5 :type "ActorComponent Object Reference"))
  (bind _returnvalue (`Actor.GetAttachParentActor` Actor))
  (bind _returnvalue_2 (`PXCityComponent.GetCityArea` (`PXDistrictVisualComponent.GetCity` (`Actor.GetComponentByClass` (`Actor.GetAttachParentActor` (`local.Actor`)) "/Script/Frostpunk2.PXDistrictVisualComponent"))))
  (bind _returnvalue_3 (`PXCityAreaComponent.GetLeftBottom2D` _returnvalue_2))
  (bind (_returnvalue_x _returnvalue_y) (`KismetMathLibrary.BreakVector2D` (* (- _returnvalue_3 (`PXCityAreaComponent.GetCityAreaCenter2D` _returnvalue_2)) (2.0 2.0))))
  (`/Engine/EditorBlueprintResources/StandardMacros.IsValid` _returnvalue
    (:`Is Valid`
      (if (`PXDistrictComponent.IsMainDistrict` (`PXDistrictVisualComponent.GetDistrict` (`Actor.GetComponentByClass` _returnvalue "/Script/Frostpunk2.PXDistrictVisualComponent")))
        (bind _returnvalue_4 (`self.GetBoolArgument` (`local.Arguments`) "Enable"))
        (set `local.ShouldEnable` _returnvalue_4)
        (`|ExecutionSequence`
          (:`then_0`
            ;[1 1 1] Gather arguments
            (bind _returnvalue_5 (`self.GetComponentArgument` (`local.Arguments`) "CityMaskDrawer" (`local.Actor`) false))
            (bind _aspxcity_mask_drawer_component (cast `PXCityMaskDrawerComponent` _returnvalue_5))
            (set `local.Drawer` _aspxcity_mask_drawer_component)
            (bind _returnvalue_6 (`self.GetFloatArgument` (`local.Arguments`) "CPURadius"))
            (set `PXCityMaskDrawerComponent.CPUGridRadius` _returnvalue_6 (`local.Drawer`))
            (bind _returnvalue_7 (`self.GetComponentArgument` (`local.Arguments`) (`self.DistrictInactivityMaskName`) (`local.Actor`) false))
            (set `local.DistrictInactivityMask` _returnvalue_7)
            (bind _returnvalue_8 (`self.GetComponentArgument` (`local.Arguments`) (`self.DistrictActivityMaskName`) (`local.Actor`) false))
            (bind _asscene_component (cast `SceneComponent` _returnvalue_8)
              (:`then`
                (set `local.DistrictActivityMaskSC` _asscene_component))
              (:`CastFailed`
                (`KismetSystemLibrary.LogString` (`KismetStringLibrary.Concat_StrStr` (`KismetStringLibrary.Conv_NameToString` (`self.DistrictActivityMaskName`)) " not found!")))))
          (:`then_1`
            ;[1 1 1] Handle CPU mask
            (`PXCityMaskSubsystem.UpdateCPUGrid` (subsystem `PXCityMaskSubsystem`) (`local.Drawer`) (not (`local.ShouldEnable`)))
            ;[1 1 1] Handle GPU mask
            (`PXComponentUtils.SetComponentEnabled` (`local.DistrictInactivityMask`) (not (`local.ShouldEnable`)) "Activity")
            (if (`local.ShouldEnable`)
              (`PXComponentUtils.SetComponentEnabled` (`local.DistrictActivityMaskSC`) true "Activity"))
            ;[1 1 1] This is required to disable lights on roads when districts are disabled. It is done like that because its hard to get roads from district.
            (`PXStateUtils.SetStateInAreaByEntry` (`|MakeArray` _returnvalue_3 (- _returnvalue_3 (`KismetMathLibrary.MakeVector2D` 0.0 _returnvalue_y)) (- _returnvalue_3 (`KismetMathLibrary.MakeVector2D` _returnvalue_x _returnvalue_y)) (- _returnvalue_3 (`KismetMathLibrary.MakeVector2D` _returnvalue_x))) (struct :`StateGuid` "5536D1364C893648D491E6891E382D31") (`local.ShouldEnable`))
            ;[1 1 1] Handle snow melting
            (if (`local.ShouldEnable`)
              (`PXCityWeatherSubsystem.FadeOut` (subsystem `PXCityWeatherSubsystem`) (`local.DistrictActivityMaskSC`) (0.0 1.0) 0.5 false)
              (else
                (`PXCityWeatherSubsystem.FadeIn` (subsystem `PXCityWeatherSubsystem`) (`local.DistrictActivityMaskSC`) (0.0 1.0) 0.5 false)))))))))