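; State behavior for district activity actors that toggles components and refreshes landscape mask captures.
; Activation and deactivation run the same function, which sets the argument-specified components to the Enabled argument, using the state entry's enablement reason.
; It then recaptures masks through PXLandscapeMaskSubsystem.
; Directly attached actors with a VAT animator have their state switched off, then set to the Enabled value.
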(event `self.OnActivate`
  (params (owner :type "Actor Object Reference") (gameInstance :type "PXGameInstance Object Reference") (arguments :type "PXStateBehaviourArguments Object Reference") (stateEntry :type "PXStateEntry Structure"))
  (`self.BehaviorFunction Multiple Arguments` arguments owner stateEntry))

(event `self.OnDeactivate`
  (params (owner :type "Actor Object Reference") (gameInstance :type "PXGameInstance Object Reference") (arguments :type "PXStateBehaviourArguments Object Reference") (stateEntry :type "PXStateEntry Structure"))
  (`self.BehaviorFunction Multiple Arguments` arguments owner stateEntry))

(fn `BehaviorFunction Multiple Arguments`
  (params (Arguments :type "PXStateBehaviourArguments Object Reference") (Actor :type "Actor Object Reference") (`State Entry` :type "PXStateEntry Structure"))
  (`|ExecutionSequence`
    (:`then_0`
      (bind _returnvalue (`self.GetComponentArguments` Arguments Actor))
      (for _array_element _returnvalue
        (bind _returnvalue_2 (`self.GetBoolArgument` (`local.Arguments`) (`KismetStringLibrary.Conv_StringToName` "Enabled")))
        (bind _returnvalue_3 (`PXEnablementUtils.GetEnablementReasonForState` (`local.State Entry`)))
        (`PXComponentUtils.SetComponentEnabled` _array_element _returnvalue_2 _returnvalue_3)))
    (:`then_1`
      (`PXLandscapeMaskSubsystem.CaptureMasks` (subsystem `PXLandscapeMaskSubsystem`))
      (for _array_element_2 (`Actor.GetAttachedActors` Actor true false)
        (if (`KismetSystemLibrary.IsValid` (`Actor.GetComponentByClass` _array_element_2 "/Script/Frostpunk2.PXVatAnimatorComponent"))
          (`PXStateUtils.SetActorStateByEntry` _array_element_2 (struct :`StateGuid` "8DCFC9E04F97E52D6521FFB25C802177") false)
          (bind _returnvalue_4 (`self.GetBoolArgument` (`local.Arguments`) "Enabled"))
          (`PXStateUtils.SetActorStateByEntry` _array_element_2 (struct :`StateGuid` "8DCFC9E04F97E52D6521FFB25C802177") _returnvalue_4))))))