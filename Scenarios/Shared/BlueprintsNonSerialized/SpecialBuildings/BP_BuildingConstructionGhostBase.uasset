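; Base Blueprint for the special-building construction ghost, previewing a building mesh and showing whether it can be placed.
; On initialization it applies the supplied static mesh and scales it uniformly to fit within the TargetDimension box, using the smallest extent ratio.
; It replaces every material slot with a dynamic instance of M_SBGhost and caches these instances.
; Placeable state changes switch their EmissiveColor between the placeable and unplaceable colors.
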(event `self.OnInitialized`
  (params (staticMesh :type "StaticMesh Object Reference"))
  ;[1 1 1] Setting the mesh from building type or fallback from config
  (`parent.OnInitialized` staticMesh)
  (`StaticMeshComponent.SetStaticMesh` (`self.BuildingStaticMesh`) staticMesh)
  (`self.FitTargetDimensions`)
  (`self.OverrideMaterials`))

(event `self.OnDeinitialized`
  ;[1 1 1] Cleanup
  (`parent.OnDeinitialized`))

(event `self.OnPlaceableStateChanged`
  (params (isPlaceable :type Boolean))
  ;[1 1 1] We can change material colors here
  (`self.SetPlaceableColor` isPlaceable))

(fn `FitTargetDimensions`
  (`SceneComponent.SetWorldScale3D` (`self.BuildingStaticMesh`) (`KismetMathLibrary.Conv_DoubleToVector` (`KismetMathLibrary.GetMinElement` (/ (`BoxComponent.GetScaledBoxExtent` (`self.TargetDimension`)) (`.BoxExtent` (`KismetSystemLibrary.GetComponentBounds` (`self.BuildingStaticMesh`))))))))

(fn `OverrideMaterials`
  (for (_ _array_index) (`MeshComponent.GetMaterials` (`self.BuildingStaticMesh`))
    (bind _returnvalue (`KismetMaterialLibrary.CreateDynamicMaterialInstance` "/Game/Scenarios/Shared/Materials/SpecialBuildingGhost/M_SBGhost.M_SBGhost"))
    (`KismetArrayLibrary.Array_AddUnique` (`self.MIDs`) _returnvalue)
    (`PrimitiveComponent.SetMaterial` (`self.BuildingStaticMesh`) _array_index _returnvalue)))

(fn `SetPlaceableColor`
  (params (isPlaceable :type Boolean))
  (for _array_element (`self.MIDs`)
    (`MaterialInstanceDynamic.SetVectorParameterValue` _array_element "EmissiveColor" (`KismetMathLibrary.SelectColor` (`self.PlaceableColor`) (`self.UnplaceableColor`) isPlaceable))))

(fn `UserConstructionScript`)