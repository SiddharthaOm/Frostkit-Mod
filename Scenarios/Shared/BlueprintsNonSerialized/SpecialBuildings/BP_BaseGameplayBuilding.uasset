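; Base Blueprint for special gameplay buildings that keeps state entries on the building and its district's deposits in sync with its lifecycle.
; On start it binds to the construction-finished event and, a tick later, activates a state on the attach parent of each deposit's owner.
; When its own construction finishes or a matching state changes, it toggles its states and copies one from its parent actor.
; Destruction switches deposit states again, noted as for deep wood removal.
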(event `self.ReceiveEndPlay`
  (params (EndPlayReason :type "EEndPlayReason Enum" :default "Destroyed"))
  (bind _returnvalue (`PXDepositUtils.GetDepositsUsedByDistrict` (`PXBuildingComponent.OwningDistrict` (`self.GetComponentByClass` "/Script/Frostpunk2.PXBuildingComponent"))))
  ;[1 1 1] For deep wood removal
  (if (`|EnumEquality` EndPlayReason "Destroyed")
    (if (`KismetArrayLibrary.Array_IsValidIndex` _returnvalue)
      (for _array_element _returnvalue
        (bind _returnvalue_2 (`self.GetAttachParentActor` (`ActorComponent.GetOwner` _array_element)))
        (`PXStateUtils.SetActorStateByEntry` _returnvalue_2 (struct :`StateGuid` "9684C1BC4762CA66E2469295AD688449"))
        (`PXStateUtils.SetActorStateByEntry` _returnvalue_2 (struct :`StateGuid` "9684C1BC4762CA66E2469295AD688449") false)))))

(event `self.ReceiveActorStarted`
  (bind _returnvalue (`PXDepositUtils.GetDepositsUsedByDistrict` (`PXBuildingComponent.OwningDistrict` (`self.GetComponentByClass` "/Script/Frostpunk2.PXBuildingComponent"))))
  ;[1 1 1] For deep wood removal
  (bind _returnvalue_2 (`|Subsystem`)
    (:`then`
      (add `PXConstructionSubsystem.ConstructionFinishedEvent` _returnvalue_2 (delegate `AddStateOnFinished`))
      (`KismetSystemLibrary.DelayUntilNextTick`)
      (if (`KismetArrayLibrary.Array_IsValidIndex` _returnvalue)
        (for _array_element _returnvalue
          (`PXStateUtils.SetActorStateByEntry` (`self.GetAttachParentActor` (`ActorComponent.GetOwner` _array_element)) (struct :`StateGuid` "9684C1BC4762CA66E2469295AD688449")))))))

(event `AddStateOnFinished`
  (params (constructionComponent :type "PXConstructionComponent Object Reference"))
  (bind _returnvalue (`self.GetComponentByClass` "/Script/Frostpunk2.PXConstructionComponent"))
  (`/Engine/EditorBlueprintResources/StandardMacros.IsValid` _returnvalue
    (:`Is Valid`
      (if (== constructionComponent _returnvalue)
        (`PXStateUtils.SetActorStateByEntry` self (struct :`StateGuid` "E02E58F040BEC2DEAFE6F9BE30186FA0"))
        (`PXStateUtils.SetActorStateByEntry` self (struct :`StateGuid` "8DCFC9E04F97E52D6521FFB25C802177"))
        (`PXStateUtils.SetActorStateByEntry` self (struct :`StateGuid` "8DCFC9E04F97E52D6521FFB25C802177") false)
        (bind _returnvalue_2 (`PXStateUtils.GetActorStateByEntry` (`self.GetAttachParentActor`) (struct :`StateGuid` "8DCFC9E04F97E52D6521FFB25C802177")))
        (`PXStateUtils.SetActorStateByEntry` self (struct :`StateGuid` "8DCFC9E04F97E52D6521FFB25C802177") _returnvalue_2)
        (remove `PXConstructionSubsystem.ConstructionFinishedEvent` (stale `self.ReceiveActorStarted` _returnvalue_2) (`|CreateDelegate` :!event `AddStateOnFinished`))))))

(event `self.PXState.ChangedStateEvent`
  (params (StateComponent :type "PXStateComponent Object Reference") (Entry :type "PXStateEntry Structure (by ref)") (Activate :type Boolean))
  (if (`PXStateUtils.AreStatesEqual` Entry (struct :`StateGuid` "7BB63F5D41127ABE8AD88B99172217DB"))
    (`PXStateUtils.SetActorStateByEntry` self (struct :`StateGuid` "8DCFC9E04F97E52D6521FFB25C802177"))
    (`PXStateUtils.SetActorStateByEntry` self (struct :`StateGuid` "8DCFC9E04F97E52D6521FFB25C802177") false)
    (bind _returnvalue (`PXStateUtils.GetActorStateByEntry` (`self.GetAttachParentActor`) (struct :`StateGuid` "8DCFC9E04F97E52D6521FFB25C802177")))
    (`PXStateUtils.SetActorStateByEntry` self (struct :`StateGuid` "8DCFC9E04F97E52D6521FFB25C802177") _returnvalue)))

(fn `UserConstructionScript`)