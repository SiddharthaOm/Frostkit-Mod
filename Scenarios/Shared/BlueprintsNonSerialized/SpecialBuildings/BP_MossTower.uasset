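; BP_MossTower is a moss filtration tower special building whose head meshes align with the map's default wind direction.
; Shortly after BeginPlay, following a brief delay, it reads DefaultWindDirection from the general weather config.
; It converts that vector to a look-at rotation from the origin and sets it as the world rotation of three head components.
; The orientation is set once, with no further updates.
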(event `self.ReceiveBeginPlay`
  (bind _returnvalue (`KismetMathLibrary.FindLookAtRotation` (`KismetMathLibrary.MakeVector` 0.0) (`PXGeneralWeatherConfig.DefaultWindDirection` (`PXGameplayUtils.GetGeneralWeatherConfig`))))
  (`KismetSystemLibrary.Delay` 0.2)
  (`SceneComponent.K2_SetWorldRotation` (`self.SM_CIT_HOU_MossFiltrationTower_D_Head`) _returnvalue false false)
  (`SceneComponent.K2_SetWorldRotation` (`self.SM_CIT_HOU_MossFiltrationTower_D_Head2`) _returnvalue false false)
  (`SceneComponent.K2_SetWorldRotation` (`self.SM_CIT_HOU_MossFiltrationTower_D_Head1`) _returnvalue false false))

(fn `UserConstructionScript`)