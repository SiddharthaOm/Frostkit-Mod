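; Base game mode that starts the multiplayer game for joining players and sets the initial input mode.
; Outside standalone, PostLogin casts the new player to BP_MP_MainPlayerController and calls MPStartGame, retrying a failed cast through a zero-length delay.
; BeginPlay puts the first player controller in Game and UI input with a visible cursor.
; MP_StartGame is an empty stub, and the default scenario loading and connected-player list logic are disconnected.
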(event `MP_StartGame`
  ;[1 1 1] SIDD>>>>> RUN THIS CODE IN THE CONTROLLER AND CALL IT FROM GAMESTATE!
)

(event `self.K2_PostLogin`
  (params (NewPlayer :type "PlayerController Object Reference"))
  ;[1 1 1] MP Game Scenario Load
  ; TODO add scenario selection
  (if (`KismetSystemLibrary.IsStandalone`)
    (`KismetSystemLibrary.PrintString` "Is Standalone!")
    (else
      (bind _asbp_mp_main_player_controller (cast `/Game/Scenarios/Shared/BlueprintsNonSerialized/Main/BP_MP_MainPlayerController` NewPlayer :!label _label)
        (:`then`
          (`/Game/Scenarios/Shared/BlueprintsNonSerialized/Main/BP_MP_MainPlayerController.MP_StartGame` _asbp_mp_main_player_controller))
        (:`CastFailed`
          (`KismetSystemLibrary.Delay` 0.0)
          (goto _label))))))

(event `self.ReceiveBeginPlay`
  ;[1 1 1] This code survives..... for now
  (`WidgetBlueprintLibrary.SetInputMode_GameAndUIEx` (`GameplayStatics.GetPlayerController` 0) null "DoNotLock" false))

(fn `UserConstructionScript`)