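; Small coal extraction slot Blueprint for procedurally generated Urbos area fillers.
; On BeginPlay it randomly either keeps its placed rotation or sets it to a fixed 90-degree turn, adding layout variety.
; When its terraform connector reports a failed connection, it enables fallback components: an empty-lot mesh, a proxy, a snow cap and a melt quad.
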(event `self.ReceiveBeginPlay`
  (switch `int` (`KismetMathLibrary.RandomInteger` 2)
    (:`0`
      (`self.K2_SetActorRotation` (struct :`Yaw` 90.0)))))

(event `self.Connector_Terraform.ConnectionFailedEvent`
  (params (connector :type "PXUrbosConnectorComponent Object Reference"))
  (`PXComponentUtils.SetComponentEnabled` (`self.SM_CIT_EXT_EmptyLot_C`) true)
  (`PXComponentUtils.SetComponentEnabled` (`self.SM_CIT_EXT_Proxy`) true)
  (`PXComponentUtils.SetComponentEnabled` (`self.GENERATED_SnowCap1`) true)
  (`PXComponentUtils.SetComponentEnabled` (`self.MeltQuad`) true))

(fn `UserConstructionScript`)