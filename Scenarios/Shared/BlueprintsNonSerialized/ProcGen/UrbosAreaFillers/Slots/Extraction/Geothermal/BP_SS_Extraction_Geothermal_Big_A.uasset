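; Big geothermal extraction slot (variant A) for the procedurally generated urban area fillers.
; On BeginPlay it has a one-in-two chance of setting its rotation to a 90-degree turn for variety.
; If the terraform connector fails to connect, it enables empty-lot, steam, melt quad and frame components.
; When that connector turns active, it disables both steam bursts, with no branch to re-enable them.
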(event `self.ReceiveBeginPlay`
  (switch `int` (`KismetMathLibrary.RandomInteger` 2)
    (:`0`
      (`self.K2_SetActorRotation` (struct :`Yaw` 90.0)))))

(event `self.Connector_Terraform.ConnectionFailedEvent`
  (params (connector :type "PXUrbosConnectorComponent Object Reference"))
  (`PXComponentUtils.SetComponentEnabled` (`self.SM_CIT_EXT_EmptyLot_C1`) true)
  (`PXComponentUtils.SetComponentEnabled` (`self.SM_CIT_PRD_suburbs_steam1`) true)
  (`PXComponentUtils.SetComponentEnabled` (`self.MeltQuad`) true)
  (`PXComponentUtils.SetComponentEnabled` (`self.Frame3_A`) true)
  (`PXComponentUtils.SetComponentEnabled` (`self.SM_CIT_PRD_suburbs_steam2`) true))

(event `self.Connector_Terraform.ChangedStateEvent`
  (params (Connector :type "PXUrbosConnectorComponent Object Reference") (Active :type Boolean))
  (if Active
    (`PXComponentUtils.SetComponentEnabled` (`self.SteamBurst1`) false "Connector")
    (`PXComponentUtils.SetComponentEnabled` (`self.SteamBurst2`) false "Connector")))

(fn `UserConstructionScript`)