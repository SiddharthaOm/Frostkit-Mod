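; BP_LogEnabler is an Urbos logistics tile actor that shows a logistics arm when its connector is active.
; Connector activation triggers a deferred building-slot refresh, enables one of four positional random spawners, and links spawned actors to the district owner for interaction.
; Deactivation disables and clears that spawner.
; A separate SnapEndpoint event traces vertically ahead to place the trail endpoint, matching the connector's yaw.
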(event `Snap Endpoint`
  (bind _trail_end_point (`self.Trail end point`))
  (bind (_returnvalue_roll _returnvalue_pitch _returnvalue_yaw) (`KismetMathLibrary.BreakRotator` (`SceneComponent.K2_GetComponentRotation` (`self.PXUrbosConnector`))))
  (bind _returnvalue (+ (`self.K2_GetActorLocation`) (* (`self.GetActorForwardVector`) (`self.DistanceOfEndpoint`))))
  (bind _outhit (`KismetSystemLibrary.LineTraceSingle` :`Start` (+ _returnvalue (0.0 0.0 4000.0)) :`End` (+ _returnvalue (0.0 0.0 -4000.0)) :`TraceChannel` "TraceTypeQuery4" :`DrawDebugType` "ForDuration" :`DrawTime` 4.0))
  (`self.K2_SetActorLocation` _trail_end_point (`.Location` (`GameplayStatics.BreakHitResult` _outhit)) false false)
  (`self.K2_SetActorRotation` _trail_end_point (`KismetMathLibrary.MakeRotator` 0.0 0.0 _returnvalue_yaw) false))

(event `self.PXUrbosConnector.ChangedStateEvent`
  (params (Connector :type "PXUrbosConnectorComponent Object Reference") (Active :type Boolean))
  (bind _returnvalue (`PXDistrictUtils.FindParentDistrictVisual` Connector))
  (bind _currentspawn (`self.CurrentSpawn`))
  ;[1 1 1] buildings slots
  (if Active
    (`PXDistrictVisualSubsystem.RefreshBuildingSlotsDeferred` (subsystem `PXDistrictVisualSubsystem`) _returnvalue :!pinned true) ; Deferred to make sure connectedTo is\nalready set on executor and enabler already\nspawned the arm
  )
  (if Active
    (bind _output_get (set `self.CurrentSpawn` (`KismetArrayLibrary.Array_Random` (`|MakeArray` (`self.PXPositionalRandomSpawn_LOG_UNIQ_A5`) (`self.PXPositionalRandomSpawn_LOG_UNIQ_A2`) (`self.PXPositionalRandomSpawn_LOG_UNIQ_A4`) (`self.PXPositionalRandomSpawn_LOG_UNIQ_A3`)))))
    (`PXComponentUtils.SetComponentEnabled` _output_get true)
    ;[0.03125 0.03125 0.03125] Interact with log arm outside of placement area
    (bind _returnvalue_2 (`PXPositionalRandomSpawnComponent.GetSpawnedActors` (`self.CurrentSpawn`)))
    (for _array_element _returnvalue_2
      (`/Engine/EditorBlueprintResources/StandardMacros.IsValid` (`PXInteractionUtils.AddInteractionComponent` _array_element (`ActorComponent.GetOwner` (`PXDistrictVisualComponent.GetDistrict` _returnvalue)))) ; thanks for pure function :V
    )
    (else
      (`/Engine/EditorBlueprintResources/StandardMacros.IsValid` _currentspawn
        (:`Is Valid`
          (`PXComponentUtils.SetComponentEnabled` _currentspawn)
          (set `self.CurrentSpawn` null))))))

(fn `UserConstructionScript`)