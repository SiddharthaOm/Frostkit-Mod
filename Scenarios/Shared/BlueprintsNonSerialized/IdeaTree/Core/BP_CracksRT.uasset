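; BP_CracksRT captures the Idea Tree's crack meshes into what appears to be a render target mask for materials.
; BeginPlay writes the capture camera's position and ortho width to MPC_IdeaTree.
; CookCracks reveals each mesh from RefAllCracksBP, adds it to the show-only list with an unlit coloration material, and captures.
; RestoreCracks reapplies the gold crack material and has RefResearchNodesBP hide unused cracks.
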(event `self.ReceiveBeginPlay`
  (bind _rt_camera (`self.RT_Camera`))
  (bind _orthowidth (`SceneCaptureComponent2D.OrthoWidth` _rt_camera))
  (`KismetMaterialLibrary.SetVectorParameterValue` "/Game/Scenarios/Shared/Materials/MaterialParameterCollection/MPC_IdeaTree.MPC_IdeaTree" "RTPosition" (`KismetMathLibrary.Conv_VectorToLinearColor` (`SceneComponent.K2_GetComponentLocation` _rt_camera)))
  (`KismetMaterialLibrary.SetVectorParameterValue` "/Game/Scenarios/Shared/Materials/MaterialParameterCollection/MPC_IdeaTree.MPC_IdeaTree" "RTCracksSize" (make `LinearColor` _orthowidth _orthowidth 1.0 1.0)))

(fn `CookCracks`
  (bind _rt_camera (`self.RT_Camera`))
  (`SceneCaptureComponent.ClearShowOnlyComponents` _rt_camera)
  (for _array_element (`PXIdeaTreeNodesActor.CracksMeshes` (`self.RefAllCracksBP`))
    (bind _returnvalue (`KismetSystemLibrary.LoadAsset_Blocking` _array_element))
    (bind _asstatic_mesh_component (cast `StaticMeshComponent` _returnvalue))
    (`SceneComponent.SetHiddenInGame` _asstatic_mesh_component false false)
    (`SceneComponent.SetVisibility` _asstatic_mesh_component true false)
    (`SceneCaptureComponent.ShowOnlyComponent` _rt_camera _asstatic_mesh_component)
    (`PrimitiveComponent.SetMaterial` _asstatic_mesh_component 0 "/Engine/EngineDebugMaterials/LevelColorationUnlitMaterial.LevelColorationUnlitMaterial")
    (`SceneCaptureComponent2D.CaptureScene` (`self.RT_Camera`))))

(fn `RestoreCracks`
  (for _array_element (`PXIdeaTreeNodesActor.CracksMeshes` (`self.RefAllCracksBP`))
    (bind _returnvalue (`KismetSystemLibrary.LoadAsset_Blocking` _array_element))
    (bind _asstatic_mesh_component (cast `StaticMeshComponent` _returnvalue))
    (`SceneComponent.SetHiddenInGame` _asstatic_mesh_component false false)
    (`SceneComponent.SetVisibility` _asstatic_mesh_component true false)
    (`PrimitiveComponent.SetMaterial` _asstatic_mesh_component 0 "/Game/Scenarios/Shared/FXs/Materials/MaterialInstnaces/MI_Gold_Cracks.MI_Gold_Cracks")
    (`/Game/Scenarios/Shared/BlueprintsNonSerialized/IdeaTree/Core/ResearchNodes/BP_ResearchNodes.HideUnusedCracks` (`self.RefResearchNodesBP`))))

(fn `UserConstructionScript`)