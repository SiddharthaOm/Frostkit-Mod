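; Mist cloud plane for the Idea Tree that adds UI sound to its animation phases.
; On BeginPlay it binds to the audio start events of a subsystem, once that subsystem is valid.
; The gold cracks and cloud phases each post a 2D audio event: golden path and mist whoosh.
; The aftershock handler is empty, and the stop-all-animation handler is empty and never bound.
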(event `StopAllAnimation_Event`)

(event `self.ReceiveBeginPlay`
  (bind _returnvalue (`|Subsystem`)
    (:`then`
      (add `PXIdeaTreeSubsystem.GoldCracksAnimationStartAudioEvent` _returnvalue (delegate `GoldCracksAnimationStartAudioEvent_Event`))
      (add `PXIdeaTreeSubsystem.CloudAnimationStartAudioEvent` _returnvalue (delegate `CloudAnimationStartAudioEvent_Event`))
      (add `PXIdeaTreeSubsystem.AftershockAnimationStartAudioEvent` _returnvalue (delegate `AftershockAnimationStartAudioEvent_Event`)))))

(event `GoldCracksAnimationStartAudioEvent_Event`
  (params (duration :type "Float (single-precision)"))
  (`/Game/Scenarios/Shared/BlueprintsNonSerialized/Audio/BPFL_AudioUtils.Post 2d Audio Event` "/Game/Scenarios/Shared/Audio/Events/UI/Research/ui_idea_tree_golden_path.ui_idea_tree_golden_path"))

(event `CloudAnimationStartAudioEvent_Event`
  (params (duration :type "Float (single-precision)"))
  (`/Game/Scenarios/Shared/BlueprintsNonSerialized/Audio/BPFL_AudioUtils.Post 2d Audio Event` "/Game/Scenarios/Shared/Audio/Events/UI/Research/ui_idea_tree_myst_whoosh.ui_idea_tree_myst_whoosh"))

(event `AftershockAnimationStartAudioEvent_Event`
  (params (duration :type "Float (single-precision)")))

(fn `UserConstructionScript`)