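; Gameplay action that activates a configured ability on the owner of the best city or district found in the context.
; A flag picks city or district, and the ability must pass an availability check.
; It either activates immediately with the context's action origin, or, with AfterTick set, hands actor, origin and ability to a fake quest named for post-tick activation.
; It supplies no gameplay factor values.
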(fn `Activate Ability`
  (params (context :type "PXGameContext Structure (by ref)"))
  (locals (owner :type "Actor Object Reference"))
  (bind _returnvalue_passed (break `PXCheckResult` (`PXAbilityUtils.IsActorAbilityAvailable` (`local.owner`) (`self.Ability`))))
  (if (`self.City Ability?`)
    (set `local.owner` (`ActorComponent.GetOwner` (`/Game/Scenarios/Shared/BlueprintsNonSerialized/SocietyUtils/BPFL_Communication_Utils.Get Best City from Context` context)))
    (else
      (set `local.owner` (`ActorComponent.GetOwner` (`/Game/Scenarios/Shared/BlueprintsNonSerialized/SocietyUtils/BPFL_Communication_Utils.Get Best District from Context` context)))))
  (if _returnvalue_passed
    (if (`self.After Tick?`)
      (bind _returnvalue (`PXQuestUtils.StartQuest` "/Game/Scenarios/Shared/BlueprintsSerialized/Quests/BP_FAKE_ActivateAbilityAfterTick_Quest.BP_FAKE_ActivateAbilityAfterTick_Quest_C"))
      (`/Game/Scenarios/Shared/BlueprintsSerialized/Quests/BP_FAKE_ActivateAbilityAfterTick_Quest.Setup Variables` _returnvalue (`local.owner`) (`PXGameplayContextUtils.TryGetActionOriginFromGameContext` (`local.context`)) (`self.Ability`))
      (else
        (`PXAbilityUtils.ActivateActorAbility` (`local.owner`) (`self.Ability`) (`PXGameplayContextUtils.TryGetActionOriginFromGameContext` (`local.context`)))))))

(fn `ExecuteAction`
  (params (context :type "PXGameContext Structure (by ref)"))
  (`self.Activate Ability` context)
  (return))

(fn `GetGameplayFactorValues`
  (params (factorValues :type "Array of PXGameplayFactorValues Structure (by ref)") (context :type "PXGameContext Structure (by ref)"))
  ;[1 1 1] Empty on purpose
  (return))