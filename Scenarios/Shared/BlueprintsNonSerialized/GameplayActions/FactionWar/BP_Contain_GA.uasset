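; Faction War gameplay action for containment that swaps one imprint for another on communities.
; When executed, it finds every community with ImprintToCheck, removes that imprint and adds ImprintToAdd.
; A disconnected, never-run branch would move population from Banned-imprint communities into Detainees and adjust detainees for faction size.
; The gameplay factor values function is empty.
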(fn `ExecuteAction`
  (params (context :type "PXGameContext Structure (by ref)"))
  (locals (NewLocalVar :type "Array of PXCommunityComponent Object Reference") (`imprint to check` :type "PXImprint Object Reference" :default "/Script/Frostpunk2.PXImprint'/Game/Scenarios/Shared/Configs/Communities/Imprints/DA_Shared_ToBeContained_Imprint.DA_Shared_ToBeContained_Imprint'") (`imprint to add` :type "PXImprint Object Reference" :default "/Script/Frostpunk2.PXImprint'/Game/Scenarios/Shared/Configs/Communities/Imprints/DA_Shared_Contained_Imprint.DA_Shared_Contained_Imprint'"))
  (bind _output_get (set `local.NewLocalVar` (`PXCommunityUtils.GetAllCommunitiesWithImprint` (`local.imprint to check`))))
  (for _array_element _output_get
    (`PXCommunityUtils.RemoveImprint` _array_element (`local.imprint to check`))
    (`PXCommunityUtils.AddImprint` _array_element (`local.imprint to add`))))

(fn `GetGameplayFactorValues`
  (params (factorValues :type "Array of PXGameplayFactorValues Structure (by ref)") (context :type "PXGameContext Structure (by ref)"))
  (return))