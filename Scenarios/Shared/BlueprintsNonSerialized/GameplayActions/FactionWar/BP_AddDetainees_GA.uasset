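; Faction War gameplay action that adds detainees by fixed, ranged or percentage amounts, if capacity allows.
; Without the Pick A Side unlock, it targets all main-city factions, the context community, or the war's initial aggressor/defender (roundup path), optionally requiring fervor.
; With the unlock, it skips target selection and adds detainees directly.
; Without capacity, it starts the FailedToDetain story arc if untracked and notifies that militants are released.
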(fn `ExecuteAction`
  (params (context :type "PXGameContext Structure (by ref)"))
  (locals (prisons :type "Array of PXBuildingType Object Reference") (`failed to detain` :type "PXParameterizedStoryArc Class Reference" :default "/Script/Engine.BlueprintGeneratedClass'/Game/Scenarios/Shared/BlueprintsSerialized/StoryArcs/FactionWar/BP_FactionWar_FailedToDetain_SA.BP_FactionWar_FailedToDetain_SA_C'"))
  (bind (_community _found) (`/Game/Scenarios/Shared/BlueprintsNonSerialized/SocietyUtils/BPFL_Communication_Utils.Get Best Community from Context` (`local.context`)))
  (bind _returnvalue (select `bool` (`self.Target Agressor?`) :`false` (`/Game/Scenarios/Shared/BlueprintsNonSerialized/SocietyUtils/BPFL_SharedScenariosStorage.Get Faction War Initial Defender`) :`true` (`/Game/Scenarios/Shared/BlueprintsNonSerialized/SocietyUtils/BPFL_SharedScenariosStorage.Get Faction War Initial Aggressor`)))
  (bind _returnvalue_2 (`/Game/Scenarios/Shared/BlueprintsNonSerialized/FactionEmergence/BPFL_FactionWarUtils.Can Add More Detainees?`))
  (if _returnvalue_2
    (if (not (`PXUnlockUtils.IsUnlockActive` (`PXNationUtils.GetPlayerNation`) "/Game/Scenarios/Shared/Configs/Unlocks/FactionWarEndings/DA_PickASide_Unlock.DA_PickASide_Unlock"))
      (if (`self.All Factions?`)
        (for _array_element (`PXFactionUtils.GetMembersFromCity` (`PXNationUtils.GetPlayerMainCity`) null)
          (`self.Handle One Faction` _array_element))
        (elif _found
          (`self.Handle One Faction` _community)
          (elif (`KismetSystemLibrary.IsValid` _returnvalue)
            (`self.Handle One Faction` _returnvalue true))))
      (elif (`self.Use Percent?`)
        (`/Game/Scenarios/Shared/BlueprintsNonSerialized/FactionEmergence/BPFL_FactionWarUtils.Add Detainees Percent of Deported Faction` (`self.Percent`))
        (return)
        (elif (`self.Use Range?`)
          (`/Game/Scenarios/Shared/BlueprintsNonSerialized/FactionEmergence/BPFL_FactionWarUtils.Add Detainees` (`PXRandomLibrary.PXRandomIntegerInRange` (`self.Min`) (`self.Max`)))
          (return)
          (else
            (`/Game/Scenarios/Shared/BlueprintsNonSerialized/FactionEmergence/BPFL_FactionWarUtils.Add Detainees` (`self.Detainees`))
            (return)))))
    (else
      (if (not (`PXStoryUtils.IsStoryArcOfClassTracked` (`local.failed to detain`)))
        (bind _returnvalue_3 (`|GenericCreateObject` (subsystem `PXStoryArcSubsystem`) (`local.failed to detain`)))
        (bind _returnvalue_4 (`PXStoryUtils.StartParameterizedStoryArc` _returnvalue_3))
        (if _returnvalue_4
          _
          (else
            _)))
      (`PXCommunicationChannelsUtils.AddNotification` (make `PXNotificationData` "Normal" (`|FormatText` "Guards forced to release detained militants due to lack of prison space"))))))

(fn `GetGameplayFactorValues`
  (params (factorValues :type "Array of PXGameplayFactorValues Structure (by ref)") (context :type "PXGameContext Structure (by ref)"))
  ;[1 1 1] Empty on purpose
  (return))

(fn `Handle One Faction`
  (params (InputPin :type "PXCommunityComponent Object Reference") (`FromRoundup?` :type Boolean))
  (if (`self.Only with Fervour?`)
    (if (> (`PXTraitType.SeverityLevel` (`PXInfluenceUtils.GetFervorTraitType` (`PXNationUtils.GetPlayerMainCity`) (`PXCommunityComponent.GetCommunityType` InputPin))) 0)
      (if `FromRoundup?` :!label _label
        (`KismetArrayLibrary.Array_Remove` (`/Game/Scenarios/Shared/BlueprintsSerialized/VariableStorage/BP_SharedVariableStorage.Roundup Target Communities` (`/Game/Scenarios/Shared/BlueprintsNonSerialized/SocietyUtils/BPFL_SharedScenariosStorage.Get Shared Variable Storage`))))
      (if (`self.Use Percent?`)
        (`/Game/Scenarios/Shared/BlueprintsNonSerialized/FactionEmergence/BPFL_FactionWarUtils.Add Detainees Percent of Passed Faction` (`self.Percent`) InputPin (struct) (`local.FromRoundup?`))
        (else
          (`/Game/Scenarios/Shared/BlueprintsNonSerialized/FactionEmergence/BPFL_FactionWarUtils.Add Detainees from Passed Faction` (`PXRandomLibrary.PXRandomIntegerInRange` (`self.Min`) (`self.Max`)) InputPin (struct) (`local.FromRoundup?`)))))
    (else
      (goto _label))))