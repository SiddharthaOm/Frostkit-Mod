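; Scenario gameplay action for Condemn Radicals that forces a configured community action on behalf of one faction's community.
; The acting community comes from the existing faction whose affinity is opposite to the Winterhome choice.
; The action origin is taken from the game context.
; When the economic layout flag is set, it also adds the wrapped action's gameplay action to the reported factor values.
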(fn `ExecuteAction`
  (params (context :type "PXGameContext Structure (by ref)"))
  (`PXCommunityActionUtils.ExecuteCommunityAction` (`self.Action`) (`PXGameplayContextUtils.TryGetActionOriginFromGameContext` context) (`.ReturnValue` (`PXFactionUtils.GetCommunityFromFaction` (`/Game/Scenarios/Shared/BlueprintsNonSerialized/SocietyUtils/BPFL_StoryArc_Utils.Get existing faction with affinity` (`/Game/Scenarios/Shared/BlueprintsNonSerialized/SocietyUtils/BPFL_Cornerstone_Utils.Get Opposite Affinity` (`/Game/Scenarios/Main/BlueprintsNonSerialized/ScenarioFunctionLibrary/BPFL_S1_ScenarioFunctionLibrary.Get Winterhome Choice Affinity`))))) true)
  (return))

(fn `GetGameplayFactorValues`
  (params (factorValues :type "Array of PXGameplayFactorValues Structure (by ref)") (context :type "PXGameContext Structure (by ref)"))
  (if (`self.Show Economic Layout`)
    (`PXGameplayActionUtils.AddGameplayActionToGameplayFactorValues` factorValues (`PXCommunityAction.GameplayAction` (`self.Action`)) context)
    (return)
    (else
      (return))))