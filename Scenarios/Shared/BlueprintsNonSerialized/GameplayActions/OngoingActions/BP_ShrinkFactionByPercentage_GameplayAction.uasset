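; Gameplay action that shrinks the context community's faction by a randomized percentage of the city's total size units.
; The random multiplier is scaled by a reverted membership population multiplier, then applied through ShrinkFactionUsingAllCommunitiesInCity with a reason and notification settings.
; An older proportional transfer to independent communities is left disconnected.
; Gameplay factor values are intentionally empty, and the trust-based scaling helper is unused here.
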(fn `ExecuteAction`
  (params (context :type "PXGameContext Structure (by ref)"))
  (bind (_community _isvalid) (`PXGameplayContextUtils.TryGetCommunityComponentFromGameContext` context))
  (if _isvalid
    (`/Engine/EditorBlueprintResources/StandardMacros.IsValid` (`PXCommunityComponent.GetFaction` _community)
      (:`Is Valid`
        (`/Game/Scenarios/Shared/BlueprintsNonSerialized/FactionEmergence/BPFL_FactionEmergenceUtils.Shrink Faction Using All Communities in City` _community (`KismetMathLibrary.FTrunc` (* (`KismetMathLibrary.Conv_IntToDouble` (`/Game/Scenarios/Shared/BlueprintsNonSerialized/Communities/BPFL_CommunityUtils.Get Total Size Units in City` (`PXGameplayContextUtils.TryGetCityFromGameContext` context))) (* (`/Game/Scenarios/Shared/BlueprintsNonSerialized/Communities/BPFL_CommunityUtils.Get Membership Population Multiplier` _community true) (`PXRandomLibrary.PXRandomFloatInRange` (`self.Multiplier Min`) (`self.Multiplier Max`))))) (`self.REASON`) true (`self.Use Custom Notification Template?`) (`self.Change Duration`))))))

(fn `Get Trust Scaling Factor`
  (params (nation :type "PXNationComponent Object Reference"))
  (returns (ReturnValue :type "Float (double-precision)"))
  (bind _returnvalue (`PXTrustUtils.GetTotalTrust` nation))
  (if (>= _returnvalue 0.0)
    (return (select `int` (`PXTraitType.SeverityLevel` (`PXTrustUtils.GetTraitTypeByTrustValue` "/Game/Scenarios/Shared/Configs/Trust/DA_OverallTrustType.DA_OverallTrustType" _returnvalue)) :`0` 0.5 :`1` 0.6 :`2` 0.7 :`3` 0.8 :`4` 1.0))
    (else
      (return 0.4))))

(fn `GetGameplayFactorValues`
  (params (factorValues :type "Array of PXGameplayFactorValues Structure (by ref)") (context :type "PXGameContext Structure (by ref)"))
  ;[1 1 1] Empty on purpose
  (return))