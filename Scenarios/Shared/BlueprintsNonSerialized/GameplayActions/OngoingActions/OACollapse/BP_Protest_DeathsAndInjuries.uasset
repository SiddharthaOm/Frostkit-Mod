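; Gameplay action that periodically kills and injures bystanders in the player's main city during protests.
; The active protest count selects a cooldown, falling back to the last map entry, checked against a shared timestamp so all protests share one timer.
; Casualties scale with city population and percentages keyed by the protesting community's strength tier.
; KillAndInjure applies deaths and injured workforce absences, then a notification reports results if anyone was injured.
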(fn `ExecuteAction`
  (params (context :type "PXGameContext Structure (by ref)"))
  (locals (RequiredSpacing :type "PXGameTime Structure"))
  (bind _strenght_trait (`/Game/Scenarios/Shared/BlueprintsNonSerialized/OngoingEvents/BPFL_OngoingAction_Utils.Get Community Strength Tier` (`PXOngoingActionComponent.GetCommunity` (`PXGameplayContextUtils.TryGetOngoingActionFromGameContext` context))))
  ;[1 1 1] Are there any AO?
  (bind _number (`/Game/Scenarios/Shared/BlueprintsNonSerialized/OngoingEvents/BPFL_OngoingAction_Utils.GetNumberOfOngoingActionsOfType` "/Game/Scenarios/Shared/Configs/OngoingActions/System_Started/DA_Protest.DA_Protest"))
  (if (> _number 0)
    (bind (_value _returnvalue) (`BlueprintMapLibrary.Map_Find` (`self.SpacingPerDistrictsAffected`) _number))
    ;[1 1 1] Does spacing match
    (if _returnvalue
      (set `local.RequiredSpacing` _value)
      ;[1 1 1] Get injure and death counts
      (if (`PXTimeUtils.Greater` (`PXTimeUtils.GetCurrentGameTime`) (`PXTimeUtils.Add` (`/Game/Scenarios/Shared/BlueprintsSerialized/VariableStorage/BP_SharedVariableStorage.TimeOfLastProtestInjuries` (`/Game/Scenarios/Shared/BlueprintsNonSerialized/SocietyUtils/BPFL_SharedScenariosStorage.Get Shared Variable Storage`)) (`local.RequiredSpacing`))) :!label _label
        (set `/Game/Scenarios/Shared/BlueprintsSerialized/VariableStorage/BP_SharedVariableStorage.TimeOfLastProtestInjuries` (`PXTimeUtils.GetCurrentGameTime`) (`/Game/Scenarios/Shared/BlueprintsNonSerialized/SocietyUtils/BPFL_SharedScenariosStorage.Get Shared Variable Storage`))
        (bind (_killed _injured) (`self.Kill and Injure` (`KismetMathLibrary.FTrunc` (* (`PXCommunityUtils.GetScaledCityPopulationSize` (`PXNationUtils.GetPlayerMainCity`)) (`BlueprintMapLibrary.Map_Find` (`self.PercentDeadPerFervor`) _strenght_trait))) (`KismetMathLibrary.FTrunc` (* (`PXCommunityUtils.GetScaledCityPopulationSize` (`PXNationUtils.GetPlayerMainCity`)) (`BlueprintMapLibrary.Map_Find` (`self.PercentInjuredPerFervor`) _strenght_trait)))))
        ;[1 1 1] Apply penalty
        (if (> _injured 0)
          (if (> _killed 0)
            (`PXCommunicationChannelsUtils.AddNotification` (make `PXNotificationData` "PopulationDeath" (`|FormatText` "{X} bystanders killed and {Y} injured in the protest" _killed _injured)))
            (else
              (`PXCommunicationChannelsUtils.AddNotification` (make `PXNotificationData` "PopulationDeath" (`|FormatText` "{X} bystanders injured in the protest" _injured)))))))
      (else
        (bind _keys (`BlueprintMapLibrary.Map_Keys` (`self.SpacingPerDistrictsAffected`)))
        (bind (_value_2 _returnvalue_2) (`BlueprintMapLibrary.Map_Find` (`self.SpacingPerDistrictsAffected`) (`KismetArrayLibrary.Array_Find` _keys (`KismetArrayLibrary.Array_LastIndex` _keys))))
        (if _returnvalue_2
          (set `local.RequiredSpacing` _value_2)
          (goto _label))))))

(fn `Kill and Injure`
  (params (KillCounts :type Integer) (`Injure Counts` :type Integer))
  (returns (Killed :type Integer) (Injured :type Integer))
  (locals (Kills :type Integer) (Injurs :type Integer))
  (bind _size_units_killed (`/Game/Scenarios/Shared/BlueprintsNonSerialized/GameplayActions/BPFL_GameplayAction_Utils.Kill Number Of Units in City` (`|FormatText` "bystanders were killed by warring factions") (`PXNationUtils.GetPlayerMainCity`) KillCounts false true true))
  (set `local.Kills` _size_units_killed)
  (bind _returnvalue (`PXAbsenceUtils.AddWorkforceCurrentAbsenceInCity` (`PXNationUtils.GetPlayerMainCity`) "/Game/Scenarios/Shared/Configs/Absences/AbsenceTypes/DA_Injured_Absence.DA_Injured_Absence" (`local.Injure Counts`)))
  (bind _output_get (set `local.Injurs` _returnvalue))
  (return (`local.Kills`) _output_get))