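; Gameplay action that ends an ongoing action resolved from the game context, using configured collapse, simultaneous-collapse and end-type settings.
; It takes the action from the context's district, otherwise from the best community, otherwise directly from the context; a found district or community without one stops the search.
; EndOngoingAction receives start and finish gameplay actions plus the community's faction name as a text tag.
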(fn `ExecuteAction`
  (params (context :type "PXGameContext Structure (by ref)"))
  (locals (`OA Data` :type "PXOngoingActionComponent Object Reference"))
  (bind (_district _isvalid) (`PXGameplayContextUtils.TryGetDistrictFromGameContext` context))
  (bind (_community _found) (`/Game/Scenarios/Shared/BlueprintsNonSerialized/SocietyUtils/BPFL_Communication_Utils.Get Best Community from Context` context))
  (bind (_ongoingaction _isvalid_2) (`PXGameplayContextUtils.TryGetOngoingActionFromGameContext` context))
  (bind _oa_data (`local.OA Data`))
  (if _isvalid
    (bind (_hasongoingaction _returnvalue) (`PXOngoingActionUtils.GetOngoingActionComponentForDistrict` _district))
    (if _hasongoingaction
      (set `local.OA Data` _returnvalue)
      (`PXOngoingActionUtils.EndOngoingAction` _oa_data (`self.Gameplay Action on Start`) (`self.Gameplay Action on Finish`) (`|MakeMap` "FACTION" (`PXFactionUtils.GetFactionInGameName` (`PXOngoingActionComponent.GetCommunity` _oa_data))) (`self.Collapse Mode`) (`self.Simultaneous Collapse`) (`self.End Type`) :!label _label)
      (return))
    (elif _found
      (bind (_hasongoingaction_2 _returnvalue_2) (`PXOngoingActionUtils.GetOngoingActionComponentForCommunity` _community))
      (if _hasongoingaction_2
        (set `local.OA Data` _returnvalue_2)
        (goto _label))
      (elif _isvalid_2
        (set `local.OA Data` _ongoingaction)
        (goto _label)))))

(fn `GetGameplayFactorValues`
  (params (factorValues :type "Array of PXGameplayFactorValues Structure (by ref)") (context :type "PXGameContext Structure (by ref)"))
  ;[1 1 1] Empty on purpose
  (return))