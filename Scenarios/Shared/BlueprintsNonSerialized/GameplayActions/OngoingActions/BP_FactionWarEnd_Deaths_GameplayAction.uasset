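; Gameplay action that applies faction war end casualties to the losing community, injuring and killing its people.
; A MainCommunityKills flag decides whether the context's main or additional community is the killer, with the other as victim.
; Casualty counts come from the next-battle raw info for that pairing and district, with injuries randomized slightly upward.
; Both reasons name winner and district; factor values are intentionally empty.
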(fn `ExecuteAction`
  (params (context :type "PXGameContext Structure (by ref)"))
  (locals (dist :type "PXDistrictComponent Object Reference") (`community to kil` :type "PXCommunityComponent Object Reference") (`killer community` :type "PXCommunityComponent Object Reference") (deaths :type Integer))
  (bind _community (`PXGameplayContextUtils.TryGetAdditionalCommunityComponentFromGameContext` context))
  (bind _community_2 (`PXGameplayContextUtils.TryGetCommunityComponentFromGameContext` context))
  (bind _community_to_kil (`local.community to kil`))
  (bind _main_community_kills_ (`self.Main Community Kills?`))
  (bind _result (`|FormatText` (`self.Format`) (`/Game/Scenarios/Shared/BlueprintsNonSerialized/Communities/BPFL_CommunityUtils.Get Community Name` (`local.killer community`)) (`/Game/Scenarios/Shared/BlueprintsNonSerialized/SocietyUtils/BPFL_Communication_Utils.Get District Name from Context` (`local.context`))))
  (set `local.dist` (`/Game/Scenarios/Shared/BlueprintsNonSerialized/SocietyUtils/BPFL_Communication_Utils.Get Best District from Context` context))
  (set `local.killer community` (select `bool` _main_community_kills_ :`false` _community :`true` _community_2))
  (set `local.community to kil` (select `bool` _main_community_kills_ :`false` _community_2 :`true` _community))
  (bind (_per_community_deaths1 _per_community_injuries_1) (`/Game/Scenarios/Shared/BlueprintsNonSerialized/FactionEmergence/BPFL_FactionWarUtils.Get Faction War Next Battle Raw Info` (`local.killer community`) (`local.community to kil`) (`local.dist`)))
  (bind _output_get (set `local.deaths` (`BlueprintMapLibrary.Map_Find` _per_community_deaths1 _community_to_kil)))
  (`|ExecutionSequence`
    (:`then_0`
      (bind _value (`BlueprintMapLibrary.Map_Find` _per_community_injuries_1 _community_to_kil))
      (`/Game/Scenarios/Shared/BlueprintsNonSerialized/FactionEmergence/BPFL_FactionWarUtils.Injure People In Community` (`local.community to kil`) _result _value (+ _value 25))
      (return))
    (:`then_1`
      (`/Game/Scenarios/Shared/BlueprintsNonSerialized/Communities/BPFL_CommunityUtils.Kill People in Community For Real` (`local.community to kil`) _output_get false _result)
      (return))))

(fn `GetGameplayFactorValues`
  (params (factorValues :type "Array of PXGameplayFactorValues Structure (by ref)") (context :type "PXGameContext Structure (by ref)"))
  ;[1 1 1] Empty on purpose
  (return))