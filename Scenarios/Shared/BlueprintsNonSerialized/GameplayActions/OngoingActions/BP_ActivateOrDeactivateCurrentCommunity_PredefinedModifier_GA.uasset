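; Ongoing gameplay action that switches a predefined modifier on or off for the current community, based on its Active flag.
; On execution it takes the nation from the game context and, if valid, sets the modifier's manual-target state on the community's owner.
; A helper picks the context's best community or, with UseAdditionalCommunity, the additional one.
; It also reports the modifier's gameplay factor values using that community as context.
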(fn `ExecuteAction`
  (params (context :type "PXGameContext Structure (by ref)"))
  (bind (_nation _isvalid) (`PXGameplayContextUtils.TryGetNationFromGameContext` context))
  (if _isvalid
    (`PXPredefinedModifierUtils.SetPredefinedModifierActiveManualTarget` _nation (`self.Predefined Modifier`) (`ActorComponent.GetOwner` (`self.Get Community` context)) (`self.Active`))
    (return)))

(fn `Get Community`
  (params (InputPin :type "PXGameContext Structure (by ref)"))
  (returns (ReturnValue :type "PXCommunityComponent Object Reference"))
  (return (select `bool` (`self.Use Additional Community?`) :`false` (`/Game/Scenarios/Shared/BlueprintsNonSerialized/SocietyUtils/BPFL_Communication_Utils.Get Best Community from Context` InputPin) :`true` (`PXGameplayContextUtils.TryGetAdditionalCommunityComponentFromGameContext` InputPin))))

(fn `GetGameplayFactorValues`
  (params (factorValues :type "Array of PXGameplayFactorValues Structure (by ref)") (context :type "PXGameContext Structure (by ref)"))
  (`PXGameplayActionUtils.AddPredefinedModifierToGameplayFactorValues` factorValues (`self.Predefined Modifier`) (`PXGameplayContextUtils.MakePXGameContext` (`self.Get Community` context)))
  (return))