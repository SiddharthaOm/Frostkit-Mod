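; BP_RazeDistrict_GameplayAction is an ongoing gameplay action that marks a district as razed by faction-war fighting.
; It takes the best district from the action context and activates the destroyed-district and razed-tag modifiers on its owner for the player's nation.
; It then shows a central notification, broadcasts a severe "Razed" absence event and adds a Razed history record.
; A tutorial highlight for razed districts is left disconnected.
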(fn `ExecuteAction`
  (params (context :type "PXGameContext Structure (by ref)"))
  (bind _district (`/Game/Scenarios/Shared/BlueprintsNonSerialized/SocietyUtils/BPFL_Communication_Utils.Get Best District from Context` context))
  (bind _returnvalue (`ActorComponent.GetOwner` _district))
  (`/Engine/EditorBlueprintResources/StandardMacros.IsValid` _district
    (:`Is Valid`
      (`PXPredefinedModifierUtils.SetPredefinedModifierActiveManualTarget` (`PXNationUtils.GetPlayerNation`) "/Game/Scenarios/Shared/Configs/PredefinedModifiers/FactionWar/DA_FactionWar_DestroyedDistrict_Modifier.DA_FactionWar_DestroyedDistrict_Modifier" _returnvalue true)
      (`PXPredefinedModifierUtils.SetPredefinedModifierActiveManualTarget` (`PXNationUtils.GetPlayerNation`) "/Game/Scenarios/Shared/Configs/PredefinedModifiers/FactionWar/DA_FactionWar_RazedTag_Modifier.DA_FactionWar_RazedTag_Modifier" _returnvalue true)
      (`PXCentralNotificationUtils.ShowCustomCentralNotificationSmall` (`|FormatText` "{DISTRICT} Destroyed in Fighting" (`/Game/Scenarios/Shared/BlueprintsNonSerialized/Cities/BPFL_CityUtils.GetDistrictFluffName` _district)) (`|FormatText` "Fighting moves elsewhere; district in need of major repairs.") "" "/Game/UI/Assets/Textures/SpecialTextures/Illustrations/CentralNotifications/UIT_CentralNotification_GeneratorDanger_Sprite.UIT_CentralNotification_GeneratorDanger_Sprite")
      (`PXUICustomEventsUtils.BroadcastDistrictAbsenceChangedEvent` _district "Dead" 0 "/Game/UI/Assets/Textures/AtlasedTextures/Icons/Frames/UIT_Fire_Icon.UIT_Fire_Icon" 0 null 3 (`|FormatText` "Razed"))
      (`PXHistoryRecordUtils.AddActorHistoryRecord` _returnvalue "/Game/Scenarios/Shared/Configs/HistoryRecords/Types/DA_HistoryRecord_Razed.DA_HistoryRecord_Razed" 1)
      (return))))