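; Ongoing gameplay action that marks an outpost territory for exploration and tells the player which resource it holds.
; It picks the first Revealed territory with a site whose outpost has a valid main resource.
; It flags that territory as an objective in the context nation's exploration data and activates the player nation's InstantExplore modifier on it.
; A notification credits the context community's seers, naming the territory and resource.
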(fn `ExecuteAction`
  (params (context :type "PXGameContext Structure (by ref)"))
  (locals (`Territory to Mark` :type "PXTerritoryComponent Object Reference") (`instant explore` :type "PXPredefinedModifier Object Reference" :default "/Script/Frostpunk2.PXPredefinedModifier'/Game/Scenarios/Main/Configs/PredefinedModifiers/DA_InstantExploreTerritory_PilgrimsSeers_Modifier.DA_InstantExploreTerritory_PilgrimsSeers_Modifier'") (resource :type "PXResource Object Reference"))
  (bind (_resource _territory) (`self.Get Territory to Mark`))
  (`/Engine/EditorBlueprintResources/StandardMacros.IsValid` _territory
    (:`Is Valid`
      (set `local.Territory to Mark` _territory)
      (set `local.resource` _resource)
      (`PXTerritoryUtils.SetTerritoryObjectiveMarkStatus` (`PXTerritoryComponent.GetExplorationComponent` (`local.Territory to Mark`) (`PXGameplayContextUtils.TryGetNationFromGameContext` (`local.context`))) true null)
      (`PXPredefinedModifierUtils.SetPredefinedModifierActiveManualTarget` (`PXNationUtils.GetPlayerNation`) (`local.instant explore`) (`ActorComponent.GetOwner` (`local.Territory to Mark`)) true)
      (`PXCommunicationChannelsUtils.AddNotification` (make `PXNotificationData` "Normal" (`|FormatText` "{FACTION}' seers have revealed much about a '{TERRITORY}' territory, a source of {RESOURCE}" (`/Game/Scenarios/Shared/BlueprintsNonSerialized/Communities/BPFL_CommunityUtils.Get Community Name` (`/Game/Scenarios/Shared/BlueprintsNonSerialized/SocietyUtils/BPFL_Communication_Utils.Get Best Community from Context` (`local.context`))) (`PXTerritoryComponent.UnexploredName` (`local.Territory to Mark`)) (`PXResource.IngameName` (`local.resource`)))))
      (return))))

(fn `Get Territory to Mark`
  (returns (Resource :type "PXResource Object Reference") (Territory :type "PXTerritoryComponent Object Reference") (site :type "PXSiteComponent Object Reference"))
  (for _array_element (`PXTerritoryUtils.GetTerritoriesByState` "Revealed")
    (for _array_element_2 (`PXTerritoryComponent.GetSites` _array_element)
      (bind _returnvalue (`PXSiteUtils.TryGetOutpostFromSite` _array_element_2))
      (`/Engine/EditorBlueprintResources/StandardMacros.IsValid` _returnvalue
        (:`Is Valid`
          (bind _returnvalue_2 (`PXOutpostUtils.GetOutpostMainResource` _returnvalue))
          (`/Engine/EditorBlueprintResources/StandardMacros.IsValid` _returnvalue_2
            (:`Is Valid`
              (return _returnvalue_2 (`PXOutpostUtils.GetOutpostTerritory` _returnvalue) _array_element_2))))))))

(fn `GetGameplayFactorValues`
  (params (factorValues :type "Array of PXGameplayFactorValues Structure (by ref)") (context :type "PXGameContext Structure (by ref)"))
  (locals (`instant explore_0` :type "PXPredefinedModifier Object Reference" :default "/Script/Frostpunk2.PXPredefinedModifier'/Game/Scenarios/Main/Configs/PredefinedModifiers/DA_InstantExploreTerritory_PilgrimsSeers_Modifier.DA_InstantExploreTerritory_PilgrimsSeers_Modifier'"))
  (return))