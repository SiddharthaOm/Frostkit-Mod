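; A gameplay action that removes a configured imprint from communities.
; With AllCommunities set, it removes the imprint from every community present in the main city.
; Otherwise it takes the community from the game context, and logs a message when that community is invalid.
; It deliberately supplies no gameplay factor values.
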(fn `ExecuteAction`
  (params (context :type "PXGameContext Structure (by ref)"))
  (bind (_community _isvalid) (`PXGameplayContextUtils.TryGetCommunityComponentFromGameContext` context))
  (if (`self.All Communities?`)
    (for _array_element (`/Game/Scenarios/Shared/BlueprintsNonSerialized/Communities/BPFL_CommunityUtils.Get All Communities Present In Main City`)
      (`PXCommunityUtils.RemoveImprint` _array_element (`self.Imprint`)))
    (else
      (`/Engine/EditorBlueprintResources/StandardMacros.IsValid` _community
        (:`Is Valid`
          (if _isvalid
            (`PXCommunityUtils.RemoveImprint` _community (`self.Imprint`))))
        (:`Is Not Valid`
          (`KismetSystemLibrary.LogString` "Tried to remove imprint from invalid community"))))))

(fn `GetGameplayFactorValues`
  (params (factorValues :type "Array of PXGameplayFactorValues Structure (by ref)") (context :type "PXGameContext Structure (by ref)"))
  ;[1 1 1] Empty on purpose
  (return))