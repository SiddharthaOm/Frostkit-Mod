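; Gameplay action effect that kills a set number of people in a community, passing along a reason and a silent-notification flag.
; An optional community type override selects the target through the stored City variable.
; Otherwise it resolves the city and takes the context's best community, or the additional one if flagged and valid.
; The kill goes through a safeguarded helper, and gameplay factor reporting is intentionally empty.
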(fn `Action Function`
  (params (context :type "PXGameContext Structure (by ref)"))
  (locals (city :type "PXCityComponent Object Reference") (`community to kill` :type "PXCommunityComponent Object Reference") (NewLocalVar :type Integer :default 0))
  (bind (_community _isvalid) (`PXGameplayContextUtils.TryGetAdditionalCommunityComponentFromGameContext` (`local.context`)))
  (`/Engine/EditorBlueprintResources/StandardMacros.IsValid` (`self.Community Type to Kill Override`)
    (:`Is Valid`
      (bind _output_get (set `local.community to kill` (`.ReturnValue` (`PXCommunityUtils.GetCommunityOfCommunityType` (`self.Community Type to Kill Override`) (`local.city`)))))
      (`/Engine/EditorBlueprintResources/StandardMacros.IsValid` _output_get
        (:`Is Valid`
          _)))
    (:`Is Not Valid`
      (set `local.city` (`/Game/Scenarios/Shared/BlueprintsNonSerialized/SocietyUtils/BPFL_Communication_Utils.Return Valid City or Choose Best` (`PXGameplayContextUtils.TryGetCityFromGameContext` context)))
      (bind _output_get_2 (set `local.community to kill` (select `bool` (and _isvalid (`self.Use Additional Community insted of Main?`)) :`false` (`/Game/Scenarios/Shared/BlueprintsNonSerialized/SocietyUtils/BPFL_Communication_Utils.Get Best Community from Context` (`local.context`)) :`true` _community)))
      (`/Engine/EditorBlueprintResources/StandardMacros.IsValid` _output_get_2
        (:`Is Valid`
          _))))
  (`/Game/Scenarios/Shared/BlueprintsNonSerialized/Communities/BPFL_CommunityUtils.Kill People in Community With Safeguard` (`local.community to kill`) (`self.Number To Kill`) (`self.Silent Notification`) (`self.Reason`)))

(fn `ExecuteAction`
  (params (context :type "PXGameContext Structure (by ref)"))
  (`self.Action Function` context))

(fn `GetGameplayFactorValues`
  (params (factorValues :type "Array of PXGameplayFactorValues Structure (by ref)") (context :type "PXGameContext Structure (by ref)"))
  ;[1 1 1] Empty on purpose
  (return))