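; Gameplay action effect that kills a percentage of a city's population for a given death reason, with optional notification and trust penalty.
; The target city comes from the context's city, community or district, falling back to the player's main city.
; The percentage is capped by an optional maximum unit count before the kill.
; A helper reports units to kill, population number and affected community types, while gameplay factor values stay empty.
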(fn `Action Function`
  (params (context :type "PXGameContext Structure (by ref)"))
  (locals (city :type "PXCityComponent Object Reference") (`community to kill` :type "PXCommunityComponent Object Reference"))
  (bind (_community _isvalid) (`PXGameplayContextUtils.TryGetCommunityComponentFromGameContext` context))
  (bind (_district _isvalid_2) (`PXGameplayContextUtils.TryGetDistrictFromGameContext` context))
  (bind (_city _isvalid_3) (`PXGameplayContextUtils.TryGetCityFromGameContext` context))
  (bind _city_2 (`local.city`))
  (if _isvalid_3
    (set `local.city` _city)
    (elif _isvalid
      (set `local.city` (`PXCommunityComponent.ParentCity` _community))
      (elif _isvalid_2
        (set `local.city` (`PXDistrictComponent.GetCity` _district))
        (else
          (set `local.city` (`PXNationUtils.GetPlayerMainCity`))))))
  (`/Game/Scenarios/Shared/BlueprintsNonSerialized/GameplayActions/BPFL_GameplayAction_Utils.Kill Percent Of City` (`self.DeathReason`) _city_2 (`/Game/Scenarios/Shared/BlueprintsNonSerialized/GameplayActions/BPFL_GameplayAction_Utils.Cap Percent of City Population at Value` _city_2 (`self.PercentChange`) (`self.(Optional) Max Raw Units To Cap At`) true) (`self.Should Send Notification`) (`self.ShouldApplyTrustPenalty`) (`self.Use Custom Notification Template`)))

(fn `ExecuteAction`
  (params (context :type "PXGameContext Structure (by ref)"))
  (`self.Action Function` context))

(fn `GetGameplayFactorValues`
  (params (factorValues :type "Array of PXGameplayFactorValues Structure (by ref)") (context :type "PXGameContext Structure (by ref)"))
  ;[1 1 1] Empty on purpose
  (return))

(fn `GetPeopleToKill`
  (params (City :type "PXCityComponent Object Reference") (Percent :type "Float (double-precision)"))
  (returns (Count :type Integer) (FluffNumber :type Integer) (`Communities to die` :type "Array of PXCommunityType Object Reference"))
  (bind _returnvalue (`/Game/Scenarios/Shared/BlueprintsNonSerialized/GameplayActions/BPFL_GameplayAction_Utils.Get Population Size Units to Kill from City` Percent City))
  (return _returnvalue (`/Game/UI/Utilities/BPFL_UI.Get Population From Size Points` _returnvalue) (`PXCommunityUtils.GetCommunityTypesFromCity` City)))