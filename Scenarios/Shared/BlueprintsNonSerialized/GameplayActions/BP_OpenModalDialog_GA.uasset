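; Gameplay action that opens a modal dialog by constructing and starting a parameterized BP_Modal_StoryArc with a hash and predefined dialog.
; As a marked hack, a context lacking a valid community is replaced by one built from the primary and secondary communities of its best district's ongoing action.
; Otherwise the context passes through unchanged.
; It intentionally reports no gameplay factor values.
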(fn `ExecuteAction`
  (params (context :type "PXGameContext Structure (by ref)"))
  (bind _returnvalue (`|GenericCreateObject` :`self` (subsystem `PXStoryArcSubsystem`) :`Class` "/Game/Scenarios/Shared/BlueprintsSerialized/StoryArcs/CommunityActions/BP_Modal_StoryArc.BP_Modal_StoryArc_C" :`Hash` (`self.Hash`) :`Predefined Dialog` (`self.Predefined Dialog`) :`Game Context` (`self.Fill In Context With OA Info` context)))
  (`PXStoryUtils.StartParameterizedStoryArc` _returnvalue)
  (return))

(fn `Fill In Context With OA Info`
  (params (context :type "PXGameContext Structure (by ref)"))
  (returns (ReturnValue :type "PXGameContext Structure"))
  (locals (community :type "PXCommunityComponent Object Reference") (district :type "PXDistrictComponent Object Reference"))
  (bind (_community _isvalid) (`PXGameplayContextUtils.TryGetCommunityComponentFromGameContext` context))
  ;[1 1 1] HACK
  (if _isvalid
    (set `local.community` _community)
    (elif true
      (bind _output_get (set `local.district` (`/Game/Scenarios/Shared/BlueprintsNonSerialized/SocietyUtils/BPFL_Communication_Utils.Get Best District from Context` context)))
      (bind (_hasongoingaction _returnvalue) (`PXOngoingActionUtils.GetOngoingActionComponentForDistrict` _output_get))
      (if _hasongoingaction
        (bind (_primary_community _secondary_community) (`/Game/Scenarios/Shared/BlueprintsNonSerialized/OngoingEvents/BPFL_OngoingAction_Utils.Get Primary and Secondary Community from OA Component` _returnvalue))
        (return (`PXGameplayContextUtils.MakePXGameContext` _primary_community _secondary_community))
        (else
          _))
      (else
        (return context))))
  (return context))

(fn `GetGameplayFactorValues`
  (params (factorValues :type "Array of PXGameplayFactorValues Structure (by ref)") (context :type "PXGameContext Structure (by ref)"))
  ;[1 1 1] Empty on purpose
  (return))