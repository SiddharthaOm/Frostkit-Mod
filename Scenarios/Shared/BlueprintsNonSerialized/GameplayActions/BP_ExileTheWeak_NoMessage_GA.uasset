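; Gameplay action that exiles the weak, removing the population absent through sickliness from the player's main city.
; ExecuteAction negates that absence count and passes it to ExileTheWeakAndNotifiy with the city's community types and a formatted population text.
; GetGameplayFactorValues adds no factors, as its Sickliness flat-change logic is left disconnected.
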(fn `ExecuteAction`
  (params (context :type "PXGameContext Structure (by ref)"))
  (locals (`units to exile` :type Integer :default 0) (fluff :type Text))
  (bind _returnvalue (`PXNationUtils.GetPlayerMainCity`))
  (bind _returnvalue_2 (`PXAbsenceUtils.GetCurrentPopulationAbsenceInCity` (`PXNationUtils.GetPlayerMainCity`) "/Game/Scenarios/Shared/Configs/Absences/AbsenceTypes/DA_Sickliness_Absence.DA_Sickliness_Absence"))
  (set `local.units to exile` (* _returnvalue_2 -1))
  (set `local.fluff` (`/Game/UI/Utilities/BPFL_UI.Get Population Size Points Display Text` _returnvalue_2))
  (`/Game/Scenarios/Shared/BlueprintsNonSerialized/GameplayActions/BPFL_GameplayAction_Utils.Exile the Weak and Notifiy` (`local.units to exile`) _returnvalue (`PXCommunityUtils.GetCommunityTypesFromCity` _returnvalue) (`local.fluff`))
  (return))

(fn `GetGameplayFactorValues`
  (params (factorValues :type "Array of PXGameplayFactorValues Structure (by ref)") (context :type "PXGameContext Structure (by ref)"))
  (locals (Sickliness :type "PXStatistic Object Reference" :default "/Script/Frostpunk2.PXStatistic'/Game/Scenarios/Shared/Configs/Statistics/Entries/DA_Sickliness.DA_Sickliness'"))
  (return))