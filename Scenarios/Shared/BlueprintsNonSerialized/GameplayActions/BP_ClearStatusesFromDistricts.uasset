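; Gameplay action that clears a configured status type from a city's districts.
; On execute, it takes the districts of the best city resolved from the context and filters them by the DistrictsToFilter tag.
; It then loops over the filtered districts and removes the status from each owning actor where that status is active.
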(fn `ExecuteAction`
  (params (context :type "PXGameContext Structure (by ref)"))
  (locals (NumberOfDistrictsToBeAffected :type Integer) (AllDistricts :type "Array of PXDistrictComponent Object Reference"))
  (bind _status (`self.Status`))
  (bind _districts (`/Game/Scenarios/Shared/BlueprintsNonSerialized/GameplayUtils/BPFL_LocalPopulation_FunctionLibrary.Filter Districts with Tag` (`self.DistrictsToFilter`) (`PXCityComponent.GetDistricts` (`/Game/Scenarios/Shared/BlueprintsNonSerialized/SocietyUtils/BPFL_Communication_Utils.Get Best City from Context` context))))
  (bind _output_get (set `local.AllDistricts` _districts))
  ;[1 1 1] Remove all active statuses
  (for _array_element _output_get
    (bind _returnvalue (`ActorComponent.GetOwner` _array_element))
    (if (`PXStatusUtils.HasActiveStatus` _returnvalue _status)
      (`PXStatusUtils.RemoveStatus` _returnvalue _status))))