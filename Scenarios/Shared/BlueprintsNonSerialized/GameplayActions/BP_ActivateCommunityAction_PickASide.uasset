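; Gameplay action that makes one side of a faction war, chosen by the UseDefender flag, perform a configured community action.
; GetCommunity picks the war's initial defender or aggressor, and ExecuteAction runs the action as that community with a leader action origin.
; Gameplay factor values are gathered from the wrapped action using that same community as context.
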(fn `Execute Action 2`
  (params (context :type "PXGameContext Structure (by ref)"))
  (locals (`Community to use` :type "PXCommunityComponent Object Reference"))
  (set `local.Community to use` (`self.Get Community`))
  (`PXCommunityActionUtils.ExecuteCommunityAction` (`self.Action`) "/Game/Scenarios/Shared/Configs/ActionOrigin/DA_LeaderActionOrigin.DA_LeaderActionOrigin" (`local.Community to use`)))

(fn `ExecuteAction`
  (params (context :type "PXGameContext Structure (by ref)"))
  (`self.Execute Action 2` context))

(fn `Get Community`
  (returns (ReturnValue :type "PXCommunityComponent Object Reference"))
  (return (select `bool` (`self.Use Defender?`) :`false` (`/Game/Scenarios/Shared/BlueprintsNonSerialized/SocietyUtils/BPFL_SharedScenariosStorage.Get Faction War Initial Aggressor`) :`true` (`/Game/Scenarios/Shared/BlueprintsNonSerialized/SocietyUtils/BPFL_SharedScenariosStorage.Get Faction War Initial Defender`))))

(fn `GetGameplayFactorValues`
  (params (factorValues :type "Array of PXGameplayFactorValues Structure (by ref)") (context :type "PXGameContext Structure (by ref)"))
  (`PXGameplayActionUtils.AddGameplayActionToGameplayFactorValues` factorValues (`PXCommunityAction.GameplayAction` (`self.Action`)) (`PXGameplayContextUtils.MakePXGameContext` (`self.Get Community`)))
  (return))