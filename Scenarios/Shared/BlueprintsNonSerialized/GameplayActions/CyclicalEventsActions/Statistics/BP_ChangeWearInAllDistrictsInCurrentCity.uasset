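; Gameplay action for cyclical events that increases wear on districts in the city taken from the game context.
; On execution it finds that city's districts matching a tag query, inactive ones included, and adds a configurable wear amount to each owning actor.
; It can then post a notification naming the city, and deliberately reports no gameplay factor values.
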(fn `BreakDistrictWithoutOngoingAction`
  (params (City :type "PXCityComponent Object Reference"))
  (locals (DistrictsWithTag :type "Array of PXDistrictComponent Object Reference"))
  ;[1 1 1] Get all eligible districs
  (bind _output_get (set `local.DistrictsWithTag` (`PXDistrictUtils.GetDistrictWithTagFromCity` City (`self.TagOfDistrictsToBreak`))))
  (for _array_element _output_get
    (`PXWearUtils.IncreaseWear` (`ActorComponent.GetOwner` _array_element) (`self.Amount`))))

(fn `ExecuteAction`
  (params (context :type "PXGameContext Structure (by ref)"))
  (bind (_city _isvalid) (`PXGameplayContextUtils.TryGetCityFromGameContext` context))
  (if _isvalid
    (`self.BreakDistrictWithoutOngoingAction` _city)
    (if (`self.Notify`)
      (`PXCommunicationChannelsUtils.AddNotification` (make `PXNotificationData` "Normal" (`|FormatText` (`self.Notification Text`) (`PXGameplayElementUtils.GetActorIngameName` (`ActorComponent.GetOwner` _city)))))
      (return))))

(fn `GetGameplayFactorValues`
  (params (factorValues :type "Array of PXGameplayFactorValues Structure (by ref)") (context :type "PXGameContext Structure (by ref)"))
  ;[1 1 1] Empty on purpose
  (return))