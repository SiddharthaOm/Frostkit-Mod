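; Cyclical-event action effect that injures people in a nation's cold districts, with chances tuned per week.
; It requires a valid nation and city in the game context, then queries active districts tagged Freezing, Very Cold, Cold and Chilly in turn.
; Each district rolls against its tier's chance; a hit injures a shared percentage of its workforce with an injured-from-cold icon.
; The GetNotificationLevel function is an empty stub.
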(fn `ExecuteAction`
  (params (context :type "PXGameContext Structure (by ref)"))
  (locals (`Freezing Tag` :type "GameplayTagQuery Structure" :default (struct :`TagDictionary` (struct :`(TagName` "HeatLevel.Freezing") :`(TagName` "District.Production") :`(TagName` "District.Extraction")) :`QueryTokenStream` "(0,1,5,2,1,1,0,1,2,1,2)" :`AutoDescription` " ALL(  ANY( HeatLevel.Freezing ),  ANY( District.Production, District.Extraction ) )")) (`Very Cold Tag` :type "GameplayTagQuery Structure" :default (struct :`TagDictionary` (struct :`(TagName` "HeatLevel.VeryCold") :`(TagName` "District.Production") :`(TagName` "District.Extraction")) :`QueryTokenStream` "(0,1,5,2,1,1,0,1,2,1,2)" :`AutoDescription` " ALL(  ANY( HeatLevel.VeryCold ),  ANY( District.Production, District.Extraction ) )")) (`Cold Tag` :type "GameplayTagQuery Structure" :default (struct :`TagDictionary` (struct :`(TagName` "HeatLevel.Cold") :`(TagName` "District.Production") :`(TagName` "District.Extraction")) :`QueryTokenStream` "(0,1,5,2,1,1,0,1,2,1,2)" :`AutoDescription` " ALL(  ANY( HeatLevel.Cold ),  ANY( District.Production, District.Extraction ) )")) (`Chilly Tag` :type "GameplayTagQuery Structure" :default (struct :`TagDictionary` (struct :`(TagName` "HeatLevel.Chilly") :`(TagName` "District.Production") :`(TagName` "District.Extraction")) :`QueryTokenStream` "(0,1,5,2,1,1,0,1,2,1,2)" :`AutoDescription` " ALL(  ANY( HeatLevel.Chilly ),  ANY( District.Production, District.Extraction ) )")) (Nation :type "PXNationComponent Object Reference") (City :type "PXCityComponent Object Reference"))
  (bind (_nation _isvalid) (`PXGameplayContextUtils.TryGetNationFromGameContext` context))
  (bind (_city _isvalid_2) (`PXGameplayContextUtils.TryGetCityFromGameContext` context))
  (if _isvalid
    (set `local.Nation` _nation)
    (if _isvalid_2
      (set `local.City` _city)
      (`|ExecutionSequence`
        (:`then_0`
          (bind _returnvalue (`PXDistrictUtils.GetDistrictWithTagFromNation` (`local.Nation`) (`local.Freezing Tag`) true null))
          (for _array_element _returnvalue
            (if (<= (`PXRandomLibrary.PXRandomFloatInRange` 0.0 1.0) (`self.Chance to Affect Freezing per Week`))
              (`/Game/Scenarios/Shared/BlueprintsNonSerialized/GameplayUtils/BPFL_LocalPopulation_FunctionLibrary.InjurePeopleInDistrictByPercentofWorkforce` _array_element (`self.Percent in district to Injure`) "/Game/UI/Assets/Textures/AtlasedTextures/Icons/Frames/UIT_InjuredFromColdIcon.UIT_InjuredFromColdIcon"))))
        (:`then_1`
          (bind _returnvalue_2 (`PXDistrictUtils.GetDistrictWithTagFromNation` (`local.Nation`) (`local.Very Cold Tag`) true null))
          (for _array_element_2 _returnvalue_2
            (if (<= (`PXRandomLibrary.PXRandomFloatInRange` 0.0 1.0) (`self.Chance to Affect Very Cold per Week`))
              (`/Game/Scenarios/Shared/BlueprintsNonSerialized/GameplayUtils/BPFL_LocalPopulation_FunctionLibrary.InjurePeopleInDistrictByPercentofWorkforce` _array_element_2 (`self.Percent in district to Injure`) "/Game/UI/Assets/Textures/AtlasedTextures/Icons/Frames/UIT_InjuredFromColdIcon.UIT_InjuredFromColdIcon"))))
        (:`then_2`
          (bind _returnvalue_3 (`PXDistrictUtils.GetDistrictWithTagFromNation` (`local.Nation`) (`local.Cold Tag`) true null))
          (for _array_element_3 _returnvalue_3
            (if (<= (`PXRandomLibrary.PXRandomFloatInRange` 0.0 1.0) (`self.Chance to Affect Cold per Week`))
              (`/Game/Scenarios/Shared/BlueprintsNonSerialized/GameplayUtils/BPFL_LocalPopulation_FunctionLibrary.InjurePeopleInDistrictByPercentofWorkforce` _array_element_3 (`self.Percent in district to Injure`) "/Game/UI/Assets/Textures/AtlasedTextures/Icons/Frames/UIT_InjuredFromColdIcon.UIT_InjuredFromColdIcon"))))
        (:`then_3`
          (bind _returnvalue_4 (`PXDistrictUtils.GetDistrictWithTagFromNation` (`local.Nation`) (`local.Chilly Tag`) true null))
          (for _array_element_4 _returnvalue_4
            (if (<= (`PXRandomLibrary.PXRandomFloatInRange` 0.0 1.0) (`self.Chance to Affect Chilly per Week`))
              (`/Game/Scenarios/Shared/BlueprintsNonSerialized/GameplayUtils/BPFL_LocalPopulation_FunctionLibrary.InjurePeopleInDistrictByPercentofWorkforce` _array_element_4 (`self.Percent in district to Injure`) "/Game/UI/Assets/Textures/AtlasedTextures/Icons/Frames/UIT_InjuredFromColdIcon.UIT_InjuredFromColdIcon"))))
        (:`then_4`
          (return))))))

(fn `Get Notification Level`
  (params (`People to Injure` :type Boolean)))