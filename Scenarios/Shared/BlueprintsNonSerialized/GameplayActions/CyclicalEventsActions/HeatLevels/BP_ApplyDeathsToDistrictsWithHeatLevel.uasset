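; Heat-level gameplay action that kills inhabitants from cold in a city's districts carrying both the DistrictToAffect and HeatLevel tags.
; Each district rolls against an occurrence chance, then loses a randomized percentage of occupants scaled by a shared cold-death multiplier.
; The current city applies deaths per district with an icon notification.
; Other cities accumulate one total, killed city-wide in districts only if the final loop index is non-zero.
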(fn `ExecuteAction`
  (params (context :type "PXGameContext Structure (by ref)"))
  (locals (City :type "PXCityComponent Object Reference") (`Total Number To Kill` :type Integer :default 0))
  (bind _city (`/Game/Scenarios/Shared/BlueprintsNonSerialized/SocietyUtils/BPFL_Communication_Utils.Get Best City from Context` context))
  (bind _city_2 (`local.City`))
  (bind _output_get (set `local.City` _city))
  (`/Engine/EditorBlueprintResources/StandardMacros.IsValid` _output_get
    (:`Is Valid`
      (bind _districts (`/Game/Scenarios/Shared/BlueprintsNonSerialized/GameplayUtils/BPFL_LocalPopulation_FunctionLibrary.Filter Districts with Tag` (`self.District to Affect`) (`PXCityComponent.GetDistricts` _city)))
      (bind _districts_2 (`/Game/Scenarios/Shared/BlueprintsNonSerialized/GameplayUtils/BPFL_LocalPopulation_FunctionLibrary.Filter Districts with Tag` (`self.Heat Level`) _districts))
      (for (_array_element _array_index) _districts_2
        (if (<= (`PXRandomLibrary.PXRandomFloatInRange` 0.0 1.0) (`self.Chance of Occurence per district`))
          (bind _out_value (`/Game/Scenarios/Shared/BlueprintsNonSerialized/GameplayUtils/BPFL_LocalPopulation_FunctionLibrary.Randomize Float  By Percent` (`self.Percent of Inhabitants to Kill`) (`self.Random Factor on number of deaths`)))
          (if (== (`PXSelectionUtils.GetCurrentCity`) (`local.City`))
            (bind _returnvalue (`KismetMathLibrary.FTrunc` (* (`/Game/Scenarios/Shared/BlueprintsSerialized/VariableStorage/BP_SharedVariableStorage.CyclicalDathsFromColdinDistrictsMultiplier` (`/Game/Scenarios/Shared/BlueprintsNonSerialized/SocietyUtils/BPFL_SharedScenariosStorage.Get Shared Variable Storage`)) (* (`.ReturnValue` (`PXPeopleAllocationUtils.GetOccupantsFromDistrict` _array_element)) _out_value))))
            (`/Game/Scenarios/Shared/BlueprintsNonSerialized/GameplayUtils/BPFL_LocalPopulation_FunctionLibrary.KillInhabitantsInDistrictByNumber` _array_element _returnvalue "/Game/UI/Assets/Textures/AtlasedTextures/Icons/Frames/UIT_DeathFromColdIcon.UIT_DeathFromColdIcon" (`self.Statistic for EndLog`) null false "{NUMBER}")
            (else
              (set `local.Total Number To Kill` (+ _returnvalue (`local.Total Number To Kill`)))))))
      (if (!= _array_index 0)
        (if (== (`PXSelectionUtils.GetCurrentCity`) _city_2)
          (return)
          (else
            (`/Game/Scenarios/Shared/BlueprintsNonSerialized/GameplayUtils/BPFL_LocalPopulation_FunctionLibrary.Kill Total Population by Number` (`local.Total Number To Kill`) _city_2 "{NUMBER} People died of Cold in {CITY}" true "DistrictsOnly" (`self.Statistic for EndLog`)))))
      (set `local.Total Number To Kill` 0))))