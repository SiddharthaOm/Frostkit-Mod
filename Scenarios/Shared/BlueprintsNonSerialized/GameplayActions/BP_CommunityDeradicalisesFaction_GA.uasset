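; Gameplay action in which a community deradicalises the existing faction matching its first core affinity.
; It shrinks that faction through all communities in the city, scaling the size transfer by city population, membership multiplier and a random range.
; It applies an influence-down modifier if the faction's strength tier is at least one.
; A trust-down modifier also applies unless the player has the relations-hit-block unlock.
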(fn `ExecuteAction`
  (params (context :type "PXGameContext Structure (by ref)"))
  (locals (`Faction Local` :type "PXFactionType Object Reference") (`Community Local` :type "PXCommunityComponent Object Reference") (`influence strength down modifier` :type "PXPredefinedModifier Object Reference" :default "/Script/Frostpunk2.PXPredefinedModifier'/Game/Scenarios/Shared/BlueprintsSerialized/StoryArcs/Modifiers/Radicalisation/DA_InfluenceStrengthDecrease_PredefinedModifier.DA_InfluenceStrengthDecrease_PredefinedModifier'") (`trust down modifier` :type "PXPredefinedModifier Object Reference" :default "/Script/Frostpunk2.PXPredefinedModifier'/Game/Scenarios/Shared/Configs/PredefinedModifiers/DA_FactionCommunityDeradicalisation_Modifier.DA_FactionCommunityDeradicalisation_Modifier'"))
  (bind _community (`PXGameplayContextUtils.TryGetCommunityComponentFromGameContext` context))
  (bind (_nation _isvalid) (`PXGameplayContextUtils.TryGetNationFromGameContext` (`local.context`)))
  (bind (_outfound _returnvalue) (`PXFactionUtils.GetCommunityFromFaction` (`local.Faction Local`)))
  (bind _factioncache1 (`/Game/Scenarios/Shared/BlueprintsNonSerialized/SocietyUtils/BPFL_StoryArc_Utils.Get existing faction with affinity` (`|GetArrayItem` (`PXCommunityUtils.GetCommunityCoreAffinities` _community))))
  (bind (_outfound_2 _returnvalue_2) (`PXFactionUtils.GetCommunityFromFaction` _factioncache1))
  (set `local.Community Local` _community)
  (if _outfound_2
    (`/Engine/EditorBlueprintResources/StandardMacros.IsValid` (`PXCommunityComponent.GetFaction` _returnvalue_2)
      (:`Is Valid`
        (set `local.Faction Local` _factioncache1)
        (`/Game/Scenarios/Shared/BlueprintsNonSerialized/FactionEmergence/BPFL_FactionEmergenceUtils.Shrink Faction Using All Communities in City` _returnvalue_2 (`KismetMathLibrary.FTrunc` (* (`KismetMathLibrary.Conv_IntToDouble` (`/Game/Scenarios/Shared/BlueprintsNonSerialized/Communities/BPFL_CommunityUtils.Get Total Size Units in City` (`PXGameplayContextUtils.TryGetCityFromGameContext` context))) (* (`/Game/Scenarios/Shared/BlueprintsNonSerialized/Communities/BPFL_CommunityUtils.Get Membership Population Multiplier` _returnvalue_2 true) (`PXRandomLibrary.PXRandomFloatInRange` (`self.Multiplier Min`) (`self.Multiplier Max`))))) (`self.Population Change Notification Text`) true true (`self.Change Duration`))
        (if (>= (`.Severity Level` (`/Game/Scenarios/Shared/BlueprintsNonSerialized/OngoingEvents/BPFL_OngoingAction_Utils.Get Community Strength Tier` (`.ReturnValue` (`PXFactionUtils.GetCommunityFromFaction` (`local.Faction Local`))))) 1)
          (`PXPredefinedModifierUtils.SetPredefinedModifierActiveManualTarget` (`PXNationUtils.GetPlayerNation`) (`local.influence strength down modifier`) (`ActorComponent.GetOwner` (`.ReturnValue` (`PXFactionUtils.GetCommunityFromFaction` (`local.Faction Local`)))) true))
        (if (not (`PXUnlockUtils.IsUnlockActive` (`PXNationUtils.GetPlayerNation`) "/Game/Scenarios/Shared/Configs/Unlocks/CA/DA_CommunityDeradicalisationRelationsHitBlock_Unlock.DA_CommunityDeradicalisationRelationsHitBlock_Unlock"))
          (if (and _isvalid _outfound)
            (`PXPredefinedModifierUtils.SetPredefinedModifierActiveManualTarget` _nation (`local.trust down modifier`) (`ActorComponent.GetOwner` _returnvalue) true)
            (return)))))))

(fn `GetGameplayFactorValues`
  (params (factorValues :type "Array of PXGameplayFactorValues Structure (by ref)") (context :type "PXGameContext Structure (by ref)"))
  ;[1 1 1] Empty on purpose
  (return))