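; Gameplay action that grows or shrinks a community by a fraction of its size, scaled by recent use of the Abuse Slaves ability.
; The fraction doubles if that ability last ran within a set time window, and Death changes are negated.
; Size is read from the context city, but the change targets the player's main city.
; An optional custom notification reports the count, with alternate text for the abuse case.
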(fn `ExecuteAction`
  (params (context :type "PXGameContext Structure (by ref)"))
  (locals (Size :type Integer :default 0) (`Abuse Slaves ability` :type "PXCommunityAction Object Reference" :default "/Script/Frostpunk2.PXCommunityAction'/Game/Scenarios/Shared/Configs/Communities/CommunityActions/Special_Group/AbuseWork/Da_AbuseSlaveWork_CommunityAction.Da_AbuseSlaveWork_CommunityAction'"))
  (bind (_city _isvalid) (`PXGameplayContextUtils.TryGetCityFromGameContext` context))
  (bind _community_type (`self.Community Type`))
  (bind _returnvalue (`KismetMathLibrary.FTrunc` (* (`KismetMathLibrary.Conv_IntToDouble` (`PXCommunityUtils.GetCommunitySize` _city _community_type)) (`KismetMathLibrary.SelectFloat` (* (`KismetMathLibrary.Abs` (`self.Size Change`)) 2.0) (`KismetMathLibrary.Abs` (`self.Size Change`)) (`PXTimeUtils.LessEqual` (`PXTimeUtils.Subtract` (`PXTimeUtils.GetCurrentGameTime`) (`PXCommunityActionUtils.GetCommunityActionExecutionInfo` (`local.Abuse Slaves ability`))) (`self.Last Time community action used`))))))
  (if _isvalid
    (`/Engine/EditorBlueprintResources/StandardMacros.IsValid` (`self.Community Type`)
      (:`Is Valid`
        (bind _returnvalue_2 (`PXCommunityUtils.ChangeCommunitySizeByPercent` (`KismetMathLibrary.SelectInt` (* _returnvalue -1) _returnvalue (`|EnumEquality` (`self.Change Type`) "Death")) (make `PXCommunitySizeChangeParameters` (`self.Change Type`) (`PXNationUtils.GetPlayerMainCity`) _community_type (`self.Reason`) (`self.Custom Notification`) false)))
        (set `local.Size` (`KismetMathLibrary.Abs_Int` _returnvalue_2))
        (if (`self.Custom Notification`)
          (`PXCommunicationChannelsUtils.AddNotification` (make `PXNotificationData` "Normal" (`|FormatText` (select `bool` (`PXTimeUtils.LessEqual` (`PXTimeUtils.Subtract` (`PXTimeUtils.GetCurrentGameTime`) (`PXCommunityActionUtils.GetCommunityActionExecutionInfo` (`local.Abuse Slaves ability`))) (`self.Last Time community action used`)) :`false` (`self.Reason`) :`true` (`self.Reason with Abuse`)) (`local.Size`) (`/Game/Scenarios/Shared/BlueprintsNonSerialized/SocietyUtils/BPFL_Communication_Utils.Get City Name from Context` (`local.context`)))))
          (return))))))

(fn `GetGameplayFactorValues`
  (params (factorValues :type "Array of PXGameplayFactorValues Structure (by ref)") (context :type "PXGameContext Structure (by ref)"))
  ;[1 1 1] Empty on purpose
  (return))