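; Gameplay action effect for ongoing-action messages that force-starts a story arc; the name indicates a fallback message as the alternative.
; ExecuteAction runs the parent logic only when the ongoing action's start message is not overridden.
; ConstructArc defers to the parent, but skips arc classes already tracked when their CheckIfTrackedBeforeForcing default is set.
; StartParametrisedFunction force-starts the supplied existing arc, and gameplay factor values pass straight to the parent.
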(fn `Construct Arc`
  (params (`Game Context` :type "PXGameContext Structure") (Class :type "/Game/Scenarios/Shared/BlueprintsSerialized/StoryArcs/ParentArcs/BP_GameplayAction_StoryArc Class Reference"))
  (returns (ReturnValue :type "/Game/Scenarios/Shared/BlueprintsSerialized/StoryArcs/ParentArcs/BP_GameplayAction_StoryArc Object Reference"))
  (if (`.Check If Tracked Before Forcing` (defaults `Object` Class))
    (if (not (`PXStoryUtils.IsStoryArcOfClassTracked` Class))
      (bind _returnvalue (`parent.Construct Arc` `Game Context` Class :!label _label))
      (return _returnvalue))
    (else
      (goto _label))))

(fn `ExecuteAction`
  (params (context :type "PXGameContext Structure (by ref)"))
  (if (not (`PXOngoingActionUtils.IsOngoingActionStartMessageOverrideed` (`PXGameplayContextUtils.TryGetOngoingActionFromGameContext` context)))
    (`parent.ExecuteAction` context)
    (return)))

(fn `GetGameplayFactorValues`
  (params (factorValues :type "Array of PXGameplayFactorValues Structure (by ref)") (context :type "PXGameContext Structure (by ref)"))
  ;[1 1 1] Empty on purpose
  (`parent.GetGameplayFactorValues` factorValues context)
  (return))

(fn `Start Parametrised Function`
  (params (parametrizedStoryArc :type "PXParameterizedStoryArc Object Reference"))
  (returns (ReturnValue :type Boolean))
  (`PXStoryUtils.ForceStartExistingArc` (`local.parametrizedStoryArc`))
  (return true))