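; Consequence-message effect variant that, by its name, starts a story arc or fallback message, using the community of an Ongoing Action (OA).
; It overrides Provide Game Context, finding the ongoing action in the incoming context or, failing that, via the context's district.
; The resulting context carries that action's community and any one of its districts.
; When neither lookup finds an action, it defers to the parent implementation.
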(fn `Provide Game Context`
  (params (InputPin :type "PXGameContext Structure (by ref)"))
  (returns (OutputPin :type "PXGameContext Structure"))
  (locals (`oa component` :type "PXOngoingActionComponent Object Reference"))
  (bind (_ongoingaction _isvalid) (`PXGameplayContextUtils.TryGetOngoingActionFromGameContext` InputPin))
  (bind (_district _isvalid_2) (`PXGameplayContextUtils.TryGetDistrictFromGameContext` InputPin))
  (bind _outputpin (`parent.Provide Game Context` InputPin))
  (bind _oa_component (`local.oa component`))
  (if _isvalid
    (set `local.oa component` _ongoingaction)
    (elif _isvalid_2
      (bind (_hasongoingaction _returnvalue) (`PXOngoingActionUtils.GetOngoingActionComponentForDistrict` _district))
      (if _hasongoingaction
        (set `local.oa component` _returnvalue)
        (else
          (return _outputpin)))
      (else
        (return _outputpin))))
  (return (`PXGameplayContextUtils.MakePXGameContext` (`PXOngoingActionComponent.GetCommunity` _oa_component) null null null (`PXOngoingActionComponent.GetAnyDistict` _oa_component))))