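; Roundup scenario gameplay action that marks either the faction war's initial aggressor or defender community as a roundup target.
; A TargetAggressor flag selects the community, which is added to the shared RoundupTargetCommunities list.
; It then force-executes the Roundup community action as that community with a leader origin, using the best district from context.
; Factor values come from the Roundup gameplay action evaluated for the same community and district.
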(fn `ExecuteAction`
  (params (context :type "PXGameContext Structure (by ref)"))
  (locals (`roundup target imprint` :type "PXImprint Object Reference" :default "/Script/Frostpunk2.PXImprint'/Game/Scenarios/Shared/Configs/Communities/Imprints/Other/DA_FactionWar_RoundUpFaction_Imprint.DA_FactionWar_RoundUpFaction_Imprint'") (`roundup ca` :type "PXCommunityAction Object Reference" :default "/Script/Frostpunk2.PXCommunityAction'/Game/Scenarios/Shared/Configs/Communities/CommunityActions/Fervour_Group/InterveneFactionWar/DA_RoundUp_CA.DA_RoundUp_CA'"))
  (`KismetArrayLibrary.Array_Add` (`/Game/Scenarios/Shared/BlueprintsSerialized/VariableStorage/BP_SharedVariableStorage.Roundup Target Communities` (`/Game/Scenarios/Shared/BlueprintsNonSerialized/SocietyUtils/BPFL_SharedScenariosStorage.Get Shared Variable Storage`)) (`self.Get Community to Use`))
  (`PXCommunityActionUtils.ExecuteCommunityAction` (`local.roundup ca`) "/Game/Scenarios/Shared/Configs/ActionOrigin/DA_LeaderActionOrigin.DA_LeaderActionOrigin" (`self.Get Community to Use`) true (`/Game/Scenarios/Shared/BlueprintsNonSerialized/SocietyUtils/BPFL_Communication_Utils.Get Best District from Context` context)))

(fn `Get Community to Use`
  (returns (ReturnValue :type "PXCommunityComponent Object Reference"))
  (return (select `bool` (`self.Target Aggressor?`) :`false` (`/Game/Scenarios/Shared/BlueprintsNonSerialized/SocietyUtils/BPFL_SharedScenariosStorage.Get Faction War Initial Defender`) :`true` (`/Game/Scenarios/Shared/BlueprintsNonSerialized/SocietyUtils/BPFL_SharedScenariosStorage.Get Faction War Initial Aggressor`))))

(fn `GetGameplayFactorValues`
  (params (factorValues :type "Array of PXGameplayFactorValues Structure (by ref)") (context :type "PXGameContext Structure (by ref)"))
  (locals (`roundup ga` :type "PXGameplayAction Object Reference" :default "/Script/Frostpunk2.PXGameplayAction'/Game/Scenarios/Shared/Configs/Communities/CommunityActions/Fervour_Group/InterveneFactionWar/DA_RoundUp_GA.DA_RoundUp_GA'"))
  (`PXGameplayActionUtils.AddGameplayActionToGameplayFactorValues` factorValues (`local.roundup ga`) (`PXGameplayContextUtils.MakePXGameContext` (`self.Get Community to Use`) null null null (`/Game/Scenarios/Shared/BlueprintsNonSerialized/SocietyUtils/BPFL_Communication_Utils.Get Best District from Context` context))))