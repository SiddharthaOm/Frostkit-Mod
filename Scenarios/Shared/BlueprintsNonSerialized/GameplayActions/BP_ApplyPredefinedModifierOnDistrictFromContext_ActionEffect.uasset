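; Gameplay action effect that activates or deactivates a predefined modifier on the district resolved from the game context.
; On execution it requires a valid nation and district, then sets the modifier's state for that nation with the district's owner as manual target.
; An optional flag applies the same state to each of the district's buildings.
; It also adds the modifier to the action's gameplay factor values, regardless of the active flag.
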(fn `ExecuteAction`
  (params (context :type "PXGameContext Structure (by ref)"))
  (bind (_nation _isvalid) (`PXGameplayContextUtils.TryGetNationFromGameContext` context))
  (bind _district (`/Game/Scenarios/Shared/BlueprintsNonSerialized/SocietyUtils/BPFL_Communication_Utils.Get Best District from Context` context))
  (if (and _isvalid (`KismetSystemLibrary.IsValid` _district))
    (`PXPredefinedModifierUtils.SetPredefinedModifierActiveManualTarget` _nation (`self.modifier`) (`ActorComponent.GetOwner` _district) (`self.Active`))
    (if (`self.Also Buildings?`)
      (for _array_element (`PXDistrictComponent.GetBuildings` (`/Game/Scenarios/Shared/BlueprintsNonSerialized/SocietyUtils/BPFL_Communication_Utils.Get Best District from Context` (`local.context`)))
        (`PXPredefinedModifierUtils.SetPredefinedModifierActiveManualTarget` _nation (`self.modifier`) (`ActorComponent.GetOwner` _array_element) (`self.Active`)))
      (return))))

(fn `GetGameplayFactorValues`
  (params (factorValues :type "Array of PXGameplayFactorValues Structure (by ref)") (context :type "PXGameContext Structure (by ref)"))
  (`PXGameplayActionUtils.AddPredefinedModifierToGameplayFactorValues` factorValues (`self.modifier`) context)
  (return))