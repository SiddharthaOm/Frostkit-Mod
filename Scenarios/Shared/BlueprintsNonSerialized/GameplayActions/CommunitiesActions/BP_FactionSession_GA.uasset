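; Gameplay action that forces a faction session on behalf of the context community, putting a policy it wants on the agenda.
; It consumes the community's stored preferred policy, skipping the session if that policy or its fallback is active, or otherwise looks one up.
; If the opposite policy in the same law previously passed with a promise made, it also starts a revenge-vote story arc.
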(fn `Also like active policy?`
  (params (policy :type "PXPolicyType Object Reference") (community :type "PXCommunityType Object Reference"))
  (returns (ReturnValue :type Boolean))
  (bind (_affinity_entry _hasaffinity) (`/Game/Scenarios/Shared/BlueprintsNonSerialized/SocietyUtils/BPFL_FactionDemandAction_Utils.Get Policy Dominant Affinity` (`/Game/Scenarios/Shared/BlueprintsNonSerialized/Policies/BPFL_PolicyUtils.Get Active Policy for Policy Law` policy)))
  (if _hasaffinity
    (return (`KismetArrayLibrary.Array_Contains` (`PXCommunityType.GetAffinities` community) _affinity_entry))))

(fn `ExecuteAction`
  (params (context :type "PXGameContext Structure (by ref)"))
  (`self.Force Session` context)
  (return))

(fn `Force Session`
  (params (context :type "PXGameContext Structure (by ref)"))
  (locals (desires :type "Array of PXDesire Structure") (policy :type "PXPolicyType Object Reference") (`Ignore negotiated check` :type Boolean :default false) (community :type "PXCommunityType Object Reference"))
  (bind (_community _isvalid) (`PXGameplayContextUtils.TryGetCommunityComponentFromGameContext` context))
  (bind _community_preferred_policy (`/Game/Scenarios/Shared/BlueprintsSerialized/VariableStorage/BP_SharedVariableStorage.Community Preferred Policy` (`/Game/Scenarios/Shared/BlueprintsNonSerialized/SocietyUtils/BPFL_SharedScenariosStorage.Get Shared Variable Storage`)))
  (bind (_value _returnvalue) (`BlueprintMapLibrary.Map_Find` _community_preferred_policy (`local.community`)))
  (if _isvalid
    (bind _output_get (set `local.community` (`PXCommunityComponent.GetCommunityType` _community)))
    (set `/Game/Scenarios/Shared/BlueprintsSerialized/VariableStorage/BP_SharedVariableStorage.Grant Agenda Community` _output_get (`/Game/Scenarios/Shared/BlueprintsNonSerialized/SocietyUtils/BPFL_SharedScenariosStorage.Get Shared Variable Storage`))
    (if _returnvalue
      (bind _output_get_2 (set `local.policy` _value))
      (`BlueprintMapLibrary.Map_Remove` _community_preferred_policy (`local.community`))
      (if (not (`/Game/Scenarios/Shared/BlueprintsNonSerialized/Policies/BPFL_PolicyUtils.Policy or Fallback is Active` _output_get_2))
        (`PXParliamentUtils.RequestSession` true (`local.policy`) false (`PXGameplayContextUtils.TryGetCommunityComponentFromGameContext` (`local.context`)) :!label _label)
        (if (`self.Likely Negotiated on Opposite Policy` (`local.policy`))
          (bind _returnvalue_2 (`|GenericCreateObject` (subsystem `PXStoryArcSubsystem`) "/Game/Scenarios/Shared/BlueprintsSerialized/StoryArcs/CommunityActions/BP_GrantAgenda_RevengeVote_StoryArc.BP_GrantAgenda_RevengeVote_StoryArc_C" (`local.policy`) (`PXTimeUtils.GetCurrentGameTime`) (`local.context`)))
          (`PXStoryUtils.StartParameterizedStoryArc` _returnvalue_2)))
      (else
        (bind (_policy_cache1 _has_valid_policy) (`/Game/Scenarios/Shared/BlueprintsNonSerialized/Policies/BPFL_PolicyUtils.Get Community Policy to Put On Agenda` (`local.community`)))
        (if (not _has_valid_policy)
          ;[1 1 1] This should never happen
          (set `local.policy` (`KismetArrayLibrary.Array_Random` (`PXPolicyUtils.GetAllInactivePolicies` (`PXPolicyUtils.GetPlayerPolicy`) true))))
        (set `local.policy` _policy_cache1)
        (goto _label)))))

(fn `GetGameplayFactorValues`
  (params (factorValues :type "Array of PXGameplayFactorValues Structure (by ref)") (context :type "PXGameContext Structure (by ref)"))
  ;[1 1 1] Empty on purpose
  (return))

(fn `Likely Negotiated on Opposite Policy`
  (params (policy :type "PXPolicyType Object Reference"))
  (returns (hasAnyItem :type Boolean))
  (return (`.hasAnyItem` (`PXParliamentUtils.GetVotingHistory` (`PXParliamentUtils.GetCurrentParliament`) 0 (`|MakeArray` (`/Game/Scenarios/Shared/BlueprintsNonSerialized/Policies/BPFL_PolicyUtils.Get Opposite Affinity Policy in Same Law` policy)) "PassedOnly" "PromiseMadeOnly" "All" "All"))))

(fn `Quest to Grant Agenda?`
  (params (context :type "PXGameContext Structure (by ref)"))
  (returns (ReturnValue :type Boolean))
  (locals (`grant agenda action` :type "PXCommunityAction Object Reference" :default "/Script/Frostpunk2.PXCommunityAction'/Game/Scenarios/Shared/Configs/Communities/CommunityActions/Relations_Group/FactionSession/DA_FactionSession_CA.DA_FactionSession_CA'"))
  (bind (_community _isvalid) (`PXGameplayContextUtils.TryGetCommunityComponentFromGameContext` context))
  (bind (_true _promisequest) (`/Game/Scenarios/Shared/BlueprintsNonSerialized/SocietyUtils/BPFL_Quest_Utils.Has Active Promise Quest?` _community))
  (bind _desire (`PXPromiseQuest.Desire` _promisequest))
  (if _isvalid
    (if _true
      (if (`|EnumEquality` (`PXDesireUtils.GetDesireType` _desire) "ActionDesire")
        (if (== (`.CommunityAction` (break `PXDesire` _desire)) (`local.grant agenda action`))
          (return true))))))