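; Gameplay action that disperses a rally by ending the ongoing community action in the district from the game context.
; On execution, it finds that district's ongoing action component and ends it with the start and finish actions and simultaneous collapse enabled.
; The acting community's in-game faction name fills a FACTION text tag.
; Gameplay factor values are intentionally left empty.
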(fn `ExecuteAction`
  (params (context :type "PXGameContext Structure (by ref)"))
  (locals (`Community in Action` :type "PXCommunityComponent Object Reference"))
  (bind (_district _isvalid) (`PXGameplayContextUtils.TryGetDistrictFromGameContext` context))
  (if _isvalid
    (bind (_hasongoingaction _returnvalue) (`PXOngoingActionUtils.GetOngoingActionComponentForDistrict` _district))
    (set `local.Community in Action` (`PXOngoingActionComponent.GetCommunity` _returnvalue))
    (`PXOngoingActionUtils.EndOngoingAction` _returnvalue (`self.Gameplay Action on Start`) (`self.Gameplay Action on Finish`) (`|MakeMap` "FACTION" (`PXFactionUtils.GetFactionInGameName` (`local.Community in Action`))) "Collapse" true null)
    (return)))

(fn `GetGameplayFactorValues`
  (params (factorValues :type "Array of PXGameplayFactorValues Structure (by ref)") (context :type "PXGameContext Structure (by ref)"))
  ;[1 1 1] Empty on purpose
  (return))