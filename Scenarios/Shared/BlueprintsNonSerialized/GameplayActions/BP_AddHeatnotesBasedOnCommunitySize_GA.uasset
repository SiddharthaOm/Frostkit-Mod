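; Gameplay action that changes the nation's stockpile of a resource (Heatnotes) in proportion to the size of the context community.
; The amount scales by a configurable multiplier, a faction boost, an optional FundAbuse imprint bonus that grows with the script's use count, and a half-funding imprint penalty.
; The same calculation feeds the gameplay factor values and execution, which can show a central notification when the stockpile change succeeds.
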(fn `ExecuteAction`
  (params (context :type "PXGameContext Structure (by ref)"))
  (locals (amount :type Integer :default 0))
  (bind (_community _isvalid) (`PXGameplayContextUtils.TryGetCommunityComponentFromGameContext` context))
  (bind (_nation _isvalid_2) (`PXGameplayContextUtils.TryGetNationFromGameContext` context))
  (bind _ingame_name (`/Game/Scenarios/Shared/BlueprintsNonSerialized/Communities/BPFL_CommunityUtils.Get Community Name` _community))
  (if _isvalid
    (if _isvalid_2
      (bind _output_get (set `local.amount` (`self.Get Heatnotes Amount` _community)))
      (bind _returnvalue (`PXStockpileUtils.TryChangeNationStockpile` _nation (`self.Resource`) _output_get))
      (if (and _returnvalue (`self.Show Notification?`))
        (`PXCentralNotificationUtils.ShowCentralNotificationOfType` "PopulationChange" (`|FormatText` (`self.Notification Title`) _ingame_name (`KismetMathLibrary.Abs_Int` (`local.amount`)) (`PXResource.IngameName` (`self.Resource`))) (`|FormatText` (`self.Notification Description`) _ingame_name (`KismetMathLibrary.Abs_Int` (`local.amount`)) (`PXResource.IngameName` (`self.Resource`))))
        (return)))))

(fn `Get FundAbuse Number`
  (params (Community :type "PXCommunityComponent Object Reference (by ref)"))
  (returns (`Times Projects Funded` :type Integer))
  (bind _returnvalue (`PXScenarioScriptSubsystem.FindScenarioScript` (subsystem `PXScenarioScriptSubsystem`) "/Game/Scenarios/Shared/BlueprintsSerialized/ScenarioScripts/StoryArcs/StoryArcsScenarioScripts/BP_FundAbuse_Script.BP_FundAbuse_Script_C")
    (:`Found`
      (return (`/Game/Scenarios/Shared/BlueprintsSerialized/ScenarioScripts/StoryArcs/StoryArcsScenarioScripts/BP_FundAbuse_Script.Get Fund Projects Use for Community` _returnvalue Community)))))

(fn `Get Half Funding Multiplier`
  (params (self2 :type "PXCommunityComponent Object Reference"))
  (returns (ReturnValue :type "Float (double-precision)"))
  (bind _half_funding_imprint (`/Game/Scenarios/Shared/Configs/ConstantsStorage/BP_SharedConstantsStorageBaseClass.Half Funding Imprint` (`/Game/Scenarios/Shared/BlueprintsNonSerialized/SocietyUtils/BPFL_SharedScenariosStorage.Get Current Scenario Constants Storage`)))
  (`/Engine/EditorBlueprintResources/StandardMacros.IsValid` _half_funding_imprint
    (:`Is Valid`
      (return (select `bool` (`PXCommunityComponent.HasActiveImprint` self2 _half_funding_imprint) :`false` 1.0 :`true` 0.5)))
    (:`Is Not Valid`
      (return 1.0))))

(fn `Get Heatnotes Amount`
  (params (self2 :type "PXCommunityComponent Object Reference"))
  (returns (ReturnValue :type Integer))
  (locals (`Faction Boost Multiplier` :type "Float (double-precision)" :default 1.4))
  (return (`KismetMathLibrary.FTrunc` (* (`KismetMathLibrary.Conv_IntToDouble` (`PXCommunityComponent.GetCommunitySize` self2)) (`self.Community Size x Heatnotes multiplier`) (select `bool` (`KismetSystemLibrary.IsValid` (`PXCommunityComponent.GetFaction` self2)) :`false` 1.0 :`true` (`local.Faction Boost Multiplier`)) (select `bool` (`self.Consider Fund Abuse Imprint?`) :`false` 1.0 :`true` (select `bool` (`PXCommunityComponent.HasActiveImprint` self2 "/Game/Scenarios/Shared/Configs/Communities/Imprints/NarrativeBased/DA_FundAbuse_IncreaseFunding_Imprint.DA_FundAbuse_IncreaseFunding_Imprint") :`false` 1.0 :`true` (+ 2.0 (* (`self.Get FundAbuse Number` self2) 0.1)))) (`self.Get Half Funding Multiplier` self2)))))

(fn `GetGameplayFactorValues`
  (params (factorValues :type "Array of PXGameplayFactorValues Structure (by ref)") (context :type "PXGameContext Structure (by ref)"))
  (bind (_community _isvalid) (`PXGameplayContextUtils.TryGetCommunityComponentFromGameContext` context))
  (if _isvalid
    (`PXGameplayActionUtils.AddIntegerToGameplayFactorValues` factorValues "/Game/Scenarios/Shared/Configs/Attributes/Categories/DA_AttributeCategory_Stockpile.DA_AttributeCategory_Stockpile" (`self.Resource`) (`self.Get Heatnotes Amount` _community))
    (return)))