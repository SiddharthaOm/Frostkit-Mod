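; Gameplay action that starts the predefined Round Up gameplay process in a city.
; On execution it takes the city from the game context and starts the process only if that city can afford it.
; Its factor values combine those of the process in the context's best city with the Detained fervour-decrease predefined modifier, which execution does not apply directly.
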(fn `ExecuteAction`
  (params (context :type "PXGameContext Structure (by ref)"))
  (bind (_city _isvalid) (`PXGameplayContextUtils.TryGetCityFromGameContext` context))
  (bind _returnvalue_passed (break `PXCheckResult` (`PXGameplayProcessUtils.CanAffordPredefinedGameplayProcessInCity` _city (`/Game/Scenarios/Shared/BlueprintsNonSerialized/FactionEmergence/BPFL_FactionWarUtils.RoundUP Gameplay process`))))
  (if _isvalid
    (if _returnvalue_passed
      (`PXGameplayProcessUtils.TryStartPredefinedGameplayProcessInCity` _city (`/Game/Scenarios/Shared/BlueprintsNonSerialized/FactionEmergence/BPFL_FactionWarUtils.RoundUP Gameplay process`))
      (return))))

(fn `GetGameplayFactorValues`
  (params (factorValues :type "Array of PXGameplayFactorValues Structure (by ref)") (context :type "PXGameContext Structure (by ref)"))
  ;[1 1 1] Empty on purpose
  (`PXGameplayActionUtils.AddPredefinedGameplayProcessToGameplayFactorValues` factorValues (`/Game/Scenarios/Shared/BlueprintsNonSerialized/SocietyUtils/BPFL_Communication_Utils.Get Best City from Context` context) (`/Game/Scenarios/Shared/BlueprintsNonSerialized/FactionEmergence/BPFL_FactionWarUtils.RoundUP Gameplay process`))
  (`PXGameplayActionUtils.AddPredefinedModifierToGameplayFactorValues` factorValues "/Game/Scenarios/Shared/Configs/PredefinedModifiers/FactionWar/DA_Detained_FervourDecrease_PredefinedModifier.DA_Detained_FervourDecrease_PredefinedModifier" context)
  (return))