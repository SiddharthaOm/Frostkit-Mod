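; BP_PickBarks_GA is a gameplay action that triggers barks between two generated speaker communities, using a bark set, an angry setting and the context's district.
; Each speaker resolves from a target type: context, additional or opposing-faction community, or an affinity-based commenter with fallbacks; Specific Community shares the affinity path.
; Legacy custom-speaker bools still force the affinity path, flagged as a temporary hack.
; Extra text defines merge with those from the game context.
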(fn `ExecuteAction`
  (params (context :type "PXGameContext Structure (by ref)"))
  (bind _context (`local.context`))
  (bind _defines_map_merged (`/Game/Scenarios/Shared/BlueprintsNonSerialized/SocietyUtils/BPFL_Communication_Utils.Merge Defines` (`self.Extra Text Defines`) (`/Game/Scenarios/Shared/BlueprintsNonSerialized/SocietyUtils/BPFL_Communication_Utils.Get Defines from Game Context` (`local.context`))))
  (`/Game/Scenarios/Shared/BlueprintsNonSerialized/SocietyUtils/BPFL_Communication_Utils.Pick Barks with Generated Speaker` (`self.Get Speaker 1 Community` _context) (`self.Get Speaker 2 Community` _context) (`self.Angry`) _defines_map_merged (`self.Bark Set`) (`/Game/Scenarios/Shared/BlueprintsNonSerialized/SocietyUtils/BPFL_Communication_Utils.Get Best District from Context` (`local.context`))))

(fn `Get Community for Target Type`
  (params (Selection :type "/Game/Scenarios/Shared/Enumerations/ENUM_CommunityActionTarget Enum" :default "NewEnumerator0") (context :type "PXGameContext Structure (by ref)") (Affinity :type "PXAffinityEntry Structure"))
  (returns (OutputPin :type "PXCommunityComponent Object Reference"))
  (bind (_community _isvalid) (`PXGameplayContextUtils.TryGetCommunityComponentFromGameContext` (`local.context`)))
  (bind (_oppositefaction _faction_component _found) (`/Game/Scenarios/Shared/BlueprintsNonSerialized/FactionEmergence/BPFL_FactionWarUtils.Get Existing Opposing Faction` (`PXCommunityComponent.GetFaction` _community)))
  (switch `/Game/Scenarios/Shared/Enumerations/ENUM_CommunityActionTarget` Selection
    (:`NewEnumerator0`
      (return (`/Game/Scenarios/Shared/BlueprintsNonSerialized/SocietyUtils/BPFL_Communication_Utils.Get Best Community from Context` (`local.context`))))
    (:`NewEnumerator1`
      (return (`PXGameplayContextUtils.TryGetAdditionalCommunityComponentFromGameContext` (`local.context`))))
    (:`NewEnumerator2`
      (if _isvalid
        (if _found
          (return _faction_component)
          (else
            _)))
      (`KismetSystemLibrary.PrintString` "Community Action could not find valid target. PickBarks_GA "))
    (:`NewEnumerator3`
      (bind (_exists _community_2) (`/Game/Scenarios/Shared/BlueprintsNonSerialized/SocietyUtils/BPFL_Cornerstone_Utils.Get X Affinity Commenter` (`local.Affinity`) true true :!label _label))
      (return _community_2))
    (:`NewEnumerator4`
      (goto _label))))

(fn `Get Speaker 1 Community`
  (params (context :type "PXGameContext Structure (by ref)"))
  (returns (ReturnValue :type "PXCommunityComponent Object Reference"))
  (bind _outputpin (`self.Get Community for Target Type` (select `bool` (`self.Custom Generated Speaker for Speaker 1`) :`false` (`self.Speaker 1 Target`) :`true` "NewEnumerator4") context (`self.Affinity Speaker 1`)))
  (return _outputpin))

(fn `Get Speaker 2 Community`
  (params (context :type "PXGameContext Structure (by ref)"))
  (returns (ReturnValue :type "PXCommunityComponent Object Reference"))
  (bind _outputpin (`self.Get Community for Target Type` (select `bool` (`self.Custom Generated Speaker for Speaker 2`) :`false` (`self.Speaker 2 Target`) :`true` "NewEnumerator4") context (`self.Affinity Speaker 2`)))
  (return _outputpin))

(fn `GetGameplayFactorValues`
  (params (factorValues :type "Array of PXGameplayFactorValues Structure (by ref)") (context :type "PXGameContext Structure (by ref)"))
  ;[1 1 1] Empty on purpose
  (return))