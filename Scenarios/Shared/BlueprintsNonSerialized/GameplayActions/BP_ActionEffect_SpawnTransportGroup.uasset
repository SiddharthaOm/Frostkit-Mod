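; Gameplay action effect that sends a unit to transport resources from the context's frostland site to the city.
; It issues the transport order with an overridden or default refugee-order cost, passes on arrival actions, then increments the frostland stockpiles-taken counter.
; It also reports cost, resources and arrival actions as gameplay factor values.
; The stockpile registration and trip-duration factor nodes never run.
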(fn `ExecuteAction`
  (params (context :type "PXGameContext Structure (by ref)"))
  (bind (_city _isvalid) (`PXGameplayContextUtils.TryGetCityFromGameContext` context))
  (bind (_orderdescription_ingamename _orderdescription_title _orderdescription_description _orderdescription_finishedordernotificationtext _orderdescription_failedordernotificationtext _orderdescription_defaultcost) (break `PXUnitOrderDescription` (`PXUnitOrderType.OrderDescription` (`PXUnitConfig.RefugeesOrder` (`PXGameplayUtils.GetUnitConfig`)))))
  (if _isvalid
    (bind _actor (`self.GetContextActor` context))
    (`PXUnitUtils.AssignUnitToTransportResourcesOrder` (`self.UnitType`) _actor (select `bool` (`self.OverrideCost`) :`false` _orderdescription_defaultcost :`true` (`self.Cost`)) (`self.Resources`) _city (`self.GameplayActionOnArrival`) (`self.GameplayPredefinedAction`))
    (`/Engine/EditorBlueprintResources/StandardMacros.IncrementInt` (`/Game/Scenarios/Shared/BlueprintsSerialized/VariableStorage/BP_SharedVariableStorage.TimesStockpilesFromFrostlandTaken` (`/Game/Scenarios/Shared/BlueprintsNonSerialized/SocietyUtils/BPFL_SharedScenariosStorage.Get Shared Variable Storage`))
      (:`  `
        (return)))))

(fn `GetContextActor`
  (params (Context :type "PXGameContext Structure"))
  (returns (Actor :type "Actor Object Reference"))
  (bind (_site _isvalid) (`PXGameplayContextUtils.TryGetSiteFromGameContext` Context))
  (if _isvalid
    (return (`ActorComponent.GetOwner` _site))
    (else
      (return null))))

(fn `GetGameplayFactorValues`
  (params (factorValues :type "Array of PXGameplayFactorValues Structure (by ref)") (context :type "PXGameContext Structure (by ref)"))
  (locals (UnitOperationCost :type "PXOperationCost Structure") (EmptyCost :type "Map of PXResource Object Reference to Integer"))
  (bind _context (`local.context`))
  (bind _city (`PXGameplayContextUtils.TryGetCityFromGameContext` _context))
  (bind _actor (`self.GetContextActor` context))
  (`/Engine/EditorBlueprintResources/StandardMacros.IsValid` _actor
    (:`Is Valid`
      (`/Engine/EditorBlueprintResources/StandardMacros.IsValid` _city
        (:`Is Valid`
          (bind _output_get (set `local.UnitOperationCost` (`PXUnitUtils.GetUnitOperationCost` (`self.UnitType`) (`local.EmptyCost`) (`PXGameplayContextUtils.TryGetNationFromGameContext` _context) _actor (`ActorComponent.GetOwner` _city))))
          (`PXGameplayActionUtils.AddResourcesToGameplayFactorValues` (`local.factorValues`) "/Game/Scenarios/Shared/Configs/Attributes/Categories/DA_AttributeCategory_FlatChange.DA_AttributeCategory_FlatChange" (select `bool` (`self.OverrideCost`) :`false` (`.DefaultCost` (break `PXUnitOrderDescription` (`PXUnitOrderType.OrderDescription` (`PXUnitConfig.RefugeesOrder` (`PXGameplayUtils.GetUnitConfig`))))) :`true` (`self.Cost`)))
          (`PXGameplayActionUtils.AddResourcesToGameplayFactorValues` (`local.factorValues`) "/Game/Scenarios/Shared/Configs/Attributes/Categories/DA_AttributeCategory_Stockpile.DA_AttributeCategory_Stockpile" (`self.Resources`))
          (`PXGameplayActionUtils.AddPredefinedActionsToGameplayFactorValues` (`local.factorValues`) (`self.GameplayPredefinedAction`) (`local.context`))
          (`/Engine/EditorBlueprintResources/StandardMacros.IsValid` (`self.GameplayActionOnArrival`)
            (:`Is Valid`
              (`PXGameplayActionUtils.AddGameplayActionToGameplayFactorValues` (`local.factorValues`) (`self.GameplayActionOnArrival`) (`local.context`)))
            (:`Is Not Valid`
              _))
          (return))))))