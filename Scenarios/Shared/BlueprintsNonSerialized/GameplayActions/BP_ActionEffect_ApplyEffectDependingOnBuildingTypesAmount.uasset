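; Gameplay action effect that changes a nation's stockpile of a configurable resource based on community size, despite the asset name referring to building types.
; The amount is community size times a multiplier, boosted when the community has a valid faction, then truncated.
; Execution applies it to the context nation and optionally shows a central notification on success.
; The same calculation feeds the stockpile gameplay factor values.
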(fn `ExecuteAction`
  (params (context :type "PXGameContext Structure (by ref)"))
  (locals (amount :type Integer :default 0))
  (bind (_community _isvalid) (`PXGameplayContextUtils.TryGetCommunityComponentFromGameContext` context))
  (bind (_nation _isvalid_2) (`PXGameplayContextUtils.TryGetNationFromGameContext` context))
  (bind _ingame_name (`/Game/Scenarios/Shared/BlueprintsNonSerialized/Communities/BPFL_CommunityUtils.Get Community Name` _community))
  (if _isvalid
    (if _isvalid_2
      (bind _output_get (set `local.amount` (`self.Get Heatnotes Amount` _community)))
      (bind _returnvalue (`PXStockpileUtils.TryChangeNationStockpile` _nation (`self.Resource`) _output_get))
      (if (and _returnvalue (`self.Show Notification?`))
        (`PXCentralNotificationUtils.ShowCentralNotificationOfType` "PopulationChange" (`|FormatText` (`self.Notification Title`) _ingame_name (`KismetMathLibrary.Abs_Int` (`local.amount`)) (`PXResource.IngameName` (`self.Resource`))) (`|FormatText` (`self.Notification Description`) _ingame_name (`KismetMathLibrary.Abs_Int` (`local.amount`)) (`PXResource.IngameName` (`self.Resource`))))
        (return)))))

(fn `Get Heatnotes Amount`
  (params (self2 :type "PXCommunityComponent Object Reference"))
  (returns (ReturnValue :type Integer))
  (locals (`Faction Boost Multiplier` :type "Float (double-precision)" :default 1.4))
  (return (`KismetMathLibrary.FTrunc` (* (`KismetMathLibrary.Conv_IntToDouble` (`PXCommunityComponent.GetCommunitySize` self2)) (`self.Community Size x Heatnotes multiplier`) (select `bool` (`KismetSystemLibrary.IsValid` (`PXCommunityComponent.GetFaction` self2)) :`false` 1.0 :`true` (`local.Faction Boost Multiplier`))))))

(fn `GetGameplayFactorValues`
  (params (factorValues :type "Array of PXGameplayFactorValues Structure (by ref)") (context :type "PXGameContext Structure (by ref)"))
  (bind (_community _isvalid) (`PXGameplayContextUtils.TryGetCommunityComponentFromGameContext` context))
  (if _isvalid
    (`PXGameplayActionUtils.AddIntegerToGameplayFactorValues` factorValues "/Game/Scenarios/Shared/Configs/Attributes/Categories/DA_AttributeCategory_Stockpile.DA_AttributeCategory_Stockpile" (`self.Resource`) (`self.Get Heatnotes Amount` _community))
    (return)))