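; A gameplay action effect that activates a configured predefined modifier on the city taken from the game context.
; ExecuteAction resolves the nation and city from the context and, when both are valid, sets the modifier active for that nation with the city's owner as manual target.
; GetGameplayFactorValues adds the same modifier's values to the reported gameplay factors.
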(fn `ExecuteAction`
  (params (context :type "PXGameContext Structure (by ref)"))
  (bind (_city _isvalid) (`PXGameplayContextUtils.TryGetCityFromGameContext` context))
  (bind (_nation _isvalid_2) (`PXGameplayContextUtils.TryGetNationFromGameContext` context))
  (if (and _isvalid_2 _isvalid)
    (`PXPredefinedModifierUtils.SetPredefinedModifierActiveManualTarget` _nation (`self.modifier`) (`ActorComponent.GetOwner` _city) true)
    (return)))

(fn `GetGameplayFactorValues`
  (params (factorValues :type "Array of PXGameplayFactorValues Structure (by ref)") (context :type "PXGameContext Structure (by ref)"))
  (`PXGameplayActionUtils.AddPredefinedModifierToGameplayFactorValues` factorValues (`self.modifier`) context)
  (return))