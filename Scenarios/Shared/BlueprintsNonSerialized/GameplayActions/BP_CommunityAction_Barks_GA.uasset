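; Gameplay action that plays a two-speaker bark exchange when a community action comes from the player leader; other origins show no default barks.
; The first speaker comes from the context's community, the second from a random community in the same city.
; The second pick prefers communities with opposite core affinities, then those lacking them, then any other community.
; Barks use generated speakers, the context's text defines and best district; gameplay factor values are intentionally empty.
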(fn `ExecuteAction`
  (params (context :type "PXGameContext Structure (by ref)"))
  (locals (community :type "PXCommunityComponent Object Reference") (`opposite community` :type "PXCommunityComponent Object Reference") (communities :type "Array of PXCommunityComponent Object Reference") (`player leader action origin` :type "PXActionOrigin Object Reference" :default "/Script/Frostpunk2.PXActionOrigin'/Game/Scenarios/Shared/Configs/ActionOrigin/DA_LeaderActionOrigin.DA_LeaderActionOrigin'"))
  (bind (_actionorigin _isvalid) (`PXGameplayContextUtils.TryGetActionOriginFromGameContext` context))
  (bind _community (`local.community`))
  (bind _context (`local.context`))
  (if _isvalid
    ;[1 1 1] Don't show default barks when not Leader action
    (if (== _actionorigin (`local.player leader action origin`))
      (bind _output_get (set `local.community` (`PXGameplayContextUtils.TryGetCommunityComponentFromGameContext` context)))
      (bind _communities_with_affinity (`/Game/Scenarios/Shared/BlueprintsNonSerialized/SocietyUtils/BPFL_Cornerstone_Utils.Get Communites With Opposite Affinity` (`PXCommunityComponent.ParentCity` _output_get) (`PXCommunityUtils.GetCommunityCoreAffinities` _output_get)))
      (bind _output_get_2 (set `local.communities` _communities_with_affinity))
      (if (not (`KismetArrayLibrary.Array_IsNotEmpty` _output_get_2))
        (bind _communities_with_affinity_2 (`/Game/Scenarios/Shared/BlueprintsNonSerialized/SocietyUtils/BPFL_Cornerstone_Utils.Get Communites Without Affinity` (`PXCommunityComponent.ParentCity` _community) (`PXCommunityUtils.GetCommunityCoreAffinities` _community)))
        (bind _output_get_3 (set `local.communities` _communities_with_affinity_2))
        (if (not (`KismetArrayLibrary.Array_IsNotEmpty` _output_get_3))
          (bind _output_get_4 (set `local.communities` (`PXCityComponent.GetCommunities` (`PXCommunityComponent.ParentCity` (`local.community`)))))
          (`KismetArrayLibrary.Array_RemoveItem` _output_get_4 (`local.community`))))
      (set `local.opposite community` (`PXRandomLibrary.PXArrayRandom` (`local.communities`)))
      (`/Game/Scenarios/Shared/BlueprintsNonSerialized/SocietyUtils/BPFL_Communication_Utils.Pick Barks with Generated Speaker` (`local.community`) (`local.opposite community`) false (`/Game/Scenarios/Shared/BlueprintsNonSerialized/SocietyUtils/BPFL_Communication_Utils.Get Defines from Game Context` _context) (`self.Bark Set`) (`/Game/Scenarios/Shared/BlueprintsNonSerialized/SocietyUtils/BPFL_Communication_Utils.Get Best District from Context` _context))
      (return))))

(fn `GetGameplayFactorValues`
  (params (factorValues :type "Array of PXGameplayFactorValues Structure (by ref)") (context :type "PXGameContext Structure (by ref)"))
  ;[1 1 1] Empty on purpose
  (return))