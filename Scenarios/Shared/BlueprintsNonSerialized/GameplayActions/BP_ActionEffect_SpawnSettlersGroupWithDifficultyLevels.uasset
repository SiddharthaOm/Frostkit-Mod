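; Gameplay action effect that orders a unit to bring a group of settlers from a Frostland site to the city, with group size set by difficulty.
; Size is looked up by entry in the difficulty setup's site randomization values.
; Execution assigns a refugees order with default or overridden cost and arrival actions, then increments a shared counter.
; Factor values preview population, cost and arrival effects; the duration preview is unwired.
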(fn `ExecuteAction`
  (params (context :type "PXGameContext Structure (by ref)"))
  (bind (_city _isvalid) (`PXGameplayContextUtils.TryGetCityFromGameContext` context))
  (if _isvalid
    (`/Engine/EditorBlueprintResources/StandardMacros.IsValid` (`self.UnitType`)
      (:`Is Valid`
        _)
      (:`Is Not Valid`
        (set `self.UnitType` "/Game/Scenarios/Shared/Configs/FrostlandExploration/FrostlandUnitExplorationType/DA_AllPurposeUnit.DA_AllPurposeUnit")))
    (bind _actor (`self.GetContextActor` context))
    (`PXUnitUtils.AssignUnitToRefugeesOrder` (`self.UnitType`) _actor (select `bool` (`self.OverrideCost`) :`false` (`.DefaultCost` (break `PXUnitOrderDescription` (`PXUnitOrderType.OrderDescription` (`PXUnitConfig.RefugeesOrder` (`PXGameplayUtils.GetUnitConfig`))))) :`true` (`self.Cost`)) (`self.CommunityType`) (`self.Get Community Size from Difficulty Level`) _city (`self.GameplayActionOnArrival`) (`self.PredefinedGameplayAction`))
    (`/Engine/EditorBlueprintResources/StandardMacros.IncrementInt` (`/Game/Scenarios/Shared/BlueprintsSerialized/VariableStorage/BP_SharedVariableStorage.TimesPeople FromFrostlandTaken` (`/Game/Scenarios/Shared/BlueprintsNonSerialized/SocietyUtils/BPFL_SharedScenariosStorage.Get Shared Variable Storage`))
      (:`  `
        (return)))))

(fn `Get Community Size from Difficulty Level`
  (returns (CommunitySize :type Integer))
  (bind _asbp_pda_sites_randomization_values (cast `/Game/Scenarios/Shared/Configs/DifficultyLevels/Categories/Frostland/SiteRandomizationValues/BP_PDA_SitesRandomizationValues` (`.SiteRandomizationValues` (break `PXDifficultyLevelSetup` (`PXDifficultyLevelUtils.GetDifficultyLevelSetup`)))))
  (if (`/Game/Scenarios/Shared/Configs/DifficultyLevels/Categories/Frostland/SiteRandomizationValues/BP_PDA_SitesRandomizationValues.Has Value for Entry` _asbp_pda_sites_randomization_values (`self.SiteRandomizationValuesEntry`))
    (return (`BlueprintMapLibrary.Map_Find` (`/Game/Scenarios/Shared/Configs/DifficultyLevels/Categories/Frostland/SiteRandomizationValues/BP_PDA_SitesRandomizationValues.SiteRandomizationValues` _asbp_pda_sites_randomization_values) (`self.SiteRandomizationValuesEntry`)))
    (else
      (return 0))))

(fn `GetContextActor`
  (params (Context :type "PXGameContext Structure"))
  (returns (Actor :type "Actor Object Reference"))
  (bind (_site _isvalid) (`PXGameplayContextUtils.TryGetSiteFromGameContext` Context))
  (if _isvalid
    (return (`ActorComponent.GetOwner` _site))
    (else
      (return null))))

(fn `GetGameplayFactorValues`
  (params (factorValues :type "Array of PXGameplayFactorValues Structure (by ref)") (context :type "PXGameContext Structure (by ref)"))
  (locals (EmptyCost :type "Map of PXResource Object Reference to Integer"))
  (bind _gameplayactiononarrival (`self.GameplayActionOnArrival`))
  (bind _actor (`self.GetContextActor` context))
  (`/Engine/EditorBlueprintResources/StandardMacros.IsValid` _actor
    (:`Is Valid`
      (`PXGameplayActionUtils.AddResourcesToGameplayFactorValues` factorValues "/Game/Scenarios/Shared/Configs/Attributes/Categories/DA_AttributeCategory_FlatChange.DA_AttributeCategory_FlatChange" (`|MakeMap` "/Game/Scenarios/Shared/Configs/Resources/Types/DA_PeopleResource.DA_PeopleResource" (`/Game/UI/Utilities/BPFL_UI.Get Population From Size Points` (`self.Get Community Size from Difficulty Level`)) :!type "PXResource Object Reference"))
      (`PXGameplayActionUtils.AddResourcesToGameplayFactorValues` factorValues "/Game/Scenarios/Shared/Configs/Attributes/Categories/DA_AttributeCategory_FlatChange.DA_AttributeCategory_FlatChange" (select `bool` (`self.OverrideCost`) :`false` (`.DefaultCost` (break `PXUnitOrderDescription` (`PXUnitOrderType.OrderDescription` (`PXUnitConfig.RefugeesOrder` (`PXGameplayUtils.GetUnitConfig`))))) :`true` (`self.Cost`)))
      (`PXGameplayActionUtils.AddPredefinedActionsToGameplayFactorValues` factorValues (`self.PredefinedGameplayAction`) context)
      (`/Engine/EditorBlueprintResources/StandardMacros.IsValid` _gameplayactiononarrival
        (:`Is Valid`
          (`PXGameplayActionUtils.AddGameplayActionToGameplayFactorValues` factorValues _gameplayactiononarrival context))
        (:`Is Not Valid`
          _))
      (return))))