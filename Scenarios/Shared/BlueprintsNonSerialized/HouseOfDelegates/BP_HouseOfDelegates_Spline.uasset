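; Spline-based camera animation Blueprint for the House of Delegates scenario, currently inert: its two events are empty and the remaining logic is disconnected.
; The unwired camera logic plays or reverses a timeline that moves a camera actor along the spline, signalling completion when finished.
; Unwired cursor-trace checks against a character trigger would start that zoom or play looping skeletal mesh animations, including cheering, switched after a delay.
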(event `CameraAnimationFinished`)

(event `PlayCameraAnimaiton`
  (params (Reverse :type Boolean)))

(event `InputAction|DebugPointHoD`
  (params (Key :type "Key Structure")))

(fn `UserConstructionScript`)