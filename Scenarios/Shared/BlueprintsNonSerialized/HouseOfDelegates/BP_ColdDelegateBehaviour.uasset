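; Behaviour that gives House of Delegates parliament characters a cold-breath steam effect from the mouth.
; On activation it waits for the delegate-set event if the representative or head mesh is missing, then filters representatives by a tag query (empty matches all).
; Matching delegates get a cold mouth steam emission point attached to a head bone, and their visible-in-view state is reset.
; Deactivation, and each re-application, destroys the previously spawned effect.
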(event `CustomEvent_0`
  (`self.OnDeactivateFunction`)
  (bind _hastags (`self.HasDesiredTags` (`PXRepresentativeComponent.GetRepresentative` (`/Game/Scenarios/Shared/BlueprintsNonSerialized/HouseOfDelegates/BP_ParliamentCharacter.PXRepresentative` (stale `self.OnActivate` _asbp_parliament_character))) :!label _label))
  (if _hastags
    (bind _returnvalue (`PXParliamentUtils.AddEmissionPointToDelegate` (stale `self.OnActivate` _asbp_parliament_character) "/Game/Scenarios/Shared/FXs/EmissionPoints/EmissionPointTypes/DA_ColdMouthSteam.DA_ColdMouthSteam"))
    (bind _output_get (set `self.SpawnedFX` _returnvalue))
    (`SceneComponent.K2_AttachToComponent` _output_get (`/Game/Scenarios/Shared/BlueprintsNonSerialized/HouseOfDelegates/BP_ParliamentCharacter.Head` (stale `self.OnActivate` _asbp_parliament_character)) (`self.BoneName`) "KeepRelative" "KeepRelative" "KeepWorld" true)
    (`SceneComponent.K2_SetRelativeRotation` (`self.SpawnedFX`) (struct :`Yaw` -90.0) false false)
    (`PXParliamentUtils.ResetVisibileInView` (`/Game/Scenarios/Shared/BlueprintsNonSerialized/HouseOfDelegates/BP_ParliamentCharacter.PXVisibleInView` (stale `self.OnActivate` _asbp_parliament_character)))
    (clear `/Game/Scenarios/Shared/BlueprintsNonSerialized/HouseOfDelegates/BP_ParliamentCharacter.CallDelegateIsSet` (stale `self.OnActivate` _asbp_parliament_character))))

(event `self.OnActivate`
  (params (owner :type "Actor Object Reference") (gameInstance :type "PXGameInstance Object Reference") (arguments :type "PXStateBehaviourArguments Object Reference") (stateEntry :type "PXStateEntry Structure"))
  (bind _asbp_parliament_character (cast `/Game/Scenarios/Shared/BlueprintsNonSerialized/HouseOfDelegates/BP_ParliamentCharacter` owner))
  (`/Engine/EditorBlueprintResources/StandardMacros.IsValid` (`PXRepresentativeComponent.GetRepresentative` (`/Game/Scenarios/Shared/BlueprintsNonSerialized/HouseOfDelegates/BP_ParliamentCharacter.PXRepresentative` _asbp_parliament_character))
    (:`Is Valid`
      (`/Engine/EditorBlueprintResources/StandardMacros.IsValid` (`SkeletalMeshComponent.SkeletalMeshAsset` (`/Game/Scenarios/Shared/BlueprintsNonSerialized/HouseOfDelegates/BP_ParliamentCharacter.Head` _asbp_parliament_character))
        (:`Is Valid`
          (goto _label))
        (:`Is Not Valid`
          _)))
    (:`Is Not Valid`
      _))
  (add `/Game/Scenarios/Shared/BlueprintsNonSerialized/HouseOfDelegates/BP_ParliamentCharacter.CallDelegateIsSet` _asbp_parliament_character (delegate `CustomEvent_0`)))

(event `self.OnDeactivate`
  (params (owner :type "Actor Object Reference") (gameInstance :type "PXGameInstance Object Reference") (arguments :type "PXStateBehaviourArguments Object Reference") (stateEntry :type "PXStateEntry Structure"))
  (`self.OnDeactivateFunction`))

(fn `HasDesiredTags`
  (params (Representative :type "PXRepresentative Object Reference"))
  (returns (hasTags :type Boolean))
  (bind _returnvalue (`PXParliamentUtils.GetRepresentativeTags` Representative))
  (`/Engine/EditorBlueprintResources/StandardMacros.IsValid` Representative
    (:`Is Valid`
      (return (or (`BlueprintGameplayTagLibrary.DoesContainerMatchTagQuery` _returnvalue (`self.DesiredTags`)) (`BlueprintGameplayTagLibrary.IsTagQueryEmpty` (`self.DesiredTags`)))))
    (:`Is Not Valid`
      (return false))))

(fn `OnDeactivateFunction`
  (bind _spawnedfx (`self.SpawnedFX`))
  (`/Engine/EditorBlueprintResources/StandardMacros.IsValid` _spawnedfx
    (:`Is Valid`
      (`SceneComponent.SetVisibility` _spawnedfx true false)
      (`ActorComponent.K2_DestroyComponent` _spawnedfx)
      (set `self.SpawnedFX` null))))