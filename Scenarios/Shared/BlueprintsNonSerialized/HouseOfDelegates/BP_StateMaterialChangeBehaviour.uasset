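; State behaviour that swaps static mesh materials on a BP_HoD_3D actor when one of its states activates or deactivates.
; Both events look up the state entry in the owner's StateMaterialsChange map, find components by key name and set materials per slot index.
; Activation first checks the state through a subsystem and clears IsAsyncActive as materials apply.
; Deactivation applies DeactivationArguments materials but takes its component list from the ActivationArguments keys.
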(event `self.OnActivate`
  (params (owner :type "Actor Object Reference") (gameInstance :type "PXGameInstance Object Reference") (arguments :type "PXStateBehaviourArguments Object Reference") (stateEntry :type "PXStateEntry Structure"))
  (set `self.Owner` owner)
  (set `self.State Entry` stateEntry)
  (bind _returnvalue (`|Subsystem`)
    (:`then`
      (bind _returnvalue_2 (`PXStateSubsystem.GetActorStateByEntry` _returnvalue (`self.Owner`) (`self.State Entry`)))
      (if _returnvalue_2
        (bind _asbp_ho_d_3d (cast `/Game/Scenarios/Shared/BlueprintsNonSerialized/HouseOfDelegates/BP_HoD_3D` (`self.Owner`)))
        (bind (_value _returnvalue_3) (`BlueprintMapLibrary.Map_Find` (`/Game/Scenarios/Shared/BlueprintsNonSerialized/HouseOfDelegates/BP_HoD_3D.StateMaterialsChange` _asbp_ho_d_3d) (`self.State Entry`)))
        (if _returnvalue_3
          (bind _activationarguments (break `/Game/Scenarios/Shared/BlueprintsNonSerialized/HouseOfDelegates/S_ComponentAndMaterialSlot` _value))
          (bind _keys (`BlueprintMapLibrary.Map_Keys` _activationarguments))
          (for _array_element _keys
            (bind _returnvalue_4 (`PXActorComponentLinkUtils.GetName` _array_element))
            (bind _returnvalue_5 (`PXComponentUtils.FindComponentByName` _returnvalue_4 (`self.Owner`)))
            (bind _asstatic_mesh_component (cast `StaticMeshComponent` _returnvalue_5))
            (for (_array_element_2 _array_index) (`.MaterialArray_8_FACBF486421F247E8C3489A72F4E259E` (break `/Game/Scenarios/Shared/BlueprintsNonSerialized/HouseOfDelegates/S_MaterialSlot` (`BlueprintMapLibrary.Map_Find` _activationarguments _array_element)))
              (`PrimitiveComponent.SetMaterial` _asstatic_mesh_component _array_index _array_element_2)
              (set `self.IsAsyncActive` false))))))))

(event `self.OnDeactivate`
  (params (owner :type "Actor Object Reference") (gameInstance :type "PXGameInstance Object Reference") (arguments :type "PXStateBehaviourArguments Object Reference") (stateEntry :type "PXStateEntry Structure"))
  (bind _asbp_ho_d_3d (cast `/Game/Scenarios/Shared/BlueprintsNonSerialized/HouseOfDelegates/BP_HoD_3D` owner))
  (bind (_value _returnvalue) (`BlueprintMapLibrary.Map_Find` (`/Game/Scenarios/Shared/BlueprintsNonSerialized/HouseOfDelegates/BP_HoD_3D.StateMaterialsChange` _asbp_ho_d_3d) stateEntry))
  (if _returnvalue
    (bind (_activationarguments _deactivationarguments) (break `/Game/Scenarios/Shared/BlueprintsNonSerialized/HouseOfDelegates/S_ComponentAndMaterialSlot` _value))
    (bind _keys (`BlueprintMapLibrary.Map_Keys` _activationarguments))
    (for _array_element _keys
      (bind _returnvalue_2 (`PXActorComponentLinkUtils.GetName` _array_element))
      (bind _returnvalue_3 (`PXComponentUtils.FindComponentByName` _returnvalue_2 owner))
      (bind _asstatic_mesh_component (cast `StaticMeshComponent` _returnvalue_3))
      (for (_array_element_2 _array_index) (`.MaterialArray_8_FACBF486421F247E8C3489A72F4E259E` (break `/Game/Scenarios/Shared/BlueprintsNonSerialized/HouseOfDelegates/S_MaterialSlot` (`BlueprintMapLibrary.Map_Find` _deactivationarguments _array_element)))
        (`PrimitiveComponent.SetMaterial` _asstatic_mesh_component _array_index _array_element_2)))))