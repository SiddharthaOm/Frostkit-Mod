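; BP_TrailUnderConstruction is a visualization actor that marks a trail segment under construction between two points.
; CreateConnections aims ConnectionTransform's X axis from Start to End and stretches its X scale to the distance, keeping Y and Z scale.
; It moves the two pin meshes to the endpoints, offset upward by each pin's relative Z.
; ConnectionTransform's location is not set here, and there is no active Tick or construction logic.
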(event `self.CreateConnections`
  (params (start :type "Vector Structure") (end :type "Vector Structure"))
  (bind (_relativelocation_x _relativelocation_y _relativelocation_z) (`KismetMathLibrary.BreakVector` (`SceneComponent.RelativeLocation` (`self.PinMeshA`))))
  (bind (_relativescale3d_x _relativescale3d_y _relativescale3d_z) (`KismetMathLibrary.BreakVector` (`SceneComponent.RelativeScale3D` (`self.ConnectionTransform`))))
  (bind (_relativelocation_x_2 _relativelocation_y_2 _relativelocation_z_2) (`KismetMathLibrary.BreakVector` (`SceneComponent.RelativeLocation` (`self.PinMeshB`))))
  (`SceneComponent.K2_SetRelativeRotation` (`self.ConnectionTransform`) (`KismetMathLibrary.Conv_VectorToRotator` (- end start)) false false)
  (`SceneComponent.SetRelativeScale3D` (`self.ConnectionTransform`) (`KismetMathLibrary.MakeVector` (`KismetMathLibrary.Vector_Distance` start end) _relativescale3d_y _relativescale3d_z))
  (`SceneComponent.K2_SetWorldLocation` (`self.PinMeshA`) (+ start (`KismetMathLibrary.MakeVector` 0.0 0.0 _relativelocation_z)) false false)
  (`SceneComponent.K2_SetWorldLocation` (`self.PinMeshB`) (+ end (`KismetMathLibrary.MakeVector` 0.0 0.0 _relativelocation_z_2)) false false))

(fn `UserConstructionScript`)