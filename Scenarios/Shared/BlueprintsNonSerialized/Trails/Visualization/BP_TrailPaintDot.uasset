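; Visual marker for one dot in trail painting, shown as a pin, point of interest, neighbour dot or blocked torus.
; Status flags pick the visible meshes by priority, while selection and connectability choose the decal material and empty-pin preview.
; Pins stretch a rotated connection mesh to their connected dot or, without one, the mouse position.
; Curve-driven animation and fading, plus unavailable states, reach materials through custom primitive data.
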(event EventRefreshSlectionStatus
  (CallFunction|UpdateSelectionState)
  (Rendering|SetVisibility (Variables|Default|GetEmptyPinMesh) (or (and (Class|PXTrailPaintDot|IsSelected) (Class|PXTrailPaintDot|HasStatus "Connectable")) (and (Class|PXTrailPaintDot|HasStatus "PointOfInterest") (not (Class|PXTrailPaintDot|HasStatus "Pin")))) true)
  (Rendering|SetVisibility (Variables|Default|GetDotMesh) (Math|Boolean|ANDBoolean (not (and (Class|PXTrailPaintDot|IsSelected) (Class|PXTrailPaintDot|HasStatus "Connectable"))) (Class|PXTrailPaintDot|HasStatus "Neighbour") (not (or (Class|PXTrailPaintDot|HasStatus "PointOfInterest") (Class|PXTrailPaintDot|HasStatus "Pin")))) false))

(event EventRefreshStatus
  (Utilities|FlowControl|Sequence
    (:then_0
      (Rendering|SetVisibility (Variables|Default|GetEmptyPinTransform) false true)
      (Rendering|SetVisibility (Variables|Default|GetPXPinTransform) false true)
      (Rendering|SetVisibility (Variables|Default|GetDotMesh) false false)
      (Rendering|SetVisibility (Variables|Default|GetTorusMesh) false false)
      (Utilities|MajorStatusSwitch
        (:Pin
          (Rendering|SetVisibility (Variables|Default|GetPXPinTransform) true true)
          (if (Utilities|IsValid (Variables|Default|GetConnectedDot))
            (CallFunction|Connectto (+ (Variables|/Script/Engine.SceneComponent|GetRelativeLocation (Variables|Default|GetPinMesh)) (Transformation|GetActorLocation (Variables|Default|GetConnectedDot))))))
        (:PointOfInterest
          (Rendering|SetVisibility (Variables|Default|GetEmptyPinTransform) true true)
          (Rendering|SetVisibility (Variables|Default|GetConnectionMesh) false false))
        (:Neighbour
          (Rendering|SetVisibility (Variables|Default|GetDotMesh) true false)
          (Rendering|SetVisibility (Variables|Default|GetConnectionMesh) false false))
        (:Blocked
          (Rendering|SetVisibility (Variables|Default|GetTorusMesh) true false))))
    (:then_1
      (Rendering|SetVisibility (Variables|Default|GetDecalPlane) (Class|PXTrailPaintDot|HasStatus "PointOfInterest") false)
      (CallFunction|UpdateSelectionState)
      (Rendering|Material|SetCustomPrimitiveDataFloat (Variables|Default|GetConnectionMesh) 0 (Math|Conversions|ToFloat(Boolean) (Class|PXTrailPaintDot|HasStatus "NextUnavailable")))
      (Rendering|Material|SetCustomPrimitiveDataFloat (Variables|Default|GetPinMesh) 0 (Math|Conversions|ToFloat(Boolean) (Class|PXTrailPaintDot|HasStatus "Unavailable"))))))

(event EventUpdateMousePos
  (params (worldMousePos :type Vector :default "0, 0, 0"))
  (if (and (Class|PXTrailPaintDot|HasStatus "Pin") (not (Utilities|IsValid (Variables|Default|GetConnectedDot))))
    (CallFunction|Connectto worldMousePos)))

(event EventSetAnimationTime
  (params (time :type Float%20%28single-precision%29) (fade :type Float%20%28single-precision%29))
  (Utilities|FlowControl|Sequence
    (:then_0
      (Rendering|Material|SetCustomPrimitiveDataFloat (Variables|Default|GetDotMesh) 0 (|(offset+((1-offset)*alpha)) (* (Math|Float|MakeLiteralFloat 0.5) (Math|Conversions|ToFloat(Boolean) (Class|PXTrailPaintDot|HasStatus "Connectable"))) time))
      (Rendering|Material|SetCustomPrimitiveDataFloat (Variables|Default|GetTorusMesh) 0 time)
      (Transformation|SetRelativeLocation (Variables|Default|GetEmptyPinMesh) (Math|Vector|MakeVector 0.0 0.0 (* (Variables|/Script/Frostpunk2.PXTrailConfig|GetMouseHeight (Class|PXGameplayUtils|GetTrailConfig)) (Math|Float|Lerp (Math|Float|MakeLiteralFloat 0.75) (Math|Curves|GetFloatValue (Variables|Default|GetPointOfInterestHeight) time) (Math|Conversions|ToFloat(Boolean) (or (Class|PXTrailPaintDot|HasStatus "Neighbour") (and (Class|PXTrailPaintDot|HasStatus "PointOfInterest") (Class|PXTrailPaintDot|HasStatus "Connectable"))))))) false false))
    (:then_1
      (Rendering|Material|SetCustomPrimitiveDataFloat (Variables|Default|GetDotMesh) 1 (Math|Curves|GetFloatValue (Variables|Default|GetFadeOpacity) fade))
      (Rendering|Material|SetCustomPrimitiveDataFloat (Variables|Default|GetDotMesh) 2 (Math|Float|Lerp (Math|Curves|GetFloatValue (Variables|Default|GetFadeOutHeight) fade) (Math|Curves|GetFloatValue (Variables|Default|GetFadeInHeight) fade) (Math|Conversions|ToFloat(Boolean) (Class|PXTrailPaintDot|HasStatus "Neighbour")))))))

(fn ConstructionScript)

(fn Connectto
  (params (InputPin :type Vector))
  (bind _connectiontransform (Variables|Default|GetConnectionTransform))
  (bind _relativescale3d (Variables|/Script/Engine.SceneComponent|GetRelativeScale3D _connectiontransform))
  (Transformation|SetRelativeRotation (Variables|Default|GetConnectionTransform) (Math|Conversions|RotationFromXVector (- InputPin (Transformation|GetWorldLocation (Variables|Default|GetPinMesh)))) false false)
  (Transformation|SetRelativeScale3D (Variables|Default|GetConnectionTransform) (Math|Vector|MakeVector (Math|Vector|Distance(Vector) (Transformation|GetWorldLocation (Variables|Default|GetPinMesh)) InputPin) (.y _relativescale3d) (.z _relativescale3d))))

(fn UpdateSelectionState
  (Rendering|Material|SetMaterial (Variables|Default|GetDecalPlane) 0 (select (Math|Boolean|ANDBoolean (Class|PXTrailPaintDot|HasStatus "Connectable") (Class|PXTrailPaintDot|IsSelected) (not (Class|PXTrailPaintDot|HasStatus "Pin"))) "/Game/Scenarios/Shared/Materials/Trails/TrailPainting/MI_POI_Decal_Selected.MI_POI_Decal_Selected" (select (Class|PXTrailPaintDot|HasStatus "Connectable") "/Game/Scenarios/Shared/Materials/Trails/TrailPainting/MI_POI_Decal.MI_POI_Decal" "/Game/Scenarios/Shared/Materials/Trails/TrailPainting/MI_POI_Decal_Disabled.MI_POI_Decal_Disabled"))))