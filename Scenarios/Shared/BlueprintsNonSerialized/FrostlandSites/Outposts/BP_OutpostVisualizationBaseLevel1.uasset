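; Level 1 base Blueprint for outpost visualization on Frostland sites.
; It calls UpdateOutpost, which is defined outside this file, when the actor starts and when the outpost is constructed, after running the parent handler in each case.
; Site activity changes, site state changes and the construction script only forward to the parent class.
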(event `self.ReceiveActorStarted`
  (`parent.ReceiveActorStarted`)
  (`self.UpdateOutpost`))

(event `self.OnSiteActivityChanged`
  (params (isActive :type Boolean))
  (`parent.OnSiteActivityChanged` isActive))

(event `self.OnSiteStateChanged`
  (params (state :type "EPXSiteState Enum" :default "Hidden"))
  (`parent.OnSiteStateChanged` state))

(event `self.OnOutpostConstructed`
  (`parent.OnOutpostConstructed`)
  (`self.UpdateOutpost`))

(fn `UserConstructionScript`
  (`parent.UserConstructionScript`))