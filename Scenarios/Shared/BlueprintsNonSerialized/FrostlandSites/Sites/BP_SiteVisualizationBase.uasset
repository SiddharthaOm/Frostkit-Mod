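; Base Blueprint for a Frostland site visualization that shows or hides the site's map pin.
; On actor start and on each site state change, it reads the site state component for the player's nation and the visualized site.
; The pin transform and its children are visible only while that state is Operational.
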(event `self.ReceiveActorStarted`
  (`self.UpdatePin`))

(event `self.OnSiteStateChanged`
  (params (state :type "EPXSiteState Enum" :default "Hidden"))
  (`self.UpdatePin`))

(fn `UpdatePin`
  (`SceneComponent.SetVisibility` (`self.PinTransform`) (`|EnumEquality` (`PXSiteStateComponent.State` (`PXSiteUtils.GetSiteStateComponent` (`PXNationUtils.GetPlayerNation`) (`PXSiteVisualizationComponent.Site` (`self.SiteVisualization`)))) "Operational") true))

(fn `UserConstructionScript`)