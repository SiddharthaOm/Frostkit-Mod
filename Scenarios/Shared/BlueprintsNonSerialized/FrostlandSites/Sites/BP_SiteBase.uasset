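; Base Blueprint for Frostland site actors that keeps each site's UI tracker pin in sync with its state.
; On actor start and on every state change, UpdateTracker creates or re-initializes the pin for Visible, Operational and Finished sites, and removes it when Hidden.
; The pin class comes from the site type's input-device-specific override, falling back to the site config's base pin class.
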(event `self.ReceiveActorStarted`
  (`self.UpdateTracker` (`PXSiteStateComponent.State` (`PXSiteUtils.GetSiteStateComponent` (`PXNationUtils.GetPlayerNation`) (`self.Site`)))))

(event `self.OnSiteStateChanged`
  (params (state :type "EPXSiteState Enum" :default "Hidden"))
  (`self.UpdateTracker` state))

(fn `UpdateTracker`
  (params (SiteState :type "EPXSiteState Enum" :default "Hidden"))
  (bind _returnvalue (`PXSiteType.GetCustomSiteTrackerForInputDevice` (`PXSiteComponent.SiteType` (`self.GetComponentByClass` "/Script/Frostpunk2.PXSiteComponent"))))
  (`/Engine/EditorBlueprintResources/StandardMacros.IsValid` (`self.Frostland Tracker Panel`)
    (:`Is Valid`
      (switch `EPXSiteState` (`local.SiteState`)
        (:`Hidden`
          (`PXTrackerUtils.RemoveTracker` (`self.Frostland Tracker Panel`))
          (set `self.Frostland Tracker Panel` null))
        (:`Visible`
          (`PXFrostlandTrackerPanel.InitializeSiteTracker` (stale _output_get) (`self.GetComponentByClass` "/Script/Frostpunk2.PXSiteComponent") :!label _label))
        (:`Operational`
          (goto _label))
        (:`Finished`
          (goto _label))))
    (:`Is Not Valid`
      (switch `EPXSiteState` (`local.SiteState`)
        (:`Visible`
          _)
        (:`Operational`
          _)
        (:`Finished`
          _))
      (bind _returnvalue_2 (`PXTrackerUtils.AddTrackerToActor` (select `bool` (`KismetSystemLibrary.IsValidClass` _returnvalue) :`false` (`PXSiteConfig.BaseFrostlandPinClass` (`PXGameplayUtils.GetSiteConfig`)) :`true` _returnvalue :!type "PXTrackerPanel Class Reference") self "TrackerLayer_InactiveFrostlandTrackers" -1 true "/Game/UI/UiWidgets/CommonWidgets/Trackers/WBP_DefaultTrackerRootPanel.WBP_DefaultTrackerRootPanel_C"))
      (bind _aspxfrostland_tracker_panel (cast `PXFrostlandTrackerPanel` _returnvalue_2))
      (bind _output_get (set `self.Frostland Tracker Panel` _aspxfrostland_tracker_panel))
      (goto _label))))

(fn `UserConstructionScript`)