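; Requirement that passes when no extremes opposing the context community's core affinities are active for the player.
; An active faction-war peace-path block unlock on the player nation passes it outright.
; Otherwise, a valid prepare quest selects the peace-specific opposite-extremes query, else it checks the player's extremes against the opposite affinities.
; The description repeats that branch without the unlock check, listing offending affinities in the not-met text.
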(fn `GetDescription`
  (params (context :type "PXGameContext Structure (by ref)"))
  (returns (ReturnValue :type Text))
  (bind _community (`PXGameplayContextUtils.TryGetCommunityComponentFromGameContext` context))
  (`/Engine/EditorBlueprintResources/StandardMacros.IsValid` (`/Game/Scenarios/Shared/BlueprintsNonSerialized/FactionEmergence/BPFL_FactionWarUtils.Get Prepare Quest`)
    (:`Is Valid`
      (bind _bad_things_names1 (`/Game/Scenarios/Shared/BlueprintsNonSerialized/FactionEmergence/BPFL_FactionWarUtils.Peace - Opposite Extremes for Community Active?` _community))
      (if (`KismetArrayLibrary.Array_IsNotEmpty` _bad_things_names1)
        (return (`|FormatText` (`self.Not Met Text Format`) (`/Game/Scenarios/Shared/BlueprintsNonSerialized/SocietyUtils/BPFL_Quest_Utils.Combine Text Array Into Single` _bad_things_names1)))))
    (:`Is Not Valid`
      (bind _opposites1 (`/Game/Scenarios/Shared/BlueprintsNonSerialized/FactionEmergence/BPFL_FactionEmergenceUtils.Get Opposite Affinity Array` (`PXCommunityUtils.GetCommunityCoreAffinities` _community)))
      (bind (_returnvalue _extreme_affinities _names1) (`/Game/Scenarios/Shared/BlueprintsNonSerialized/FactionEmergence/BPFL_FactionWarUtils.Player Is Extreme on Any Of Affinities` _opposites1))
      (if _returnvalue
        (return (`|FormatText` (`self.Not Met Text Format`) (`/Game/Scenarios/Shared/BlueprintsNonSerialized/SocietyUtils/BPFL_Quest_Utils.Combine Text Array Into Single` _names1)))))))

(fn `IsConditionFulfilled`
  (params (context :type "PXGameContext Structure (by ref)"))
  (returns (ReturnValue :type Boolean))
  (bind _community (`PXGameplayContextUtils.TryGetCommunityComponentFromGameContext` context))
  (if (`PXUnlockUtils.IsUnlockActive` (`PXNationUtils.GetPlayerNation`) "/Game/Scenarios/Shared/Configs/Unlocks/FactionWarEndings/DA_FactionWar_PeacePath_PolicyBuilding_Block_Unlock.DA_FactionWar_PeacePath_PolicyBuilding_Block_Unlock")
    (return true)
    (else
      (`/Engine/EditorBlueprintResources/StandardMacros.IsValid` (`/Game/Scenarios/Shared/BlueprintsNonSerialized/FactionEmergence/BPFL_FactionWarUtils.Get Prepare Quest`)
        (:`Is Valid`
          (bind _bad_things_names1 (`/Game/Scenarios/Shared/BlueprintsNonSerialized/FactionEmergence/BPFL_FactionWarUtils.Peace - Opposite Extremes for Community Active?` _community))
          (return (`KismetArrayLibrary.Array_IsEmpty` _bad_things_names1)))
        (:`Is Not Valid`
          (bind _opposites1 (`/Game/Scenarios/Shared/BlueprintsNonSerialized/FactionEmergence/BPFL_FactionEmergenceUtils.Get Opposite Affinity Array` (`PXCommunityUtils.GetCommunityCoreAffinities` _community)))
          (bind _returnvalue (`/Game/Scenarios/Shared/BlueprintsNonSerialized/FactionEmergence/BPFL_FactionWarUtils.Player Is Extreme on Any Of Affinities` _opposites1))
          (return (not _returnvalue)))))))