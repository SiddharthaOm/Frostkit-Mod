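; Scenario requirement Blueprint that checks whether the player can afford to clean up asbestos.
; A shared AsbestosCost function derives the cost from the housing district count via a base cost and percentage multiplier, then compares it to the main city's resource stockpile.
; IsConditionFulfilled returns that comparison and caches the cost in AsbestosCleanupCost, while GetDescription shows the cost as required prefabs.
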(fn `Asbestos Cost`
  (returns (ReturnValue :type Boolean) (ReturnValue2 :type "Float (double-precision)"))
  (bind _returnvalue (`/Game/Scenarios/Shared/BlueprintsNonSerialized/SocietyUtils/BPFL_StoryArc_Utils.Get Cost based on housing districts amount` (`self.Housing Fresh cost`) (`self.Part of the cost multiplier`)))
  (return (>= (`PXStockpileUtils.GetCityStockpileOfResource` (`PXNationUtils.GetPlayerMainCity`) (`self.Resource`)) _returnvalue) (`KismetMathLibrary.Conv_IntToDouble` _returnvalue)))

(fn `GetDescription`
  (params (context :type "PXGameContext Structure (by ref)"))
  (returns (ReturnValue :type Text))
  (return (`|FormatText` "Requires {X} prefabs to clean up the asbestos" (`.ReturnValue2` (`self.Asbestos Cost`)))))

(fn `IsConditionFulfilled`
  (params (context :type "PXGameContext Structure (by ref)"))
  (returns (ReturnValue :type Boolean))
  (bind (_returnvalue _returnvalue2) (`self.Asbestos Cost`))
  (set `self.Asbestos Cleanup Cost` _returnvalue2)
  (return _returnvalue))