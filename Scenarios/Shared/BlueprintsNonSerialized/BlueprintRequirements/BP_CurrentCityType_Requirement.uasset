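; Blueprint requirement that passes only when the city in the current game context is of the configured CityType.
; It resolves the city from the context's City first, then from a Community's parent city, then from a District's city, and fails if none is found.
; The description text is fixed as "Only possible in The City", regardless of the CityType value.
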(fn `GetDescription`
  (params (context :type "PXGameContext Structure (by ref)"))
  (returns (ReturnValue :type Text))
  (return (`|FormatText` "Only possible in The City")))

(fn `IsConditionFulfilled`
  (params (context :type "PXGameContext Structure (by ref)"))
  (returns (ReturnValue :type Boolean))
  (bind (_city _isvalid) (`PXGameplayContextUtils.TryGetCityFromGameContext` context))
  (bind (_community _isvalid_2) (`PXGameplayContextUtils.TryGetCommunityComponentFromGameContext` context))
  (bind (_district _isvalid_3) (`PXGameplayContextUtils.TryGetDistrictFromGameContext` context))
  (if _isvalid
    (return (== (`|ConvertAsset` (`PXCityComponent.GetType` _city)) (`self.CityType`)))
    (elif _isvalid_2
      (return (== (`|ConvertAsset` (`PXCityComponent.GetType` (`PXCommunityComponent.ParentCity` _community))) (`self.CityType`)))
      (elif _isvalid_3
        (return (== (`|ConvertAsset` (`PXCityComponent.GetType` (`PXDistrictComponent.GetCity` _district))) (`self.CityType`)))
        (else
          (return false))))))