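; Blueprint requirement that passes only when the city in the game context is the resettlement (deportation) colony.
; The condition check resolves the city from the context and compares it to the ResettlementCity held by the resettlement destination owner.
; It fails if the context city, the owner or the resettlement city is invalid.
; The description reads "Must be resettlement colony".
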(fn `GetDescription`
  (params (context :type "PXGameContext Structure (by ref)"))
  (returns (ReturnValue :type Text))
  (return (`|FormatText` "Must be resettlement colony")))

(fn `IsConditionFulfilled`
  (params (context :type "PXGameContext Structure (by ref)"))
  (returns (ReturnValue :type Boolean))
  (bind (_returnvalue _valid _resettlement_city) (`/Game/Scenarios/Shared/BlueprintsNonSerialized/FactionEmergence/BPFL_FactionWarUtils.Get Resettlement Destination Owner`))
  (bind (_city _isvalid) (`PXGameplayContextUtils.TryGetCityFromGameContext` context))
  (if _isvalid
    (if _valid
      (`/Engine/EditorBlueprintResources/StandardMacros.IsValid` _resettlement_city
        (:`Is Valid`
          (return (== _city _resettlement_city)))
        (:`Is Not Valid`
          (return false)))
      (else
        (return false)))
    (else
      (return false))))