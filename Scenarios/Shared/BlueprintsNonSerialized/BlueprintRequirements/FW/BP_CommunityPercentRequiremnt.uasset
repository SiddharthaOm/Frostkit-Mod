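; Blueprint requirement that checks what share of a city's population belongs to a given community type.
; It resolves the city from the context and divides the community's size by the scaled city population, giving a fraction rather than a 0-100 percent.
; That ratio is tested against Value using the selected comparison operator.
; A population of zero or less skips the comparison, avoiding division by zero.
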(fn `IsConditionFulfilled`
  (params (context :type "PXGameContext Structure (by ref)"))
  (returns (ReturnValue :type Boolean))
  (locals (CurrentCommunityPercent :type "Float (double-precision)"))
  (bind _city (`/Game/Scenarios/Shared/BlueprintsNonSerialized/SocietyUtils/BPFL_Communication_Utils.Get Best City from Context` context))
  (bind _returnvalue (`PXCommunityUtils.GetScaledCityPopulationSize` _city))
  (if (not (<= _returnvalue 0))
    (set `local.CurrentCommunityPercent` (/ (`KismetMathLibrary.Conv_IntToDouble` (`PXCommunityUtils.GetCommunitySize` _city (`self.CommunityType`))) (`KismetMathLibrary.Conv_IntToDouble` _returnvalue)))
    (switch `EPXComparisonType` (`self.ComparisonType`)
      (:`LessThan`
        (return (< (`local.CurrentCommunityPercent`) (`self.Value`))))
      (:`LessThanOrEqualTo`
        (return (<= (`local.CurrentCommunityPercent`) (`self.Value`))))
      (:`EqualTo`
        (return (== (`local.CurrentCommunityPercent`) (`self.Value`))))
      (:`GreaterThanOrEqualTo`
        (return (>= (`local.CurrentCommunityPercent`) (`self.Value`))))
      (:`GreaterThan`
        (return (> (`local.CurrentCommunityPercent`) (`self.Value`)))))))