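; Blueprint requirement that is fulfilled only when no embraced Cornerstone matches the affinities of the community in context.
; A shared helper takes the community's core affinities, or their opposites when UseOpposite is set, and collects embraced Cornerstones with a matching affinity.
; When any match, GetDescription names them and explains they make the community an irremovable part of society, with singular or plural wording.
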(fn `Get Embraced Cornerstones for Community`
  (params (context :type "PXGameContext Structure (by ref)"))
  (returns (`Any embraced?` :type Boolean) (`embraced cs1` :type "Array of PXCornerstone Object Reference"))
  (locals (`embraced cs` :type "Array of PXCornerstone Object Reference") (`affinities to check` :type "Array of PXAffinityEntry Structure"))
  (bind _embraced_cs (`local.embraced cs`))
  (bind _returnvalue (`PXCommunityUtils.GetCommunityCoreAffinities` (`PXGameplayContextUtils.TryGetCommunityComponentFromGameContext` context)))
  (bind _opposites1 (`/Game/Scenarios/Shared/BlueprintsNonSerialized/FactionEmergence/BPFL_FactionEmergenceUtils.Get Opposite Affinity Array` _returnvalue))
  (set `local.affinities to check` (select `bool` (`self.Use Opposite?`) :`false` _returnvalue :`true` _opposites1))
  (for _array_element (`/Game/Scenarios/Shared/BlueprintsNonSerialized/SocietyUtils/BPFL_Cornerstone_Utils.Get Embraced Cornerstones`)
    (if (`KismetArrayLibrary.Array_Contains` (`local.affinities to check`) (`PXCornerstone.Affinity` _array_element))
      (`KismetArrayLibrary.Array_AddUnique` (`local.embraced cs`) _array_element)))
  (return (`KismetArrayLibrary.Array_IsNotEmpty` _embraced_cs) _embraced_cs))

(fn `GetDescription`
  (params (context :type "PXGameContext Structure (by ref)"))
  (returns (ReturnValue :type Text))
  (locals (`embraced names` :type "Array of Text") (`embraced cs` :type "Array of PXCornerstone Object Reference"))
  (bind _thing_text (`/Game/Scenarios/Shared/BlueprintsNonSerialized/SocietyUtils/BPFL_Quest_Utils.Combine Text Array Into Single` (`local.embraced names`)))
  (bind (_any_embraced_ _embraced_cs1) (`self.Get Embraced Cornerstones for Community` context))
  (if _any_embraced_
    (bind _output_get (set `local.embraced cs` _embraced_cs1))
    (for _array_element _output_get
      (`KismetArrayLibrary.Array_Add` (`local.embraced names`) (`PXCornerstone.InGameName` _array_element)))
    (return (select `bool` (> (`KismetArrayLibrary.Array_Length` (`local.embraced cs`)) 1) :`false` (`|FormatText` "You have embraced a Cornerstone ({CORNERSTONES}) which they support, making them an irremovable part of your society." _thing_text) :`true` (`|FormatText` "You have embraced Cornerstones ({CORNERSTONES}) which they support, making them an irremovable part of your society." _thing_text)))))

(fn `IsConditionFulfilled`
  (params (context :type "PXGameContext Structure (by ref)"))
  (returns (ReturnValue :type Boolean))
  (locals (`affinities to check` :type "Array of PXAffinityEntry Structure"))
  (bind _any_embraced_ (`self.Get Embraced Cornerstones for Community` context))
  (return (not _any_embraced_)))