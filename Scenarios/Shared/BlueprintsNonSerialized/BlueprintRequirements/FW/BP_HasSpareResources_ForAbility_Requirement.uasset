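; Blueprint requirement that checks whether a city has enough spare capacity of a chosen resource to afford at least one ability from a configured list.
; IsConditionFulfilled resolves the city from the context and passes as soon as any ability's cost in that resource fits; the district it also fetches is unused.
; GetDescription finds the least expensive ability for that resource and reports the missing capacity as "Requires X more Resource".
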(fn `GetDescription`
  (params (context :type "PXGameContext Structure (by ref)"))
  (returns (ReturnValue :type Text))
  (locals (NewLocalVar :type "Array of PXAbility Object Reference"))
  (bind _resource_cost_to_check (`self.Resource Cost to Check`))
  (bind _output_get (set `local.NewLocalVar` (`self.Abilities to check`)))
  (bind _lowest_cost1 (`/Game/Scenarios/Shared/BlueprintsNonSerialized/GameplayActions/BPFL_GameplayAction_Utils.Get Least Expensive Ability` _output_get _resource_cost_to_check))
  (return (`|FormatText` "Requires {AMOUNT} more {RESOURCE}" (`.Missing capacity` (`/Game/Scenarios/Shared/BlueprintsNonSerialized/GameplayActions/BPFL_GameplayAction_Utils.Has Spare Resource Capacity` _resource_cost_to_check (`/Game/Scenarios/Shared/BlueprintsNonSerialized/SocietyUtils/BPFL_Communication_Utils.Get Best City from Context` context) _lowest_cost1)) (`PXResource.IngameName` _resource_cost_to_check))))

(fn `IsConditionFulfilled`
  (params (context :type "PXGameContext Structure (by ref)"))
  (returns (ReturnValue :type Boolean))
  (locals (dist :type "PXDistrictComponent Object Reference"))
  (set `local.dist` (`/Game/Scenarios/Shared/BlueprintsNonSerialized/SocietyUtils/BPFL_Communication_Utils.Get Best District from Context` context))
  (for _array_element (`self.Abilities to check`)
    (if (`/Game/Scenarios/Shared/BlueprintsNonSerialized/GameplayActions/BPFL_GameplayAction_Utils.Has Spare Resource Capacity` (`self.Resource Cost to Check`) (`/Game/Scenarios/Shared/BlueprintsNonSerialized/SocietyUtils/BPFL_Communication_Utils.Get Best City from Context` (`local.context`)) (`BlueprintMapLibrary.Map_Find` (`PXAbility.ResourcesCost` _array_element) (`self.Resource Cost to Check`)))
      (return true)))
  (return false))