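; Zoom story requirement that checks whether the current city area is in a high or low tension state.
; It looks up actor state entries on the area's owner and ORs the results together.
; The HighTension flag selects whether that result is returned directly or inverted, so one Blueprint covers both cases.
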(fn `IsConditionFulfilled`
  (params (context :type "PXGameContext Structure (by ref)"))
  (returns (ReturnValue :type Boolean))
  (locals (Condition :type Boolean :default false) (Owner :type "Actor Object Reference"))
  (set `local.Owner` (`ActorComponent.GetOwner` (`PXSelectionUtils.GetCurrentCityArea`)))
  (if true
    (bind _returnvalue (`PXStateUtils.GetActorStateByEntry` (`local.Owner`) (struct :`StateGuid` "BED5067B481B4978712C78B93BF8B621")))
    (bind _returnvalue_2 (or _returnvalue _returnvalue))
    (return (select `bool` (`self.HighTension`) :`false` (not _returnvalue_2) :`true` _returnvalue_2))
    (else
      (return false))))