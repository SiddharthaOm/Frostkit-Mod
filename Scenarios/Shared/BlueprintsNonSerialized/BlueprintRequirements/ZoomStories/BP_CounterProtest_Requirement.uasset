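; Scenario requirement for the CounterProtest zoom story that tests an actor state tied to the district in the game context.
; It resolves the district from the context, reads the state of its owning actor through GetActorStateByEntry, and fails if no valid district is found.
; An Opposite flag inverts the state result, but not the missing-district failure.
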(fn `ChooseOpposite`
  (params (A :type Boolean))
  (returns (ReturnValue :type Boolean))
  (return (select `bool` (`self.Opposite`) :`false` A :`true` (not A))))

(fn `IsConditionFulfilled`
  (params (context :type "PXGameContext Structure (by ref)"))
  (returns (ReturnValue :type Boolean))
  (bind (_district _isvalid) (`PXGameplayContextUtils.TryGetDistrictFromGameContext` context))
  (if _isvalid
    (bind _returnvalue (`PXStateUtils.GetActorStateByEntry` (`ActorComponent.GetOwner` _district) (struct :`StateGuid` "A92FDE9546B80B704E054191A30CB69E")))
    (return (`self.ChooseOpposite` _returnvalue))
    (else
      (return false))))