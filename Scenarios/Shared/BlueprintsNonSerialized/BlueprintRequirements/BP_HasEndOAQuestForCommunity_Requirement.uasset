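; Blueprint requirement that is met when a community has a UI-visible promise quest to negotiate the end of an ongoing action.
; It takes the community from the game context, falling back to the community behind the context district's ongoing action.
; It then scans that community type's promises for the quest.
; The description text switches to a failed-promise message while any post-silent variant of the quest is active.
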(fn `GetDescription`
  (params (context :type "PXGameContext Structure (by ref)"))
  (returns (ReturnValue :type Text))
  (return (select `bool` (`PXQuestUtils.IsAnyQuestOfTypeActive` "/Game/Scenarios/Shared/BlueprintsSerialized/Quests/Demands/BP_NegotiateEndOngoingAction_PostSilent_Quest.BP_NegotiateEndOngoingAction_PostSilent_Quest_C") :`false` (`|FormatText` "No outstanding promise quest for this community") :`true` (`|FormatText` "Already negotiated with them and failed to carry out your promise"))))

(fn `IsConditionFulfilled`
  (params (context :type "PXGameContext Structure (by ref)"))
  (returns (ReturnValue :type Boolean))
  (locals (Community :type "PXCommunityComponent Object Reference"))
  (bind (_community _isvalid) (`PXGameplayContextUtils.TryGetCommunityComponentFromGameContext` context))
  (bind (_district _isvalid_2) (`PXGameplayContextUtils.TryGetDistrictFromGameContext` context))
  (if _isvalid
    (set `local.Community` _community)
    (bind _returnvalue (`PXDesireUtils.GetCommunityPromises` (`PXCommunityComponent.GetCommunityType` (`local.Community`)) :!label _label))
    (for _array_element _returnvalue
      (bind _asbp_negotiate_end_ongoing_action_quest (cast `/Game/Scenarios/Shared/BlueprintsSerialized/Quests/Demands/BP_NegotiateEndOngoingAction_Quest` _array_element))
      (if (`PXQuest.VisibleOnUI` _asbp_negotiate_end_ongoing_action_quest)
        (return true)))
    (return false)
    (elif _isvalid_2
      (bind (_hasongoingaction _returnvalue_2) (`PXOngoingActionUtils.GetOngoingActionComponentForDistrict` _district))
      (if _hasongoingaction
        (set `local.Community` (`PXOngoingActionComponent.GetCommunity` _returnvalue_2))
        (goto _label)))))