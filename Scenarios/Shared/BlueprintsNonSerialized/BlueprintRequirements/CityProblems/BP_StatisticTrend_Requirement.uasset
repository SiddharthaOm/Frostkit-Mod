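; A city-problem requirement that checks whether a chosen city statistic is trending up or down.
; It resolves the city from the game context, then compares that statistic's target value with its current value.
; The Increasing flag sets the direction: the condition holds when the target is strictly above the current value if set, or strictly below it otherwise.
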(fn `IsConditionFulfilled`
  (params (context :type "PXGameContext Structure (by ref)"))
  (returns (ReturnValue :type Boolean))
  (locals (City :type "PXCityComponent Object Reference"))
  (bind (_city _isvalid) (`PXGameplayContextUtils.TryGetCityFromGameContext` context))
  (if _isvalid
    (set `local.City` _city)
    (if (`self.Increasing`)
      (return (> (`/Game/Scenarios/Shared/BlueprintsNonSerialized/Cities/BPFL_CityUtils.GetTargetStatisticValue` (`local.City`) (`self.Statistic`)) (`/Game/Scenarios/Shared/BlueprintsNonSerialized/Cities/BPFL_CityUtils.GetCurrentStatisticValue` (`local.City`) (`self.Statistic`))))
      (else
        (return (> (`/Game/Scenarios/Shared/BlueprintsNonSerialized/Cities/BPFL_CityUtils.GetCurrentStatisticValue` (`local.City`) (`self.Statistic`)) (`/Game/Scenarios/Shared/BlueprintsNonSerialized/Cities/BPFL_CityUtils.GetTargetStatisticValue` (`local.City`) (`self.Statistic`))))))))