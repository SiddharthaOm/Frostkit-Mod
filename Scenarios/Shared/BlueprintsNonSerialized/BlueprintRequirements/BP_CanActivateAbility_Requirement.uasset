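; A Blueprint requirement that is fulfilled when a given Ability is available to a city or district actor.
; The CityAbility flag picks whether that actor is the owner of a city or of the best district from the context; an invalid lookup fails.
; PerformCheck takes the pass result from the availability check but builds failure reasons from the unlock and affordability checks.
; GetDescription formats those reasons into an "Unavailable because" text, adding leading dashes for multiple reasons.
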(fn `GetDescription`
  (params (context :type "PXGameContext Structure (by ref)"))
  (returns (ReturnValue :type Text))
  (bind (_returnvalue_passed _return_value_failed_reasons) (`self.Perform Check` context))
  (bind _returnvalue (`PXTextUtils.JoinTexts` _return_value_failed_reasons " \n<negative>-</>"))
  (return (`|FormatText` "{MAIN} \n \nUnavailable because: \n<negative>{REQUIREMENTS}</> \n" (`|FormatText` "{ABILITY} cannot be activated" (`PXAbility.IngameName` (`self.Ability`))) (`KismetMathLibrary.SelectText` (`|FormatText` "<negative>-</>{FailedReasons}" _returnvalue) _returnvalue (> (`KismetArrayLibrary.Array_Length` _return_value_failed_reasons) 1)))))

(fn `IsConditionFulfilled`
  (params (context :type "PXGameContext Structure (by ref)"))
  (returns (ReturnValue :type Boolean))
  (locals (owner :type "Actor Object Reference"))
  (bind _returnvalue_passed (`self.Perform Check` context))
  (return _returnvalue_passed))

(fn `Perform Check`
  (params (context :type "PXGameContext Structure (by ref)"))
  (returns (ReturnValue_Passed :type Boolean) (`Return Value Failed Reasons` :type "Array of Text") (`Return Value Passed Reasons` :type "Array of Text"))
  (locals (owner :type "Actor Object Reference") (`failed reasons out` :type "Array of Text"))
  (bind _district (`/Game/Scenarios/Shared/BlueprintsNonSerialized/SocietyUtils/BPFL_Communication_Utils.Get Best District from Context` context))
  (bind _ability (`self.Ability`))
  (bind _owner (`local.owner`))
  (bind _city1 (`/Game/Scenarios/Shared/BlueprintsNonSerialized/SocietyUtils/BPFL_Communication_Utils.Return Valid City or Choose Best` (`PXGameplayContextUtils.TryGetCityFromGameContext` context)))
  (bind (_returnvalue_passed _returnvalue_failedreasons _returnvalue_passedreasons) (break `PXCheckResult` (`PXAbilityUtils.IsActorAbilityAvailable` _owner _ability)))
  (bind (_returnvalue_passed_2 _returnvalue_failedreasons_2) (break `PXCheckResult` (`PXAbilityUtils.CanAffordActorAbility` _owner _ability)))
  (bind (_returnvalue_passed_3 _returnvalue_failedreasons_3) (break `PXCheckResult` (`PXAbilityUtils.HasActorUnlockedAbility` _owner _ability)))
  (if (`self.City Ability?`)
    (`/Engine/EditorBlueprintResources/StandardMacros.IsValid` _city1
      (:`Is Valid`
        (set `local.owner` (`ActorComponent.GetOwner` _city1)))
      (:`Is Not Valid`
        (return false)))
    (elif (`KismetSystemLibrary.IsValid` _district)
      (set `local.owner` (`ActorComponent.GetOwner` _district))
      (else
        (return false))))
  (set `local.failed reasons out` (`/Game/UI/Utilities/BPFL_UI.ClearTextsArrayFromBlankOnPurpose` _returnvalue_failedreasons_3))
  (`KismetArrayLibrary.Array_Append` (`local.failed reasons out`) (`/Game/UI/Utilities/BPFL_UI.ClearTextsArrayFromBlankOnPurpose` _returnvalue_failedreasons_2))
  (return _returnvalue_passed (`local.failed reasons out`) _returnvalue_passedreasons))