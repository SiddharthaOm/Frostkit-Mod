(fn `Get Additional Demand to Use`
  (params (City1 :type "PXCityComponent Object Reference") (context1 :type "PXGameContext Structure"))
  (returns (ReturnValue :type Integer))
  (locals (`size to use` :type Integer :default 0) (City :type "PXCityComponent Object Reference") (context :type "PXGameContext Structure (by ref)"))
  (bind (_community _found) (`/Game/Scenarios/Shared/BlueprintsNonSerialized/SocietyUtils/BPFL_Communication_Utils.Get Best Community from Context` (`local.context`)))
  (set `local.City` City1)
  (set `local.context` context1)
  (if (`self.Use All Communities?`)
    (set `local.size to use` (select `bool` (`self.Only Factions?`) :`false` (`PXCommunityUtils.GetScaledCityPopulationSize` (`local.City`)) :`true` (`/Game/Scenarios/Shared/BlueprintsNonSerialized/FactionEmergence/BPFL_FactionWarUtils.Get combined faction size`)))
    (return (`KismetMathLibrary.FTrunc` (* (`self.Get Multiplier` (`local.City`)) (`local.size to use`))))
    (elif _found
      (set `local.size to use` (`PXCommunityComponent.GetCommunitySize` _community))
      (return (`KismetMathLibrary.FTrunc` (* (`self.Get Multiplier` (`local.City`)) (`local.size to use`)))))))

(fn `Get Multiplier`
  (params (self2 :type "ActorComponent Object Reference"))
  (returns (ReturnValue :type "Float (double-precision)"))
  (locals (`multiplier to use` :type "Float (double-precision)" :default 0.0))
  (if (`self.Change if Ability is Active?`)
    (`/Engine/EditorBlueprintResources/StandardMacros.IsValid` (`self.Ability`)
      (:`Is Valid`
        (if (`PXAbilityUtils.IsActorAbilityActive` (`ActorComponent.GetOwner` self2) (`self.Ability`))
          (set `local.multiplier to use` (`self.Additional Demand x SizePoints Multiplier if Active`))
          (else
            (set `local.multiplier to use` (`self.Additional Demand x SizePoints Multiplier`) :!label _label))))
      (:`Is Not Valid`
        (goto _label)))
    (else
      (goto _label)))
  (return (`local.multiplier to use`)))

(fn `GetDescription`
  (params (context :type "PXGameContext Structure (by ref)"))
  (returns (ReturnValue :type Text))
  (bind _city (`/Game/Scenarios/Shared/BlueprintsNonSerialized/SocietyUtils/BPFL_Communication_Utils.Get Best City from Context` context))
  (bind _resource (`self.Resource`))
  (bind _city1 (`/Game/Scenarios/Shared/BlueprintsNonSerialized/SocietyUtils/BPFL_Communication_Utils.Return Valid City or Choose Best` _city))
  (return (`|FormatText` "Requires {AMOUNT} {RESOURCE}" (`KismetMathLibrary.Abs_Int` (- (`self.Get Additional Demand to Use` _city context) (- (`PXEconomyUtils.GetSupplyOfResource` _city1 _resource) (`PXEconomyUtils.GetDemandOfResource` _city1 _resource)))) (`PXResource.IngameName` (`self.Resource`)))))

(fn `IsConditionFulfilled`
  (params (context :type "PXGameContext Structure (by ref)"))
  (returns (ReturnValue :type Boolean))
  (locals (City :type "PXCityComponent Object Reference") (district :type "PXDistrictComponent Object Reference") (`additional demand to use` :type Integer :default 0))
  (bind (_city _isvalid) (`PXGameplayContextUtils.TryGetCityFromGameContext` context))
  (bind (_district _isvalid_2) (`PXGameplayContextUtils.TryGetDistrictFromGameContext` context))
  (bind (_community _isvalid_3) (`PXGameplayContextUtils.TryGetCommunityComponentFromGameContext` context))
  (bind _resource (`self.Resource`))
  (bind _district_2 (`local.district`))
  (bind _city1 (`/Game/Scenarios/Shared/BlueprintsNonSerialized/SocietyUtils/BPFL_Communication_Utils.Return Valid City or Choose Best` (`local.City`)))
  (if _isvalid_2
    (bind _output_get (set `local.district` _district))
    (set `local.City` (`PXDistrictComponent.GetCity` _output_get))
    (if (`self.Change if Ability is Active?`) :!label _label
      (`/Engine/EditorBlueprintResources/StandardMacros.IsValid` (`self.Ability`)
        (:`Is Valid`
          (`/Engine/EditorBlueprintResources/StandardMacros.IsValid` _district_2
            (:`Is Valid`
              (if (`PXAbilityUtils.IsActorAbilityActive` (`ActorComponent.GetOwner` _district_2) (`self.Ability`))
                (set `local.additional demand to use` 0 :!label _label_2)
                (else
                  (if (`PXAbilityUtils.IsActorAbilityActive` (`ActorComponent.GetOwner` (`local.City`)) (`self.Ability`)) :!label _label_3
                    (goto _label_2)
                    (else
                      (set `local.additional demand to use` (`self.Get Additional Demand to Use` (`local.City`) (`local.context`)) :!label _label_4))))))
            (:`Is Not Valid`
              (goto _label_3))))
        (:`Is Not Valid`
          (goto _label_4)))
      (else
        (goto _label_4)))
    (return (>= (- (`PXEconomyUtils.GetSupplyOfResource` _city1 _resource) (`PXEconomyUtils.GetDemandOfResource` _city1 _resource)) (`local.additional demand to use`)))
    (elif _isvalid
      (set `local.City` _city)
      (goto _label)
      (elif _isvalid_3
        (set `local.City` (`PXCommunityComponent.ParentCity` _community))
        (goto _label)))))