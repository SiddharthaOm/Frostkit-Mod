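; Blueprint requirement that checks whether the community in the game context has a policy it desires.
; It passes if a valid policy exists for that community type to put on the agenda.
; It also passes if shared variable storage holds a preferred policy for that community type and neither that policy nor its fallback is active.
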(fn `Has Valid Requested Policy`
  (params (Key :type "PXCommunityType Object Reference (by ref)"))
  (returns (ReturnValue :type Boolean))
  (bind (_value _returnvalue) (`BlueprintMapLibrary.Map_Find` (`/Game/Scenarios/Shared/BlueprintsSerialized/VariableStorage/BP_SharedVariableStorage.Community Preferred Policy` (`/Game/Scenarios/Shared/BlueprintsNonSerialized/SocietyUtils/BPFL_SharedScenariosStorage.Get Shared Variable Storage`)) Key))
  (if _returnvalue
    (return (not (`/Game/Scenarios/Shared/BlueprintsNonSerialized/Policies/BPFL_PolicyUtils.Policy or Fallback is Active` _value)))))

(fn `IsConditionFulfilled`
  (params (context :type "PXGameContext Structure (by ref)"))
  (returns (ReturnValue :type Boolean))
  (bind _returnvalue (`PXCommunityComponent.GetCommunityType` (`PXGameplayContextUtils.TryGetCommunityComponentFromGameContext` context)))
  (bind (_policy_cache1 _has_valid_policy) (`/Game/Scenarios/Shared/BlueprintsNonSerialized/Policies/BPFL_PolicyUtils.Get Community Policy to Put On Agenda` _returnvalue))
  (return (or _has_valid_policy (`self.Has Valid Requested Policy` _returnvalue))))