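; BP_AbsenteesPercent_Requirement is a condition that checks how much of a city's workforce is absent for a given absence type.
; It resolves the city from the game context, then scales the total workforce plus current absentees (excluding non-workforce) by a target percentage, truncated to a whole number.
; The current absence count for that type is compared against this target using a configurable comparison type.
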(fn `IsConditionFulfilled`
  (params (context :type "PXGameContext Structure (by ref)"))
  (returns (ReturnValue :type Boolean))
  (locals (City :type "PXCityComponent Object Reference") (`Target Absence` :type Integer) (CurrentAbsence :type Integer))
  (bind (_city _isvalid) (`PXGameplayContextUtils.TryGetCityFromGameContext` context))
  (bind _city_2 (`local.City`))
  (if _isvalid
    (set `local.City` _city)
    (set `local.Target Absence` (`KismetMathLibrary.FTrunc` (* (`self.Target Percent`) (+ (`PXWorkforceUtils.GetCityTotalWorkforce` _city_2) (`PXAbsenceUtils.GetTotalCurrentWorkforceAbsenceInCityForUI` _city_2)))))
    (set `local.CurrentAbsence` (`PXAbsenceUtils.GetCurrentWorkforceAbsenceInCity` _city_2 (`self.Absence Type`)))
    (return (`PXGameplayUtils.CompareIntegers` (`local.CurrentAbsence`) (`local.Target Absence`) (`self.CheckType`)))))