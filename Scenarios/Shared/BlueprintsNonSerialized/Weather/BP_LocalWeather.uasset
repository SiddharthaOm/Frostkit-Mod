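; Local weather actor that drives cloud visuals for one weather layer from its PXWeatherComponent.
; On weather initialization it caches the layer and sizes the cloud area from mesh bounds.
; Each tick it rotates the cloud fill FX, publishes position, size and yaw to a material parameter collection for volumetric clouds, and writes cursor positions for a proof-of-concept flashlight.
; Render-target mask painting from procedural mesh UVs exists but is disconnected.
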(event `self.ReceiveBeginPlay`)

(event `self.WeatherInitialized`
  (`self.Initialize Variables`)
  (set `self.CloudMaskSize` (* (* (`.SphereRadius` (`KismetSystemLibrary.GetComponentBounds` (`.Mesh` (break `PXWeatherLayer` (`self.Weather`))))) 2.0) 1.1)))

(event `self.ReceiveTick`
  (params (DeltaSeconds :type "Float (single-precision)"))
  (`self.Update Cloud Animation`)
  (`self.Update Flashlight`)
  (`self.Update Volume Cloud`))

(event `self.ReceiveEndPlay`
  (params (EndPlayReason :type "EEndPlayReason Enum" :default "Destroyed"))
  (switch `EEndPlayReason` EndPlayReason))

(fn `ConstructMask`
  (params (InProcMesh :type "ProceduralMeshComponent Object Reference"))
  (returns (RTmask :type "CanvasRenderTarget2D Object Reference"))
  (locals (index :type Integer) (MaskTris :type "Array of CanvasUVTri Structure"))
  (bind _index (`local.index`))
  (bind _returnvalue (* (`self.MaskSize`) (0.75 0.75)))
  (bind _returnvalue_2 (* (`self.MaskSize`) (0.125 0.125)))
  (set `local.index` 0)
  (bind (_vertices _triangles _normals _uvs) (`KismetProceduralMeshLibrary.GetSectionFromProceduralMesh` InProcMesh))
  (while (< _index (`KismetArrayLibrary.Array_Length` _triangles))
    (`KismetArrayLibrary.Array_Add` (`local.MaskTris`) (make `CanvasUVTri` (+ (* (`|GetArrayItem` _uvs (`|GetArrayItem` _triangles _index)) _returnvalue) _returnvalue_2) (0.0 0.0) (struct :`R` 1.0 :`G` 1.0 :`B` 1.0 :`A` 1.0) (+ (* (`|GetArrayItem` _uvs (`|GetArrayItem` _triangles (+ _index 1))) _returnvalue) _returnvalue_2) (0.0 0.0) (struct :`R` 1.0 :`G` 1.0 :`B` 1.0 :`A` 1.0) (+ (* (`|GetArrayItem` _uvs (`|GetArrayItem` _triangles (+ _index 2))) _returnvalue) _returnvalue_2) (0.0 0.0) (struct :`R` 1.0 :`G` 1.0 :`B` 1.0 :`A` 1.0)))
    (set `local.index` (+ (`local.index`) 3)))
  (bind _returnvalue_3 (`CanvasRenderTarget2D.CreateCanvasRenderTarget2D` "/Script/Engine.CanvasRenderTarget2D" 256 256))
  (`KismetRenderingLibrary.ClearRenderTarget2D` _returnvalue_3 (struct))
  (bind (_canvas _size _context) (`KismetRenderingLibrary.BeginDrawCanvasToRenderTarget` _returnvalue_3))
  (`Canvas.K2_DrawTriangle` _canvas "/Engine/EditorLandscapeResources/WhiteSquareTexture.WhiteSquareTexture" (`local.MaskTris`))
  (`KismetRenderingLibrary.EndDrawCanvasToRenderTarget` _context)
  (return _returnvalue_3))

(fn `ContructMaskWithExistsingCRT`
  (params (InProcMesh :type "ProceduralMeshComponent Object Reference") (RTMask :type "CanvasRenderTarget2D Object Reference") (CanalColor :type "LinearColor Structure"))
  (locals (index :type Integer) (MaskTris :type "Array of CanvasUVTri Structure"))
  (bind _index (`local.index`))
  (bind _returnvalue (* (`self.MaskSize`) (0.75 0.75)))
  (bind _returnvalue_2 (* (`self.MaskSize`) (0.125 0.125)))
  (set `local.index` 0)
  (bind (_vertices _triangles _normals _uvs) (`KismetProceduralMeshLibrary.GetSectionFromProceduralMesh` InProcMesh))
  (while (< _index (`KismetArrayLibrary.Array_Length` _triangles))
    (`KismetArrayLibrary.Array_Add` (`local.MaskTris`) (make `CanvasUVTri` (+ (* (`|GetArrayItem` _uvs (`|GetArrayItem` _triangles _index)) _returnvalue) _returnvalue_2) (0.0 0.0) CanalColor (+ (* (`|GetArrayItem` _uvs (`|GetArrayItem` _triangles (+ _index 1))) _returnvalue) _returnvalue_2) (0.0 0.0) CanalColor (+ (* (`|GetArrayItem` _uvs (`|GetArrayItem` _triangles (+ _index 2))) _returnvalue) _returnvalue_2) (0.0 0.0) CanalColor))
    (set `local.index` (+ (`local.index`) 3)))
  (bind (_canvas _size _context) (`KismetRenderingLibrary.BeginDrawCanvasToRenderTarget` RTMask))
  (`Canvas.K2_DrawTriangle` _canvas "/Game/Scenarios/Shared/FXs/Textures/Alphas/T_WindowTest_A.T_WindowTest_A" (`local.MaskTris`))
  (`KismetRenderingLibrary.EndDrawCanvasToRenderTarget` _context)
  (return))

(fn `Initialize Niagara`
  (if (`KismetSystemLibrary.IsValid` (`.Level` (break `PXWeatherLayer` (`self.Weather`))))
    _))

(fn `Initialize Variables`
  (set `self.WeatherLayers` (`self.GetLayers`))
  (set `self.WeatherMeshes` (`self.GetMeshes`))
  (set `self.Weather` (`PXWeatherComponent.GetLayer` (`self.GetComponentByClass` "/Script/Frostpunk2.PXWeatherComponent"))))

(fn `Initialize Weather`
  (bind (_area _size _level _weather _boundingbox _mesh) (break `PXWeatherLayer` (`self.Weather`)))
  (`KismetRenderingLibrary.ClearRenderTarget2D` (`self.CRT_CloudsMask1`) (struct))
  (`KismetRenderingLibrary.ClearRenderTarget2D` (`self.CRT_CloudsMask2`) (struct))
  (set `self.CloudMaskSize` (* (`.SphereRadius` (`KismetSystemLibrary.GetComponentBounds` _mesh)) 2.0))
  ;[1 1 1] added rendering to RT for volume clouds
  (switch `int` (`PXWeatherLevel.Level` _level)
    (:`1`
      (`self.ContructMaskWithExistsingCRT` _mesh (`self.CRT_CloudsMask1`) (struct :`R` 1.0 :`A` 1.0)))
    (:`2`
      (`self.ContructMaskWithExistsingCRT` _mesh (`self.CRT_CloudsMask2`) (struct :`G` 1.0 :`A` 1.0)))))

(fn `Update Cloud Animation`
  (`FXSystemComponent.SetVectorParameter` (`.FXCloudFill` (break `PXWeatherLayer` (`self.Weather`))) "Rotation" (`KismetMathLibrary.Conv_RotatorToVector` (`SceneComponent.K2_GetComponentRotation` (`self.Transform`)))))

(fn `Update Flashlight`
  (bind _returnvalue (`GameplayStatics.GetPlayerController` 0))
  (bind (_locationx _locationy) (`PlayerController.GetMousePosition` _returnvalue))
  (bind (_worldlocation _worlddirection) (`PlayerController.DeprojectMousePositionToWorld` _returnvalue))
  (bind (_t _intersection) (`KismetMathLibrary.LinePlaneIntersection_OriginNormal` _worldlocation (+ _worldlocation (* _worlddirection 1000000000.0)) (0.0 0.0 35362.0) (0.0 0.0 1.0)))
  ;[1 1 1] FlashLight poc
  (if (`PlayerController.bShowMouseCursor` _returnvalue)
    (`GameUserSettings.GetGameUserSettings`)
    (`KismetMaterialLibrary.SetVectorParameterValue` "/Game/Scenarios/Shared/Materials/Weather/MPC_CursorPosition.MPC_CursorPosition" "CursorPos" (make `LinearColor` _locationx _locationy 0.0 1.0))
    (`KismetMaterialLibrary.SetVectorParameterValue` "/Game/Scenarios/Shared/Materials/Weather/MPC_CursorPosition.MPC_CursorPosition" "WorldCursorPos" (make `LinearColor` (.x _intersection) (.y _intersection) (.z _intersection) 1.0))))

(fn `Update Volume Cloud`
  (bind (_returnvalue_roll _returnvalue_pitch _returnvalue_yaw) (`KismetMathLibrary.BreakRotator` (`self.K2_GetActorRotation`)))
  (bind (_returnvalue_x _returnvalue_y) (`KismetMathLibrary.BreakVector` (`self.K2_GetActorLocation`)))
  (bind _cloudmasksize (`self.CloudMaskSize`))
  ;[1 1 1] location of local weather for vol cloud
  (`KismetMaterialLibrary.SetVectorParameterValue` "/Game/Scenarios/Shared/Materials/MaterialParameterCollection/MPC_GlobalMaterialParameters.MPC_GlobalMaterialParameters" "LocalWeatherPositionAndSize" (make `LinearColor` _returnvalue_x _returnvalue_y _cloudmasksize _cloudmasksize))
  (`KismetMaterialLibrary.SetScalarParameterValue` "/Game/Scenarios/Shared/Materials/MaterialParameterCollection/MPC_GlobalMaterialParameters.MPC_GlobalMaterialParameters" "LocalWeatherRotationZ" _returnvalue_yaw))

(fn `UserConstructionScript`)