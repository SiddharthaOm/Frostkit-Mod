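; Weather effect actor that keeps a Niagara snow effect on the player camera and triggers a burst when the temperature drops.
; On start it snaps the Snow component to the first player camera manager's root and binds to the temperature subsystem's visual-only level change event.
; Each drop in degrees increments a counter written to the TempChange Niagara variable, whose change signals the spawn burst.
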(event `self.ReceiveActorStarted`
  (bind _returnvalue (`GameplayStatics.GetPlayerCameraManager` 0))
  (set `self.Camera` _returnvalue)
  (`SceneComponent.K2_AttachToComponent` (`self.Snow`) (`Actor.RootComponent` _returnvalue) "None" "SnapToTarget" "SnapToTarget" "KeepWorld" true)
  (add `PXTemperatureSubsystem.TemperatureLevelChangedEvent_VisualOnly` (subsystem `PXTemperatureSubsystem`) (delegate `TemperatureLevelChangedEvent_Event`)))

(event `TemperatureLevelChangedEvent_Event`
  (params (newLevel :type "PXTemperatureLevel Object Reference") (oldLevel :type "PXTemperatureLevel Object Reference"))
  ;[1 1 1] On temperature lowered - niagara Spawn burst
  (if (< (`PXTemperatureLevel.Degrees` newLevel) (`PXTemperatureLevel.Degrees` oldLevel))
    (bind _output_get (set `self.TempInt` (+ (`self.TempInt`) 1)))
    (`NiagaraComponent.SetVariableInt` (`self.Snow`) "TempChange" _output_get)))

(fn `UserConstructionScript`)