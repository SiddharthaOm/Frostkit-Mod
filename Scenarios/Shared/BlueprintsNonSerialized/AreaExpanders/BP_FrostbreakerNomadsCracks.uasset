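; Frostbreaker Nomads cracks decal actor that fades out when its area expander is removed.
; On start it subscribes to the area expander subsystem's removal event, matching the expander through the visual component on its grandparent attach actor.
; A match sets a kill flag, after which Tick lowers a fade value over the fade duration into the decal's dynamic material, holding it while paused.
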(event `self.ReceiveActorStarted`
  (add `PXAreaExpanderSubsystem.AreaExpanderRemoved` (subsystem `PXAreaExpanderSubsystem`) (delegate `AreaExpanderRemoved_Event`)))

(event `AreaExpanderRemoved_Event`
  (params (areaExpaner :type "PXAreaExpanderComponent Object Reference"))
  (if (== areaExpaner (`PXAreaExpanderVisualComponent.GetAreaExpanderComponent` (`self.GetComponentByClass` (`self.GetAttachParentActor` (`self.GetAttachParentActor`)) "/Script/Frostpunk2.PXAreaExpanderVisualComponent")))
    (set `self.Kill` true)))

(event `self.ReceiveTick`
  (params (DeltaSeconds :type "Float (single-precision)"))
  (if (`self.Kill`)
    (`|Subsystem`
      (:`then`
        (if (`PXTimeUtils.IsPaused`)
          (bind _asmaterial_instance_dynamic (cast `MaterialInstanceDynamic` (`DecalComponent.GetDecalMaterial` (`self.Decal`))))
          (`MaterialInstanceDynamic.SetScalarParameterValue` _asmaterial_instance_dynamic (`self.Parameter Name`) (`self.Fade Out Progress Value`))
          (else
            (bind _output_get (set `self.Fade Out Progress Value` (- (`self.Fade Out Progress Value`) (/ DeltaSeconds (`self.Fade Duration`)))))
            (bind _asmaterial_instance_dynamic_2 (cast `MaterialInstanceDynamic` (`DecalComponent.GetDecalMaterial` (`self.Decal`))))
            (`MaterialInstanceDynamic.SetScalarParameterValue` _asmaterial_instance_dynamic_2 (`self.Parameter Name`) _output_get)))))))

(fn `UserConstructionScript`)