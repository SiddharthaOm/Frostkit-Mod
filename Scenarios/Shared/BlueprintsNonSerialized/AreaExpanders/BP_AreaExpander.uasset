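; BP_AreaExpander is the actor for an area expansion tile, linking its expander component to a tracker UI panel.
; On start it plays the tile-select construction sound and attaches a WBP_AreaExpanderTracker panel to itself.
; Once that tracker is initialized, immediately or via its initialization event, it passes its PXAreaExpanderComponent to the panel.
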(event `self.ReceiveActorStarted`
  (`/Game/Scenarios/Shared/BlueprintsNonSerialized/Audio/BPFL_AudioUtils.Post 2d Audio Event` "/Game/Scenarios/Shared/Audio/Events/UI/Construction/ui_construction_expand_area_select_tile.ui_construction_expand_area_select_tile")
  (bind _returnvalue (`PXTrackerUtils.AddTrackerToActor` "/Game/UI/UiWidgets/CommonWidgets/Trackers/WBP_AreaExpanderTracker.WBP_AreaExpanderTracker_C" self "TrackerLayer_World" -1 true null))
  (if (`PXTrackerPanel.IsTrackerInitialized` _returnvalue)
    (`self.OnTrackerInitializedEvent` _returnvalue)
    (else
      (add `PXTrackerPanel.OnTrackerInitializedEvent` _returnvalue (delegate `OnTrackerInitializedEvent`)))))

(event `OnTrackerInitializedEvent`
  (params (trackerPanel :type "PXTrackerPanel Object Reference"))
  (bind _aswbp_area_expander_tracker (cast `/Game/UI/UiWidgets/CommonWidgets/Trackers/WBP_AreaExpanderTracker` trackerPanel))
  (`/Game/UI/UiWidgets/CommonWidgets/Trackers/WBP_AreaExpanderTracker.InitializeAreaExpanderTracker` _aswbp_area_expander_tracker (`self.GetComponentByClass` "/Script/Frostpunk2.PXAreaExpanderComponent")))

(fn `UserConstructionScript`)