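; BP_CityArea is a city area actor that switches its actor states to reflect the main city's statistics and embraced Cornerstones.
; On start it binds to statistic-change and Cornerstone events, refreshing supported statistics on both and activating the Cornerstone's state on the latter.
; While the tension context is active, each statistic's last reached trait threshold selects a state from its state group.
; A newly applied state also triggers a follow-up state update involving a faction-war check.
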(event `self.ReceiveActorStarted`
  (bind _returnvalue (`|Subsystem`)
    (:`then`
      (add `PXStatisticSubsystem.CurrentStatisticChangedEvent` _returnvalue (delegate `OnCurrentStatisticChanged`))
      (bind _returnvalue_2 (`|Subsystem`)
        (:`then`
          (add `PXCornerstoneSubsystem.CornerstoneEmbraced` _returnvalue_2 (delegate `OnCornerstoneEmbaraced`)))))))

(event `OnCornerstoneEmbaraced`
  (params (Cornerstone :type "PXCornerstone Object Reference"))
  (bind _returnvalue (`PXCityAreaComponent.GetMainCity` (`self.FP2City`)))
  (for _array_element (`PXStatisticUtils.GetSupportedStatistics` _returnvalue)
    (`self.UpdateStatisticState` _returnvalue _array_element))
  (`self.UpdateCornerstoneState` (`PXCityAreaComponent.GetMainCity` (`self.FP2City`)) Cornerstone))

(event `OnCurrentStatisticChanged`
  (params (statisticHolder :type "PXStatisticHolderComponent Object Reference"))
  (bind _returnvalue (`PXStatisticUtils.GetCityFromStatisticHolder` statisticHolder))
  (for _array_element (`PXStatisticUtils.GetSupportedStatistics` _returnvalue)
    (`self.UpdateStatisticState` _returnvalue _array_element)))

(fn `UpdateCornerstoneState`
  (params (City :type "PXCityComponent Object Reference") (Cornerstone :type "PXCornerstone Object Reference"))
  (bind _cornerstonestate (`PXCornerstone.CornerstoneState` Cornerstone))
  (if (not (`PXStateUtils.IsStateEntryEmpty` _cornerstonestate))
    (`PXStateUtils.SetActorStateByEntry` self _cornerstonestate)))

(fn `UpdateStatisticState`
  (params (City :type "PXCityComponent Object Reference") (Statistic :type "PXStatistic Object Reference"))
  (locals (CurrentStatLocal :type Integer) (CurrentStateLocal :type Name) (CurrentTrait :type "PXTraitType Object Reference"))
  (bind _returnvalue (`PXStateUtils.GetStateEntryFromGroup` (`PXStatistic.StateGroup` Statistic) (`local.CurrentStateLocal`)))
  (bind _returnvalue_2 (`PXCityAreaComponent.GetMainCity` (`self.FP2City`)))
  (if (`PXContextUtils.IsContextActive` "/Game/Scenarios/Shared/Configs/Contexts/Simple/DA_TensionAvailableContext.DA_TensionAvailableContext")
    (if (== City _returnvalue_2)
      (if (`KismetSystemLibrary.IsValid` Statistic)
        (if (`KismetSystemLibrary.IsValid` (`PXStatistic.StateGroup` Statistic))
          (set `local.CurrentStatLocal` (`/Game/Scenarios/Shared/BlueprintsNonSerialized/Cities/BPFL_CityUtils.GetCurrentStatisticValue` _returnvalue_2 Statistic))
          (for _array_element (`PXStatistic.ResultingTraits` Statistic)
            (bind (_triggeringvalue _traittype) (break `PXTraitAndBorder` _array_element))
            (if (>= (`local.CurrentStatLocal`) _triggeringvalue)
              (set `local.CurrentStateLocal` (`PXTraitType.StateName` _traittype))))
          (bind _returnvalue_3 (`|Subsystem`)
            (:`then`
              (bind _returnvalue_4 (`PXStateSubsystem.GetActorStateByEntry` _returnvalue_3 self _returnvalue))
              (if _returnvalue_4
                _
                (elif (not (`PXStateUtils.IsStateEntryEmpty` _returnvalue))
                  (`PXStateUtils.SetActorStateByEntry` self _returnvalue)
                  (bind _returnvalue_5 (`PXStateUtils.GetActorStateByEntry` self (struct :`StateGuid` "BED5067B481B4978712C78B93BF8B621")))
                  (if _returnvalue_5
                    (if (`/Game/Scenarios/Shared/BlueprintsNonSerialized/OngoingEvents/BPFL_OngoingAction_Utils.Is Any Action of type Ongoing?` "/Game/Scenarios/Shared/Configs/OngoingActions/System_Started/DA_FactionWar.DA_FactionWar")
                      (`PXStateUtils.SetActorStateByEntry` self (struct :`StateGuid` "AB6FBA1B4CB03C33680F8487529AFF73")))
                    (else
                      (`PXStateUtils.SetActorStateByEntry` self (struct :`StateGuid` "AB6FBA1B4CB03C33680F8487529AFF73") false))))))))))))

(fn `UserConstructionScript`)