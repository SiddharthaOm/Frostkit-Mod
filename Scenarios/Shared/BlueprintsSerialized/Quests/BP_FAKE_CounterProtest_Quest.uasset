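; Quest that resolves a counter-protest collapse when finished, as its start event is empty.
; FinishQuest ends the action in a district, waits a collapse-tier duration, then ends the whole action if it spans several districts.
; The end gameplay action scales with the stronger community's severity tier.
; If the opposing faction is weaker, a shared flag makes the first collapse send a members-leave choice message, while later ones shrink that faction with a notification.
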(event `self.ReceiveStartQuest`)

(event `self.ReceiveFinishQuest`
  (params (bSuccess :type Boolean))
  (bind _ongoing_action (`self.Ongoing Action`))
  (bind _non_oa_community (`self.Non OA Community`))
  (bind _returnvalue (`PXOngoingActionComponent.GetCommunity` _ongoing_action))
  (bind _returnvalue_2 (`KismetMathLibrary.FTrunc` (* (`KismetMathLibrary.Conv_IntToDouble` (`self.Size Transfer`)) (`/Game/Scenarios/Shared/BlueprintsNonSerialized/Communities/BPFL_CommunityUtils.Get Membership Population Multiplier` _non_oa_community true))))
  (set `self.OA Community` _returnvalue)
  (set `self.Non OA Community` (`.Faction Component` (`/Game/Scenarios/Shared/BlueprintsNonSerialized/FactionEmergence/BPFL_FactionWarUtils.Get Existing Opposing Faction` (`PXCommunityComponent.GetFaction` _returnvalue))))
  (set `self.Districts in OA` (`KismetArrayLibrary.Array_Length` (`PXOngoingActionComponent.GetDistricts` _ongoing_action)))
  (set `self.Collapse End GA` (`self.Get Collapse End GA`))
  (`PXOngoingActionUtils.EndOngoingActionInDistrict` :`district` (`self.District`) :`gameplayActionOnStart` "/Game/Scenarios/Shared/Configs/GameplayActions/OngoingActionsMessages/DA_CounterProtest_FullCollapse_Start_GA.DA_CounterProtest_FullCollapse_Start_GA" :`gameplayActionOnFinish` (select `bool` (<= (`self.Districts in OA`) 1) :`true` (`self.Collapse End GA`)) :`endType` "/Game/Scenarios/Shared/Configs/OngoingActions/EndTypes/DA_Protest_CounterProtest_EndType.DA_Protest_CounterProtest_EndType")
  (bind _keys (`BlueprintMapLibrary.Map_Keys` (`PXOngoingActionType.CollapseTimeTiers` (`PXOngoingActionComponent.GetActionType` (`self.Ongoing Action`)))))
  (`PXAsyncWaitForDurationPassed.AsyncAction_WaitForDurationPassed` (`|GetArrayItem` _keys)
    (:`Completed`
      (`|ExecutionSequence`
        (:`then_0`
          (if (not (<= (`self.Districts in OA`) 1))
            (`PXOngoingActionUtils.EndOngoingAction` :`ongoingAction` (`self.Ongoing Action`) :`gameplayActionOnFinish` (`self.Collapse End GA`) :`endType` "/Game/Scenarios/Shared/Configs/OngoingActions/EndTypes/DA_Protest_CounterProtest_EndType.DA_Protest_CounterProtest_EndType")
            (set `/Game/Scenarios/Shared/BlueprintsSerialized/VariableStorage/BP_SharedVariableStorage.Guns SNOPS Manual Trigger` true (`/Game/Scenarios/Shared/BlueprintsNonSerialized/SocietyUtils/BPFL_SharedScenariosStorage.Get Shared Variable Storage`))))
        (:`then_1`
          (if (< (`.Severity Level` (`/Game/Scenarios/Shared/BlueprintsNonSerialized/OngoingEvents/BPFL_OngoingAction_Utils.Get Community Strength Tier` (`self.Non OA Community`))) (`.Severity Level` (`/Game/Scenarios/Shared/BlueprintsNonSerialized/OngoingEvents/BPFL_OngoingAction_Utils.Get Community Strength Tier` (`self.OA Community`))))
            (if (`/Game/Scenarios/Shared/BlueprintsSerialized/VariableStorage/BP_SharedVariableStorage.Counter Protesters Left Once` (`/Game/Scenarios/Shared/BlueprintsNonSerialized/SocietyUtils/BPFL_SharedScenariosStorage.Get Shared Variable Storage`))
              (`/Game/Scenarios/Shared/BlueprintsNonSerialized/FactionEmergence/BPFL_FactionEmergenceUtils.Shrink Faction Using All Communities in City` _non_oa_community _returnvalue_2 (`|FormatText` (`self.Format`) (`KismetTextLibrary.Conv_IntToText` _returnvalue_2)) true true)
              (else
                (set `/Game/Scenarios/Shared/BlueprintsSerialized/VariableStorage/BP_SharedVariableStorage.Counter Protesters Left Once` true (`/Game/Scenarios/Shared/BlueprintsNonSerialized/SocietyUtils/BPFL_SharedScenariosStorage.Get Shared Variable Storage`))
                (bind _decision (`/Game/Scenarios/Shared/BlueprintsNonSerialized/SocietyUtils/BPFL_Communication_Utils.Send Config Message` "/Game/Scenarios/Shared/Configs/Messages/Lenses/OngoingActions_RandomEvents/Rally/DA_CounterProtest_MembersLeave_Lens.DA_CounterProtest_MembersLeave_Lens" (`PXOngoingActionComponent.GetAnyDistict` (`self.Ongoing Action`)) (`self.Non OA Community`) null (`|MakeMap` "COUNTER_FACTION" (`PXFactionUtils.GetFactionInGameName` (`self.Non OA Community`))) null null (struct) true))
                (`PXAsyncWaitForAnyChoice.AsyncAction_WaitForAnyChoice` _decision)))))))))

(fn `Get Collapse End GA`
  (returns (ReturnValue :type "PXGameplayAction Object Reference"))
  (bind (_strenght_trait _ingame_name _severity_level) (`/Game/Scenarios/Shared/BlueprintsNonSerialized/OngoingEvents/BPFL_OngoingAction_Utils.Get Community Strength Tier` (`self.OA Community`)))
  (bind (_strenght_trait_2 _ingame_name_2 _severity_level_2) (`/Game/Scenarios/Shared/BlueprintsNonSerialized/OngoingEvents/BPFL_OngoingAction_Utils.Get Community Strength Tier` (`self.Non OA Community`)))
  (bind _returnvalue (select `bool` (> _severity_level _severity_level_2) :`false` _severity_level_2 :`true` _severity_level))
  (return (select `bool` (>= _returnvalue 3) :`false` (select `int` _returnvalue :`0` "/Game/Scenarios/Shared/Configs/GameplayActions/OngoingActionsMessages/DA_CounterProtest_FullCollapse_End_GA.DA_CounterProtest_FullCollapse_End_GA" :`1` "/Game/Scenarios/Shared/Configs/GameplayActions/OngoingActionsMessages/DA_CounterProtest_FullCollapse_End_GA.DA_CounterProtest_FullCollapse_End_GA" :`2` "/Game/Scenarios/Shared/Configs/GameplayActions/OngoingActionsMessages/DA_CounterProtest_FullCollapse_End_Fervour_2_GA.DA_CounterProtest_FullCollapse_End_Fervour_2_GA" :`3` "/Game/Scenarios/Shared/Configs/GameplayActions/OngoingActionsMessages/DA_CounterProtest_FullCollapse_End_Fervour_3_GA.DA_CounterProtest_FullCollapse_End_Fervour_3_GA" :!type "PXGameplayAction Object Reference") :`true` "/Game/Scenarios/Shared/Configs/GameplayActions/OngoingActionsMessages/DA_CounterProtest_FullCollapse_End_Fervour_3_GA.DA_CounterProtest_FullCollapse_End_Fervour_3_GA")))