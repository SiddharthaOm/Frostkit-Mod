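; Endless quest for a promise negotiated with a community to end its ongoing action, typically a protest.
; It listens for ongoing action changes and fails if that community's action finishes without being in the Collapsing state.
; On success it collapses the action, then either starts a radicalisation story arc or raises the opposing faction's Fervour.
; Failure raises the community's own Fervour unless a shared flag blocks it.
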(event `self.ReceiveStartQuest`
  (`self.SetEndlessDuration` self)
  (add `PXOngoingActionSubsystem.OngoingActionChangedEvent` (subsystem `PXOngoingActionSubsystem`) (delegate `On Ongoing Action End`)))

(event `On Ongoing Action End`
  (params (changeType :type "EPXOngoingActionChangeType Enum" :default "Start") (ongoingAction :type "PXOngoingActionComponent Object Reference"))
  (bind (_outfound _returnvalue) (`PXCommunityUtils.GetCommunityOfCommunityType` (`self.GetCommunityType` self)))
  (`/Engine/EditorBlueprintResources/StandardMacros.IsValid` (`self.GetCommunityType` self)
    (:`Is Valid`
      (if (not (`|EnumEquality` (`PXOngoingActionComponent.GetState` ongoingAction) "Collapsing"))
        (if (and (`|EnumEquality` changeType "Finish") (or (== (`PXOngoingActionComponent.GetCommunity` ongoingAction) _returnvalue) (== (`PXOngoingActionComponent.GetSecondaryCommunity` ongoingAction) _returnvalue)))
          (`self.FinishQuest` false))))))

(event `self.ReceiveFinishQuest`
  (params (bSuccess :type Boolean))
  (bind (_outfound _returnvalue) (`PXCommunityUtils.GetCommunityOfCommunityType` (`self.GetCommunityType` self)))
  (bind (_outfound_2 _returnvalue_2) (`PXCommunityUtils.GetCommunityOfCommunityType` (`self.GetCommunityType` self)))
  (bind (_outfound_3 _returnvalue_3) (`PXCommunityUtils.GetCommunityOfCommunityType` (`self.GetCommunityType` self)))
  (`/Game/Scenarios/Main/BlueprintsNonSerialized/ScenarioFunctionLibrary/BPFL_S1_Endlog_Utils.Log Endlog Fact and Date` (`self.Negotiated Protest Endlog`) (`PXCommunityType.IngameName` (`self.GetCommunityType` self)))
  (remove `PXOngoingActionSubsystem.OngoingActionChangedEvent` (subsystem `PXOngoingActionSubsystem`) (delegate `On Ongoing Action End`))
  (if bSuccess
    (bind _hasongoingaction (`PXOngoingActionUtils.GetOngoingActionComponentForCommunity` _returnvalue_3))
    (if _hasongoingaction
      (bind (_hasongoingaction_2 _returnvalue_4) (`PXOngoingActionUtils.GetOngoingActionComponentForCommunity` _returnvalue_2))
      (`PXOngoingActionComponent.SetCollapseAssociatedState` _returnvalue_4 (struct :`StateGuid` "AC13D35B4D14C166CAF5CEB1DAC3D756"))
      (`PXOngoingActionUtils.EndOngoingAction` _returnvalue_4 "/Game/Scenarios/Shared/Configs/GameplayActions/OngoingActionsMessages/DA_NegotiateEndOngoingAction_Start_GA.DA_NegotiateEndOngoingAction_Start_GA" "/Game/Scenarios/Shared/Configs/GameplayActions/OngoingActionsMessages/DA_NegotiateEndOngoingAction_End_GA.DA_NegotiateEndOngoingAction_End_GA" (`|MakeMap` "FACTION" (`PXFactionUtils.GetFactionInGameName` _returnvalue_2)) "Collapse" true (`self.Protest End Type`))
      ;[1 1 1] Radicalize Opposite If Protest
      (set `self.Faction Component` (`.Faction Component` (`/Game/Scenarios/Shared/BlueprintsNonSerialized/FactionEmergence/BPFL_FactionWarUtils.Get Existing Opposing Faction` (`PXCommunityComponent.GetFaction` _returnvalue))))
      (if (`KismetArrayLibrary.Array_IsNotEmpty` (`/Game/Scenarios/Shared/BlueprintsSerialized/VariableStorage/BP_SharedVariableStorage.Radicalisation Negotiation Ghosts` (`/Game/Scenarios/Shared/BlueprintsNonSerialized/SocietyUtils/BPFL_SharedScenariosStorage.Get Shared Variable Storage`)))
        (bind _returnvalue_5 (`|GenericCreateObject` (subsystem `PXStoryArcSubsystem`) "/Game/Scenarios/Shared/BlueprintsSerialized/StoryArcs/Cornerstones/RadicalisationGhosts/Children/BP_RadicalisationGhosts_NegotiatedWithProtesters_SA.BP_RadicalisationGhosts_NegotiatedWithProtesters_SA_C" (`self.Faction Component`)))
        (`PXStoryUtils.StartParameterizedStoryArc` _returnvalue_5)
        (else
          (bind (_hasongoingaction_3 _returnvalue_6) (`PXOngoingActionUtils.GetOngoingActionComponentForCommunity` _returnvalue))
          (if _hasongoingaction_3
            (`PXAsyncWaitForOngoingActionFinished.AsyncAction_WaitForOngoingActionFinished` (`PXOngoingActionComponent.GetActionType` _returnvalue_6)
              (:`Completed`
                _)))
          (`/Game/Scenarios/Shared/BlueprintsNonSerialized/Communities/BPFL_CommunityUtils.DisplayCommunityNotification` (`self.Faction Component`) (`|FormatText` "{FACTION}' Fervour rises due to negotiations with protesters" (`PXFactionUtils.GetFactionInGameName` (`self.Faction Component`))))
          (`PXPredefinedModifierUtils.SetPredefinedModifierActiveManualTarget` (`PXNationUtils.GetPlayerNation`) (`self.Predefined Modifier`) (`ActorComponent.GetOwner` (`self.Faction Component`)) true))))
    (elif (not (`/Game/Scenarios/Shared/BlueprintsSerialized/VariableStorage/BP_SharedVariableStorage.Block Radicalisation From Unfufilled Negotiation` (`/Game/Scenarios/Shared/BlueprintsNonSerialized/SocietyUtils/BPFL_SharedScenariosStorage.Get Shared Variable Storage`)))
      (`self.Add Fervour on Fail` _returnvalue_3))))

(fn `Add Fervour on Fail`
  (params (Community :type "PXCommunityComponent Object Reference"))
  (`PXPredefinedModifierUtils.SetPredefinedModifierActiveManualTarget` (`PXNationUtils.GetPlayerNation`) (`self.Predefined Modifier`) (`ActorComponent.GetOwner` Community) true)
  (`/Game/Scenarios/Shared/BlueprintsNonSerialized/Communities/BPFL_CommunityUtils.DisplayCommunityNotification` Community (`|FormatText` "{FACTION}' Fervour rises due unfulfilled protest promise" (`PXFactionUtils.GetFactionInGameName` Community))))

(fn `Reactivate Buildings in District`
  (params (self2 :type "PXDistrictComponent Object Reference"))
  (for _array_element (`PXDistrictComponent.GetBuildings` self2)
    (bind _returnvalue (`ActorComponent.GetOwner` _array_element))
    (`PXActivityUtils.RemoveDeactivationReason` _returnvalue "/Game/Scenarios/Shared/Configs/Activity/DeactivationTypes/DA_DeactivationReason_Protest.DA_DeactivationReason_Protest")
    (`PXActivityUtils.ActivateLogic` _returnvalue)))