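; BP_PacifyPromise_Quest is a demand quest for a pacify promise tied to a community, an affinity and a choice.
; SetVariables stores those three values for later use.
; When the quest finishes, it runs the parent logic, starts a wait-for-duration async action, passes the result to mild desires outcome handling, and calls PeaceAgreementReached on shared variable storage, with no branch on success.
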(event `self.ReceiveFinishQuest`
  (params (bSuccess :type Boolean))
  (bind _output_get (set `self.Success` bSuccess))
  (`parent.ReceiveFinishQuest` _output_get)
  (`PXAsyncWaitForDurationPassed.AsyncAction_WaitForDurationPassed` (struct :`ScaledTicks` 10)
    (:`Completed`
      (`/Game/Scenarios/Shared/BlueprintsNonSerialized/SocietyUtils/BPFL_Desires_Utils.Handle Mild Desires Quest Outcome` (`self.Success`) (`self.Community`) (`self.affinity`) (`self.Choice`))
      (`/Game/Scenarios/Shared/BlueprintsSerialized/VariableStorage/BP_SharedVariableStorage.PeaceAgreementReached` (`/Game/Scenarios/Shared/BlueprintsNonSerialized/SocietyUtils/BPFL_SharedScenariosStorage.Get Shared Variable Storage`)))))

(fn `Set Variables`
  (params (Community :type "PXCommunityComponent Object Reference") (affinity :type "PXAffinityEntry Structure") (Choice :type Integer))
  (set `self.Community` Community)
  (set `self.affinity` affinity)
  (set `self.Choice` Choice))