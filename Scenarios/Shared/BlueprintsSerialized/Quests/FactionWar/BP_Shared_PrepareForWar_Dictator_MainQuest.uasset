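; Main quest for the Dictator path of preparing for faction war: pass Captain's Authority, secure rule, then contain factions.
; An in-progress unlock starts a countdown objective, restarting its wait if lost, while a parallel timer completes it regardless and unlocks Containment.
; KickoffEliminate, called externally, adds a containment objective tracked through community imprint changes.
; Finishing clears containment ability unlocks and blocks deactivation, deconstruction and actions on aggressor containment districts and buildings.
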(event `self.ReceiveStartQuest`
  (bind _returnvalue (`PXNationUtils.GetPlayerNation`))
  (bind _secure_rule_objective (`self.Secure Rule objective`))
  (`self.Starting Stuff`)
  (`self.Add Captains Authority Objective`)
  (`self.Add Ban Factions Objective`)
  (`|ExecutionSequence`
    (:`then_0`
      (if (not (`/Game/Scenarios/Shared/BlueprintsNonSerialized/Policies/BPFL_PolicyUtils.IsPolicyActive` (`self.Captain's Authority Policy`)))
        (`PXAsyncWaitForUnlock.AsyncAction_WaitForUnlock` "/Game/Scenarios/Shared/Configs/Unlocks/Other/DA_CaptainsBigLensSeen_Unlock.DA_CaptainsBigLensSeen_Unlock" true
          (:`Completed`
            _)))
      (`PXAsyncWaitForDurationPassed.AsyncAction_WaitForDurationPassed` (struct :`ScaledTicks` 10)
        (:`Completed`
          (`PXQuestObjective.ModifyObjectiveName` (`self.Secure Rule objective`) (`self.Get New Ban Factions Name`)))))
    (:`then_1`
      (`PXAsyncWaitForUnlock.AsyncAction_WaitForUnlock` (`self.secure unity in progress Unlock Type`) true :!label _label
        (:`Completed`
          (set `self.wait obj start time` (`PXTimeUtils.GetCurrentGameTime`))
          (`PXQuestObjective.ModifyObjectiveProgress` _secure_rule_objective 0)
          (`PXQuestObjective.ModifyObjectiveName` _secure_rule_objective (`self.Get Wait Objective Name`))
          (set `self.wait obj` (`self.Secure Rule objective`))
          (`|ExecutionSequence`
            (:`then_0`
              ;[1 1 1] Update name with countdown
              (`PXAsyncWaitForDurationPassed.AsyncAction_WaitForDurationPassed` (struct :`ScaledTicks` 10) :!label _label_2
                (:`Completed`
                  (if (not (`PXQuestObjective.IsObjectiveFinished` (`self.wait obj`)))
                    (if (`PXUnlockUtils.IsUnlockActive` (`PXNationUtils.GetPlayerNation`) (`self.secure unity in progress Unlock Type`))
                      (`PXQuestObjective.ModifyObjectiveName` (`self.wait obj`) (`self.Get Wait Objective Name`))
                      (goto _label_2)
                      (else
                        (`PXQuestObjective.ModifyObjectiveName` (`self.wait obj`) (`self.Get New Ban Factions Name`))
                        (`self.Restart Wait for Unity Flow`)))))))
            (:`then_1`
              ;[1 1 1] Just wait for duration, don't care if ability active
              (`PXAsyncWaitForDurationPassed.AsyncAction_WaitForDurationPassed` (`PXAbility.Duration` (`self.Secure Rule Ability`))
                (:`Completed`
                  (`PXQuestUtils.FinishObjective` (`self.wait obj`))
                  (`PXUnlockUtils.SetUnlockActive` _returnvalue (`self.Containment Unlock`) true)
                  (`PXUnlockUtils.SetUnlockActive` _returnvalue (`self.secure unity in progress Unlock Type`)))))))))))

(event `Restart Wait for Unity Flow`
  (goto _label))

(event `Kickoff Eliminate`
  (params (`Factions to eliminate` :type "Array of PXCommunityComponent Object Reference"))
  (set `self.Factions To Eliminate` `Factions to eliminate`)
  (`self.Add Eliminate Objective`))

(event `self.ReceiveFinishQuest`
  (params (bSuccess :type Boolean))
  (bind _returnvalue (`PXNationUtils.GetPlayerNation`))
  (`parent.ReceiveFinishQuest` bSuccess)
  (`PXUnlockUtils.SetUnlockActive` (`PXNationUtils.GetPlayerNation`) (`self.dictator unlock`) true)
  (`PXUnlockUtils.SetUnlockActive` _returnvalue "/Game/Scenarios/Shared/Configs/Unlocks/FactionWarEndings/DA_Dictator_Relocate_Visibility_Unlock.DA_Dictator_Relocate_Visibility_Unlock")
  (`PXUnlockUtils.SetUnlockActive` _returnvalue "/Game/Scenarios/Shared/Configs/Unlocks/FactionWarEndings/DA_Dictator_ContainmentDefenderAbility_Unlock.DA_Dictator_ContainmentDefenderAbility_Unlock")
  (`PXUnlockUtils.SetUnlockActive` _returnvalue "/Game/Scenarios/Shared/Configs/Unlocks/FactionWarEndings/DA_Dictator_ContainmentAggressorAbility_Unlock.DA_Dictator_ContainmentAggressorAbility_Unlock")
  (for _array_element (`PXDistrictUtils.GetDistrictWithTagFromCity` (`PXNationUtils.GetPlayerMainCity`) (struct :`TagDictionary` (struct :`(TagName` "District.Containment.Aggressor") :`(TagName` "District.Containment.Defender")) :`QueryTokenStream` "(0,1,1,2,0,1)" :`AutoDescription` " ANY( District.Containment.Aggressor, District.Containment.Defender )"))
    (bind _returnvalue_2 (`ActorComponent.GetOwner` _array_element))
    (`PXActivityUtils.BlockPlayerDeactivation` _returnvalue_2 "/Game/Scenarios/Shared/Configs/Activity/PlayerDeactivityBlockage/DA_PlotArmourBlockage.DA_PlotArmourBlockage")
    (`PXDeconstructionUtils.BlockDeconstruction` _returnvalue_2 "/Game/Scenarios/Shared/Configs/Deconstructions/Blockages/DA_FactionEnclaveBlockage.DA_FactionEnclaveBlockage")
    ;[1 1 1] Block actions
    (`PXPredefinedModifierUtils.SetPredefinedModifierActiveManualTarget` (`PXNationUtils.GetPlayerNation`) "/Game/Scenarios/Shared/Configs/PredefinedModifiers/FactionWar/DA_Dictator_Containment_Blockage_Modifier.DA_Dictator_Containment_Blockage_Modifier" _returnvalue_2 true)
    (for _array_element_2 (`PXDistrictComponent.GetBuildings` _array_element)
      (bind _returnvalue_3 (`ActorComponent.GetOwner` _array_element_2))
      (`PXActivityUtils.BlockPlayerDeactivation` _returnvalue_3 "/Game/Scenarios/Shared/Configs/Activity/PlayerDeactivityBlockage/DA_PlotArmourBlockage.DA_PlotArmourBlockage")
      (`PXDeconstructionUtils.BlockDeconstruction` _returnvalue_3 "/Game/Scenarios/Shared/Configs/Deconstructions/Blockages/DA_FactionEnclaveBlockage.DA_FactionEnclaveBlockage")
      ;[1 1 1] Block Actions
      (`PXPredefinedModifierUtils.SetPredefinedModifierActiveManualTarget` (`PXNationUtils.GetPlayerNation`) "/Game/Scenarios/Shared/Configs/PredefinedModifiers/FactionWar/DA_Dictator_Containment_Blockage_Modifier.DA_Dictator_Containment_Blockage_Modifier" _returnvalue_3 true))))

(fn `Add Ban Factions Objective`
  (`PXUnlockUtils.SetUnlockActive` (`PXNationUtils.GetPlayerNation`) (`self.Dictator ban factions Unlock`) true)
  (bind _returnvalue (`self.AddQuestObjective` self (`|FormatText` "Unify the City behind its Captain") "" 0 1 false null "DebugObjectiveName"))
  (set `self.Secure Rule objective` _returnvalue))

(fn `Add Ban Single Faction Objectives`
  (for _array_element (`PXFactionUtils.GetMembersFromCity` (`PXNationUtils.GetPlayerMainCity`) null)
    (`PXQuestUtils.AddCommunityActionQuestObjective` null (`|FormatText` "Ban {FACTION} only" (`/Game/Scenarios/Shared/BlueprintsNonSerialized/Communities/BPFL_CommunityUtils.Get Community Name` _array_element)) "" (`self.Ban Faction Action`) null false true null)))

(fn `Add Captains Authority Objective`
  (bind _captain_s_authority_policy (`self.Captain's Authority Policy`))
  (bind _returnvalue (`PXQuestUtils.AddPolicyQuestObjective` (make `PXObjectiveParameters` (`|FormatText` "Pass '{POLICY}'" (`PXPolicyType.IngameName` _captain_s_authority_policy)) "" false 1 null self) (make `PXPolicyObjectiveParameters` _captain_s_authority_policy)))
  (bind _output_get (set `self.captains authority objective` _returnvalue))
  (if (`/Game/Scenarios/Shared/BlueprintsNonSerialized/Policies/BPFL_PolicyUtils.IsPolicyActive` (`self.Captain's Authority Policy`))
    (`PXQuestObjective.ProgressObjective` _output_get 1)))

(fn `Add Eliminate Objective`
  (bind _returnvalue (`self.AddQuestObjective` (`self.Get Eliminate Objective Name`) "" 0 (`KismetArrayLibrary.Array_Length` (`self.Factions To Eliminate`)) false null))
  (set `self.eliminate objective` _returnvalue)
  (add `PXCommunitySubsystem.ImprintsChangedEvent` (subsystem `PXCommunitySubsystem`) (`|CreateDelegate` :!event `Update Eliminate`)))

(fn `Get combined size`
  (returns (ReturnValue :type Integer))
  (for _array_element (`self.Factions To Eliminate`)
    (`/Engine/EditorBlueprintResources/StandardMacros.IsValid` _array_element)))

(fn `Get Eliminate Objective Name`
  (returns (Result :type Text))
  (return (`|FormatText` "Contain {FACTIONS} " (`/Game/Scenarios/Shared/BlueprintsNonSerialized/SocietyUtils/BPFL_Quest_Utils.Combine Text Array Into Single` (`/Game/Scenarios/Shared/BlueprintsNonSerialized/SocietyUtils/BPFL_Cornerstone_Utils.Get Community Names` (`self.Factions To Eliminate`))))))

(fn `Get End War Objective Name`
  (returns (Result :type Text))
  (return (`|FormatText` "End the fighting <optional>Currently affected districts:</> <semibold>{X}</>" (`KismetArrayLibrary.Array_Length` (`PXOngoingActionUtils.GetDistrictsWithOngoingActions`)))))

(fn `Get New Ban Factions Name`
  (returns (Result :type Text))
  (return (`|FormatText` "Ban Factions using the '{ABILITY}' City Ability " (`PXAbility.IngameName` (`self.Secure Rule Ability`)))))

(fn `Get Wait Objective Name`
  (returns (Result :type Text))
  (bind _duration (`PXAbility.Duration` (`self.Secure Rule Ability`)))
  (return (`|FormatText` (`self.Wait objective text`) (`PXTextUtils.GameTimeToTextMostImportant` _duration) (`PXTextUtils.GameTimeToTextMostImportant` (`PXTimeUtils.Subtract` (`PXTimeUtils.Add` _duration (`self.wait obj start time`)) (`PXTimeUtils.GetCurrentGameTime`))))))

(fn `Starting Stuff`
  (bind _returnvalue (`PXNationUtils.GetPlayerNation`))
  (`PXUnlockUtils.SetUnlockActive` _returnvalue (`self.dictator unlock`) true)
  (`PXUnlockUtils.SetUnlockActive` _returnvalue (`self.Final Charter Unlock`) true))

(fn `Update Eliminate`
  (params (community :type "PXCommunityComponent Object Reference"))
  (locals (cache :type "PXCommunityComponent Object Reference"))
  (for _array_element (`self.Factions To Eliminate`)
    (bind _output_get (set `local.cache` _array_element))
    (`/Engine/EditorBlueprintResources/StandardMacros.IsValid` _output_get
      (:`Is Valid`
        (if (`PXCommunityComponent.HasActiveImprint` _output_get (`self.contained imprint`))
          (`KismetArrayLibrary.Array_RemoveItem` (`self.Factions To Eliminate`) (`local.cache`))
          (`PXQuestObjective.ProgressObjective` (`self.eliminate objective`) 1
            (:`Finished`
              (remove `PXCommunitySubsystem.ImprintsChangedEvent` (subsystem `PXCommunitySubsystem`) (`|CreateDelegate` :!event `Update Eliminate`))
              (`self.FinishQuest` true))))))))