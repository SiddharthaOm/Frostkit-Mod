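; Main quest for the Faction War peace path, unlocking peace actions and guiding the player toward Peace Accords.
; It builds objectives to undo extreme laws and buildings as one combined objective, negotiate with both warring factions, optionally protect embattled districts, and pass the accords.
; Subsystem events refresh progress; completing required objectives or a 100-aye accords vote finishes the quest.
; Fervour, deradicalise and end-war helpers remain, but startup does not call them.
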(event `self.ReceiveStartQuest`
  (`self.Initial Unlocks`)
  (`self.Add Undo Extremes Objective`)
  (`self.Add Pacify Objective` false)
  (`self.Add Protect Districts Objective`)
  (`self.Add Peace Treaty Objective`)
  (`self.Initial Progress`)
  (`self.Bind Update Objective`))

(event `self.ReceiveObjectiveFinished`
  (params (objective :type "PXQuestObjective Object Reference"))
  (if (== objective (`self.Extremes Objective`))
    (`PXAsyncOpenPredefinedDialog.AsyncAction_OpenPredefinedDialog` "/Game/Scenarios/Shared/Configs/Messages/Dialogs/FactionWar/DA_FactionWar_Peace_UndoneExtremes_Dialog.DA_FactionWar_Peace_UndoneExtremes_Dialog"
      (:`Completed`
        (`PXUnlockUtils.SetUnlockActive` (`PXNationUtils.GetPlayerNation`) "/Game/Scenarios/Shared/Configs/Unlocks/FactionWarEndings/DA_FactionWar_PeacePath_PolicyBuilding_Block_Unlock.DA_FactionWar_PeacePath_PolicyBuilding_Block_Unlock" true)))))

(event `self.ReceiveFinishQuest`
  (params (bSuccess :type Boolean))
  (`parent.ReceiveFinishQuest` bSuccess)
  (`PXUnlockUtils.SetUnlockActive` (`PXNationUtils.GetPlayerNation`) "/Game/Scenarios/Shared/Configs/Unlocks/FactionWarEndings/DA_PeacePath_Unlock.DA_PeacePath_Unlock"))

(fn `Add Deradicalise Objective`
  (params (isOptional :type Boolean))
  (bind _returnvalue (`PXQuestUtils.AddCommunityActionQuestObjective` null (`|FormatText` "Ask the {INDEPENDENTS} to deradicalise the factions" (`/Game/Scenarios/Shared/BlueprintsNonSerialized/SocietyUtils/BPFL_Quest_Utils.Combine Text Array Into Single` (`/Game/Scenarios/Shared/BlueprintsNonSerialized/SocietyUtils/BPFL_Cornerstone_Utils.Get Community Names` (`self.Get Communities for Relations Objective`)))) "" (`self.Good relations community action`) null true isOptional null))
  (set `self.deradicalise objective` _returnvalue))

(fn `Add End War Objective`
  (params (`Aggressor faction` :type "PXCommunityComponent Object Reference"))
  (`self.Fervour Main Objective` false))

(fn `Add Fervour Silent Objectives`
  (bind _zero_fists (`self.Zero Fists`))
  (bind _returnvalue (`PXQuestUtils.StartQuestInPlace` "Silent fervour quest" "" (struct) "SideQuest" "DebugQuestName" false true 0.0 false))
  (bind _output_get (set `self.fervour quest` _returnvalue))
  (`BlueprintMapLibrary.Map_Add` (`self.Quest -> Objective Map`) _output_get (`self.fervour objective`))
  (for _array_element (`PXFactionUtils.GetMembersFromCity` (`PXNationUtils.GetPlayerMainCity`) null)
    (`PXQuestUtils.AddFervorTraitQuestObjective` (`self.fervour quest`) (`|FormatText` "Reduce {FACTION}' fervour to {ZERO_TIER}" (`/Game/Scenarios/Shared/BlueprintsNonSerialized/Communities/BPFL_CommunityUtils.Get Community Name` _array_element) (`PXTraitType.IngameName` _zero_fists)) "" (`PXCommunityComponent.GetCommunityType` _array_element) _zero_fists "LessThanOrEqualTo" false null)))

(fn `Add Pacify Objective`
  (params (isOptional :type Boolean))
  (bind _returnvalue (`self.AddQuestObjective` (`|FormatText` "Negotiate an end to militancy with the {AGGRESSOR}" (`.Faction War Aggressor Name` (`/Game/Scenarios/Shared/BlueprintsNonSerialized/SocietyUtils/BPFL_SharedScenariosStorage.Get Faction War Initial Aggressor`))) "" 0 1 false null))
  (set `self.aggressor pacify obj` _returnvalue)
  (bind _returnvalue_2 (`self.AddQuestObjective` (`|FormatText` "Negotiate an end to militancy with the {DEFENDER}" (`.Faction War Defender Name` (`/Game/Scenarios/Shared/BlueprintsNonSerialized/SocietyUtils/BPFL_SharedScenariosStorage.Get Faction War Initial Defender`))) "" 0 1 false null))
  (set `self.defender pacify obj` _returnvalue_2)
  (add `PXCommunitySubsystem.ImprintsChangedEvent` (subsystem `PXCommunitySubsystem`) (`|CreateDelegate` :!event `Update Pacify Obj`))
  (add `PXQuestSubsystem.QuestFinishEvent` (subsystem `PXQuestSubsystem`) (`|CreateDelegate` :!event `Update Negotiate Obj on Quest Finish`)))

(fn `Add Peace Treaty Objective`
  (returns (Output_Get :type "PXQuestObjective Object Reference"))
  (`PXPolicyUtils.SetCurrentPolicyInFallbackGroup` (`PXPolicyUtils.GetPlayerPolicy`) (`self.Peace Policy`))
  (`PXUnlockUtils.SetUnlockActive` (`PXNationUtils.GetPlayerNation`) "/Game/Scenarios/Shared/Configs/Unlocks/FactionWarEndings/DA_PeaceTreaty_Unlock.DA_PeaceTreaty_Unlock" true)
  (bind _returnvalue (`PXQuestUtils.AddPolicyQuestObjective` (make `PXObjectiveParameters` (`|FormatText` "Pass 'Peace Accords' using the 'Propose Peace Accords' Ability") "" false 1 null self) (make `PXPolicyObjectiveParameters` (`self.Peace Policy`) "Pass" (`|MakeArray` "/Game/Scenarios/Shared/Configs/Policies/Rule/Special/PeaceTreaty/DA_PeaceAccords_Policy.DA_PeaceAccords_Policy" :!type "PXPolicyType Object Reference"))))
  (bind _output_get (set `self.Peace Objective` _returnvalue))
  (add `PXParliamentSubsystem.VoteFinishedEvent` (subsystem `PXParliamentSubsystem`) (`|CreateDelegate` :!event `Force Peace Treaty Objective`))
  (return _output_get))

(fn `Add Protect Districts Objective`
  (bind _returnvalue (subsystem `PXOngoingActionSubsystem`))
  (bind _returnvalue_2 (subsystem `PXAbilitySubsystem`))
  (bind (_protected_districts1 _number_protected _number_total) (`/Game/Scenarios/Shared/BlueprintsNonSerialized/FactionEmergence/BPFL_FactionWarUtils.Get Protected Districts`))
  (bind _returnvalue_3 (`self.AddQuestObjective` (`self.Get Protect Obj Name`) "" _number_protected _number_total true null))
  (set `self.protected objective` _returnvalue_3)
  (add `PXOngoingActionSubsystem.OngoingActionChangedEvent` _returnvalue (`|CreateDelegate` :!event `Update Protect on War Changed`))
  (add `PXOngoingActionSubsystem.OngoingActionDistrictChangedEvent` _returnvalue (`|CreateDelegate` :!event `Update Protect on War Dist Changed`))
  (add `PXAbilitySubsystem.AbilityActivatedEvent` _returnvalue_2 (`|CreateDelegate` :!event `Update Protect on Ability Act`))
  (add `PXAbilitySubsystem.AbilityDeactivatedEvent` _returnvalue_2 (`|CreateDelegate` :!event `Update Protect on Ability Act`)))

(fn `Add Tag to Must Destroy Buildings`
  (params (Array :type "Array of PXBuildingComponent Object Reference"))
  (locals (cache :type "Actor Object Reference"))
  (for _array_element Array
    (bind _output_get (set `local.cache` (`ActorComponent.GetOwner` _array_element)))
    (`PXPredefinedModifierUtils.SetPredefinedModifierActiveManualTarget` (`PXNationUtils.GetPlayerNation`) "/Game/Scenarios/Shared/Configs/PredefinedModifiers/FactionWar/DA_Peace_RadicalBuildingToDestroy_Predefinied.DA_Peace_RadicalBuildingToDestroy_Predefinied" _output_get true)))

(fn `Add Undo Extremes Objective`
  (locals (`extreme policies` :type "Array of PXPolicyType Object Reference") (`extreme buildings` :type "Array of PXBuildingComponent Object Reference") (`added types` :type "Array of PXBuildingType Object Reference") (`first policy` :type "PXPolicyType Object Reference") (`first building` :type "PXBuildingComponent Object Reference"))
  (bind _result (`|FormatText` "Undo all extreme measures in the city"))
  (bind _extreme_buildings (`local.extreme buildings`))
  (bind _extreme_policies (`local.extreme policies`))
  (bind (_extreme_active_things _extreme_active_law_output _extreme_existing_buildings_output _extreme_existing_building_types1) (`/Game/Scenarios/Shared/BlueprintsNonSerialized/SocietyUtils/BPFL_Cornerstone_Utils.Get All Extreme Building and Laws in Main City`))
  (if (> _extreme_active_things 0)
    (bind _output_get (set `local.extreme policies` _extreme_active_law_output))
    (set `self.extreme policies global` _output_get)
    (bind _output_get_2 (set `local.extreme buildings` _extreme_existing_buildings_output))
    (bind _output_get_3 (set `self.extreme buildings global` _output_get_2))
    (`self.Add Tag to Must Destroy Buildings` _output_get_3)
    (set `self.Extreme building types global` _extreme_existing_building_types1)
    (if (`KismetArrayLibrary.Array_IsNotEmpty` _extreme_policies)
      (bind _output_get_4 (set `local.first policy` (`|GetArrayItem` _extreme_policies)))
      (`KismetArrayLibrary.Array_RemoveItem` (`local.extreme policies`) _output_get_4)
      (bind _returnvalue (`PXQuestUtils.AddPolicyQuestObjective` (make `PXObjectiveParameters` _result "" false 1 null self) (make `PXPolicyObjectiveParameters` (`local.first policy`) "Repeal")))
      (set `self.Extremes Objective` _returnvalue)
      (else
        (bind _output_get_5 (set `local.first building` (`|GetArrayItem` _extreme_buildings)))
        (`KismetArrayLibrary.Array_RemoveItem` _extreme_buildings _output_get_5)
        (bind _returnvalue_2 (`PXQuestUtils.AddBuildingQuestObjective` (make `PXObjectiveParameters` _result "" false 1 null self) (`self.Get Destroy Building Params` (`local.first building`))))
        (set `self.Extremes Objective` _returnvalue_2)
        (`KismetArrayLibrary.Array_Add` (`local.added types`) (`PXBuildingComponent.Type` (`local.first building`)))))
    (for _array_element (`local.extreme policies`)
      (`PXQuestUtils.CombinePolicyQuestObjective` (`self.Extremes Objective`) (make `PXPolicyObjectiveParameters` _array_element "Repeal")))
    (for _array_element_2 (`local.extreme buildings`)
      (bind _type (`PXBuildingComponent.Type` _array_element_2))
      (if (not (`KismetArrayLibrary.Array_Contains` (`local.added types`) _type))
        _
        (else
          _))
      (`KismetArrayLibrary.Array_Add` (`local.added types`) _type)
      (`PXQuestUtils.CombineBuildingQuestObjective` (`self.Extremes Objective`) (`self.Get Destroy Building Params` _array_element_2)))
    (else
      ;[1 1 1] Block doing any more Extremes if none present at start
      (`PXUnlockUtils.SetUnlockActive` (`PXNationUtils.GetPlayerNation`) (`self.Peace No Extreme Policy / Building Unlock`) true))))

(fn `Bind Update Objective`
  (add `PXQuestSubsystem.QuestObjectiveProgressEvent` (subsystem `PXQuestSubsystem`) (`|CreateDelegate` :!event `Update Objectives`)))

(fn `Fervour Main Objective`
  (params (isOptional :type Boolean))
  (bind _returnvalue (`self.AddQuestObjective` (`|FormatText` "Reduce all factions' fervour to {ZERO_TIER}" (`PXTraitType.IngameName` (`self.Zero Fists`))) "" 0 (`KismetArrayLibrary.Array_Length` (`PXFactionUtils.GetMembersFromCity` (`PXNationUtils.GetPlayerMainCity`) null)) isOptional null))
  (set `self.fervour objective` _returnvalue)
  (`self.Add Fervour Silent Objectives`))

(fn `Force Peace Treaty Objective`
  (params (parliament :type "PXParliamentComponent Object Reference") (affectedPolicy :type "PXPolicyType Object Reference") (results :type "PXVoteResultData Structure"))
  (if (== affectedPolicy (`self.Peace Policy`))
    (if (== (`.AyeCount` (break `PXVoteResultData` results)) 100)
      (remove `PXParliamentSubsystem.VoteFinishedEvent` (subsystem `PXParliamentSubsystem`) (`|CreateDelegate` :!event `Force Peace Treaty Objective`))
      (`PXQuestObjective.ProgressObjective` (`self.Peace Objective`) 1
        (:`NotFinished`
          _)
        (:`Finished`
          _))
      (`self.FinishQuest` true))))

(fn `Get Communities for Relations Objective`
  (returns (ReturnValue :type "Array of PXCommunityComponent Object Reference"))
  (return (`PXFactionUtils.GetIndependentCommunitiesFromCity` (`PXNationUtils.GetPlayerMainCity`))))

(fn `Get Destroy Building Params`
  (params (self2 :type "PXBuildingComponent Object Reference"))
  (returns (PXBuildingObjectiveParameters :type "PXBuildingObjectiveParameters Structure"))
  (return (make `PXBuildingObjectiveParameters` :`BuildingType` (`PXBuildingComponent.Type` self2) :`QuestType` "Destroy" :`OptionalSpecificBuilding` self2 :`OptionalCity` (`PXNationUtils.GetPlayerMainCity`) :`CheckProgressAtStart` false)))

(fn `Get Finished Quest Objectives`
  (params (self2 :type "PXQuest Object Reference"))
  (returns (finished1 :type "Array of PXQuestObjective Object Reference") (ReturnValue :type Integer))
  (locals (finished :type "Array of PXQuestObjective Object Reference"))
  (bind _finished (`local.finished`))
  (for _array_element (`self.GetQuestObjectives` self2)
    (if (`PXQuestObjective.IsObjectiveFinished` _array_element)
      (`KismetArrayLibrary.Array_Add` (`local.finished`) _array_element)))
  (return _finished (`KismetArrayLibrary.Array_Length` _finished)))

(fn `Get Protect Obj Name`
  (returns (Result :type Text))
  (return (`|FormatText` "Use <semibold>'{PROTECT_EITHER}'</> District Ability on all districts engulfed in fighting" (`PXAbility.IngameName` (`self.protect generic ability`)))))

(fn `Initial Progress`
  (bind _keys (`BlueprintMapLibrary.Map_Keys` (`self.Quest -> Objective Map`)))
  (for _array_element _keys
    (bind (_finished1 _returnvalue) (`self.Get Finished Quest Objectives` _array_element))
    (`PXQuestObjective.ModifyObjectiveProgress` (`BlueprintMapLibrary.Map_Find` (`self.Quest -> Objective Map`) _array_element) _returnvalue)))

(fn `Initial Unlocks`
  (bind _returnvalue (`PXNationUtils.GetPlayerNation`))
  (`PXUnlockUtils.SetUnlockActive` _returnvalue "/Game/Scenarios/Shared/Configs/Unlocks/FactionWarEndings/DA_PeacePath_Unlock.DA_PeacePath_Unlock" true)
  (`PXUnlockUtils.SetUnlockActive` _returnvalue "/Game/Scenarios/Shared/Configs/Unlocks/OA/DA_GoodRelations_Arc_CA.DA_GoodRelations_Arc_CA" true)
  (`PXUnlockUtils.SetUnlockActive` _returnvalue "/Game/Scenarios/Shared/Configs/Unlocks/OA/DA_GoodRelations_Deradicalise_CA.DA_GoodRelations_Deradicalise_CA" true)
  (`PXUnlockUtils.SetUnlockActive` _returnvalue "/Game/Scenarios/Shared/Configs/Unlocks/Other/DA_PacifyUnlock_Unlock.DA_PacifyUnlock_Unlock" true))

(fn `Modal After Fervour Objective`
  (if (not (`self.fervour modal shown`))
    (`/Game/Scenarios/Shared/BlueprintsNonSerialized/Audio/BPFL_AudioUtils.Post 2d Audio Event` "/Game/Scenarios/Shared/Audio/Events/Music/Chapter_05/S06_NL_Quest_Notify_07.S06_NL_Quest_Notify_07")
    (`PXCommunicationChannelsUtils.OpenPredefinedDialog` (`self.Fervor Gone Dialog`) (`|MakeMap` "" :!valuetype "Text") null)
    (set `self.fervour modal shown` true)))

(fn `Update End War Objective`
  (params (changeType :type "EPXOngoingActionChangeType Enum" :default "HintsStart") (ongoingAction :type "PXOngoingActionComponent Object Reference"))
  (if (`|EnumEquality` changeType "Finish")
    (`PXQuestObjective.ModifyObjectiveProgress` (`self.end wars objective`) (select `bool` (`/Game/Scenarios/Shared/BlueprintsNonSerialized/OngoingEvents/BPFL_OngoingAction_Utils.Is Any Action of type Ongoing?` "/Game/Scenarios/Shared/Configs/OngoingActions/System_Started/DA_FactionWar.DA_FactionWar") :`false` 1))))

(fn `Update Negotiate Obj on Quest Finish`
  (params (Quest :type "PXQuest Object Reference") (bSuccess :type Boolean))
  (`self.Update Pacify Obj` null))

(fn `Update Objectives`
  (params (Objective :type "PXQuestObjective Object Reference") (OldProgress :type Integer))
  (bind _returnvalue (`PXQuestObjective.GetOwnerQuest` Objective))
  (bind _fervour_objective (`self.fervour objective`))
  (bind (_value _returnvalue_2) (`BlueprintMapLibrary.Map_Find` (`self.Quest -> Objective Map`) _returnvalue))
  (bind (_finished1 _returnvalue_3) (`self.Get Finished Quest Objectives` _returnvalue))
  (if _returnvalue_2
    (`PXQuestObjective.ModifyObjectiveProgress` _value _returnvalue_3)
    (if (and (== _value _fervour_objective) (`PXQuestObjective.IsObjectiveFinished` _fervour_objective))
      (`self.Modal After Fervour Objective`)))
  (if (`/Game/Scenarios/Shared/BlueprintsNonSerialized/SocietyUtils/BPFL_Quest_Utils.Are All Objectives Finished` self true)
    (remove `PXQuestSubsystem.QuestObjectiveProgressEvent` (subsystem `PXQuestSubsystem`) (`|CreateDelegate` :!event `Update Objectives`))
    (`self.FinishQuest` true)))

(fn `Update Pacify Obj`
  (params (community :type "PXCommunityComponent Object Reference"))
  (`|ExecutionSequence`
    (:`then_0`
      (if (not (`PXQuestObjective.IsObjectiveFinished` (`self.aggressor pacify obj`)))
        (if (`PXCommunityComponent.HasActiveImprint` (`/Game/Scenarios/Shared/BlueprintsNonSerialized/SocietyUtils/BPFL_SharedScenariosStorage.Get Faction War Initial Aggressor`) (`self.militancy imprint`))
          (`PXQuestUtils.FinishObjective` (`self.aggressor pacify obj`)))))
    (:`then_1`
      (if (not (`PXQuestObjective.IsObjectiveFinished` (`self.defender pacify obj`)))
        (if (`PXCommunityComponent.HasActiveImprint` (`/Game/Scenarios/Shared/BlueprintsNonSerialized/SocietyUtils/BPFL_SharedScenariosStorage.Get Faction War Initial Defender`) (`self.militancy imprint`))
          (`PXQuestUtils.FinishObjective` (`self.defender pacify obj`)))))))

(fn `Update Protect on Ability Act`
  (params (AbilityComponent :type "PXAbilityComponent Object Reference"))
  (`self.Update Protect on War Changed` "HintsStart"))

(fn `Update Protect on War Changed`
  (params (changeType :type "EPXOngoingActionChangeType Enum" :default "HintsStart") (ongoingAction :type "PXOngoingActionComponent Object Reference"))
  (bind _protected_objective (`self.protected objective`))
  (bind (_protected_districts1 _number_protected _number_total _some_unprotected1) (`/Game/Scenarios/Shared/BlueprintsNonSerialized/FactionEmergence/BPFL_FactionWarUtils.Get Protected Districts`))
  (if (or (!= _number_protected (`PXQuestObjective.GetObjectiveProgress` _protected_objective)) (!= (`PXQuestObjective.GetObjectiveMaxProgress` _protected_objective) _number_total))
    (`PXQuestObjective.ModifyObjective` _protected_objective "" "" _number_protected _number_total)
    (`PXUnlockUtils.SetUnlockActive` (`PXNationUtils.GetPlayerNation`) (`self.all dist protected unlock`) (not _some_unprotected1))))

(fn `Update Protect on War Dist Changed`
  (params (changeType :type "EPXOngoingActionChangeType Enum" :default "HintsStart") (action :type "PXOngoingActionComponent Object Reference") (district :type "PXDistrictComponent Object Reference"))
  (`self.Update Protect on War Changed` "HintsStart"))