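; Quest that asks the player to raise relations with a protesting community to a target trust trait.
; The community comes from shared variable storage and feeds a greater-than-or-equal trust objective with a formatted name.
; Async waits cover the quest duration and the end of that community's ongoing protest action.
; The failure path removes the community from the protest relation-fix quest list and finishes the quest unsuccessfully.
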(event `self.ReceiveStartQuest`
  (set `self.Protesting Community` (`/Game/Scenarios/Shared/BlueprintsSerialized/VariableStorage/BP_SharedVariableStorage.Community to Fix Relations in Protest` (`/Game/Scenarios/Shared/BlueprintsNonSerialized/SocietyUtils/BPFL_SharedScenariosStorage.Get Shared Variable Storage`)))
  (`PXQuestUtils.AddTrustQuestObjective` null (`|FormatText` "Increase Relations with {FACTION} to {RELATIONS}" (`PXCommunityType.IngameName` (`self.Protesting Community`)) (`PXTraitType.IngameName` (`self.Trust Trait`))) "" (`self.Protesting Community`) (`self.Trust Trait`) "GreaterThanOrEqualTo" false null)
  (`PXAsyncWaitForDurationPassed.AsyncAction_WaitForDurationPassed` (struct :`ScaledTicks` 10)
    (:`Completed`
      (bind (_hasongoingaction _returnvalue) (`PXOngoingActionUtils.GetOngoingActionComponentForCommunity` (`.ReturnValue` (`PXCommunityUtils.GetCommunityOfCommunityType` (`self.Protesting Community`)))))
      (set `self.Protest` _returnvalue)
      (`PXAsyncWaitForOngoingActionFinished.AsyncAction_WaitForOngoingActionFinished` (`PXOngoingActionComponent.GetActionType` (`self.Protest`))
        (:`Completed`
          (`KismetArrayLibrary.Array_RemoveItem` (`/Game/Scenarios/Shared/BlueprintsSerialized/VariableStorage/BP_SharedVariableStorage.Protest Relation Fix Quests with Communities` (`/Game/Scenarios/Shared/BlueprintsNonSerialized/SocietyUtils/BPFL_SharedScenariosStorage.Get Shared Variable Storage`)) (`self.Protesting Community`))
          (`PXQuestUtils.FinishQuest` self))))))