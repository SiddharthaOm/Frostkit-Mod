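; Scenario notification script that tells the player when the temperature level rises or drops and how heat demand changes as a result.
; On BeginPlay it registers for the temperature level changed event on a validated subsystem.
; The change handler compares new and old degrees, then shows a central notification with matching text and illustration.
; Notifications are suppressed while the player nation has the block-temperature-notification unlock active.
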(event `self.ReceiveBeginPlay`
  (bind _returnvalue (`|Subsystem`)
    (:`then`
      (add `PXTemperatureSubsystem.TemperatureLevelChangedEvent` _returnvalue (`|CreateDelegate` :!event `OnTemperatureChange`)))))

(fn `Is Temperature Increasing`
  (params (`New Temp Level` :type "PXTemperatureLevel Object Reference") (`Old Temp Level` :type "PXTemperatureLevel Object Reference"))
  (returns (ReturnValue :type Boolean))
  (return (> (`PXTemperatureLevel.Degrees` `New Temp Level`) (`PXTemperatureLevel.Degrees` `Old Temp Level`))))

(fn `OnTemperatureChange`
  (params (newLevel :type "PXTemperatureLevel Object Reference") (oldLevel :type "PXTemperatureLevel Object Reference"))
  (if (not (`PXUnlockUtils.IsUnlockActive` (`PXNationUtils.GetPlayerNation`) "/Game/Scenarios/Shared/Configs/Unlocks/NotificationsControllers/DA_BlockTemperatureNotification.DA_BlockTemperatureNotification"))
    (if (`self.Is Temperature Increasing` newLevel oldLevel)
      (`PXCentralNotificationUtils.ShowCentralNotification` "Custom" (`|FormatText` "Temperature rise") (`|FormatText` "Heat demand is decreased") "" "/Game/UI/Assets/Textures/SpecialTextures/Illustrations/CentralNotifications/UIT_CentralNotification_TemperatureRises_Sprite.UIT_CentralNotification_TemperatureRises_Sprite" "/Game/UI/Assets/Textures/AtlasedTextures/Icons/Frames/UIT_FuelIcon.UIT_FuelIcon" false "BottomLeft")
      (else
        (`PXCentralNotificationUtils.ShowCentralNotification` "Custom" (`|FormatText` "Temperature drop") (`|FormatText` "Heat demand is increased") "" "/Game/UI/Assets/Textures/SpecialTextures/Illustrations/CentralNotifications/UIT_CentralNotification_TemperatureDrops_Sprite.UIT_CentralNotification_TemperatureDrops_Sprite" "/Game/UI/Assets/Textures/AtlasedTextures/Icons/Frames/UIT_FuelIcon.UIT_FuelIcon" false "BottomLeft")))))