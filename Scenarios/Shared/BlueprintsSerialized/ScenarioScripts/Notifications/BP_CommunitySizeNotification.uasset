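; Scenario script that notifies the player of community and city population size changes.
; On BeginPlay it binds to the community subsystems' change events, acting only on changes flagged to notify.
; Deaths add notifications formatted from the supplied reason; city growth adds a growth or natural-death notification by sign, plus a central "Population increased" popup regardless of sign.
; Community growth notifications are unsupported, leaving that text helper as a debug-print stub.
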(event `self.ReceiveBeginPlay`
  (bind _returnvalue (`|Subsystem`)
    (:`then`
      (add `PXCommunitySubsystem.CommunitySizeChangedEvent` _returnvalue (`|CreateDelegate` :!event `OnCommunitySizeChanged`))
      (add `PXCommunitySubsystem.PopulationSizeChangedEvent` (subsystem `PXCommunitySubsystem`) (`|CreateDelegate` :!event `OnPopulationSizeChanged`)))))

(fn `Get Community Death Text`
  (params (Params :type "PXCommunitySizeChangedEventParameters Structure (by ref)"))
  (returns (`Death text` :type Text))
  (bind (_params_community _params_change) (break `PXCommunitySizeChangedEventParameters` (`local.Params`)))
  (bind (_community _change _transfermatches _reason) (break `PXCommunitySizeChangedEventParameters` (`local.Params`)))
  (bind _returnvalue (`KismetMathLibrary.Abs_Int` _params_change))
  (bind _ingame_name (`/Game/Scenarios/Shared/BlueprintsNonSerialized/Cities/BPFL_CityUtils.Get City Ingame Name` (`PXCommunityComponent.ParentCity` _community)))
  (return (`|FormatText` _reason _returnvalue (`PXFactionUtils.GetFactionOrCommunityInGameNameText` _community) _ingame_name _returnvalue _returnvalue _ingame_name)))

(fn `Get Community Growth Text`
  (params (Params :type "PXCommunitySizeChangedEventParameters Structure (by ref)"))
  (returns (Result :type Text))
  (bind (_params_community _params_change) (break `PXCommunitySizeChangedEventParameters` (`local.Params`)))
  (bind (_params_community_2 _params_change_2) (break `PXCommunitySizeChangedEventParameters` (`local.Params`)))
  (`KismetSystemLibrary.PrintString` (`KismetTextLibrary.Conv_TextToString` (`|FormatText` "{PopulationSize} {MoreOrLess} {Community} live among us" (`KismetMathLibrary.Abs_Int` _params_change) (select `bool` (> _params_change_2 0) :`false` "less" :`true` "more" :!type "Text") (`PXCommunityType.IngameName` (`PXCommunityComponent.GetCommunityType` (`.Community` (break `PXCommunitySizeChangedEventParameters` (`local.Params`))))))))
  (return ""))

(fn `Get Natural Growth Text`
  (params (Change :type Integer) (City :type "PXCityComponent Object Reference"))
  (returns (ReturnValue :type Text))
  (bind _returnvalue (`KismetMathLibrary.Abs_Int` (`local.Change`)))
  (bind _returnvalue_2 (`PXGameplayElementUtils.GetActorIngameName` (`ActorComponent.GetOwner` (`local.City`))))
  (return (select `bool` (> (`local.Change`) 0) :`false` (`|FormatText` "{PopulationSize} people died of natural reasons in {CITY}" _returnvalue _returnvalue_2) :`true` (`|FormatText` "Population grew by {PopulationSize} in {CITY}" _returnvalue _returnvalue_2))))

(fn `Get Population Death Text`
  (params (Params :type "PXPopulationSizeChangedEventParameters Structure (by ref)"))
  (returns (Result :type Text))
  (bind (_city _change _reason) (break `PXPopulationSizeChangedEventParameters` Params))
  (bind _returnvalue (`KismetMathLibrary.Abs_Int` _change))
  (bind _returnvalue_2 (`PXGameplayElementUtils.GetActorIngameName` (`ActorComponent.GetOwner` _city)))
  (return (`|FormatText` _reason _returnvalue _returnvalue_2 _returnvalue _returnvalue _returnvalue_2)))

(fn `OnCommunitySizeChanged`
  (params (params :type "PXCommunitySizeChangedEventParameters Structure"))
  (if params_ShouldNotify
    (switch `EPXCommunitySizeChangeReason` params_ChangeType
      (:`Death`
        (`PXCommunicationChannelsUtils.AddNotification` (make `PXNotificationData` "PopulationDeath" (`self.Get Community Death Text` (`local.params`))))))))

(fn `OnPopulationSizeChanged`
  (params (params :type "PXPopulationSizeChangedEventParameters Structure"))
  (locals (ChangeValue :type Integer))
  (bind (_params_city _params_change) (break `PXPopulationSizeChangedEventParameters` (`local.params`)))
  (bind (_params_city_2 _params_change_2) (break `PXPopulationSizeChangedEventParameters` (`local.params`)))
  (bind _returnvalue (`self.Get Natural Growth Text` _params_change _params_city))
  (if params_ShouldNotify
    (switch `EPXCommunitySizeChangeReason` params_ChangeType
      (:`Death`
        (`PXCommunicationChannelsUtils.AddNotification` (make `PXNotificationData` "PopulationDeath" (`self.Get Population Death Text` (`local.params`)) "/Game/UI/Assets/Textures/SpecialTextures/Illustrations/CentralNotifications/UIT_CentralNotification_PopulationLoss_Sprite.UIT_CentralNotification_PopulationLoss_Sprite")))
      (:`Growth`
        (`PXCommunicationChannelsUtils.AddNotification` (make `PXNotificationData` (select `bool` (> _params_change_2 0) :`false` "PopulationDeath" :`true` "PopulationGrowth" :!type "EPXNotificationType Enum") _returnvalue))
        (`PXCentralNotificationUtils.ShowCentralNotificationOfType` "PopulationChange" "Population increased" _returnvalue "Growth" "/Game/UI/Assets/Textures/SpecialTextures/Illustrations/CentralNotifications/UIT_CentralNotification_PopulationGrowth_Sprite.UIT_CentralNotification_PopulationGrowth_Sprite")))))