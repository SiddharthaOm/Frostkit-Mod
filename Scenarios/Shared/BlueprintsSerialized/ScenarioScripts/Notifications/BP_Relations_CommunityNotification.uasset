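; Scenario notification script that tells the player when relations with a community in their main city improve or worsen.
; It listens to the trust subsystem's community standing event and queues changes above a threshold in a map of community to direction.
; A guarded timed wait batches the queue, keeping only the latest direction per community.
; It then shows the notifications if fewer than three communities are queued, otherwise discards them all silently.
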(event `self.ReceiveBeginPlay`
  (add `PXTrustSubsystem.CommunityStandingChangedEvent` (subsystem `PXTrustSubsystem`) (`|CreateDelegate` :!event `Relations Change Community Notification`)))

(event `Queued Notifications`
  (if (not (`self.Already Queuing?`))
    (set `self.Already Queuing?` true)
    (`PXAsyncWaitForDurationPassed.AsyncAction_WaitForDurationPassed` (struct :`ScaledTicks` 10)
      (:`Completed`
        (if (< (`BlueprintMapLibrary.Map_Length` (`self.Queued Communities`)) 3)
          (bind _keys (`BlueprintMapLibrary.Map_Keys` (`self.Queued Communities`)))
          (for _array_element _keys
            (`self.Show Notification` (`BlueprintMapLibrary.Map_Find` (`self.Queued Communities`) _array_element) _array_element))
          (`BlueprintMapLibrary.Map_Clear` (`self.Queued Communities`))
          (set `self.Already Queuing?` false)
          (else
            (`BlueprintMapLibrary.Map_Clear` (`self.Queued Communities`))
            (set `self.Already Queuing?` false)))))))

(fn `Relations Change Community Notification`
  (params (communityType :type "PXCommunityType Object Reference") (oldStanding :type "Float (single-precision)") (newStanding :type "Float (single-precision)"))
  (locals (`community comp` :type "PXCommunityComponent Object Reference"))
  (bind (_outfound _returnvalue) (`PXCommunityUtils.GetCommunityOfCommunityType` communityType (`PXNationUtils.GetPlayerMainCity`)))
  (if _outfound
    (set `local.community comp` _returnvalue)
    (if (> (`KismetMathLibrary.Abs` (- (`local.oldStanding`) (`local.newStanding`))) (`self.Threshold to trigger`))
      (`BlueprintMapLibrary.Map_Add` (`self.Queued Communities`) (`local.community comp`) (< (`local.oldStanding`) (`local.newStanding`)))
      (`self.Queued Notifications`))))

(fn `Show Notification`
  (params (Condition :type Boolean) (`community comp1` :type "PXCommunityComponent Object Reference"))
  (locals (`community comp` :type "PXCommunityComponent Object Reference"))
  (set `local.community comp` `community comp1`)
  (if Condition
    (`/Game/Scenarios/Shared/BlueprintsNonSerialized/Communities/BPFL_CommunityUtils.DisplayCommunityNotification` (`local.community comp`) (`|FormatText` (`self.Relations Improve Text`) (`/Game/Scenarios/Shared/BlueprintsNonSerialized/Communities/BPFL_CommunityUtils.Get Community Name` (`local.community comp`))))
    (else
      (`/Game/Scenarios/Shared/BlueprintsNonSerialized/Communities/BPFL_CommunityUtils.DisplayCommunityNotification` (`local.community comp`) (`|FormatText` (`self.Relations Worsen Text`) (`/Game/Scenarios/Shared/BlueprintsNonSerialized/Communities/BPFL_CommunityUtils.Get Community Name` (`local.community comp`)))))))