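; Notification script that shows a central notification when a storm hits or a whiteout ends in one of the player's cities.
; On BeginPlay it binds to a subsystem's weather level change event, then skips notifications if a blocking unlock is active or the city belongs to another nation.
; A rising level shows the storm alert with the new level's description; any other change shows the survival message.
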(event `self.ReceiveBeginPlay`
  (add `PXWeatherTargetSubsystem.WeatherLevelChangedEvent` (`|Subsystem`) (`|CreateDelegate` :!event `On Weather Changed`)))

(fn `IsPlayerNation`
  (params (city :type "PXCityComponent Object Reference"))
  (returns (ReturnValue :type Boolean))
  (return (== (`PXNationUtils.GetCityNation` city) (`PXNationUtils.GetPlayerNation`))))

(fn `On Weather Changed`
  (params (weatherTarget :type "PXWeatherTargetComponent Object Reference") (oldWeatherLevel :type "PXWeatherLevel Object Reference") (newWeatherLevel :type "PXWeatherLevel Object Reference"))
  (locals (City :type "PXCityComponent Object Reference"))
  (if (not (`PXUnlockUtils.IsUnlockActive` (`PXNationUtils.GetPlayerNation`) "/Game/Scenarios/Shared/Configs/Unlocks/Other/DA_BlockWhiteoutNotificationsFromScript.DA_BlockWhiteoutNotificationsFromScript"))
    (bind _output_get (set `local.City` (`Actor.GetComponentByClass` (`ActorComponent.GetOwner` (`local.weatherTarget`)) "/Script/Frostpunk2.PXCityComponent")))
    (`/Engine/EditorBlueprintResources/StandardMacros.IsValid` _output_get
      (:`Is Valid`
        ;[1 1 1] Don't Show Notifications for cities that do not belong to the player
        (if (`self.IsPlayerNation` (`local.City`))
          (if (< (`PXWeatherLevel.Level` (`local.oldWeatherLevel`)) (`PXWeatherLevel.Level` (`local.newWeatherLevel`)))
            (`PXCentralNotificationUtils.ShowCentralNotification` "ColonyCreation" (`|FormatText` "Storm hits {cityName}" (`PXGameplayElementUtils.GetActorIngameName` (`ActorComponent.GetOwner` (`local.City`)))) (`PXWeatherLevel.Description` (`local.newWeatherLevel`)) "" "/Game/UI/Assets/Textures/SpecialTextures/Illustrations/CentralNotifications/UIT_CentralNotification_StormHits_Sprite.UIT_CentralNotification_StormHits_Sprite" null false "TepLeft")
            (else
              (`PXCentralNotificationUtils.ShowCentralNotification` "ColonyCreation" (`|FormatText` "Whiteout ends in {cityName}" (`PXGameplayElementUtils.GetActorIngameName` (`ActorComponent.GetOwner` (`local.City`)))) (`|FormatText` "The City Survived ") "" "/Game/UI/Assets/Textures/SpecialTextures/Illustrations/CentralNotifications/UIT_CentralNotification_StormLeaves_Sprite.UIT_CentralNotification_StormLeaves_Sprite" null false "TepLeft"))))))))