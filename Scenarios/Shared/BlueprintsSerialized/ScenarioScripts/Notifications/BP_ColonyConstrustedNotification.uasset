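; Scenario script that shows a central "colony constructed" notification when a city finishes construction.
; On BeginPlay it binds to the construction subsystem's finished event and filters for owners with a city component.
; It skips the player's main city and any colonies listed as excluded in the current scenario's constants storage.
; The notification shows the city's in-game name and the creation panel image from its city area's UI config.
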(event `self.ReceiveBeginPlay`
  (add `PXConstructionSubsystem.ConstructionFinishedEvent` (subsystem `PXConstructionSubsystem`) (`|CreateDelegate` :!event `OnColonyConstructionFinished`)))

(fn `OnColonyConstructionFinished`
  (params (constructionComponent :type "PXConstructionComponent Object Reference"))
  (bind _output_get (set `self.CityComponent` (`Actor.GetComponentByClass` (`ActorComponent.GetOwner` constructionComponent) "/Script/Frostpunk2.PXCityComponent")))
  (`/Engine/EditorBlueprintResources/StandardMacros.IsValid` _output_get
    (:`Is Valid`
      (if (!= (`PXNationUtils.GetPlayerMainCity`) (`PXCityComponent.GetType` (`self.CityComponent`)))
        (if (not (`KismetArrayLibrary.Array_Contains` (`/Game/Scenarios/Shared/Configs/ConstantsStorage/BP_SharedConstantsStorageBaseClass.Excluded Colonies from Notifications` (`/Game/Scenarios/Shared/BlueprintsNonSerialized/SocietyUtils/BPFL_SharedScenariosStorage.Get Current Scenario Constants Storage`)) (`PXCityComponent.GetType` (`self.CityComponent`))))
          (`self.ShowNotification` (`self.CityComponent`)))))))

(fn `ShowNotification`
  (params (CityComponent :type "PXCityComponent Object Reference"))
  (bind _returnvalue_citycreationpanelimage (break `PXCityTileAssetsConfig` (`PXCityAreaUtils.GetCityAreaUiAssetsConfig` (`PXCityComponent.GetCityArea` CityComponent))))
  (`PXCentralNotificationUtils.ShowCentralNotificationOfType` "ColonyCreation" (`|FormatText` "{CityName} constructed" (`PXGameplayElementUtils.GetActorIngameName` (`ActorComponent.GetOwner` CityComponent))) "" "" (`|ConvertAsset` _returnvalue_citycreationpanelimage)))