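; Scenario script that tracks whether extreme policies and buildings represent both opposing affinities on the same axis.
; On BeginPlay it binds to policy change, construction finished and deconstruction events, each refreshing the cached extreme policy or building affinities.
; It then merges both lists and, for each axis to check, writes a contrasting-extremes flag to shared variable storage, true when both affinities of that axis are present.
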(event `self.ReceiveBeginPlay`
  (add `PXPolicySubsystem.PolicyChangedEvent` (subsystem `PXPolicySubsystem`) (`|CreateDelegate` :!event `Check On Policy Changed`))
  (add `PXConstructionSubsystem.ConstructionFinishedEvent` (subsystem `PXConstructionSubsystem`) (`|CreateDelegate` :!event `Check On Construction`))
  (add `PXDeconstructionSubsystem.DeconstructionChangedEvent` (subsystem `PXDeconstructionSubsystem`) (`|CreateDelegate` :!event `Check On Deconstruction`)))

(fn `Check for Opposite Extremes`
  (locals (`extreme affinities` :type "Array of PXAffinityEntry Structure") (`axes to check` :type "Array of PXAffinityAxisEntry Structure"))
  (bind _extreme_affinities (`local.extreme affinities`))
  (bind _output_get (set `local.extreme affinities` (`self.Extreme Building Affinities`)))
  (`KismetArrayLibrary.Array_Append` _output_get (`self.Extreme Policy Affinities`))
  (for _array_element (`local.axes to check`)
    (bind (_data _firstaffinity _secondaffinity) (`EntriesBlueprintFunctionLibrary.GetAffinityAxisDetails` _array_element))
    (`/Game/Scenarios/Shared/BlueprintsSerialized/VariableStorage/BP_SharedVariableStorage.Update Contrasting Extremes On Axis` (`/Game/Scenarios/Shared/BlueprintsNonSerialized/SocietyUtils/BPFL_SharedScenariosStorage.Get Shared Variable Storage`) _array_element (and (`KismetArrayLibrary.Array_Contains` _extreme_affinities _firstaffinity) (`KismetArrayLibrary.Array_Contains` _extreme_affinities _secondaffinity)))))

(fn `Check On Construction`
  (params (constructionComponent :type "PXConstructionComponent Object Reference"))
  (locals (NewLocalVar_0 :type "Array of PXAffinityEntry Structure"))
  (set `self.Extreme Building Affinities` (`.extreme building affinities` (`/Game/Scenarios/Shared/BlueprintsNonSerialized/SocietyUtils/BPFL_Quest_Utils.Extreme Buildings` (`local.NewLocalVar_0`))))
  (`self.Check for Opposite Extremes`))

(fn `Check On Deconstruction`
  (params (deconstruction :type "PXDeconstructionComponent Object Reference") (reason :type "EPXDeconstructionChangeReason Enum" :default "Started"))
  (locals (NewLocalVar_1 :type "Array of PXAffinityEntry Structure"))
  (set `self.Extreme Building Affinities` (`.extreme building affinities` (`/Game/Scenarios/Shared/BlueprintsNonSerialized/SocietyUtils/BPFL_Quest_Utils.Extreme Buildings` (`local.NewLocalVar_1`))))
  (`self.Check for Opposite Extremes`))

(fn `Check On Policy Changed`
  (params (policyComponent :type "PXPolicyComponent Object Reference") (previousPolicy :type "PXPolicyType Object Reference") (activePolicy :type "PXPolicyType Object Reference"))
  (locals (NewLocalVar :type "Array of PXAffinityEntry Structure"))
  (set `self.Extreme Policy Affinities` (`.extreme policy affinities1` (`/Game/Scenarios/Shared/BlueprintsNonSerialized/SocietyUtils/BPFL_Quest_Utils.Extreme Policies` (`local.NewLocalVar`))))
  (`self.Check for Opposite Extremes`))