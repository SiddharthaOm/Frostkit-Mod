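; Achievement script for Paradise City: unlocks when the player's main city holds a target population with no significant problems for a set duration.
; It listens to economy change events, checking city size and that each tracked statistic stays at or below a fixed threshold.
; Meeting both conditions sets a game-time deadline, and any failed check clears it.
; Once a check passes at or after the deadline, it unlocks the achievement and unbinds.
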(event `self.ReceiveBeginPlay`
  (if (not (`PXAchievementsUtils.IsAchievementUnlocked` (`self.Achievement Config`)))
    (bind _returnvalue (`|Subsystem`)
      (:`then`
        (add `PXEconomySubsystem.EconomyChangedEvent` _returnvalue (delegate `OnEconomyChange`))))))

(event `OnEconomyChange`
  (params (economy :type "PXEconomyComponent Object Reference"))
  (bind _returnvalue (`PXNationUtils.GetPlayerMainCity`))
  (if (>= (`/Game/Scenarios/Shared/BlueprintsNonSerialized/Communities/BPFL_CommunityUtils.Get Total Size Units in City` _returnvalue) (`self.TargetPopulation`))
    (if (`self.CheckIfProblemsAbsent` _returnvalue)
      (if (`PXTimeUtils.NotEqual` (`self.Timestamp`))
        (if (`PXTimeUtils.GreaterEqual` (`PXTimeUtils.GetCurrentGameTime`) (`self.Timestamp`))
          (`ElbAchievementsSubsystem.UnlockAchievement` (subsystem `PXAchievementsSubsystem`) (`self.Achievement Config`))
          (remove `PXEconomySubsystem.EconomyChangedEvent` (`|Subsystem`) (delegate `OnEconomyChange`)))
        (else
          (set `self.Timestamp` (`PXTimeUtils.Add` (`PXTimeUtils.GetCurrentGameTime`) (`self.WaitTarget`)))))
      (else
        (set `self.Timestamp` (struct) :!label _label)))
    (else
      (goto _label))))

(fn `CheckIfProblemsAbsent`
  (params (City :type "PXCityComponent Object Reference"))
  (returns (ProblemsAbsent :type Boolean))
  (locals (Problem :type Boolean) (NoProblem :type Boolean))
  (for _array_element (`self.Stats`)
    (if (<= (`PXStatisticUtils.GetCurrentStatisticValue` City _array_element) 10.0)
      (set `local.NoProblem` true)
      (else
        (set `local.NoProblem` false)
        (break))))
  (return (`local.NoProblem`)))