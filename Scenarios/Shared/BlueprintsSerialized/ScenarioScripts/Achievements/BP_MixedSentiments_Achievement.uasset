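; Achievement script that unlocks the Mixed Sentiments achievement when a protest and a rally are ongoing at the same time.
; On BeginPlay, if the achievement is still locked, it listens for ongoing action changes from the ongoing action subsystem.
; Whenever an action starts, it counts active protests and rallies, then unlocks the achievement and unbinds once at least one of each exists.
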(event `self.ReceiveBeginPlay`
  (if (not (`PXAchievementsUtils.IsAchievementUnlocked` (`self.AchievementConfig`)))
    (add `PXOngoingActionSubsystem.OngoingActionChangedEvent` (subsystem `PXOngoingActionSubsystem`) (delegate `On Ongoing Action Changed`))))

(event `On Ongoing Action Changed`
  (params (changeType :type "EPXOngoingActionChangeType Enum" :default "HintsStart") (ongoingAction :type "PXOngoingActionComponent Object Reference"))
  (if (`|EnumEquality` changeType "Start")
    (bind _number (`/Game/Scenarios/Shared/BlueprintsNonSerialized/OngoingEvents/BPFL_OngoingAction_Utils.GetNumberOfOngoingActionsOfType` "/Game/Scenarios/Shared/Configs/OngoingActions/System_Started/DA_Protest.DA_Protest"))
    (bind _number_2 (`/Game/Scenarios/Shared/BlueprintsNonSerialized/OngoingEvents/BPFL_OngoingAction_Utils.GetNumberOfOngoingActionsOfType` "/Game/Scenarios/Shared/Configs/OngoingActions/System_Started/DA_Rally.DA_Rally"))
    (if (and (>= _number_2 1) (>= _number 1))
      (`ElbAchievementsSubsystem.UnlockAchievement` (subsystem `PXAchievementsSubsystem`) (`self.AchievementConfig`))
      (remove `PXOngoingActionSubsystem.OngoingActionChangedEvent` (subsystem `PXOngoingActionSubsystem`) (delegate `On Ongoing Action Changed`)))))