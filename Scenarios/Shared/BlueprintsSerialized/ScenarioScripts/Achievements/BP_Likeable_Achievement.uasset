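; Scenario achievement script for "Likeable", which unlocks when the game is won without the player's communities falling into poor standing.
; On BeginPlay, if still locked, it binds to community standing changes and the game win event.
; Each standing change rescans all player-nation communities; any at Standing_0 or Standing_1 unbinds both events, disqualifying the run.
; A win while still bound unlocks the achievement and unbinds.
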(event `self.ReceiveBeginPlay`
  (if (not (`PXAchievementsUtils.IsAchievementUnlocked` (`self.AchievementConfig`)))
    (bind _returnvalue (`|Subsystem`)
      (:`then`
        (add `PXTrustSubsystem.CommunityStandingChangedEvent` _returnvalue (`|CreateDelegate` :!event `OnCommunityStandingChanged`))
        (add `/Game/Scenarios/Shared/BlueprintsSerialized/VariableStorage/BP_SharedVariableStorage.GameWinEvent` (`/Game/Scenarios/Shared/BlueprintsNonSerialized/SocietyUtils/BPFL_SharedScenariosStorage.Get Shared Variable Storage`) (`|CreateDelegate` :!event `OnGameFinished`))))))

(event `OnGameFinished`
  (`ElbAchievementsSubsystem.UnlockAchievement` (subsystem `PXAchievementsSubsystem`) (`self.AchievementConfig`))
  (remove `PXTrustSubsystem.CommunityStandingChangedEvent` (`|Subsystem`) (`|CreateDelegate` :!event `OnCommunityStandingChanged`) :!label _label)
  (remove `/Game/Scenarios/Shared/BlueprintsSerialized/VariableStorage/BP_SharedVariableStorage.GameWinEvent` (`/Game/Scenarios/Shared/BlueprintsNonSerialized/SocietyUtils/BPFL_SharedScenariosStorage.Get Shared Variable Storage`) (`|CreateDelegate` :!event `OnGameFinished`)))

(event `OnCommunityStandingChanged`
  (params (communityType :type "PXCommunityType Object Reference") (oldStanding :type "Float (single-precision)") (newStanding :type "Float (single-precision)"))
  (bind _output_get (set `self.AllCommunities` (`PXCommunityUtils.GetAllCommunitiesFromNation` (`PXNationUtils.GetPlayerNation`))))
  (for _array_element _output_get
    (bind _returnvalue (`/Game/Scenarios/Shared/BlueprintsNonSerialized/FactionEmergence/BPFL_FactionEmergenceUtils.Get Community Relations Trait Helper` _array_element))
    (if (or (== _returnvalue "/Game/Scenarios/Shared/Configs/Traits/Traits/DA_Standing_1.DA_Standing_1") (== _returnvalue "/Game/Scenarios/Shared/Configs/Traits/Traits/DA_Standing_0.DA_Standing_0"))
      (goto _label))))