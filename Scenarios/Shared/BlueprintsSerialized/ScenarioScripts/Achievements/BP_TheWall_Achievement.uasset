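; Achievement script for The Wall, unlocked by finishing the game without ever taking in people from the Frostland.
; A routine with no active trigger in this graph binds a handler to the game win event while the achievement is still locked.
; Another untriggered chain checks the shared-storage count of Frostland people taken, unlocks through the achievements subsystem if zero, then unbinds from the win event.
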(event `self.ReceiveBeginPlay`)

(event `OnGameFinished`
  (remove `/Game/Scenarios/Shared/BlueprintsSerialized/VariableStorage/BP_SharedVariableStorage.GameWinEvent` (`/Game/Scenarios/Shared/BlueprintsNonSerialized/SocietyUtils/BPFL_SharedScenariosStorage.Get Shared Variable Storage`) (`|CreateDelegate` :!event `OnGameFinished`)))