(event `self.ReceiveBeginPlay`)

(event `OnGameFinished`
  (remove `/Game/Scenarios/Shared/BlueprintsSerialized/VariableStorage/BP_SharedVariableStorage.GameWinEvent` (`/Game/Scenarios/Shared/BlueprintsNonSerialized/SocietyUtils/BPFL_SharedScenariosStorage.Get Shared Variable Storage`) (delegate `OnGameFinished`)))

(fn `CanUnlockAchievement`
  (returns (Result :type Boolean))
  (locals (Parliament :type "PXParliamentComponent Object Reference") (Items :type "Array of PXVotingHistoryItem Structure"))
  (bind _output_get (set `local.Parliament` (`PXParliamentUtils.GetParliamentOfCity` (`PXNationUtils.GetPlayerMainCity`))))
  (`/Engine/EditorBlueprintResources/StandardMacros.IsValid` _output_get
    (:`Is Valid`
      (bind _output_get_2 (set `local.Items` (`PXParliamentUtils.GetVotingHistory` :`parliament` (`local.Parliament`) :`passFilter` "All" :`promiseFilter` "All" :`swayFilter` "All" :`recountFilter` "All")))
      (for _array_element _output_get_2
        (if (not (`.SessionRequested` (break `PXVotingHistoryItem` _array_element)))
          (return false)))
      (return true))
    (:`Is Not Valid`
      (return false))))