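; Achievement script for Green Power, unlocked when the player's main city runs on enough steam at a target squalor level.
; On BeginPlay it binds to the economy changed event unless the achievement is already unlocked.
; Each change checks that steam supply, fulfilled Warmth and required Warmth all reach the same steam target, and that the Squalor trait matches its target.
; Success unlocks the achievement and unbinds the listener.
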(event `self.ReceiveBeginPlay`
  (if (not (`PXAchievementsUtils.IsAchievementUnlocked` (`self.AchievementConfig`)))
    (bind _returnvalue (`|Subsystem`)
      (:`then`
        (add `PXEconomySubsystem.EconomyChangedEvent` _returnvalue (delegate `OnEconomyChange`))))))

(event `OnEconomyChange`
  (params (economy :type "PXEconomyComponent Object Reference"))
  (bind _returnvalue (`PXNationUtils.GetPlayerMainCity`))
  (bind _steamtarger (`self.SteamTarger`))
  (if (>= (`PXEconomyUtils.GetSupplyOfResource` _returnvalue "/Game/Scenarios/Shared/Configs/Resources/Types/DA_SteamResource.DA_SteamResource") (`self.SteamTarger`))
    (if (and (>= (`PXNeedUtils.GetCityNeedFulfilled` _returnvalue "/Game/Scenarios/Shared/Configs/Needs/Needs/DA_Warmth.DA_Warmth") _steamtarger) (>= (`PXNeedUtils.GetCityNeedRequired` _returnvalue "/Game/Scenarios/Shared/Configs/Needs/Needs/DA_Warmth.DA_Warmth") _steamtarger) (== (`/Game/Scenarios/Shared/BlueprintsNonSerialized/SocietyUtils/BPFL_CanBeStarted_Utils.Get Stat Trait from Int` _returnvalue "/Game/Scenarios/Shared/Configs/Statistics/Entries/DA_Squalor.DA_Squalor" (`/Game/Scenarios/Shared/BlueprintsNonSerialized/Cities/BPFL_CityUtils.GetCurrentStatisticValue` _returnvalue "/Game/Scenarios/Shared/Configs/Statistics/Entries/DA_Squalor.DA_Squalor")) (`self.TargetSqualor`)))
      (`ElbAchievementsSubsystem.UnlockAchievement` (subsystem `PXAchievementsSubsystem`) (`self.AchievementConfig`))
      (remove `PXEconomySubsystem.EconomyChangedEvent` (`|Subsystem`) (delegate `OnEconomyChange`)))))