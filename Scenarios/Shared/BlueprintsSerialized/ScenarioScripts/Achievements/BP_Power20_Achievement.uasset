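; Scenario achievement script that unlocks an achievement for keeping enough non-hub districts at Comfortable heat or above for a target time.
; While the achievement is locked, heat level changes trigger a count of qualifying districts across player cities.
; Reaching the required count records a start time and binds a week-passed check; falling short resets both.
; Once enough time has elapsed, it unbinds both events and unlocks the achievement.
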(event `self.ReceiveBeginPlay`
  (if (not (`PXAchievementsUtils.IsAchievementUnlocked` (`self.AchievementConfig`)))
    (bind _returnvalue (`|Subsystem`)
      (:`then`
        (add `PXHeatLevelSubsystem.HeatLevelChangedEvent` _returnvalue (`|CreateDelegate` :!event `DistrictTemperatureCheck`))))))

(fn `DistrictTemperatureCheck`
  (params (heatComponent :type "PXHeatLevelComponent Object Reference") (oldHeatLevel :type "PXHeatLevelType Object Reference"))
  (locals (AllDistrictsWithHeatLevel :type "Array of PXDistrictComponent Object Reference"))
  (for _array_element (`PXNationUtils.GetAllPlayerCities`)
    (for _array_element_2 (`PXDistrictUtils.FilterDistrictsByHeatLevel` (`PXCityComponent.GetDistricts` _array_element) "/Game/Scenarios/Shared/Configs/Heat/HeatLevels/DA_HeatLevel_6_Comfortable.DA_HeatLevel_6_Comfortable")
      (if (not (`PXTagUtils.HasGameplayTag` (`ActorComponent.GetOwner` _array_element_2) (struct :`TagName` "District.Hub")))
        (`KismetArrayLibrary.Array_Add` (`local.AllDistrictsWithHeatLevel`))))
    (if (>= (`KismetArrayLibrary.Array_Length` (`local.AllDistrictsWithHeatLevel`)) (`self.WarmDistrictsRequired`))
      (if (`PXTimeUtils.Equal` (`self.CheckStartingTime`))
        (set `self.CheckStartingTime` (`PXTimeUtils.GetCurrentGameTime`))
        (bind _returnvalue (`|Subsystem`)
          (:`then`
            (add `PXTimeSubsystem.WeekPassedEvent` _returnvalue (`|CreateDelegate` :!event `WeeksRequiredCheck`)))))
      (else
        (set `self.CheckStartingTime` (struct))
        (bind _returnvalue_2 (`|Subsystem`)
          (:`then`
            (remove `PXTimeSubsystem.WeekPassedEvent` _returnvalue_2 (`|CreateDelegate` :!event `WeeksRequiredCheck`))))))))

(fn `WeeksRequiredCheck`
  (params (CurrentGameTime :type "PXGameTime Structure"))
  (if (`PXTimeUtils.GreaterEqual` (`PXTimeUtils.Subtract` CurrentGameTime (`self.CheckStartingTime`)) (`self.TargetTime`))
    (bind _returnvalue (`|Subsystem`)
      (:`then`
        (remove `PXHeatLevelSubsystem.HeatLevelChangedEvent` _returnvalue (`|CreateDelegate` :!event `DistrictTemperatureCheck`))
        (bind _returnvalue_2 (`|Subsystem`)
          (:`then`
            (remove `PXTimeSubsystem.WeekPassedEvent` _returnvalue_2 (`|CreateDelegate` :!event `WeeksRequiredCheck`))
            (`ElbAchievementsSubsystem.UnlockAchievement` (subsystem `PXAchievementsSubsystem`) (`self.AchievementConfig`))))))))