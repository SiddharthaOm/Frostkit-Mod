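; Scenario achievement script that unlocks the Confident achievement when the game is won without any trust or tension fail.
; On BeginPlay it binds to the shared game-win event unless already unlocked.
; On win it checks whether any quest type in the TrustFail and TensionFail lists is active or finished, then unlocks and unbinds.
; The no-op OnQuestStart event remains solely for save/load parity and must not be deleted.
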(event `self.ReceiveBeginPlay`
  (if (not (`PXAchievementsUtils.IsAchievementUnlocked` (`self.AchievementConfig`)))
    (add `/Game/Scenarios/Shared/BlueprintsSerialized/VariableStorage/BP_SharedVariableStorage.GameWinEvent` (`/Game/Scenarios/Shared/BlueprintsNonSerialized/SocietyUtils/BPFL_SharedScenariosStorage.Get Shared Variable Storage`) (`|CreateDelegate` :!event `OnGameFinished`))))

(event `OnQuestStart`
  (params (Quest :type "PXQuest Object Reference"))
  ;[1 0 0] THIS MUST STAY. NEVER DELETE IT. ON 09.09.2024 for REVIEW PATCH BUILD WE HAD TO FIX THE ACHIEVEMENT AND REMOVED THE BIND TO ON QUEST STARTED AND IMPLEMENTATION FOR THAT EVENT. BUT THE EVENT MUST STAY FOR SAVE LOAD PARITY
  (`/Engine/EditorBlueprintResources/StandardMacros.IsValid` Quest))

(event `OnGameFinished`
  (if (not (or (`self.Has Any Tension Fail Happened`) (`self.Has Any Trust Fail Happened`)))
    (`ElbAchievementsSubsystem.UnlockAchievement` (subsystem `PXAchievementsSubsystem`) (`self.AchievementConfig`))
    (remove `/Game/Scenarios/Shared/BlueprintsSerialized/VariableStorage/BP_SharedVariableStorage.GameWinEvent` (`/Game/Scenarios/Shared/BlueprintsNonSerialized/SocietyUtils/BPFL_SharedScenariosStorage.Get Shared Variable Storage`) (`|CreateDelegate` :!event `OnGameFinished`))
    (remove `PXQuestSubsystem.QuestStartEvent` (`|Subsystem`) (`|CreateDelegate` :!event `OnQuestStart`))))

(fn `Has Any Tension Fail Happened`
  (returns (`Return value` :type Boolean))
  (locals (Happened :type Boolean))
  (set `local.Happened` false)
  (for _array_element (`self.TensionFail`)
    (if (or (`PXQuestUtils.IsAnyQuestOfTypeActive` _array_element) (`PXQuestUtils.IsAnyQuestOfTypeFinished` _array_element))
      (set `local.Happened` true)))
  (return (`local.Happened`)))

(fn `Has Any Trust Fail Happened`
  (returns (`Return value` :type Boolean))
  (locals (Happened :type Boolean))
  (set `local.Happened` false)
  (for _array_element (`self.TrustFail`)
    (if (or (`PXQuestUtils.IsAnyQuestOfTypeActive` _array_element) (`PXQuestUtils.IsAnyQuestOfTypeFinished` _array_element))
      (set `local.Happened` true)))
  (return (`local.Happened`)))