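; Blood achievement script Blueprint that, as wired, never unlocks its achievement because the key logic is disconnected.
; Quest start and game finish handlers only unbind from the quest-start and game-win events.
; Unconnected chains hold the difficulty-gated binding (Hard or above, not yet unlocked), the unlock call and a PXPromiseQuest class check that would stop tracking.
; BeginPlay is empty.
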(event `self.ReceiveBeginPlay`)

(event `OnQuestStart`
  (params (Quest :type "PXQuest Object Reference"))
  (remove `PXQuestSubsystem.QuestStartEvent` (`|Subsystem`) (`|CreateDelegate` :!event `OnQuestStart`) :!label _label)
  (remove `/Game/Scenarios/Shared/BlueprintsSerialized/VariableStorage/BP_SharedVariableStorage.GameWinEvent` (`/Game/Scenarios/Shared/BlueprintsNonSerialized/SocietyUtils/BPFL_SharedScenariosStorage.Get Shared Variable Storage`) (`|CreateDelegate` :!event `OnGameFinished`)))

(event `OnGameFinished`
  (goto _label))