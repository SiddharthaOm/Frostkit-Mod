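; Achievement script that unlocks an achievement when the game is won without any community member dying.
; On BeginPlay, if the achievement is still locked, it binds to the community size changed event and the game win event from shared variable storage.
; A change of type Death unbinds both listeners, forfeiting the achievement for the session.
; A win unlocks the configured achievement through the achievements subsystem, then unbinds as well.
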(event `self.ReceiveBeginPlay`
  (if (not (`PXAchievementsUtils.IsAchievementUnlocked` (`self.Achievement Config`)))
    (bind _returnvalue (`|Subsystem`)
      (:`then`
        (add `PXCommunitySubsystem.CommunitySizeChangedEvent` _returnvalue (`|CreateDelegate` :!event `OnDeath`))
        (add `/Game/Scenarios/Shared/BlueprintsSerialized/VariableStorage/BP_SharedVariableStorage.GameWinEvent` (`/Game/Scenarios/Shared/BlueprintsNonSerialized/SocietyUtils/BPFL_SharedScenariosStorage.Get Shared Variable Storage`) (`|CreateDelegate` :!event `OnGameFinished`))))))

(event `OnDeath`
  (params (params :type "PXCommunitySizeChangedEventParameters Structure"))
  (if (`|EnumEquality` (`.ChangeType` (break `PXCommunitySizeChangedEventParameters` params)) "Death")
    (remove `PXCommunitySubsystem.CommunitySizeChangedEvent` (`|Subsystem`) (`|CreateDelegate` :!event `OnDeath`) :!label _label)
    (remove `/Game/Scenarios/Shared/BlueprintsSerialized/VariableStorage/BP_SharedVariableStorage.GameWinEvent` (`/Game/Scenarios/Shared/BlueprintsNonSerialized/SocietyUtils/BPFL_SharedScenariosStorage.Get Shared Variable Storage`) (`|CreateDelegate` :!event `OnGameFinished`))))

(event `OnGameFinished`
  (`ElbAchievementsSubsystem.UnlockAchievement` (subsystem `PXAchievementsSubsystem`) (`self.Achievement Config`))
  (goto _label))