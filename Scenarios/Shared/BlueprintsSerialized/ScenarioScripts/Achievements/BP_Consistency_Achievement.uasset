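; Achievement script that unlocks the configured Consistency achievement if the game is won without the player collecting two opposing affinities.
; While the achievement is locked, it binds to game win, parliament vote and research topic change events.
; Affinities from finished research and non-session-requested vote policies accumulate in PlayerAffinities.
; An affinity whose opposite is already recorded unbinds all listeners, forfeiting the achievement for that run.
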(event `self.ReceiveBeginPlay`
  (if (not (`PXAchievementsUtils.IsAchievementUnlocked` (`self.Achievement Config`)))
    (add `/Game/Scenarios/Shared/BlueprintsSerialized/VariableStorage/BP_SharedVariableStorage.GameWinEvent` (`/Game/Scenarios/Shared/BlueprintsNonSerialized/SocietyUtils/BPFL_SharedScenariosStorage.Get Shared Variable Storage`) (`|CreateDelegate` :!event `OnGameFinished`))
    (`|Subsystem`
      (:`then`
        (`/Game/Scenarios/Shared/BlueprintsNonSerialized/HouseOfDelegates/BPFL_HoD_Functions.Bind Event To Parliament Vote Finished` (`|CreateDelegate` :!event `OnVoteFinished`))
        (bind _returnvalue (`|Subsystem`)
          (:`then`
            (add `PXResearchSubsystem.ResearchTopicChangedEvent` _returnvalue (`|CreateDelegate` :!event `OnResearchFinished`))))))))

(event `OnGameFinished`
  (`ElbAchievementsSubsystem.UnlockAchievement` (subsystem `PXAchievementsSubsystem`) (`self.Achievement Config`))
  (remove `PXParliamentSubsystem.VoteFinishedEvent` (`|Subsystem`) (`|CreateDelegate` :!event `OnVoteFinished`) :!label _label)
  (remove `PXResearchSubsystem.ResearchTopicChangedEvent` (`|Subsystem`) (`|CreateDelegate` :!event `OnResearchFinished`))
  (remove `/Game/Scenarios/Shared/BlueprintsSerialized/VariableStorage/BP_SharedVariableStorage.GameWinEvent` (`/Game/Scenarios/Shared/BlueprintsNonSerialized/SocietyUtils/BPFL_SharedScenariosStorage.Get Shared Variable Storage`) (`|CreateDelegate` :!event `OnGameFinished`)))

(event `OnVoteFinished`
  (params (parliament :type "PXParliamentComponent Object Reference") (affectedPolicy :type "PXPolicyType Object Reference") (results :type "PXVoteResultData Structure"))
  (bind (_timestamp _sessionindex _policy _passed _results _promisemade _swayused _recountedvotes _sessionrequested) (break `PXVotingHistoryItem` (`.latestItem` (`PXParliamentUtils.GetVotingHistory` :`parliament` parliament :`passFilter` "All" :`promiseFilter` "All" :`swayFilter` "All" :`recountFilter` "All"))))
  (if (not _sessionrequested)
    (bind _output_get (set `self.Temp Affinity Changes` (`PXPolicyType.AffinityChanges` _policy)))
    (if (!= (`KismetArrayLibrary.Array_Length` _output_get) 0)
      (for _array_element _output_get
        (bind _affinityentry (break `PXAffinityValue` (`.AffinityValue` (break `PXAffinityChange` _array_element))))
        (if (not (`KismetArrayLibrary.Array_Contains` (`self.PlayerAffinities`) _affinityentry))
          (bind (_data_ingamename _data_shortdescription _data_axis _data_axisdirection _data_oppositeaffinity) (break `PXAffinity` (`EntriesBlueprintFunctionLibrary.GetAffinityDetails` _affinityentry)))
          (if (`KismetArrayLibrary.Array_Contains` (`self.PlayerAffinities`) _data_oppositeaffinity)
            (goto _label)
            (else
              (`KismetArrayLibrary.Array_AddUnique` (`self.PlayerAffinities`) _affinityentry))))))))

(event `OnResearchFinished`
  (params (topic :type "PXResearchTopic Object Reference") (outcome :type "PXResearchOutcome Object Reference") (community :type "PXCommunityComponent Object Reference") (changeReason :type "EPXResearchChangeReason Enum" :default "Started") (silent :type Boolean))
  (bind _affinity (`PXResearchOutcome.Affinity` outcome))
  (bind (_data_ingamename _data_shortdescription _data_axis _data_axisdirection _data_oppositeaffinity) (break `PXAffinity` (`EntriesBlueprintFunctionLibrary.GetAffinityDetails` _affinity)))
  (if (`|EnumEquality` changeReason "Finished")
    (if (not (`PXAffinityUtils.Equal` _affinity))
      (if (`KismetArrayLibrary.Array_Contains` (`self.PlayerAffinities`) _affinity)
        _
        (elif (`KismetArrayLibrary.Array_Contains` (`self.PlayerAffinities`) _data_oppositeaffinity)
          (goto _label)
          (else
            (`KismetArrayLibrary.Array_AddUnique` (`self.PlayerAffinities`) _affinity)))))))