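; Sandbox scenario weather timeline that schedules temperature shifts and storms on the player's main city.
; BeginPlay picks a preset by weather difficulty or Serenity mode, randomly choosing one of two temperature timelines with four storms, and records the first storm's timing.
; Storm level and shape are drawn randomly from pools, with Serenity using its own levels.
; Logic ticks append a repeating late-game temperature-and-storm loop whenever the refresh timestamp is reached.
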(event `self.ReceiveBeginPlay`
  (add `PXTimeSubsystem.LogicTickEvent` (subsystem `PXTimeSubsystem`) (delegate `OnLogicTickEvent`))
  (if (`.SerenityMode` (break `PXScenarioRuntimeSettings` (`PXWorldManagementSubsystem.GetActiveScenarioRuntimeSettings` (subsystem `PXWorldManagementSubsystem`))))
    (`self.DIFFICULTY LEVEL: SERENITY`)
    (else
      (`self.Difficulty level check`
        (:`MODERATE`
          (`self.DIFFICULTY LEVEL: MODERATE`))
        (:`CHALLENGING`
          (`self.DIFFICULTY LEVEL: CHALLENGING`))
        (:`HARD`
          (`self.DIFFICULTY LEVEL: HARD`))
        (:`EXTREME`
          (`self.DIFFICULTY LEVEL: EXTREME`))))))

(event `OnLogicTickEvent`
  (params (DeltaGameTime :type "PXGameTime Structure") (CurrentGameTime :type "PXGameTime Structure"))
  ;[1 1 1] LATE GAME WEATHER LOOP
  (if (`PXTimeUtils.GreaterEqual` CurrentGameTime (`self.RefreshTimestamp`))
    (if (`.SerenityMode` (break `PXScenarioRuntimeSettings` (`PXWorldManagementSubsystem.GetActiveScenarioRuntimeSettings` (subsystem `PXWorldManagementSubsystem`))))
      (`self.Late Game Loop Serenity (~300 weeks)`)
      (else
        (`self.Late Game Loop (~300 weeks)`)))))

(fn `DIFFICULTY LEVEL: CHALLENGING`
  (switch `int` (`PXRandomLibrary.PXRandomIntegerInRange` 0 1)
    (:`0`
      (`|ExecutionSequence`
        (:`then_0`
          (`PXTemperatureUtils.SetTemperatureLevelChangeAt` (struct :`ScaledTicks` 67200) 1)
          (`PXTemperatureUtils.SetTemperatureLevelChangeAt` (struct :`ScaledTicks` 84000) -1)
          (`PXTemperatureUtils.SetTemperatureLevelChangeAt` (struct :`ScaledTicks` 117600) 1)
          (`PXTemperatureUtils.SetTemperatureLevelChangeAt` (struct :`ScaledTicks` 184800) 1)
          (`PXTemperatureUtils.SetTemperatureLevelChangeAt` (struct :`ScaledTicks` 235200) -1)
          (`PXTemperatureUtils.SetTemperatureLevelChangeAt` (struct :`ScaledTicks` 386400) 1)
          (`PXTemperatureUtils.SetTemperatureLevelChangeAt` (struct :`ScaledTicks` 436800) 1)
          (`PXTemperatureUtils.SetTemperatureLevelChangeAt` (struct :`ScaledTicks` 487200) -1)
          (`PXTemperatureUtils.SetTemperatureLevelChangeAt` (struct :`ScaledTicks` 688800) 1)
          (`PXTemperatureUtils.SetTemperatureLevelChangeAt` (struct :`ScaledTicks` 722400) 1)
          (`PXTemperatureUtils.SetTemperatureLevelChangeAt` (struct :`ScaledTicks` 789600) 1)
          (`PXTemperatureUtils.SetTemperatureLevelChangeAt` (struct :`ScaledTicks` 856800) -1)
          (`PXTemperatureUtils.SetTemperatureLevelChangeAt` (struct :`ScaledTicks` 1041600) 1)
          (`PXTemperatureUtils.SetTemperatureLevelChangeAt` (struct :`ScaledTicks` 1075200) -1)
          (`PXTemperatureUtils.SetTemperatureLevelChangeAt` (struct :`ScaledTicks` 1159200) 1)
          (`PXTemperatureUtils.SetTemperatureLevelChangeAt` (struct :`ScaledTicks` 1444800) 1)
          (`PXTemperatureUtils.SetTemperatureLevelChangeAt` (struct :`ScaledTicks` 1495200) 1)
          (`PXTemperatureUtils.SetTemperatureLevelChangeAt` (struct :`ScaledTicks` 1579200) -1)
          (bind _returnvalue (`PXTemperatureUtils.GetLastTemperatureTimelineEntryTimestamp`))
          (set `self.RefreshTimestamp` (`PXTimeUtils.Subtract` _returnvalue (struct :`ScaledTicks` 134400))))
        (:`then_1`
          (set `/Game/Scenarios/Sandbox/BlueprintsNonSerialized/BP_Sandbox_Constants_BaseClass.Sandbox Beta Storm Timing` (`self.Normal 0 First Storm Timestamp`) (`/Game/Scenarios/Sandbox/BlueprintsNonSerialized/BPFL_SandboxStorage.Get Sandbox Constants Storage`))
          (`self.RandomStormSpawnerFixedTime` (struct :`ScaledTicks` 50400) (`self.Normal 0 First Storm Timestamp`) (`self.FirstStormPossibleWhiteouts`) (`self.WeatherShapeVariant_Base`))
          (`self.RandomStormSpawnerFixedTime` (struct :`ScaledTicks` 84000) (struct :`ScaledTicks` 588000) (`self.All Weather Levels`) (`self.WeatherShapeVariant_Base`))
          (`self.RandomStormSpawnerFixedTime` (struct :`ScaledTicks` 84000) (struct :`ScaledTicks` 924000) (`self.All Weather Levels`) (`self.WeatherShapeVariant_LateGame`))
          (`self.RandomStormSpawnerFixedTime` (struct :`ScaledTicks` 117600) (struct :`ScaledTicks` 1310400) (`self.All Weather Levels`) (`self.WeatherShapeVariant_LateGame`)))))
    (:`1`
      (`|ExecutionSequence`
        (:`then_0`
          (`PXTemperatureUtils.SetTemperatureLevelChangeAt` (struct :`ScaledTicks` 67200) 1)
          (`PXTemperatureUtils.SetTemperatureLevelChangeAt` (struct :`ScaledTicks` 84000) -1)
          (`PXTemperatureUtils.SetTemperatureLevelChangeAt` (struct :`ScaledTicks` 100800) 1)
          (`PXTemperatureUtils.SetTemperatureLevelChangeAt` (struct :`ScaledTicks` 201600) 1)
          (`PXTemperatureUtils.SetTemperatureLevelChangeAt` (struct :`ScaledTicks` 235200) -1)
          (`PXTemperatureUtils.SetTemperatureLevelChangeAt` (struct :`ScaledTicks` 369600) 1)
          (`PXTemperatureUtils.SetTemperatureLevelChangeAt` (struct :`ScaledTicks` 453600) 1)
          (`PXTemperatureUtils.SetTemperatureLevelChangeAt` (struct :`ScaledTicks` 504000) -1)
          (`PXTemperatureUtils.SetTemperatureLevelChangeAt` (struct :`ScaledTicks` 705600) 1)
          (`PXTemperatureUtils.SetTemperatureLevelChangeAt` (struct :`ScaledTicks` 739200) 1)
          (`PXTemperatureUtils.SetTemperatureLevelChangeAt` (struct :`ScaledTicks` 772800) 1)
          (`PXTemperatureUtils.SetTemperatureLevelChangeAt` (struct :`ScaledTicks` 840000) -1)
          (`PXTemperatureUtils.SetTemperatureLevelChangeAt` (struct :`ScaledTicks` 1041600) 1)
          (`PXTemperatureUtils.SetTemperatureLevelChangeAt` (struct :`ScaledTicks` 1075200) -1)
          (`PXTemperatureUtils.SetTemperatureLevelChangeAt` (struct :`ScaledTicks` 1176000) 1)
          (`PXTemperatureUtils.SetTemperatureLevelChangeAt` (struct :`ScaledTicks` 1444800) 1)
          (`PXTemperatureUtils.SetTemperatureLevelChangeAt` (struct :`ScaledTicks` 1478400) 1)
          (`PXTemperatureUtils.SetTemperatureLevelChangeAt` (struct :`ScaledTicks` 1562400) -1)
          (bind _returnvalue_2 (`PXTemperatureUtils.GetLastTemperatureTimelineEntryTimestamp`))
          (set `self.RefreshTimestamp` (`PXTimeUtils.Subtract` _returnvalue_2 (struct :`ScaledTicks` 134400))))
        (:`then_1`
          (set `/Game/Scenarios/Sandbox/BlueprintsNonSerialized/BP_Sandbox_Constants_BaseClass.Sandbox Beta Storm Timing` (`self.Normal 1 First Storm Timestamp`) (`/Game/Scenarios/Sandbox/BlueprintsNonSerialized/BPFL_SandboxStorage.Get Sandbox Constants Storage`))
          (`self.RandomStormSpawnerFixedTime` (struct :`ScaledTicks` 50400) (`self.Normal 1 First Storm Timestamp`) (`self.FirstStormPossibleWhiteouts`) (`self.WeatherShapeVariant_Base`))
          (`self.RandomStormSpawnerFixedTime` (struct :`ScaledTicks` 84000) (struct :`ScaledTicks` 604800) (`self.All Weather Levels`) (`self.WeatherShapeVariant_Base`))
          (`self.RandomStormSpawnerFixedTime` (struct :`ScaledTicks` 84000) (struct :`ScaledTicks` 940800) (`self.All Weather Levels`) (`self.WeatherShapeVariant_LateGame`))
          (`self.RandomStormSpawnerFixedTime` (struct :`ScaledTicks` 117600) (struct :`ScaledTicks` 1293600) (`self.All Weather Levels`) (`self.WeatherShapeVariant_LateGame`)))))))

(fn `DIFFICULTY LEVEL: EXTREME`
  (switch `int` (`PXRandomLibrary.PXRandomIntegerInRange` 0 1)
    (:`0`
      (`|ExecutionSequence`
        (:`then_0`
          (`PXTemperatureUtils.SetTemperatureLevelChangeAt` (struct :`ScaledTicks` 84000) 1)
          (`PXTemperatureUtils.SetTemperatureLevelChangeAt` (struct :`ScaledTicks` 151200) 1)
          (`PXTemperatureUtils.SetTemperatureLevelChangeAt` (struct :`ScaledTicks` 201600) 1)
          (`PXTemperatureUtils.SetTemperatureLevelChangeAt` (struct :`ScaledTicks` 252000) -1)
          (`PXTemperatureUtils.SetTemperatureLevelChangeAt` (struct :`ScaledTicks` 403200) 1)
          (`PXTemperatureUtils.SetTemperatureLevelChangeAt` (struct :`ScaledTicks` 420000) 1)
          (`PXTemperatureUtils.SetTemperatureLevelChangeAt` (struct :`ScaledTicks` 504000) -1)
          (`PXTemperatureUtils.SetTemperatureLevelChangeAt` (struct :`ScaledTicks` 688800) 1)
          (`PXTemperatureUtils.SetTemperatureLevelChangeAt` (struct :`ScaledTicks` 722400) 1)
          (`PXTemperatureUtils.SetTemperatureLevelChangeAt` (struct :`ScaledTicks` 772800) 1)
          (`PXTemperatureUtils.SetTemperatureLevelChangeAt` (struct :`ScaledTicks` 823200) -1)
          (`PXTemperatureUtils.SetTemperatureLevelChangeAt` (struct :`ScaledTicks` 1024800) 1)
          (`PXTemperatureUtils.SetTemperatureLevelChangeAt` (struct :`ScaledTicks` 1058400) -1)
          (`PXTemperatureUtils.SetTemperatureLevelChangeAt` (struct :`ScaledTicks` 1142400) 1)
          (`PXTemperatureUtils.SetTemperatureLevelChangeAt` (struct :`ScaledTicks` 1444800) 1)
          (`PXTemperatureUtils.SetTemperatureLevelChangeAt` (struct :`ScaledTicks` 1478400) 1)
          (`PXTemperatureUtils.SetTemperatureLevelChangeAt` (struct :`ScaledTicks` 1579200) -1)
          (bind _returnvalue (`PXTemperatureUtils.GetLastTemperatureTimelineEntryTimestamp`))
          (set `self.RefreshTimestamp` (`PXTimeUtils.Subtract` _returnvalue (struct :`ScaledTicks` 134400))))
        (:`then_1`
          (set `/Game/Scenarios/Sandbox/BlueprintsNonSerialized/BP_Sandbox_Constants_BaseClass.Sandbox Beta Storm Timing` (`self.Extreme 0 First Storm Timestamp`) (`/Game/Scenarios/Sandbox/BlueprintsNonSerialized/BPFL_SandboxStorage.Get Sandbox Constants Storage`))
          (`self.RandomStormSpawnerFixedTime` (struct :`ScaledTicks` 67200) (`self.Extreme 0 First Storm Timestamp`) (`self.FirstStormPossibleWhiteouts`) (`self.WeatherShapeVariant_Base`))
          (`self.RandomStormSpawnerFixedTime` (struct :`ScaledTicks` 100800) (struct :`ScaledTicks` 571200) (`self.All Weather Levels`) (`self.WeatherShapeVariant_Base`))
          (`self.RandomStormSpawnerFixedTime` (struct :`ScaledTicks` 100800) (struct :`ScaledTicks` 907200) (`self.All Weather Levels`) (`self.WeatherShapeVariant_LateGame`))
          (`self.RandomStormSpawnerFixedTime` (struct :`ScaledTicks` 134400) (struct :`ScaledTicks` 1293600) (`self.All Weather Levels`) (`self.WeatherShapeVariant_LateGame`)))))
    (:`1`
      (`|ExecutionSequence`
        (:`then_0`
          (`PXTemperatureUtils.SetTemperatureLevelChangeAt` (struct :`ScaledTicks` 67200) 1)
          (`PXTemperatureUtils.SetTemperatureLevelChangeAt` (struct :`ScaledTicks` 134400) 1)
          (`PXTemperatureUtils.SetTemperatureLevelChangeAt` (struct :`ScaledTicks` 184800) 1)
          (`PXTemperatureUtils.SetTemperatureLevelChangeAt` (struct :`ScaledTicks` 235200) -1)
          (`PXTemperatureUtils.SetTemperatureLevelChangeAt` (struct :`ScaledTicks` 403200) 1)
          (`PXTemperatureUtils.SetTemperatureLevelChangeAt` (struct :`ScaledTicks` 436800) 1)
          (`PXTemperatureUtils.SetTemperatureLevelChangeAt` (struct :`ScaledTicks` 520800) -1)
          (`PXTemperatureUtils.SetTemperatureLevelChangeAt` (struct :`ScaledTicks` 672000) 1)
          (`PXTemperatureUtils.SetTemperatureLevelChangeAt` (struct :`ScaledTicks` 705600) 1)
          (`PXTemperatureUtils.SetTemperatureLevelChangeAt` (struct :`ScaledTicks` 756000) 1)
          (`PXTemperatureUtils.SetTemperatureLevelChangeAt` (struct :`ScaledTicks` 806400) -1)
          (`PXTemperatureUtils.SetTemperatureLevelChangeAt` (struct :`ScaledTicks` 1041600) 1)
          (`PXTemperatureUtils.SetTemperatureLevelChangeAt` (struct :`ScaledTicks` 1075200) -1)
          (`PXTemperatureUtils.SetTemperatureLevelChangeAt` (struct :`ScaledTicks` 1125600) 1)
          (`PXTemperatureUtils.SetTemperatureLevelChangeAt` (struct :`ScaledTicks` 1428000) 1)
          (`PXTemperatureUtils.SetTemperatureLevelChangeAt` (struct :`ScaledTicks` 1478400) 1)
          (`PXTemperatureUtils.SetTemperatureLevelChangeAt` (struct :`ScaledTicks` 1596000) -1)
          (bind _returnvalue_2 (`PXTemperatureUtils.GetLastTemperatureTimelineEntryTimestamp`))
          (set `self.RefreshTimestamp` (`PXTimeUtils.Subtract` _returnvalue_2 (struct :`ScaledTicks` 134400))))
        (:`then_1`
          (set `/Game/Scenarios/Sandbox/BlueprintsNonSerialized/BP_Sandbox_Constants_BaseClass.Sandbox Beta Storm Timing` (`self.Extreme 0 First Storm Timestamp`) (`/Game/Scenarios/Sandbox/BlueprintsNonSerialized/BPFL_SandboxStorage.Get Sandbox Constants Storage`))
          (`self.RandomStormSpawnerFixedTime` (struct :`ScaledTicks` 67200) (`self.Extreme 0 First Storm Timestamp`) (`self.FirstStormPossibleWhiteouts`) (`self.WeatherShapeVariant_Base`))
          (`self.RandomStormSpawnerFixedTime` (struct :`ScaledTicks` 100800) (struct :`ScaledTicks` 571200) (`self.All Weather Levels`) (`self.WeatherShapeVariant_Base`))
          (`self.RandomStormSpawnerFixedTime` (struct :`ScaledTicks` 100800) (struct :`ScaledTicks` 924000) (`self.All Weather Levels`) (`self.WeatherShapeVariant_LateGame`))
          (`self.RandomStormSpawnerFixedTime` (struct :`ScaledTicks` 134400) (struct :`ScaledTicks` 1276800) (`self.All Weather Levels`) (`self.WeatherShapeVariant_LateGame`)))))))

(fn `DIFFICULTY LEVEL: HARD`
  (switch `int` (`PXRandomLibrary.PXRandomIntegerInRange` 0 1)
    (:`0`
      (`|ExecutionSequence`
        (:`then_0`
          (`PXTemperatureUtils.SetTemperatureLevelChangeAt` (struct :`ScaledTicks` 33600) 1)
          (`PXTemperatureUtils.SetTemperatureLevelChangeAt` (struct :`ScaledTicks` 50400) -1)
          (`PXTemperatureUtils.SetTemperatureLevelChangeAt` (struct :`ScaledTicks` 100800) 1)
          (`PXTemperatureUtils.SetTemperatureLevelChangeAt` (struct :`ScaledTicks` 168000) 1)
          (`PXTemperatureUtils.SetTemperatureLevelChangeAt` (struct :`ScaledTicks` 252000) -1)
          (`PXTemperatureUtils.SetTemperatureLevelChangeAt` (struct :`ScaledTicks` 369600) 1)
          (`PXTemperatureUtils.SetTemperatureLevelChangeAt` (struct :`ScaledTicks` 420000) 1)
          (`PXTemperatureUtils.SetTemperatureLevelChangeAt` (struct :`ScaledTicks` 504000) -1)
          (`PXTemperatureUtils.SetTemperatureLevelChangeAt` (struct :`ScaledTicks` 672000) 1)
          (`PXTemperatureUtils.SetTemperatureLevelChangeAt` (struct :`ScaledTicks` 705600) 1)
          (`PXTemperatureUtils.SetTemperatureLevelChangeAt` (struct :`ScaledTicks` 772800) 1)
          (`PXTemperatureUtils.SetTemperatureLevelChangeAt` (struct :`ScaledTicks` 873600) -1)
          (`PXTemperatureUtils.SetTemperatureLevelChangeAt` (struct :`ScaledTicks` 1024800) 1)
          (`PXTemperatureUtils.SetTemperatureLevelChangeAt` (struct :`ScaledTicks` 1058400) -1)
          (`PXTemperatureUtils.SetTemperatureLevelChangeAt` (struct :`ScaledTicks` 1142400) 1)
          (`PXTemperatureUtils.SetTemperatureLevelChangeAt` (struct :`ScaledTicks` 1428000) 1)
          (`PXTemperatureUtils.SetTemperatureLevelChangeAt` (struct :`ScaledTicks` 1461600) 1)
          (`PXTemperatureUtils.SetTemperatureLevelChangeAt` (struct :`ScaledTicks` 1612800) -1)
          (bind _returnvalue (`PXTemperatureUtils.GetLastTemperatureTimelineEntryTimestamp`))
          (set `self.RefreshTimestamp` (`PXTimeUtils.Subtract` _returnvalue (struct :`ScaledTicks` 134400))))
        (:`then_1`
          (set `/Game/Scenarios/Sandbox/BlueprintsNonSerialized/BP_Sandbox_Constants_BaseClass.Sandbox Beta Storm Timing` (`self.Hard 0 First Storm Timestamp`) (`/Game/Scenarios/Sandbox/BlueprintsNonSerialized/BPFL_SandboxStorage.Get Sandbox Constants Storage`))
          (`self.RandomStormSpawnerFixedTime` (struct :`ScaledTicks` 50400) (`self.Hard 0 First Storm Timestamp`) (`self.FirstStormPossibleWhiteouts`) (`self.WeatherShapeVariant_Base`))
          (`self.RandomStormSpawnerFixedTime` (struct :`ScaledTicks` 84000) (struct :`ScaledTicks` 571200) (`self.All Weather Levels`) (`self.WeatherShapeVariant_Base`))
          (`self.RandomStormSpawnerFixedTime` (struct :`ScaledTicks` 84000) (struct :`ScaledTicks` 924000) (`self.All Weather Levels`) (`self.WeatherShapeVariant_LateGame`))
          (`self.RandomStormSpawnerFixedTime` (struct :`ScaledTicks` 117600) (struct :`ScaledTicks` 1293600) (`self.All Weather Levels`) (`self.WeatherShapeVariant_LateGame`)))))
    (:`1`
      (`|ExecutionSequence`
        (:`then_0`
          (`PXTemperatureUtils.SetTemperatureLevelChangeAt` (struct :`ScaledTicks` 33600) 1)
          (`PXTemperatureUtils.SetTemperatureLevelChangeAt` (struct :`ScaledTicks` 50400) -1)
          (`PXTemperatureUtils.SetTemperatureLevelChangeAt` (struct :`ScaledTicks` 84000) 1)
          (`PXTemperatureUtils.SetTemperatureLevelChangeAt` (struct :`ScaledTicks` 168000) 1)
          (`PXTemperatureUtils.SetTemperatureLevelChangeAt` (struct :`ScaledTicks` 235200) -1)
          (`PXTemperatureUtils.SetTemperatureLevelChangeAt` (struct :`ScaledTicks` 352800) 1)
          (`PXTemperatureUtils.SetTemperatureLevelChangeAt` (struct :`ScaledTicks` 403200) 1)
          (`PXTemperatureUtils.SetTemperatureLevelChangeAt` (struct :`ScaledTicks` 504000) -1)
          (`PXTemperatureUtils.SetTemperatureLevelChangeAt` (struct :`ScaledTicks` 688800) 1)
          (`PXTemperatureUtils.SetTemperatureLevelChangeAt` (struct :`ScaledTicks` 722400) 1)
          (`PXTemperatureUtils.SetTemperatureLevelChangeAt` (struct :`ScaledTicks` 756000) 1)
          (`PXTemperatureUtils.SetTemperatureLevelChangeAt` (struct :`ScaledTicks` 856800) -1)
          (`PXTemperatureUtils.SetTemperatureLevelChangeAt` (struct :`ScaledTicks` 1024800) 1)
          (`PXTemperatureUtils.SetTemperatureLevelChangeAt` (struct :`ScaledTicks` 1058400) -1)
          (`PXTemperatureUtils.SetTemperatureLevelChangeAt` (struct :`ScaledTicks` 1125600) 1)
          (`PXTemperatureUtils.SetTemperatureLevelChangeAt` (struct :`ScaledTicks` 1444800) 1)
          (`PXTemperatureUtils.SetTemperatureLevelChangeAt` (struct :`ScaledTicks` 1478400) 1)
          (`PXTemperatureUtils.SetTemperatureLevelChangeAt` (struct :`ScaledTicks` 1612800) -1)
          (bind _returnvalue_2 (`PXTemperatureUtils.GetLastTemperatureTimelineEntryTimestamp`))
          (set `self.RefreshTimestamp` (`PXTimeUtils.Subtract` _returnvalue_2 (struct :`ScaledTicks` 134400))))
        (:`then_1`
          (set `/Game/Scenarios/Sandbox/BlueprintsNonSerialized/BP_Sandbox_Constants_BaseClass.Sandbox Beta Storm Timing` (`self.Hard 1 First Storm Timestamp`) (`/Game/Scenarios/Sandbox/BlueprintsNonSerialized/BPFL_SandboxStorage.Get Sandbox Constants Storage`))
          (`self.RandomStormSpawnerFixedTime` (struct :`ScaledTicks` 50400) (`self.Hard 1 First Storm Timestamp`) (`self.FirstStormPossibleWhiteouts`) (`self.WeatherShapeVariant_Base`))
          (`self.RandomStormSpawnerFixedTime` (struct :`ScaledTicks` 84000) (struct :`ScaledTicks` 588000) (`self.All Weather Levels`) (`self.WeatherShapeVariant_Base`))
          (`self.RandomStormSpawnerFixedTime` (struct :`ScaledTicks` 84000) (struct :`ScaledTicks` 924000) (`self.All Weather Levels`) (`self.WeatherShapeVariant_LateGame`))
          (`self.RandomStormSpawnerFixedTime` (struct :`ScaledTicks` 117600) (struct :`ScaledTicks` 1310400) (`self.All Weather Levels`) (`self.WeatherShapeVariant_LateGame`)))))))

(fn `DIFFICULTY LEVEL: MODERATE`
  (switch `int` (`PXRandomLibrary.PXRandomIntegerInRange` 0 1)
    (:`0`
      (`|ExecutionSequence`
        (:`then_0`
          (`PXTemperatureUtils.SetTemperatureLevelChangeAt` (struct :`ScaledTicks` 67200) 1)
          (`PXTemperatureUtils.SetTemperatureLevelChangeAt` (struct :`ScaledTicks` 84000) -1)
          (`PXTemperatureUtils.SetTemperatureLevelChangeAt` (struct :`ScaledTicks` 134400) 1)
          (`PXTemperatureUtils.SetTemperatureLevelChangeAt` (struct :`ScaledTicks` 201600) 1)
          (`PXTemperatureUtils.SetTemperatureLevelChangeAt` (struct :`ScaledTicks` 235200) -1)
          (`PXTemperatureUtils.SetTemperatureLevelChangeAt` (struct :`ScaledTicks` 403200) 1)
          (`PXTemperatureUtils.SetTemperatureLevelChangeAt` (struct :`ScaledTicks` 436800) 1)
          (`PXTemperatureUtils.SetTemperatureLevelChangeAt` (struct :`ScaledTicks` 470400) -1)
          (`PXTemperatureUtils.SetTemperatureLevelChangeAt` (struct :`ScaledTicks` 688800) 1)
          (`PXTemperatureUtils.SetTemperatureLevelChangeAt` (struct :`ScaledTicks` 756000) 1)
          (`PXTemperatureUtils.SetTemperatureLevelChangeAt` (struct :`ScaledTicks` 789600) 1)
          (`PXTemperatureUtils.SetTemperatureLevelChangeAt` (struct :`ScaledTicks` 840000) -1)
          (`PXTemperatureUtils.SetTemperatureLevelChangeAt` (struct :`ScaledTicks` 1024800) 1)
          (`PXTemperatureUtils.SetTemperatureLevelChangeAt` (struct :`ScaledTicks` 1058400) -1)
          (`PXTemperatureUtils.SetTemperatureLevelChangeAt` (struct :`ScaledTicks` 1192800) 1)
          (`PXTemperatureUtils.SetTemperatureLevelChangeAt` (struct :`ScaledTicks` 1260000) -1)
          (`PXTemperatureUtils.SetTemperatureLevelChangeAt` (struct :`ScaledTicks` 1444800) 1)
          (`PXTemperatureUtils.SetTemperatureLevelChangeAt` (struct :`ScaledTicks` 1495200) 1)
          (`PXTemperatureUtils.SetTemperatureLevelChangeAt` (struct :`ScaledTicks` 1579200) -1)
          (bind _returnvalue (`PXTemperatureUtils.GetLastTemperatureTimelineEntryTimestamp`))
          (set `self.RefreshTimestamp` (`PXTimeUtils.Subtract` _returnvalue (struct :`ScaledTicks` 168000))))
        (:`then_1`
          (set `/Game/Scenarios/Sandbox/BlueprintsNonSerialized/BP_Sandbox_Constants_BaseClass.Sandbox Beta Storm Timing` (`self.Easy 0 First Storm Timestamp`) (`/Game/Scenarios/Sandbox/BlueprintsNonSerialized/BPFL_SandboxStorage.Get Sandbox Constants Storage`))
          (`self.RandomStormSpawnerFixedTime` (struct :`ScaledTicks` 50400) (`self.Easy 0 First Storm Timestamp`) (`self.FirstStormPossibleWhiteouts`) (`self.WeatherShapeVariant_Base`))
          (`self.RandomStormSpawnerFixedTime` (struct :`ScaledTicks` 67200) (struct :`ScaledTicks` 604800) (`self.All Weather Levels`) (`self.WeatherShapeVariant_Base`))
          (`self.RandomStormSpawnerFixedTime` (struct :`ScaledTicks` 67200) (struct :`ScaledTicks` 940800) (`self.All Weather Levels`) (`self.WeatherShapeVariant_LateGame`))
          (`self.RandomStormSpawnerFixedTime` (struct :`ScaledTicks` 100800) (struct :`ScaledTicks` 1327200) (`self.All Weather Levels`) (`self.WeatherShapeVariant_LateGame`)))))
    (:`1`
      (`|ExecutionSequence`
        (:`then_0`
          (`PXTemperatureUtils.SetTemperatureLevelChangeAt` (struct :`ScaledTicks` 67200) 1)
          (`PXTemperatureUtils.SetTemperatureLevelChangeAt` (struct :`ScaledTicks` 84000) -1)
          (`PXTemperatureUtils.SetTemperatureLevelChangeAt` (struct :`ScaledTicks` 151200) 1)
          (`PXTemperatureUtils.SetTemperatureLevelChangeAt` (struct :`ScaledTicks` 201600) 1)
          (`PXTemperatureUtils.SetTemperatureLevelChangeAt` (struct :`ScaledTicks` 252000) -1)
          (`PXTemperatureUtils.SetTemperatureLevelChangeAt` (struct :`ScaledTicks` 403200) 1)
          (`PXTemperatureUtils.SetTemperatureLevelChangeAt` (struct :`ScaledTicks` 453600) 1)
          (`PXTemperatureUtils.SetTemperatureLevelChangeAt` (struct :`ScaledTicks` 487200) -1)
          (`PXTemperatureUtils.SetTemperatureLevelChangeAt` (struct :`ScaledTicks` 688800) 1)
          (`PXTemperatureUtils.SetTemperatureLevelChangeAt` (struct :`ScaledTicks` 739200) 1)
          (`PXTemperatureUtils.SetTemperatureLevelChangeAt` (struct :`ScaledTicks` 789600) 1)
          (`PXTemperatureUtils.SetTemperatureLevelChangeAt` (struct :`ScaledTicks` 823200) -1)
          (`PXTemperatureUtils.SetTemperatureLevelChangeAt` (struct :`ScaledTicks` 1024800) 1)
          (`PXTemperatureUtils.SetTemperatureLevelChangeAt` (struct :`ScaledTicks` 1058400) -1)
          (`PXTemperatureUtils.SetTemperatureLevelChangeAt` (struct :`ScaledTicks` 1209600) 1)
          (`PXTemperatureUtils.SetTemperatureLevelChangeAt` (struct :`ScaledTicks` 1260000) -1)
          (`PXTemperatureUtils.SetTemperatureLevelChangeAt` (struct :`ScaledTicks` 1444800) 1)
          (`PXTemperatureUtils.SetTemperatureLevelChangeAt` (struct :`ScaledTicks` 1478400) 1)
          (`PXTemperatureUtils.SetTemperatureLevelChangeAt` (struct :`ScaledTicks` 1562400) -1)
          (bind _returnvalue_2 (`PXTemperatureUtils.GetLastTemperatureTimelineEntryTimestamp`))
          (set `self.RefreshTimestamp` (`PXTimeUtils.Subtract` _returnvalue_2 (struct :`ScaledTicks` 168000))))
        (:`then_1`
          (set `/Game/Scenarios/Sandbox/BlueprintsNonSerialized/BP_Sandbox_Constants_BaseClass.Sandbox Beta Storm Timing` (`self.Easy 1 First Storm Timestamp`) (`/Game/Scenarios/Sandbox/BlueprintsNonSerialized/BPFL_SandboxStorage.Get Sandbox Constants Storage`))
          (`self.RandomStormSpawnerFixedTime` (struct :`ScaledTicks` 50400) (`self.Easy 1 First Storm Timestamp`) (`self.FirstStormPossibleWhiteouts`) (`self.WeatherShapeVariant_Base`))
          (`self.RandomStormSpawnerFixedTime` (struct :`ScaledTicks` 67200) (struct :`ScaledTicks` 604800) (`self.All Weather Levels`) (`self.WeatherShapeVariant_Base`))
          (`self.RandomStormSpawnerFixedTime` (struct :`ScaledTicks` 67200) (struct :`ScaledTicks` 940800) (`self.All Weather Levels`) (`self.WeatherShapeVariant_LateGame`))
          (`self.RandomStormSpawnerFixedTime` (struct :`ScaledTicks` 100800) (struct :`ScaledTicks` 1327200) (`self.All Weather Levels`) (`self.WeatherShapeVariant_LateGame`)))))))

(fn `DIFFICULTY LEVEL: SERENITY`
  (switch `int` (`PXRandomLibrary.PXRandomIntegerInRange` 0 1)
    (:`0`
      (`|ExecutionSequence`
        (:`then_0`
          (`PXTemperatureUtils.SetTemperatureLevelChangeAt` (struct :`ScaledTicks` 67200) 1)
          (`PXTemperatureUtils.SetTemperatureLevelChangeAt` (struct :`ScaledTicks` 84000) -1)
          (`PXTemperatureUtils.SetTemperatureLevelChangeAt` (struct :`ScaledTicks` 134400) 1)
          (`PXTemperatureUtils.SetTemperatureLevelChangeAt` (struct :`ScaledTicks` 201600) 1)
          (`PXTemperatureUtils.SetTemperatureLevelChangeAt` (struct :`ScaledTicks` 235200) -1)
          (`PXTemperatureUtils.SetTemperatureLevelChangeAt` (struct :`ScaledTicks` 403200) 1)
          (`PXTemperatureUtils.SetTemperatureLevelChangeAt` (struct :`ScaledTicks` 436800) 1)
          (`PXTemperatureUtils.SetTemperatureLevelChangeAt` (struct :`ScaledTicks` 470400) -1)
          (`PXTemperatureUtils.SetTemperatureLevelChangeAt` (struct :`ScaledTicks` 688800) 1)
          (`PXTemperatureUtils.SetTemperatureLevelChangeAt` (struct :`ScaledTicks` 756000) 1)
          (`PXTemperatureUtils.SetTemperatureLevelChangeAt` (struct :`ScaledTicks` 789600) 1)
          (`PXTemperatureUtils.SetTemperatureLevelChangeAt` (struct :`ScaledTicks` 840000) -1)
          (`PXTemperatureUtils.SetTemperatureLevelChangeAt` (struct :`ScaledTicks` 1024800) 1)
          (`PXTemperatureUtils.SetTemperatureLevelChangeAt` (struct :`ScaledTicks` 1058400) -1)
          (`PXTemperatureUtils.SetTemperatureLevelChangeAt` (struct :`ScaledTicks` 1192800) 1)
          (`PXTemperatureUtils.SetTemperatureLevelChangeAt` (struct :`ScaledTicks` 1260000) -1)
          (`PXTemperatureUtils.SetTemperatureLevelChangeAt` (struct :`ScaledTicks` 1444800) 1)
          (`PXTemperatureUtils.SetTemperatureLevelChangeAt` (struct :`ScaledTicks` 1495200) 1)
          (`PXTemperatureUtils.SetTemperatureLevelChangeAt` (struct :`ScaledTicks` 1579200) -1)
          (bind _returnvalue (`PXTemperatureUtils.GetLastTemperatureTimelineEntryTimestamp`))
          (set `self.RefreshTimestamp` (`PXTimeUtils.Subtract` _returnvalue (struct :`ScaledTicks` 168000))))
        (:`then_1`
          (set `/Game/Scenarios/Sandbox/BlueprintsNonSerialized/BP_Sandbox_Constants_BaseClass.Sandbox Beta Storm Timing` (`self.Easy 0 First Storm Timestamp`) (`/Game/Scenarios/Sandbox/BlueprintsNonSerialized/BPFL_SandboxStorage.Get Sandbox Constants Storage`))
          (`self.RandomStormSpawnerFixedTime` (struct :`ScaledTicks` 50400) (`self.Easy 0 First Storm Timestamp`) (`self.Serenity Weather Levels`) (`self.WeatherShapeVariant_Base`))
          (`self.RandomStormSpawnerFixedTime` (struct :`ScaledTicks` 67200) (struct :`ScaledTicks` 604800) (`self.Serenity Weather Levels`) (`self.WeatherShapeVariant_Base`))
          (`self.RandomStormSpawnerFixedTime` (struct :`ScaledTicks` 67200) (struct :`ScaledTicks` 940800) (`self.Serenity Weather Levels`) (`self.WeatherShapeVariant_LateGame`))
          (`self.RandomStormSpawnerFixedTime` (struct :`ScaledTicks` 100800) (struct :`ScaledTicks` 1327200) (`self.Serenity Weather Levels`) (`self.WeatherShapeVariant_LateGame`)))))
    (:`1`
      (`|ExecutionSequence`
        (:`then_0`
          (`PXTemperatureUtils.SetTemperatureLevelChangeAt` (struct :`ScaledTicks` 84000) 1)
          (`PXTemperatureUtils.SetTemperatureLevelChangeAt` (struct :`ScaledTicks` 100800) -1)
          (`PXTemperatureUtils.SetTemperatureLevelChangeAt` (struct :`ScaledTicks` 151200) 1)
          (`PXTemperatureUtils.SetTemperatureLevelChangeAt` (struct :`ScaledTicks` 201600) 1)
          (`PXTemperatureUtils.SetTemperatureLevelChangeAt` (struct :`ScaledTicks` 252000) -1)
          (`PXTemperatureUtils.SetTemperatureLevelChangeAt` (struct :`ScaledTicks` 403200) 1)
          (`PXTemperatureUtils.SetTemperatureLevelChangeAt` (struct :`ScaledTicks` 453600) 1)
          (`PXTemperatureUtils.SetTemperatureLevelChangeAt` (struct :`ScaledTicks` 487200) -1)
          (`PXTemperatureUtils.SetTemperatureLevelChangeAt` (struct :`ScaledTicks` 688800) 1)
          (`PXTemperatureUtils.SetTemperatureLevelChangeAt` (struct :`ScaledTicks` 739200) 1)
          (`PXTemperatureUtils.SetTemperatureLevelChangeAt` (struct :`ScaledTicks` 789600) 1)
          (`PXTemperatureUtils.SetTemperatureLevelChangeAt` (struct :`ScaledTicks` 823200) -1)
          (`PXTemperatureUtils.SetTemperatureLevelChangeAt` (struct :`ScaledTicks` 1024800) 1)
          (`PXTemperatureUtils.SetTemperatureLevelChangeAt` (struct :`ScaledTicks` 1058400) -1)
          (`PXTemperatureUtils.SetTemperatureLevelChangeAt` (struct :`ScaledTicks` 1209600) 1)
          (`PXTemperatureUtils.SetTemperatureLevelChangeAt` (struct :`ScaledTicks` 1260000) -1)
          (`PXTemperatureUtils.SetTemperatureLevelChangeAt` (struct :`ScaledTicks` 1444800) 1)
          (`PXTemperatureUtils.SetTemperatureLevelChangeAt` (struct :`ScaledTicks` 1478400) 1)
          (`PXTemperatureUtils.SetTemperatureLevelChangeAt` (struct :`ScaledTicks` 1562400) -1)
          (bind _returnvalue_2 (`PXTemperatureUtils.GetLastTemperatureTimelineEntryTimestamp`))
          (set `self.RefreshTimestamp` (`PXTimeUtils.Subtract` _returnvalue_2 (struct :`ScaledTicks` 168000))))
        (:`then_1`
          (set `/Game/Scenarios/Sandbox/BlueprintsNonSerialized/BP_Sandbox_Constants_BaseClass.Sandbox Beta Storm Timing` (`self.Easy 1 First Storm Timestamp`) (`/Game/Scenarios/Sandbox/BlueprintsNonSerialized/BPFL_SandboxStorage.Get Sandbox Constants Storage`))
          (`self.RandomStormSpawnerFixedTime` (struct :`ScaledTicks` 33600) (`self.Easy 1 First Storm Timestamp`) (`self.Serenity Weather Levels`) (`self.WeatherShapeVariant_Base`))
          (`self.RandomStormSpawnerFixedTime` (struct :`ScaledTicks` 50400) (struct :`ScaledTicks` 604800) (`self.Serenity Weather Levels`) (`self.WeatherShapeVariant_Base`))
          (`self.RandomStormSpawnerFixedTime` (struct :`ScaledTicks` 50400) (struct :`ScaledTicks` 940800) (`self.Serenity Weather Levels`) (`self.WeatherShapeVariant_LateGame`))
          (`self.RandomStormSpawnerFixedTime` (struct :`ScaledTicks` 67200) (struct :`ScaledTicks` 1327200) (`self.Serenity Weather Levels`) (`self.WeatherShapeVariant_LateGame`)))))))

(fn `Late Game Loop (~300 weeks)`
  (`PXTemperatureUtils.AddTemperatureLevelChange` (struct :`ScaledTicks` 33600) 1)
  (`self.RandomStormSpawnerOffset` (struct :`ScaledTicks` 134400) (struct :`ScaledTicks` 67200) (`self.All Weather Levels - Lategame loop`) (`self.WeatherShapeVariant_LateGame`))
  (`PXTemperatureUtils.AddTemperatureLevelChange` (struct :`ScaledTicks` 268800) -2)
  (`PXTemperatureUtils.AddTemperatureLevelChange` (struct :`ScaledTicks` 67200) 1)
  (`PXTemperatureUtils.AddTemperatureLevelChange` (struct :`ScaledTicks` 100800) 1)
  (`PXTemperatureUtils.AddTemperatureLevelChange` (struct :`ScaledTicks` 84000) -1)
  (bind _returnvalue (`PXTemperatureUtils.GetLastTemperatureTimelineEntryTimestamp`))
  (set `self.RefreshTimestamp` (`PXTimeUtils.Subtract` _returnvalue (struct :`ScaledTicks` 134400))))

(fn `Late Game Loop Serenity (~300 weeks)`
  (`PXTemperatureUtils.AddTemperatureLevelChange` (struct :`ScaledTicks` 33600) 1)
  (`self.RandomStormSpawnerOffset` (struct :`ScaledTicks` 134400) (struct :`ScaledTicks` 67200) (`self.Serenity Weather Levels`) (`self.WeatherShapeVariant_LateGame`))
  (`PXTemperatureUtils.AddTemperatureLevelChange` (struct :`ScaledTicks` 268800) -2)
  (`PXTemperatureUtils.AddTemperatureLevelChange` (struct :`ScaledTicks` 67200) 1)
  (`PXTemperatureUtils.AddTemperatureLevelChange` (struct :`ScaledTicks` 100800) 1)
  (`PXTemperatureUtils.AddTemperatureLevelChange` (struct :`ScaledTicks` 84000) -1)
  (bind _returnvalue (`PXTemperatureUtils.GetLastTemperatureTimelineEntryTimestamp`))
  (set `self.RefreshTimestamp` (`PXTimeUtils.Subtract` _returnvalue (struct :`ScaledTicks` 134400))))

(fn `RandomStormSpawnerFixedTime`
  (params (StormDuration :type "PXGameTime Structure") (ArriveTimestamp :type "PXGameTime Structure") (PossibleWeatherLevels :type "Array of PXWeatherLevel Object Reference") (PossibleWeatherShapes :type "Array of PXWeatherShapeTemplate Class Reference"))
  (`PXWeatherUtils.ScheduleWeatherAtCity` (`PXRandomLibrary.PXArrayRandom` PossibleWeatherShapes) (`PXRandomLibrary.PXArrayRandom` PossibleWeatherLevels) (`PXNationUtils.GetPlayerMainCity`) (`local.ArriveTimestamp`) (`local.StormDuration`) 4.0)
  (return))

(fn `RandomStormSpawnerOffset`
  (params (StormDuration :type "PXGameTime Structure") (`Time Offset` :type "PXGameTime Structure") (PossibleWeatherLevels :type "Array of PXWeatherLevel Object Reference") (PossibleWeatherShapes :type "Array of PXWeatherShapeTemplate Class Reference"))
  (locals (ArriveTimestamp :type "PXGameTime Structure"))
  (bind _returnvalue (`PXTemperatureUtils.GetLastTemperatureTimelineEntryTimestamp`))
  (set `local.ArriveTimestamp` (`PXTimeUtils.Add` _returnvalue (`local.Time Offset`)))
  (`PXWeatherUtils.ScheduleWeatherAtCity` (`PXRandomLibrary.PXArrayRandom` PossibleWeatherShapes) (`PXRandomLibrary.PXArrayRandom` PossibleWeatherLevels) (`PXNationUtils.GetPlayerMainCity`) (`local.ArriveTimestamp`) (`local.StormDuration`) 4.0)
  (return))

(fn `WiteoutTesting`
  (`|ExecutionSequence`
    (:`then_0`
      (`PXTemperatureUtils.SetTemperatureLevelChangeAt` (struct :`ScaledTicks` 1680000) 1)
      (bind _returnvalue (`PXTemperatureUtils.GetLastTemperatureTimelineEntryTimestamp`))
      (set `self.RefreshTimestamp` (`PXTimeUtils.Subtract` _returnvalue (struct :`ScaledTicks` 168000))))
    (:`then_1`
      (`self.RandomStormSpawnerFixedTime` (struct :`ScaledTicks` 67200) (struct :`ScaledTicks` 84000) (`self.FirstStormPossibleWhiteouts`) (`self.WeatherShapeVariant_Base`))
      (`self.RandomStormSpawnerFixedTime` (struct :`ScaledTicks` 84000) (struct :`ScaledTicks` 201600) (`self.All Weather Levels`) (`self.WeatherShapeVariant_Base`))
      (`self.RandomStormSpawnerFixedTime` (struct :`ScaledTicks` 100800) (struct :`ScaledTicks` 336000) (`self.All Weather Levels`) (`self.WeatherShapeVariant_LateGame`))
      (`self.RandomStormSpawnerFixedTime` (struct :`ScaledTicks` 117600) (struct :`ScaledTicks` 504000) (`self.All Weather Levels`) (`self.WeatherShapeVariant_LateGame`)))))