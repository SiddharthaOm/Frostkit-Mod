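; Flow script that plays the story arc beats of the faction war preparation phase until the PrepareForWar quest finishes or the beats run out.
; After an initial timed wait, it caches the quest from shared variable storage and works recursively through the Beats queue.
; Each beat class becomes an arc, started if eligible, and only a started arc flagged BlocksFlow holds up the next beat.
; SetGameContext builds the arcs' context from the main city's first two communities.
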(event `Next Beat`
  (bind _beats (`self.Beats`))
  (if (not (`PXQuest.IsQuestFinished` (`self.Quest`))) :!label _label
    (if (`KismetArrayLibrary.Array_IsNotEmpty` _beats)
      (bind (_returnvalue _returnvalue1) (`self.Start Arc` (`|GetArrayItem` _beats)))
      (bind _output_get (set `self.Beat Arc object` _returnvalue))
      (if (and (`/Game/Scenarios/Shared/BlueprintsSerialized/StoryArcs/FactionWar/BP_FactionWarBeat_Parent.Blocks Flow?` _output_get) _returnvalue1)
        (`PXAsyncWaitForStoryArc.AsyncAction_WaitForStoryArc` (`self.Beat Arc object`)
          (:`Completed`
            _)))
      (`KismetArrayLibrary.Array_Remove` (`self.Beats`))
      (`self.Next Beat`))))

(event `self.ReceiveBeginPlay`
  (`PXAsyncWaitForDurationPassed.AsyncAction_WaitForDurationPassed` (struct :`ScaledTicks` 10)
    (:`Completed`
      (`self.Set Quest`)
      (goto _label))))

(fn `Set Game Context`
  (bind _returnvalue (`PXFactionUtils.GetMembersFromCity` (`PXNationUtils.GetPlayerMainCity`) null))
  (set `self.Game Context` (`PXGameplayContextUtils.MakePXGameContext` (`|GetArrayItem` _returnvalue) (`|GetArrayItem` _returnvalue 1))))

(fn `Set Quest`
  (set `self.Quest` (`/Game/Scenarios/Shared/BlueprintsSerialized/VariableStorage/BP_SharedVariableStorage.Prepare for War Quest` (`/Game/Scenarios/Shared/BlueprintsNonSerialized/SocietyUtils/BPFL_SharedScenariosStorage.Get Shared Variable Storage`))))

(fn `Start Arc`
  (params (`Beat StoryArc` :type "/Game/Scenarios/Shared/BlueprintsSerialized/StoryArcs/FactionWar/BP_FactionWarBeat_Parent Class Reference"))
  (returns (ReturnValue :type "/Game/Scenarios/Shared/BlueprintsSerialized/StoryArcs/FactionWar/BP_FactionWarBeat_Parent Object Reference") (ReturnValue1 :type Boolean))
  (locals (`arc local` :type "/Game/Scenarios/Shared/BlueprintsSerialized/StoryArcs/FactionWar/BP_FactionWarBeat_Parent Object Reference"))
  (bind _arc_local (`local.arc local`))
  (bind _returnvalue (`|GenericCreateObject` (subsystem `PXStoryArcSubsystem`) `Beat StoryArc` (`self.Game Context`)))
  (bind _output_get (set `local.arc local` _returnvalue))
  (bind _returnvalue_2 (`/Game/Scenarios/Shared/BlueprintsSerialized/StoryArcs/ParentArcs/BP_GameplayAction_StoryArc.CanBeStarted Core` _output_get))
  (if _returnvalue_2
    (bind _returnvalue_3 (`PXStoryUtils.StartParameterizedStoryArc` _arc_local))
    (return _arc_local _returnvalue_3)
    (else
      (return _arc_local false))))