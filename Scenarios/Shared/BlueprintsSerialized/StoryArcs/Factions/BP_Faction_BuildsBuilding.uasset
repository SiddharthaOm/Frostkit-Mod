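; Story arc in which a faction community holding a rally proposes constructing a building it desires in the rally's district.
; It can start once a timer expires during the rally, given a matching building desire and enough city workforce.
; It blocks rally events while presenting a lens choice; the first option applies the Heatnotes construction cost and creates the building, though a debug print flags this as broken.
; On finish, it lifts the block after a delay.
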(event `self.OnStarted`
  (bind _faction_community (`self.Faction community`))
  (bind _building_type_to_build (`self.Building type to build`))
  (bind _district_to_build_in (`self.District to build in`))
  (set `/Game/Scenarios/Shared/BlueprintsSerialized/VariableStorage/BP_SharedVariableStorage.RallyFreeBuilding` (`self.Building type to build`) (`/Game/Scenarios/Shared/BlueprintsNonSerialized/SocietyUtils/BPFL_SharedScenariosStorage.Get Shared Variable Storage`))
  (`PXStoryUtils.AddStoryArcBlockReason` (struct :`TagName` "StoryArcTag.RallyEvents") "/Game/Scenarios/Shared/Configs/BlockReasons/DA_RallyEvent_Block.DA_RallyEvent_Block")
  (bind _decision (`/Game/Scenarios/Shared/BlueprintsNonSerialized/SocietyUtils/BPFL_Communication_Utils.Send Lens With Community Art` (`self.OA SmallLens`) (`self.District to build in`) (`PXCommunityComponent.GetCommunityType` _faction_community) (`|MakeMap` "FACTION" (`/Game/Scenarios/Shared/BlueprintsNonSerialized/Communities/BPFL_CommunityUtils.Get Community Name` _faction_community) "BUILDING" (`PXBuildingType.IngameName` (`self.Building type to build`)) "DISTRICT" (`PXDistrictType.IngameName` (`PXDistrictComponent.DistrictType` _district_to_build_in))) (`PXGameplayContextUtils.MakePXGameContext` _faction_community null null null _district_to_build_in) (struct) false (make `/Game/Scenarios/Shared/BlueprintsNonSerialized/SocietyUtils/F_DesiresArray_Struct` (`|MakeArray` (`self.Get Immediate Desire`)))))
  (bind _choice (`PXAsyncWaitForChoice.AsyncAction_WaitForChoice` _decision)
    (:`Completed`
      (switch `int` _choice
        (:`0`
          (`PXStockpileUtils.TryChangeNationStockpile` (`PXNationUtils.GetPlayerNation`) "/Game/Scenarios/Shared/Configs/Resources/Types/DA_Core_Heatnotes.DA_Core_Heatnotes" (`BlueprintMapLibrary.Map_Find` (`PXOperationUtils.GetStockpileCostFromOperationCost` (`PXBuildingUtils.GetBuildingTypeConstructionCost` (`PXNationUtils.GetCityNation` (`PXDistrictComponent.GetCity` (`self.District to build in`))) _building_type_to_build)) "/Game/Scenarios/Shared/Configs/Resources/Types/DA_Core_Heatnotes.DA_Core_Heatnotes"))
          (bind _returnvalue (`PXBuildingUtils.CreateBuilding` (`self.District to build in`) _building_type_to_build "/Game/Scenarios/Shared/Configs/ActionOrigin/DA_OtherActionOrigin.DA_OtherActionOrigin"))
          (set `self.building component` _returnvalue)
          (`KismetSystemLibrary.PrintString` "a building should have been built but its broken"))))))

(event `self.OnFinished`
  (`PXAsyncWaitForDurationPassed.AsyncAction_WaitForDurationPassed` (struct :`ScaledTicks` 168000)
    (:`Completed`
      (`PXStoryUtils.RemoveStoryArcBlockReason` (struct :`TagName` "StoryArcTag.RallyEvents") "/Game/Scenarios/Shared/Configs/BlockReasons/DA_RallyEvent_Block.DA_RallyEvent_Block"))))

(fn `CanBeStarted`
  (returns (ReturnValue :type Boolean))
  (bind (_returnvalue _ongoing_actions1) (`/Game/Scenarios/Shared/BlueprintsNonSerialized/OngoingEvents/BPFL_OngoingAction_Utils.Is Any Action of type Ongoing?` "/Game/Scenarios/Shared/Configs/OngoingActions/System_Started/DA_Rally.DA_Rally"))
  (if _returnvalue
    (set `self.OA Data` (`|GetArrayItem` _ongoing_actions1))
    (`self.Set Timer`)
    (if (`self.Timer has expired?` (struct :`ScaledTicks` 50400))
      (bind _output_get (set `self.Faction community` (`PXOngoingActionComponent.GetCommunity` (`self.OA Data`))))
      (bind _output_get_2 (set `self.District to build in` (`PXOngoingActionComponent.GetAnyDistict` (`self.OA Data`))))
      (bind (_buildingdesire _found) (`/Game/Scenarios/Shared/BlueprintsNonSerialized/SocietyUtils/BPFL_FactionDemandAction_Utils.Get Possible Building Desire for Community in District` _output_get _output_get_2))
      (if _found
        (set `self.Building type to build` (`.Building` (break `PXDesire` _buildingdesire)))
        (if (> (`PXWorkforceUtils.GetCityAvailableWorkforce` (`PXNationUtils.GetPlayerMainCity`)) (`KismetMathLibrary.Abs_Int` (`PXOperationUtils.GetWorkforceCostFromOperationCost` (`PXBuildingUtils.GetBuildingTypeConstructionCost` (`PXNationUtils.GetPlayerNation`) (`self.Building type to build`)))))
          (return true)
          (else
            (return false)))
        (else
          (return false))))
    (else
      (`self.Restart Timer`))))

(fn `Get Immediate Desire`
  (returns (ReturnValue :type "PXDesire Structure"))
  (bind _returnvalue (`PXDesireUtils.MakeBuildingDesire` (`self.Building type to build`) 1))
  (return _returnvalue))