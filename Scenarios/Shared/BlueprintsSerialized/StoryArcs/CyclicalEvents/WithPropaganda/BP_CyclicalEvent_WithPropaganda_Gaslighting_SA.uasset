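; A cyclical propaganda story arc event about gaslighting, in which a woman is dealt with by the player's nation.
; It extends the parent's text defines with an ASYLUM entry chosen by whether the player's nation has an active Lunatic Asylum.
; With one, the text says she was tossed into that building, named by its in-game name; otherwise it says she was arrested.
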(fn `Get Defines`
  (returns (Map :type "Map of String to Text"))
  (bind _defines_map_merged (`/Game/Scenarios/Shared/BlueprintsNonSerialized/SocietyUtils/BPFL_Communication_Utils.Merge Defines` (`parent.Get Defines`) (`|MakeMap` "ASYLUM" (select `bool` (`PXBuildingUtils.HasAnyBuildingOfTypeInNation` (`PXNationUtils.GetPlayerNation`) (`self.Lunatic Asylum`) true) :`false` (`|FormatText` "NO ASYLUM: She has been arrested.") :`true` (`|FormatText` "YES ASYLUM: She has been tossed in the {BUILDING}" (`PXBuildingType.IngameName` (`self.Lunatic Asylum`)))))))
  (return _defines_map_merged))