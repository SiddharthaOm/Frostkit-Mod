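; Story arc that plays angry barks when a faction war ongoing action's "speed started" event fires in a district.
; On start, it gets the district's ongoing action component and uses its primary and secondary communities as the two generated speakers.
; It fills the barkset's text placeholders with attacker, defender, predicted battle outcome, context community, opposing faction and district names.
; The core start check always passes.
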(event `self.OnStarted`
  (bind _game_context (`self.Game Context`))
  (bind _district (`PXGameplayContextUtils.TryGetDistrictFromGameContext` _game_context))
  (bind (_primary_community _secondary_community) (`/Game/Scenarios/Shared/BlueprintsNonSerialized/OngoingEvents/BPFL_OngoingAction_Utils.Get Primary and Secondary Community from OA Component` (`self.OA Component`)))
  (bind _community (`PXGameplayContextUtils.TryGetCommunityComponentFromGameContext` _game_context))
  (bind _ingame_name (`/Game/Scenarios/Shared/BlueprintsNonSerialized/Communities/BPFL_CommunityUtils.Get Community Name` _community))
  (bind (_hasongoingaction _returnvalue) (`PXOngoingActionUtils.GetOngoingActionComponentForDistrict` (`/Game/Scenarios/Shared/BlueprintsNonSerialized/SocietyUtils/BPFL_Communication_Utils.Get Best District from Context` _game_context)))
  ;[1 1 1] IMPLEMENT BARKS / MESSAGE HERE
  (set `self.OA Component` _returnvalue)
  (`/Game/Scenarios/Shared/BlueprintsNonSerialized/SocietyUtils/BPFL_Communication_Utils.Pick Barks with Generated Speaker` _primary_community _secondary_community true (`|MakeMap` "ATTACKERS" (`/Game/Scenarios/Shared/BlueprintsNonSerialized/Communities/BPFL_CommunityUtils.Get Community Name` _primary_community) "DEFENDERS" (`/Game/Scenarios/Shared/BlueprintsNonSerialized/Communities/BPFL_CommunityUtils.Get Community Name` _secondary_community) "PREDICTED_OUTCOME" (`/Game/Scenarios/Shared/BlueprintsNonSerialized/FactionEmergence/BPFL_FactionWarUtils.Get Faction War Next Battle Text` _primary_community _secondary_community) "COMMUNITY" _ingame_name "TARGET_COMMUNITY" (`/Game/Scenarios/Shared/BlueprintsNonSerialized/Communities/BPFL_CommunityUtils.Get Community Name` (`.Faction Component` (`/Game/Scenarios/Shared/BlueprintsNonSerialized/FactionEmergence/BPFL_FactionWarUtils.Get Existing Opposing Faction` (`PXCommunityComponent.GetFaction` _community)))) "DISTRICT" (`PXDistrictType.IngameName` (`PXDistrictComponent.DistrictType` _district)) "FACTION" _ingame_name) (`self.speed Started Barkset`) _district))

(fn `CanBeStarted Core`
  (returns (ReturnValue :type Boolean))
  (return true))