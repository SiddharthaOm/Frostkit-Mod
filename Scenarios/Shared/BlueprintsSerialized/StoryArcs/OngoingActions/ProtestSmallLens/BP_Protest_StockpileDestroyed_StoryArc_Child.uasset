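; Protest story arc child that destroys a city stockpile when the protest's spread district is a depot.
; The start check maps depot type to resource, requires at least 1000 in the player's main city, and caps the loss amount.
; Coal depots randomly target coal or oil if oil also qualifies, keeping the coal-based amount.
; On finish it deducts that amount from the district's city; the resource name feeds text defines.
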(event `self.OnFinished`
  (`PXStockpileUtils.TryChangeCityStockpile` (`PXDistrictComponent.GetCity` (`self.Spread District`)) (`self.Resource Type`) (* (`self.Stockpile Amount`) -1)))

(fn `Can Be Started Core`
  (returns (Return :type Boolean))
  (locals (`Buildings in District` :type "Array of PXBuildingComponent Object Reference"))
  (bind _returnvalue (`PXStockpileUtils.GetCityStockpileOfResource` (`PXNationUtils.GetPlayerMainCity`) (`self.Resource Type`)))
  (bind _return (`parent.Can Be Started Core`))
  (if _return
    (if (`KismetArrayLibrary.Array_Contains` (`self.Depot District Types`) (`PXDistrictComponent.DistrictType` (`self.Spread District`)))
      (set `self.Depot Type` (`PXDistrictComponent.DistrictType` (`self.Spread District`)))
      (set `self.Resource Type` (`BlueprintMapLibrary.Map_Find` (`self.Depot Type to Resource`) (`self.Depot Type`)))
      (if (>= _returnvalue 1000)
        (set `self.Stockpile Amount` (`KismetMathLibrary.Clamp` _returnvalue 0 30000))
        (if (== (`self.Resource Type`) (`self.Coal Resource`))
          (if (>= (`PXStockpileUtils.GetCityStockpileOfResource` (`PXNationUtils.GetPlayerMainCity`) (`self.Oil Resource`)) 1000)
            (set `self.Resource Type` (select `bool` (`PXRandomLibrary.PXRandomBool`) :`false` (`self.Oil Resource`) :`true` (`self.Coal Resource`)))
            (return true)
            (else
              _)))
        (return true)))))

(fn `Make Defines`
  (returns (Map :type "Map of String to Text"))
  (`BlueprintMapLibrary.Map_Add` (`self.Defines Map`) "STOCKPILE" (`PXResource.IngameName` (`self.Resource Type`)))
  (bind _defines_map_merged (`/Game/Scenarios/Shared/BlueprintsNonSerialized/SocietyUtils/BPFL_Communication_Utils.Merge Defines` (`self.Defines Map`) (`parent.Make Defines`)))
  (return _defines_map_merged))