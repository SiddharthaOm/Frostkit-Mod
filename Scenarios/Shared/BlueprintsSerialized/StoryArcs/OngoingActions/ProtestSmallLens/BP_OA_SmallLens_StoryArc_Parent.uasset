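; Parent Blueprint for story-arc ongoing actions that show a small lens message with a choice, tied to a community and district.
; On start it sends the message with district, faction and opposing-faction text defines, then waits for any choice before applying effects.
; Art comes from either the message config or the community type, depending on the CustomArt flag.
; Start condition and post-choice effects are default stubs for children to override.
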(event `self.OnStarted`
  (bind _decision (`self.Send Spread Message` (`self.Get Spread Message`) (`self.Spread District`) (`PXOngoingActionComponent.GetCommunity` (`self.OA Data`)) (`self.Make Defines`)))
  (bind _output_get (set `self.Decision` _decision))
  (`PXAsyncWaitForAnyChoice.AsyncAction_WaitForAnyChoice` _output_get
    (:`Completed`
      (`self.Effects After Choice`))))

(fn `Can Be Started Core`
  (returns (Return :type Boolean))
  (return true))

(fn `CanBeStarted`
  (returns (ReturnValue :type Boolean))
  (bind _return (`self.Can Be Started Core`))
  (return _return))

(fn `Effects After Choice`)

(fn `Get Spread Message`
  (returns (message :type "PXLens Soft Object Reference"))
  (return (`self.OA SmallLens`)))

(fn `Make Defines`
  (returns (Map :type "Map of String to Text"))
  (bind _returnvalue (`PXOngoingActionComponent.GetCommunity` (`self.OA Data`)))
  (return (`|MakeMap` "DISTRICT" (`PXDistrictType.IngameName` (`PXDistrictComponent.DistrictType` (`self.Spread District`))) "OPP_FACTION" (`PXFactionType.IngameName` (`/Game/Scenarios/Shared/BlueprintsNonSerialized/FactionEmergence/BPFL_FactionWarUtils.Get Existing Opposing Faction` (`PXCommunityComponent.GetFaction` _returnvalue))) "FACTION" (`PXFactionUtils.GetFactionOrCommunityInGameNameText` _returnvalue))))

(fn `Send Spread Message`
  (params (message :type "PXLens Soft Object Reference") (`Optional District` :type "PXDistrictComponent Object Reference") (`Optional Context Community` :type "PXCommunityComponent Object Reference") (textDefines :type "Map of String to Text"))
  (returns (Decision :type "PXDecision Object Reference"))
  (if (`self.Custom Art`)
    (bind _decision (`/Game/Scenarios/Shared/BlueprintsNonSerialized/SocietyUtils/BPFL_Communication_Utils.Send Config Message` message `Optional District` `Optional Context Community` null textDefines))
    (return _decision)
    (else
      (bind _decision_2 (`/Game/Scenarios/Shared/BlueprintsNonSerialized/SocietyUtils/BPFL_Communication_Utils.Send Lens With Community Art` message `Optional District` (`PXCommunityComponent.GetCommunityType` `Optional Context Community`) textDefines (`PXGameplayContextUtils.MakePXGameContext` `Optional Context Community` null null null `Optional District`)))
      (return _decision_2))))