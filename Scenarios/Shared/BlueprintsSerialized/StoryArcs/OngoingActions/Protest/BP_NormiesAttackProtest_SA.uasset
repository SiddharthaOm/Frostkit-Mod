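; Story arc in which an independent community disrupts an ongoing faction protest in an Extraction district of the player's main city.
; It starts once a timer expires while the first ongoing protest covers such a district and an independent community type opposing one of the protesting faction's affinities exists.
; On start it shows a message, waits for a choice, then ends the protest in that district.
; After a duration it launches the "Again" follow-up arc.
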(event `self.OnStarted`
  (bind _decision (`/Game/Scenarios/Shared/BlueprintsNonSerialized/SocietyUtils/BPFL_Communication_Utils.Send Config Message` (`self.Lens`) (`self.Critical District`) (`.ReturnValue` (`PXCommunityUtils.GetCommunityOfCommunityType` (`self.Independent Community`))) null (`|MakeMap` "FACTION" (`PXFactionUtils.GetFactionInGameName` (`PXOngoingActionComponent.GetCommunity` (`self.Ongoing Action`))) "COMMUNITY" (`/Game/Scenarios/Shared/BlueprintsNonSerialized/Communities/BPFL_CommunityUtils.Get Independents Affinity And Ingame Name` (`.ReturnValue` (`PXCommunityUtils.GetCommunityOfCommunityType` (`self.Independent Community`)))) "DISTRICT" (`PXDistrictType.IngameName` (`PXDistrictComponent.DistrictType` (`self.Critical District`))) "ACTION" (`PXOngoingActionType.IngameName` (`PXOngoingActionComponent.GetActionType` (`self.Ongoing Action`))))))
  (`PXAsyncWaitForAnyChoice.AsyncAction_WaitForAnyChoice` _decision
    (:`Completed`
      (`self.Collapse Protest on Critical District`))))

(event `self.OnFinished`
  (`PXAsyncWaitForDurationPassed.AsyncAction_WaitForDurationPassed` (struct :`ScaledTicks` 84000)
    (:`Completed`
      (bind _returnvalue (`|GenericCreateObject` (subsystem `PXStoryArcSubsystem`) "/Game/Scenarios/Shared/BlueprintsSerialized/StoryArcs/OngoingActions/Protest/BP_NormiesAttackProtest_Again_SA.BP_NormiesAttackProtest_Again_SA_C"))
      (`PXStoryUtils.StartParameterizedStoryArc` _returnvalue))))

(fn `CanBeStarted`
  (returns (ReturnValue :type Boolean))
  (bind (_returnvalue _ongoing_actions1) (`/Game/Scenarios/Shared/BlueprintsNonSerialized/OngoingEvents/BPFL_OngoingAction_Utils.Is Any Action of type Ongoing?` "/Game/Scenarios/Shared/Configs/OngoingActions/System_Started/DA_Protest.DA_Protest"))
  (`self.Define Critical Districts`)
  (if _returnvalue
    (set `self.Ongoing Action` (`|GetArrayItem` _ongoing_actions1))
    (for _array_element (`PXFactionUtils.GetFactionAffinities` (`PXNationUtils.GetPlayerNation`) (`PXCommunityComponent.GetFaction` (`PXOngoingActionComponent.GetCommunity` (`self.Ongoing Action`))))
      (bind _returnvalue_2 (`PXCommunityUtils.GetIndependentsTypeFromAffinity` (`PXNationUtils.GetPlayerNation`) (`/Game/Scenarios/Shared/BlueprintsNonSerialized/SocietyUtils/BPFL_Cornerstone_Utils.Get Opposite Affinity` _array_element)))
      (`/Engine/EditorBlueprintResources/StandardMacros.IsValid` _returnvalue_2
        (:`Is Valid`
          (set `self.Independent Community` _returnvalue_2)
          (break))))
    (`/Engine/EditorBlueprintResources/StandardMacros.IsValid` (`self.Independent Community`)
      (:`Is Valid`
        (for _array_element_2 (`self.Critical Districts`)
          (if (`KismetArrayLibrary.Array_Contains` (`PXOngoingActionComponent.GetDistricts` (`self.Ongoing Action`)) _array_element_2)
            (set `self.Critical District` _array_element_2)
            (break)))
        (`/Engine/EditorBlueprintResources/StandardMacros.IsValid` (`self.Critical District`)
          (:`Is Valid`
            (`self.Set Timer`)
            (if (`self.Timer has expired?` (struct :`ScaledTicks` 16800))
              (return true)))
          (:`Is Not Valid`
            (`self.Restart Timer`)
            (return false))))
      (:`Is Not Valid`
        (`self.Restart Timer`)
        (return false)))
    (else
      (`self.Restart Timer`)
      (return false))))

(fn `Collapse Protest on Critical District`
  (`PXOngoingActionUtils.EndOngoingActionInDistrict` :`district` (`self.Critical District`) :`endType` "/Game/Scenarios/Shared/Configs/OngoingActions/EndTypes/DA_Protest_Short_Default_EndType.DA_Protest_Short_Default_EndType"))

(fn `Define Critical Districts`
  (set `self.Critical Districts` (`PXDistrictUtils.GetDistrictWithTagFromCity` (`PXNationUtils.GetPlayerMainCity`) (struct :`TagDictionary` (struct :`(TagName` "District.Extraction") :`(TagName` "District.FoodSupply")) :`QueryTokenStream` "(0,1,1,2,0,1)" :`AutoDescription` " ANY( District.Extraction, District.FoodSupply )")))
  (return))