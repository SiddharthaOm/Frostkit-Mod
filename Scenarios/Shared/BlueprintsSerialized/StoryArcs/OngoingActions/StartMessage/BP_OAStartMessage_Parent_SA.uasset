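; Parent story arc for Ongoing Action start messages, showing a decision lens with community art and faction name for the action's community and district.
; On start it registers the decision as awaited by the action, waits asynchronously for the choice and passes it to HandleChoice, a stub alongside default per-choice desires.
; An unlock can suppress these default lenses when an action is force-started; finishing clears a CA-block unlock on the player nation.
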(event `self.OnStarted`
  (set `self.Community` (`PXGameplayContextUtils.TryGetCommunityComponentFromGameContext` (`self.Game Context`)))
  (bind _decision (`self.Send Message` (`self.Get Message Defines`) (`PXCommunityComponent.GetCommunityType` (`self.Community`)) (`PXOngoingActionComponent.GetAnyDistict` (`PXGameplayContextUtils.TryGetOngoingActionFromGameContext` (`self.Game Context`)))))
  (bind _output_get (set `self.Decision` _decision))
  (`/Engine/EditorBlueprintResources/StandardMacros.IsValid` _output_get
    (:`Is Valid`
      (`PXOngoingActionUtils.SetOngoingActionDecisionAwaitedForStart` (`PXGameplayContextUtils.TryGetOngoingActionFromGameContext` (`self.Game Context`)) _output_get)
      (bind _choice (`PXAsyncWaitForChoice.AsyncAction_WaitForChoice` (`self.Decision`))
        (:`Completed`
          (bind _output_get_2 (set `self.Choice` _choice))
          (`self.Handle Choice` _output_get_2 (`self.Decision`)))))))

(event `self.OnFinished`
  (`PXUnlockUtils.SetUnlockActive` (`PXNationUtils.GetPlayerNation`) "/Game/Scenarios/Shared/Configs/Unlocks/OngoingActions/DA_OngoingAction_CABlock_Unlock.DA_OngoingAction_CABlock_Unlock"))

(fn `CanBeStarted Core`
  (returns (ReturnValue :type Boolean))
  ;[1 1 1] Must set this unlock to TRUE when force starting an OA to disable these default start lenses
  (if (not (`PXUnlockUtils.IsUnlockActive` (`PXNationUtils.GetPlayerNation`) (`self.OA Start Disabled Unlock`)))
    (set `self.Community` (`PXGameplayContextUtils.TryGetCommunityComponentFromGameContext` (`self.Game Context`)))
    (bind _returnvalue (`parent.CanBeStarted Core`))
    (return _returnvalue)))

(fn `Desire per Choice`
  (returns (ReturnValue :type "PXCommunicationChannelsDesiresPerChoiceArray Structure"))
  (return (`PXCommunicationChannelsUtils.CreateDesiresPerChoiceArray` _)))

(fn `Get Message Defines`
  (returns (Defines :type "Map of String to Text"))
  (return (`|MakeMap` "FACTION" (`PXFactionUtils.GetFactionOrCommunityInGameNameText` (`self.Community`)))))

(fn `Handle Choice`
  (params (Selection :type Integer) (Decision :type "PXDecision Object Reference"))
  (switch `int` Selection))

(fn `Send Message`
  (params (textDefines :type "Map of String to Text") (Community :type "PXCommunityType Object Reference") (`Optional District` :type "PXDistrictComponent Object Reference"))
  (returns (Decision :type "PXDecision Object Reference"))
  (bind _decision (`/Game/Scenarios/Shared/BlueprintsNonSerialized/SocietyUtils/BPFL_Communication_Utils.Send OA Start Lens With Community Art` (`self.Lens Config`) `Optional District` Community textDefines (`self.Game Context`) (`self.Desire per Choice`)))
  (return _decision))