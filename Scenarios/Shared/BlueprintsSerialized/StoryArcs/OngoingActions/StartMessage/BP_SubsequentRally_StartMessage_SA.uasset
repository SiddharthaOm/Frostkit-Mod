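; Start message for a subsequent rally ongoing action in a story arc, supplying the text placeholders that announce a community's rallying.
; It overrides GetMessageDefines to set a fixed one-district spread line, plus the name and description of the community's faction-specific community action.
; These local defines are merged with the parent class's defines and returned.
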(fn `Get Message Defines`
  (returns (Defines :type "Map of String to Text"))
  (bind _returnvalue (`/Game/Scenarios/Shared/BlueprintsNonSerialized/OngoingEvents/BPFL_OngoingAction_Utils.Get Faction Specific Community Action for Community` (`self.Community`)))
  (`BlueprintMapLibrary.Map_Add` (`self.Local Defines Map`) "SPREAD" (`|FormatText` "They have begun rallying in 1 District"))
  (`BlueprintMapLibrary.Map_Add` (`self.Local Defines Map`) "COMMUNITY_ACTION" (`/Game/Scenarios/Shared/BlueprintsNonSerialized/SocietyUtils/BPFL_Desires_Utils.Get Community Action Name` _returnvalue))
  (`BlueprintMapLibrary.Map_Add` (`self.Local Defines Map`) "CA_DESC" (`PXGameplayAction.Description` (`PXCommunityAction.GameplayAction` _returnvalue)))
  (bind _defines_map_merged (`/Game/Scenarios/Shared/BlueprintsNonSerialized/SocietyUtils/BPFL_Communication_Utils.Merge Defines` (`self.Local Defines Map`) (`parent.Get Message Defines`)))
  (return _defines_map_merged))