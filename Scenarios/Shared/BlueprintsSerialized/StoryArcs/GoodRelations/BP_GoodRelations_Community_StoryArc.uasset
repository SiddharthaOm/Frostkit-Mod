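; Community story arc that offers the player a deradicalisation choice when an independent community has good relations.
; It starts only if such a community shares its first affinity with a faction of sufficient strength and size, with imprints and past actions blocking repeats.
; On start it imprints the community, sends a choice lens naming both sides, and executes the deradicalisation community action on the first choice.
; The unlock call is disconnected.
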(event `self.OnStarted`
  (bind (_found _community_cache1 _community_type_cache1 _faction_cache1) (`self.Find Good Relations Candidates`))
  (if _found
    (set `self.Community with Good Relations` _community_cache1)
    (set `self.Community Type` _community_type_cache1)
    (set `self.Faction Community` _faction_cache1)
    (`PXCommunityUtils.AddImprint` (`self.Community with Good Relations`) (`self.Good Relations Choice Imprint`))
    (bind _decision (`/Game/Scenarios/Shared/BlueprintsNonSerialized/SocietyUtils/BPFL_Communication_Utils.Send Lens With Community Art` "/Game/Scenarios/Shared/Configs/Messages/Lenses/GoodRelations/DA_GoodRelations_Generic_Lens.DA_GoodRelations_Generic_Lens" null (`self.Community Type`) (`|MakeMap` "COMMUNITY" (`PXFactionUtils.GetFactionOrCommunityInGameNameText` (`self.Community with Good Relations`)) "FACTION" (`PXFactionUtils.GetFactionOrCommunityInGameNameText` (`self.Faction Community`)) "CHOICE_TRANSFER" (`/Game/UI/Utilities/BPFL_UI.Get Population Size Points Display Text` (`self.Choice Transfer`)) "RELATIONS" (`PXTraitType.IngameName` (`self.Bad Relations`))) (`PXGameplayContextUtils.MakePXGameContext` (`self.Community with Good Relations`)) (struct) true))
    (bind _choice (`PXAsyncWaitForChoice.AsyncAction_WaitForChoice` _decision)
      (:`Completed`
        (switch `int` _choice
          (:`0`
            (`PXCommunityActionUtils.ExecuteCommunityAction` "/Game/Scenarios/Shared/Configs/Communities/CommunityActions/Favours_Group/Deradicalisation/DA_GoodRelations_Deradicalisation_CA.DA_GoodRelations_Deradicalisation_CA" "/Game/Scenarios/Shared/Configs/ActionOrigin/DA_LeaderActionOrigin.DA_LeaderActionOrigin" (`.ReturnValue` (`PXCommunityUtils.GetCommunityOfCommunityType` (`self.Community Type`))))))))))

(fn `CanBeStarted`
  (returns (ReturnValue :type Boolean))
  (locals (`community cache` :type "PXCommunityComponent Object Reference") (`faction cache` :type "PXCommunityComponent Object Reference") (`community type cache` :type "PXCommunityType Object Reference"))
  (bind _found (`self.Find Good Relations Candidates`))
  (return _found))

(fn `Find Good Relations Candidates`
  (returns (Found :type Boolean) (`community cache1` :type "PXCommunityComponent Object Reference") (`community type cache1` :type "PXCommunityType Object Reference") (`faction cache1` :type "PXCommunityComponent Object Reference"))
  (locals (`community cache` :type "PXCommunityComponent Object Reference") (`community type cache` :type "PXCommunityType Object Reference") (`faction cache` :type "PXCommunityComponent Object Reference") (NewLocalVar :type "Array of PXCommunityComponent Object Reference"))
  (bind _community_cache (`local.community cache`))
  (bind _factioncache1 (`/Game/Scenarios/Shared/BlueprintsNonSerialized/SocietyUtils/BPFL_StoryArc_Utils.Get existing faction with affinity` (`|GetArrayItem` (`PXCommunityType.GetAffinities` (`local.community type cache`)))))
  (bind (_outfound _returnvalue) (`PXFactionUtils.GetCommunityFromFaction` _factioncache1))
  (bind _output_get (set `local.NewLocalVar` (`PXFactionUtils.GetAllIndependentCommunities`)))
  (for _array_element _output_get
    (bind _output_get_2 (set `local.community cache` _array_element))
    (`/Engine/EditorBlueprintResources/StandardMacros.IsValid` _output_get_2
      (:`Is Valid`
        (if (not (`PXCommunityActionUtils.WasCommunityActionEverExecuted` (`self.Good Relations CA`) (`local.community cache`)))
          (if (and (>= (`PXTraitType.SeverityLevel` (`/Game/Scenarios/Shared/BlueprintsNonSerialized/FactionEmergence/BPFL_FactionEmergenceUtils.Get Community Relations Trait Helper` _community_cache)) (`self.Relations Tier`)) (not (`PXCommunityComponent.HasActiveImprint` _community_cache (`self.Good Relations Sympathiser Imprint`))) (not (`PXCommunityComponent.HasActiveImprint` _community_cache (`self.Do Nothing Imprint`))))
            (set `local.community type cache` (`PXCommunityComponent.GetCommunityType` (`local.community cache`)))
            (if (`KismetArrayLibrary.Array_IsNotEmpty` (`PXCommunityType.GetAffinities` (`local.community type cache`)))
              (`/Engine/EditorBlueprintResources/StandardMacros.IsValid` _factioncache1
                (:`Is Valid`
                  (if _outfound
                    (set `local.faction cache` _returnvalue)
                    (if (> (`.Severity Level` (`/Game/Scenarios/Shared/BlueprintsNonSerialized/OngoingEvents/BPFL_OngoingAction_Utils.Get Community Strength Tier` (`local.faction cache`))) 0)
                      (if (not (<= (`PXCommunityComponent.GetCommunitySize` (`local.faction cache`)) 4))
                        (if (not (`self.Previous Good Relations Imprint?`))
                          (return true (`local.community cache`) (`local.community type cache`) (`local.faction cache`))))))))))))))
  (return false null null null))

(fn `Previous Good Relations Imprint?`
  (returns (ReturnValue :type Boolean))
  (`/Engine/EditorBlueprintResources/StandardMacros.IsValid` (`self.Good Relations Choice Imprint`)
    (:`Is Valid`
      (if (`PXCommunityUtils.IsThereAnyCommunityWithImprint` (`self.Good Relations Choice Imprint`))
        (return true)
        (else
          (return false))))
    (:`Is Not Valid`
      (return false))))