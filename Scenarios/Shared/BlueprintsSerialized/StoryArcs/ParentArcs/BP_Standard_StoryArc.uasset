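; BP_Standard_StoryArc is a parent story arc Blueprint that provides shared setup-parameter functions and a game-time timer.
; Each instance reports setup parameters, hashes by its own object pointer and never matches another arc's parameters.
; Set Timer records the start time once, and Restart Timer clears that latch to record it again.
; The expiry check uses a positive passed-in duration, otherwise the stored TimerDuration.
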(fn `GetParametersHash`
  (returns (ReturnValue :type Integer))
  (return (`self.GetThisObjectPointerHash`)))

(fn `HasSetupParameters`
  (returns (ReturnValue :type Boolean))
  (return true))

(fn `HasThisSameParameters`
  (params (selfPtr :type "PXParameterizedStoryArc Object Reference") (otherStoryArc :type "PXParameterizedStoryArc Object Reference"))
  (returns (ReturnValue :type Boolean))
  (return false))

(fn `Restart Timer`
  (set `self.Timer is Set` false)
  (`self.Set Timer`)
  (return))

(fn `Set Timer`
  (if (not (`self.Timer is Set`))
    (set `self.Timer Start` (`PXTimeUtils.GetCurrentGameTime`))
    (set `self.Timer is Set` true)
    (return)
    (else
      (return))))

(fn `Timer has expired?`
  (params (Duration :type "PXGameTime Structure"))
  (returns (ReturnValue :type Boolean))
  (return (`/Game/Scenarios/Shared/BlueprintsNonSerialized/SocietyUtils/BPFL_CanBeStarted_Utils.Duration has passed since start time` (select `bool` (`PXTimeUtils.Greater` Duration) :`false` (`self.Timer Duration`) :`true` Duration) (`self.Timer Start`))))