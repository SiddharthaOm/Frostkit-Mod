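; Story arc where an independent community with bad relations radicalises, shifting population to the faction sharing its first affinity.
; A lens offers a relations-improvement quest, harsh action or encouragement; size-one or sympathiser-imprinted communities skip it and transfer directly.
; Transfers scale with community size, except the fixed size-one case.
; Trust-change events drive the quest objective; OnFinished awaits its result, shows a dialog, transfers population on failure and sets the arc-done unlock.
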(event `self.OnStarted`
  (bind (_return _local_community_with_bad_relations1 _local_community_type1 _local_faction_type1 _local_faction_community1) (`self.Find Bad Relations Communities`))
  (set `self.Community with bad relations` _local_community_with_bad_relations1)
  (set `self.Community Type` _local_community_type1)
  (set `self.Faction type` _local_faction_type1)
  (set `self.Faction Community` _local_faction_community1)
  (if (not (== (`PXCommunityComponent.GetCommunitySize` (`self.Community with bad relations`)) 1))
    (`self.Setup Transfer Amounts`)
    (if (not (`PXCommunityComponent.HasActiveImprint` (`self.Community with bad relations`) "/Game/Scenarios/Shared/Configs/Communities/Imprints/BadRelations/DA_BadRelations_Sympathiser_Imprint.DA_BadRelations_Sympathiser_Imprint"))
      (bind _decision (`/Game/Scenarios/Shared/BlueprintsNonSerialized/SocietyUtils/BPFL_Communication_Utils.Send Lens With Community Art` (`self.Get Lens Config`) null (`self.Community Type`) (`|MakeMap` "COMMUNITY" (`PXCommunityType.IngameName` (`self.Community Type`)) "FACTION" (`PXFactionType.IngameName` (`self.Faction type`)) "QUEST_TRANSFER" (`/Game/UI/Utilities/BPFL_UI.Get Population Size Points Display Text` (`self.Quest Transfer`)) "HARSH_TRANSFER" (`/Game/UI/Utilities/BPFL_UI.Get Population Size Points Display Text` (`self.Harsh Transfer`)) "ENCOURAGE_TRANSFER" (`/Game/UI/Utilities/BPFL_UI.Get Population Size Points Display Text` (`self.Encourage Transfer`)) "RELATIONS" (`PXTraitType.IngameName` (`self.Bad Relations`)) "WEEKS" (`KismetTextLibrary.Conv_IntToText` (`PXTimeSubsystem.GetTotalWeeks` (`self.Quest Duration`)))) (`PXGameplayContextUtils.MakePXGameContext` (`self.Community with bad relations`)) (struct) true))
      (bind _choice (`PXAsyncWaitForChoice.AsyncAction_WaitForChoice` _decision)
        (:`Completed`
          (switch `int` _choice
            (:`0`
              (bind _returnvalue (`PXQuestUtils.StartQuestInPlace` (`|FormatText` "Stop {COMMUNITY} Radicalisation" (`PXCommunityType.IngameName` (`self.Community Type`))) "" (`self.Quest Duration`) "MainQuest" "DebugQuestName" true))
              (bind _output_get (set `self.quest object` _returnvalue))
              (bind _returnvalue_2 (`PXQuest.AddQuestObjective` _output_get (`|FormatText` "Improve relations with {COMMUNITY} to {TIER} or better" (`PXCommunityType.IngameName` (`self.Community Type`)) (`PXTraitType.IngameName` (`self.Minimum Improve Tier`))) "" 0 1 false null "DebugObjectiveName"))
              (set `self.objective ` _returnvalue_2)
              (add `PXTrustSubsystem.TrustChangedEvent` (subsystem `PXTrustSubsystem`) (`|CreateDelegate` :!event `Update Relations Objective`)))
            (:`1`
              (`/Game/Scenarios/Shared/BlueprintsNonSerialized/FactionEmergence/BPFL_FactionEmergenceUtils.Transfer Size From Community to Matching Faction` (`self.Harsh Transfer`) (`|FormatText` (`self.bad relations harhs transfer reason`) (`/Game/Scenarios/Shared/BlueprintsNonSerialized/Communities/BPFL_CommunityUtils.Get Community Name` (`self.Community with bad relations`)) (`/Game/Scenarios/Shared/BlueprintsNonSerialized/Communities/BPFL_CommunityUtils.Get Community Name` (`self.Faction Community`))) (`self.Community with bad relations`) true true (struct :`ScaledTicks` 8400))
              (`PXUnlockUtils.SetUnlockActive` (`PXNationUtils.GetPlayerNation`) "/Game/Scenarios/Shared/DA_BadRelationsArcDone_Unlock.DA_BadRelationsArcDone_Unlock" true :!label _label))
            (:`2`
              (`/Game/Scenarios/Shared/BlueprintsNonSerialized/FactionEmergence/BPFL_FactionEmergenceUtils.Transfer Size From Community to Matching Faction` (`self.Encourage Transfer`) (`|FormatText` (`self.bad relations encouragee transfer reason`) (`/Game/Scenarios/Shared/BlueprintsNonSerialized/Communities/BPFL_CommunityUtils.Get Community Name` (`self.Community with bad relations`)) (`/Game/Scenarios/Shared/BlueprintsNonSerialized/Communities/BPFL_CommunityUtils.Get Community Name` (`self.Faction Community`))) (`self.Community with bad relations`) true false (struct :`ScaledTicks` 8400))
              (goto _label)))))
      (else
        (`/Game/Scenarios/Shared/BlueprintsNonSerialized/FactionEmergence/BPFL_FactionEmergenceUtils.Transfer Size From Community to Matching Faction` (`self.Subsequent Transfer`) (`|FormatText` (`self.Bad Relations Subsequent Transfer Reason`) (`/Game/Scenarios/Shared/BlueprintsNonSerialized/Communities/BPFL_CommunityUtils.Get Community Name` (`self.Community with bad relations`)) (`/Game/Scenarios/Shared/BlueprintsNonSerialized/Communities/BPFL_CommunityUtils.Get Community Name` (`self.Faction Community`))) (`self.Community with bad relations`) true true (struct :`ScaledTicks` 25200))))
    (else
      (`/Game/Scenarios/Shared/BlueprintsNonSerialized/FactionEmergence/BPFL_FactionEmergenceUtils.Transfer Size From Community to Matching Faction` 1 (`|FormatText` "as they join their identity with the faction") (`self.Community with bad relations`) true true))))

(event `self.OnFinished`
  (if (not (`PXUnlockUtils.IsUnlockActive` (`PXNationUtils.GetPlayerNation`) "/Game/Scenarios/Shared/DA_BadRelationsArcDone_Unlock.DA_BadRelationsArcDone_Unlock"))
    (`/Engine/EditorBlueprintResources/StandardMacros.IsValid` (`self.quest object`)
      (:`Is Valid`
        (bind _succeeded (`PXAsyncWaitForQuest.AsyncAction_WaitForQuest` (`self.quest object`))
          (:`Completed`
            (if _succeeded
              (`PXAsyncOpenPredefinedDialog.AsyncAction_OpenPredefinedDialog` "/Game/Scenarios/Shared/Configs/Messages/Dialogs/StoryArcs/DA_BadRelationsSuccess.DA_BadRelationsSuccess" (`|MakeMap` "COMMUNITY" (`PXCommunityType.IngameName` (`self.Community Type`)) "FACTION" (`PXFactionType.IngameName` (`self.Faction type`)))
                (:`Completed`
                  _))
              (else
                (`PXAsyncOpenPredefinedDialog.AsyncAction_OpenPredefinedDialog` "/Game/Scenarios/Shared/Configs/Messages/Dialogs/StoryArcs/DA_BadRelationsFail.DA_BadRelationsFail" (`|MakeMap` "COMMUNITY" (`PXCommunityType.IngameName` (`self.Community Type`)) "QUEST_TRANSFER" (`/Game/UI/Utilities/BPFL_UI.Get Population Size Points Display Text` (`self.Quest Transfer`)) "FACTION" (`PXFactionType.IngameName` (`self.Faction type`)))
                  (:`Completed`
                    (`/Game/Scenarios/Shared/BlueprintsNonSerialized/FactionEmergence/BPFL_FactionEmergenceUtils.Transfer Size From Community to Matching Faction` (`self.Quest Transfer`) (`|FormatText` (`self.bad relations quest failed transfer reason`) (`/Game/Scenarios/Shared/BlueprintsNonSerialized/Communities/BPFL_CommunityUtils.Get Community Name` (`self.Community with bad relations`)) (`/Game/Scenarios/Shared/BlueprintsNonSerialized/Communities/BPFL_CommunityUtils.Get Community Name` (`self.Faction Community`))) (`self.Community with bad relations`) true false (struct :`ScaledTicks` 8400))))))
            (`PXUnlockUtils.SetUnlockActive` (`PXNationUtils.GetPlayerNation`) "/Game/Scenarios/Shared/DA_BadRelationsArcDone_Unlock.DA_BadRelationsArcDone_Unlock" true)))))))

(fn `CanBeStarted`
  (returns (ReturnValue :type Boolean))
  (bind _quest_object (`self.quest object`))
  (`/Engine/EditorBlueprintResources/StandardMacros.IsValid` _quest_object
    (:`Is Valid`
      (if (`PXQuest.IsQuestFinished` _quest_object)
        (bind (_return _local_community_with_bad_relations1 _local_community_type1 _local_faction_type1 _local_faction_community1) (`self.Find Bad Relations Communities` :!label _label))
        (return (and _return (< (`PXTraitType.SeverityLevel` (`/Game/Scenarios/Shared/BlueprintsNonSerialized/FactionEmergence/BPFL_FactionEmergenceUtils.Get Community Relations Trait Helper` _local_faction_community1)) 4)))))
    (:`Is Not Valid`
      (goto _label))))

(fn `Find Bad Relations Communities`
  (returns (Return :type Boolean) (`Local Community with Bad Relations1` :type "PXCommunityComponent Object Reference") (`Local Community Type1` :type "PXCommunityType Object Reference") (`Local Faction Type1` :type "PXFactionType Object Reference") (`Local Faction Community1` :type "PXCommunityComponent Object Reference"))
  (locals (`Local Community with Bad Relations` :type "PXCommunityComponent Object Reference") (`Local Community Type` :type "PXCommunityType Object Reference") (`Local Faction Type` :type "PXFactionType Object Reference") (`Local Faction Community` :type "PXCommunityComponent Object Reference"))
  (bind _returnvalue (`PXCommunityType.GetAffinities` (`local.Local Community Type`)))
  (bind _factioncache1 (`/Game/Scenarios/Shared/BlueprintsNonSerialized/SocietyUtils/BPFL_StoryArc_Utils.Get existing faction with affinity` (`|GetArrayItem` _returnvalue)))
  (for _array_element (`PXFactionUtils.GetAllIndependentCommunities`)
    (bind _output_get (set `local.Local Community with Bad Relations` _array_element))
    (if (<= (`PXTraitType.SeverityLevel` (`/Game/Scenarios/Shared/BlueprintsNonSerialized/FactionEmergence/BPFL_FactionEmergenceUtils.Get Community Relations Trait Helper` (`local.Local Community with Bad Relations`))) 1)
      (set `local.Local Community Type` (`PXCommunityComponent.GetCommunityType` _output_get))
      (if (`KismetArrayLibrary.Array_IsNotEmpty` _returnvalue)
        (`/Engine/EditorBlueprintResources/StandardMacros.IsValid` _factioncache1
          (:`Is Valid`
            (bind _output_get_2 (set `local.Local Faction Type` _factioncache1))
            (bind (_outfound _returnvalue_2) (`PXFactionUtils.GetCommunityFromFaction` _output_get_2))
            (if _outfound
              (set `local.Local Faction Community` _returnvalue_2)
              (return true (`local.Local Community with Bad Relations`) (`local.Local Community Type`) (`local.Local Faction Type`) (`local.Local Faction Community`))))))))
  (return false null null null null))

(fn `Get Lens Config`
  (returns (`Lens Config` :type "PXLens Soft Object Reference"))
  (return (`self.Generic Lens Config`)))

(fn `Previous Bad Relations Imprints?`
  (returns (ReturnValue :type Boolean))
  (bind _community_with_bad_relations (`self.Community with bad relations`))
  (bind _faction_community (`self.Faction Community`))
  (return (not (or (`PXCommunityComponent.HasActiveImprint` _community_with_bad_relations (`self.Bad Relations Quest Failed Imprint`)) (`PXCommunityComponent.HasActiveImprint` _community_with_bad_relations (`self.Bad Relations Harsh mprint_`)) (`PXCommunityComponent.HasActiveImprint` _community_with_bad_relations (`self.Bad Relations encourage imprint`)) (`PXCommunityComponent.HasActiveImprint` _faction_community (`self.Bad Relations Quest Failed Imprint`)) (`PXCommunityComponent.HasActiveImprint` _faction_community (`self.Bad Relations Harsh mprint_`)) (`PXCommunityComponent.HasActiveImprint` _faction_community (`self.Bad Relations encourage imprint`))))))

(fn `Setup Transfer Amounts`
  (bind _returnvalue (`KismetMathLibrary.Conv_IntToDouble` (`PXCommunityComponent.GetCommunitySize` (`self.Community with bad relations`))))
  (set `self.Quest Transfer` (`KismetMathLibrary.FTrunc` (* _returnvalue (`self.Quest Transfer %`))))
  (set `self.Harsh Transfer` (`KismetMathLibrary.FTrunc` (* _returnvalue (`self.Harsh Transfer %`))))
  (set `self.Encourage Transfer` (`KismetMathLibrary.FTrunc` (* _returnvalue (`self.Encourage Transfer %`))))
  (set `self.Subsequent Transfer` (`KismetMathLibrary.FTrunc` (* _returnvalue (`self.Subsequent Transfer %`)))))

(fn `Update Relations Objective`
  (if (>= (`PXTraitType.SeverityLevel` (`/Game/Scenarios/Shared/BlueprintsNonSerialized/FactionEmergence/BPFL_FactionEmergenceUtils.Get Community Relations Trait Helper` (`.ReturnValue` (`PXCommunityUtils.GetCommunityOfCommunityType` (`self.Community Type`))))) (`PXTraitType.SeverityLevel` (`self.Minimum Improve Tier`)))
    (`PXQuestObjective.ProgressObjective` (`self.objective `) 1
      (:`Finished`
        (remove `PXTrustSubsystem.TrustChangedEvent` (subsystem `PXTrustSubsystem`) (`|CreateDelegate` :!event `Update Relations Objective`))))))