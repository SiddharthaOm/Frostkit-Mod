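; Faction War story arc that triggers game over when the war's initial defender faction dies out during a pogrom.
; It can start once the defender community is invalid or its size is at or below MinSize.
; On start it shows a modal lens using the opposite faction's community, since the dead one has no info to display.
; After the choice, it fails the prepare quest, logs a PogromFail analytics event and ends the game.
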(event `self.OnStarted`
  (bind _dead_community_type (`self.Get community type for lens`))
  (bind (_outfound _returnvalue) (`PXFactionUtils.GetCommunityFromFaction` (`/Game/Scenarios/Shared/BlueprintsNonSerialized/FactionEmergence/BPFL_FactionWarUtils.Get Fully Opposite Faction` (`PXCommunityType.Faction` _dead_community_type))))
  (bind _returnvalue_2 (`PXCommunityComponent.GetCommunityType` _returnvalue))
  ;[1 1 1] Since the dead faction is dead, we can't show community info about it, so we have to use the other faction
  (bind _decision (`/Game/Scenarios/Shared/BlueprintsNonSerialized/SocietyUtils/BPFL_Communication_Utils.Send Modal Lens with Community Art` (`self.Lens Config`) null _returnvalue_2 (`|MakeMap` "DEFENDER" (`PXCommunityType.IngameName` _dead_community_type) "AGGRESSOR" (`PXCommunityType.IngameName` _returnvalue_2)) (`PXGameplayContextUtils.MakePXGameContext` _returnvalue) (struct) true))
  (`PXAsyncWaitForChoice.AsyncAction_WaitForChoice` _decision
    (:`Completed`
      (`PXQuestUtils.FinishQuest` (`/Game/Scenarios/Shared/BlueprintsNonSerialized/FactionEmergence/BPFL_FactionWarUtils.Get Prepare Quest`))
      (bind _returnvalue_3 (`PXAnalyticsSubsystem.GetMainCityNameFromSubsystem` (subsystem `PXAnalyticsSubsystem`)))
      (`PXAnalyticsSubsystem.LogEvent` (`|Subsystem`) _returnvalue_3 "" "Gameplay" "GameOver" "PogromFail" (`KismetStringLibrary.Concat_StrStr` "GoneFaction:" (`KismetTextLibrary.Conv_TextToString` (`PXCommunityType.IngameName` (`self.Get community type for lens`)))) "")
      (`/Game/Scenarios/Shared/BlueprintsNonSerialized/EndGame/BPFL_EndGameUtils.End Game` "NewEnumerator0"))))

(fn `Aggressor Has Died?`
  (returns (ReturnValue :type Boolean) (`Faction War Aggressor Type` :type "PXCommunityType Object Reference"))
  (bind (_faction_war_aggressor _faction_war_aggressor_type) (`/Game/Scenarios/Shared/BlueprintsNonSerialized/SocietyUtils/BPFL_SharedScenariosStorage.Get Faction War Initial Aggressor`))
  (bind _returnvalue (`self.Faction Has Died?` _faction_war_aggressor))
  (return _returnvalue _faction_war_aggressor_type))

(fn `CanBeStarted`
  (returns (ReturnValue :type Boolean))
  (bind _returnvalue (`self.Defender Has Died?`))
  (if _returnvalue
    (return true)
    (else
      (return false))))

(fn `CanBeStarted Core`
  (returns (ReturnValue :type Boolean))
  (return true))

(fn `Defender Has Died?`
  (returns (ReturnValue :type Boolean) (`Faction War Defender Type` :type "PXCommunityType Object Reference"))
  (bind (_defender _faction_war_defender_type) (`/Game/Scenarios/Shared/BlueprintsNonSerialized/SocietyUtils/BPFL_SharedScenariosStorage.Get Faction War Initial Defender`))
  (bind _returnvalue (`self.Faction Has Died?` _defender))
  (return _returnvalue _faction_war_defender_type))

(fn `Faction Has Died?`
  (params (InputPin :type "PXCommunityComponent Object Reference"))
  (returns (ReturnValue :type Boolean))
  (bind _returnvalue (<= (`PXCommunityComponent.GetCommunitySize` InputPin) (`self.Min Size`)))
  (`/Engine/EditorBlueprintResources/StandardMacros.IsValid` InputPin
    (:`Is Valid`
      (if _returnvalue
        (return _returnvalue)))
    (:`Is Not Valid`
      (return true))))

(fn `Get community type for lens`
  (returns (`Dead community Type` :type "PXCommunityType Object Reference"))
  (return (`.Faction War Defender Type` (`/Game/Scenarios/Shared/BlueprintsNonSerialized/SocietyUtils/BPFL_SharedScenariosStorage.Get Faction War Initial Defender`))))