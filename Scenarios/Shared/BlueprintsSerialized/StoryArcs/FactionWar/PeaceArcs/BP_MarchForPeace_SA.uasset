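; Faction War story arc offering a March for Peace decision in the player's main city, citing a tenth of the workforce as absentees and naming independent communities.
; It can start only with enough trust, an Abandoned Militancy imprint on some community and a faction war in progress.
; The first choice shrinks each of the city's faction members proportionally, then waits for a major-event story beat.
; Followup text defines name the war's aggressor and its opposite under one shared key.
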(event `self.OnStarted`
  (bind _decision (`/Game/Scenarios/Shared/BlueprintsNonSerialized/SocietyUtils/BPFL_Communication_Utils.Send Config Message` (`self.March For Peace Lens`) null null null (`|MakeMap` "ABSENTEES_NUMBER" (`KismetTextLibrary.Conv_IntToText` (`KismetMathLibrary.FTrunc` (* 0.1 (`PXWorkforceUtils.GetCityTotalWorkforce` (`PXNationUtils.GetPlayerMainCity`))))) "INDEPENDENTS" (`/Game/Scenarios/Shared/BlueprintsNonSerialized/SocietyUtils/BPFL_Quest_Utils.Combine Text Array Into Single` (`/Game/Scenarios/Shared/BlueprintsNonSerialized/SocietyUtils/BPFL_Cornerstone_Utils.Get Community Names` (`PXFactionUtils.GetIndependentCommunitiesFromCity` (`PXNationUtils.GetPlayerMainCity`))))) null null (struct) true))
  (bind _output_get (set `self.Decision` _decision))
  (bind _choice (`PXAsyncWaitForChoice.AsyncAction_WaitForChoice` _output_get)
    (:`Completed`
      (switch `int` _choice
        (:`0`
          (for _array_element (`PXFactionUtils.GetMembersFromCity` (`PXNationUtils.GetPlayerMainCity`) null)
            (`/Game/Scenarios/Shared/BlueprintsNonSerialized/FactionEmergence/BPFL_FactionEmergenceUtils.Shrink Faction` _array_element (/ (`PXCommunityComponent.GetCommunitySize` _array_element) (`self.Divisor`)) (`|FormatText` "Peacekeepers reducing size") true (`self.Change Duration`) true false (`self.Leave At Least That Much Size In Each Community`)))
          (`PXAsyncWaitForStoryBeat.AsyncAction_WaitForStoryBeat` "/Game/Scenarios/Shared/Configs/StoryBeat/DA_MajorEventStoryBeat.DA_MajorEventStoryBeat" "/Game/Scenarios/Shared/Configs/StoryBeat/Lanes/DA_Main_Lane.DA_Main_Lane"))))))

(fn `CanBeStarted`
  (returns (ReturnValue :type Boolean))
  (bind (_returnvalue _ongoing_actions1) (`/Game/Scenarios/Shared/BlueprintsNonSerialized/OngoingEvents/BPFL_OngoingAction_Utils.Is Any Action of type Ongoing?` "/Game/Scenarios/Shared/Configs/OngoingActions/System_Started/DA_FactionWar.DA_FactionWar"))
  (bind _returnvalue_2 (`/Game/Scenarios/Shared/BlueprintsNonSerialized/SocietyUtils/BPFL_Trust_Utils.Trust Trait is At Least` (`self.Minimum Acceptable Trust Trait`)))
  (if _returnvalue_2
    (if (`KismetArrayLibrary.Array_IsNotEmpty` (`PXCommunityUtils.GetAllCommunitiesWithImprint` "/Game/Scenarios/Shared/Configs/Communities/Imprints/Other/DA_FactionWar_AbandonedMilitancy_Imprint.DA_FactionWar_AbandonedMilitancy_Imprint"))
      (if _returnvalue
        (for _array_element _ongoing_actions1
          (if (`|EnumEquality` (`PXOngoingActionComponent.GetState` _array_element) "InProgress")
            (bind _returnvalue_3 (`parent.CanBeStarted`))
            (return _returnvalue_3)))
        (return false)
        (else
          (return false)))
      (else
        (return false)))
    (else
      (return false))))

(fn `CanBeStarted Core`
  (returns (ReturnValue :type Boolean))
  (return true))

(fn `Followup Defines`
  (returns (Map :type "Map of String to Text"))
  (locals (NewLocalVar :type "Map of String to Text"))
  (bind _faction_war_aggressor (`/Game/Scenarios/Shared/BlueprintsNonSerialized/SocietyUtils/BPFL_SharedScenariosStorage.Get Faction War Initial Aggressor`))
  (`BlueprintMapLibrary.Map_Add` (`local.NewLocalVar`) "STRONGEST_FACTION" (`/Game/Scenarios/Shared/BlueprintsNonSerialized/Communities/BPFL_CommunityUtils.Get Community Name` _faction_war_aggressor))
  (`BlueprintMapLibrary.Map_Add` (`local.NewLocalVar`) "STRONGEST_FACTION" (`/Game/Scenarios/Shared/BlueprintsNonSerialized/Communities/BPFL_CommunityUtils.Get Community Name` (`.ReturnValue` (`PXFactionUtils.GetCommunityFromFaction` (`/Game/Scenarios/Shared/BlueprintsNonSerialized/FactionEmergence/BPFL_FactionWarUtils.Get Fully Opposite Faction` (`PXCommunityComponent.GetFaction` _faction_war_aggressor))))))
  (return (`local.NewLocalVar`)))

(fn `GetParametersHash`
  (returns (ReturnValue :type Integer))
  (return (`PXStoryUtils.GetHashForUObjectParameter` (`PXCommunicationChannelsUtils.ToObject` (`self.March For Peace Lens`)))))