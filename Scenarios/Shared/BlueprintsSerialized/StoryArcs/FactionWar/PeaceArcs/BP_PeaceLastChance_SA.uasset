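; Faction War peace story arc that presents a "last chance for peace" message to the player.
; It can start only while the peace policy is not active.
; On start it sends the PeaceLastChanceLens config message, tied to the main district of the player's main city, then waits asynchronously for any choice.
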(event `self.OnStarted`
  (bind _decision (`/Game/Scenarios/Shared/BlueprintsNonSerialized/SocietyUtils/BPFL_Communication_Utils.Send Config Message` (`self.Peace Last Chance Lens`) (`PXCityComponent.GetMainDistrict` (`PXNationUtils.GetPlayerMainCity`)) null null (`self.Text Defines`)))
  (`PXAsyncWaitForAnyChoice.AsyncAction_WaitForAnyChoice` _decision))

(fn `CanBeStarted`
  (returns (ReturnValue :type Boolean))
  (if (not (`/Game/Scenarios/Shared/BlueprintsNonSerialized/Policies/BPFL_PolicyUtils.IsPolicyActive` (`self.Peace Policy`)))
    (return true)))