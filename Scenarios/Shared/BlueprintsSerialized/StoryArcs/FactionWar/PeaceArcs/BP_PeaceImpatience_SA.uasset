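; Faction War story arc that pressures the player to pass an unlocked but inactive peace law, escalating to game over.
; After a timeout it sends a warning and puts a countdown on the preparation quest, then force-starts a Last Chance arc.
; It then forces a Parliament vote on the Peace Accords, ending the game if they fail.
; Each async step rechecks that the policy is inactive and the war stage active.
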(event `self.OnStarted`
  (if (`self.Recheck Start Requirements`)
    (bind _decision (`/Game/Scenarios/Shared/BlueprintsNonSerialized/SocietyUtils/BPFL_Communication_Utils.Send Config Message` (`self.Peace Impatience Lens`) (`PXCityComponent.GetMainDistrict` (`PXNationUtils.GetPlayerMainCity`)) null null (`|MakeMap` "LAW" (`PXPolicyType.IngameName` (`self.Peace Policy`)) "WEEKS" (`PXTextUtils.GameTimeToTextMostImportant` (`self.Time after warning`)))))
    (`PXAsyncWaitForAnyChoice.AsyncAction_WaitForAnyChoice` _decision
      (:`Completed`
        (if (`self.Recheck Start Requirements`)
          (`PXQuest.SetQuestDuration` (`/Game/Scenarios/Shared/BlueprintsNonSerialized/FactionEmergence/BPFL_FactionWarUtils.Get Prepare Quest`) (`PXTimeUtils.Add` (`PXTimeUtils.Subtract` (`PXTimeUtils.GetCurrentGameTime`) (`PXQuest.GetQuestStartTime` (`/Game/Scenarios/Shared/BlueprintsNonSerialized/FactionEmergence/BPFL_FactionWarUtils.Get Prepare Quest`))) (`self.Time after warning`) (struct :`ScaledTicks` 240)))
          (`PXAsyncWaitForDurationPassed.AsyncAction_WaitForDurationPassed` (`self.Time after warning`)
            (:`Completed`
              (if (`self.Recheck Start Requirements`)
                (`PXQuest.SetEndlessDuration` (`/Game/Scenarios/Shared/BlueprintsNonSerialized/FactionEmergence/BPFL_FactionWarUtils.Get Prepare Quest`))
                (bind _returnvalue (`|GenericCreateObject` (subsystem `PXStoryArcSubsystem`) "/Game/Scenarios/Shared/BlueprintsSerialized/StoryArcs/FactionWar/PeaceArcs/BP_PeaceLastChance_SA.BP_PeaceLastChance_SA_C" (`self.Peace Defines`) (`self.Peace Last Chance Lens`)))
                (`PXStoryUtils.ForceStartExistingArc` _returnvalue)
                (set `self.Peace Last Chance Arc` _returnvalue)
                (`PXAsyncWaitForDurationPassed.AsyncAction_WaitForDurationPassed` (struct :`ScaledTicks` 10)
                  (:`Completed`
                    (`PXAsyncWaitForStoryArc.AsyncAction_WaitForStoryArc` (`self.Peace Last Chance Arc`)
                      (:`Completed`
                        (if (`self.Recheck Start Requirements`)
                          (`PXParliamentUtils.RequestSession` true (`self.Peace Accords Law`) true)
                          (`/Game/Scenarios/Shared/BlueprintsNonSerialized/Parliament/BPFL_ParliamentUtilities.Enter Parliament (No transition)`)
                          (`PXAsyncWaitForNextVote.AsyncAction_WaitForNextVote`
                            (:`Completed`
                              (if (`self.Recheck Start Requirements`)
                                (if (not (`/Game/Scenarios/Shared/BlueprintsNonSerialized/Policies/BPFL_PolicyUtils.IsPolicyActive` (`self.Peace Accords Law`)))
                                  (bind _decision_2 (`/Game/Scenarios/Shared/BlueprintsNonSerialized/SocietyUtils/BPFL_Communication_Utils.Send Config Message` (`self.Game Over Message`) null null null (`|MakeMap` "" :!valuetype "Text")))
                                  (`PXAsyncWaitForAnyChoice.AsyncAction_WaitForAnyChoice` _decision_2
                                    (:`Completed`
                                      (`PXQuestUtils.FinishQuest` (`/Game/Scenarios/Shared/BlueprintsNonSerialized/FactionEmergence/BPFL_FactionWarUtils.Get Prepare Quest`))
                                      (`/Game/Scenarios/Shared/BlueprintsNonSerialized/EndGame/BPFL_EndGameUtils.End Game` "NewEnumerator0"))))))))))))))))))))

(fn `CanBeStarted`
  (returns (ReturnValue :type Boolean))
  (bind _returnvalue (`PXPolicyUtils.GetPlayerPolicy`))
  (bind _peace_policy (`self.Peace Policy`))
  (if (and (not (`/Game/Scenarios/Shared/BlueprintsNonSerialized/Policies/BPFL_PolicyUtils.IsPolicyActive` _peace_policy)) (`PXPolicyUtils.IsLawUnlocked` _returnvalue (`PXPolicyUtils.GetLaw` _returnvalue _peace_policy)))
    (`self.Set Timer`)
    (return (`self.Timer has expired?` (`self.Timeout Duration`)))))

(fn `Peace Defines`
  (returns (Map :type "Map of String to Text"))
  (return (`|MakeMap` "LAW" (`PXPolicyType.IngameName` (`self.Peace Accords Law`)))))

(fn `Recheck Start Requirements`
  (returns (ReturnValue :type Boolean))
  (return (and (not (`/Game/Scenarios/Shared/BlueprintsNonSerialized/Policies/BPFL_PolicyUtils.IsPolicyActive` (`self.Peace Policy`))) (`PXUnlockUtils.IsUnlockActive` (`PXNationUtils.GetPlayerNation`) (`self.faction war stage unlock`)))))