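; Faction War story arc step that offers the player a first choice between crushing the war and enforcing peace in a district.
; An active Pick a Side unlock swaps the Crush ability for Speed Victory and uses an alternate lens message.
; Both options display informational ability desires, and the awaited choice activates that ability on the context district's owner.
; The gameplay factor override is empty, with its guard-cost logic left disconnected.
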(event `self.OnStarted`
  (bind _returnvalue (`PXNationUtils.GetPlayerMainCity`))
  (bind _returnvalue_2 (`ActorComponent.GetOwner` (`/Game/Scenarios/Shared/BlueprintsNonSerialized/SocietyUtils/BPFL_Communication_Utils.Get Best District from Context` (`self.Game Context`))))
  (bind _output_get (set `self.Crush Ability for path` (select `bool` (`PXUnlockUtils.IsUnlockActive` (`PXNationUtils.GetPlayerNation`) "/Game/Scenarios/Shared/Configs/Unlocks/FactionWarEndings/DA_PickASide_Unlock.DA_PickASide_Unlock") :`false` "/Game/Scenarios/Shared/Configs/Abilities/DistrictAbilities/FactionWar/DA_Crush_InFactionWar_DistrictAbility.DA_Crush_InFactionWar_DistrictAbility" :`true` "/Game/Scenarios/Shared/Configs/Abilities/DistrictAbilities/FactionWar/DA_SpeedVictory_InFactionWar_DistrictAbility.DA_SpeedVictory_InFactionWar_DistrictAbility" :!type "PXAbility Object Reference")))
  (bind _returnvalue_3 (`PXDesireUtils.MakeAbilityDesire` _output_get _returnvalue))
  (`KismetArrayLibrary.Array_Add` (`self.desire array`) _returnvalue_3)
  (bind _returnvalue_4 (`PXDesireUtils.MakeAbilityDesire` (`self.Enforce Peace Ability`) _returnvalue))
  (`KismetArrayLibrary.Array_Add` (`self.desire array`) _returnvalue_4)
  (bind _decision (`/Game/Scenarios/Shared/BlueprintsNonSerialized/SocietyUtils/BPFL_Communication_Utils.Send Config Message` (select `bool` (`PXUnlockUtils.IsUnlockActive` (`PXNationUtils.GetPlayerNation`) "/Game/Scenarios/Shared/Configs/Unlocks/FactionWarEndings/DA_PickASide_Unlock.DA_PickASide_Unlock") :`false` (`self.Lens Config`) :`true` (`self.Lens Config_PickASide`) :!type "PXCommunicationChannelMessage Soft Object Reference") (`/Game/Scenarios/Shared/BlueprintsNonSerialized/SocietyUtils/BPFL_Communication_Utils.Get Best District from Context` (`self.Game Context`)) null null (`|MakeMap` "CRUSH_ABILITY" (`PXAbility.IngameName` (`self.Crush Ability for path`)) "ENFORCE_ABILITY" (`PXAbility.IngameName` (`self.Enforce Peace Ability`))) null null (`/Game/Scenarios/Shared/BlueprintsNonSerialized/SocietyUtils/BPFL_Communication_Utils.Single Desire Per Choice Helper` (`self.desire array`) true) true))
  (bind _output_get_2 (set `self.Decision` _decision))
  (bind _choice (`PXAsyncWaitForChoice.AsyncAction_WaitForChoice` _output_get_2)
    (:`Completed`
      (switch `int` _choice
        (:`0`
          (`PXAbilityUtils.ActivateActorAbility` _returnvalue_2 (`self.Crush Ability for path`) "/Game/Scenarios/Shared/Configs/ActionOrigin/DA_LeaderActionOrigin.DA_LeaderActionOrigin"))
        (:`1`
          (`PXAbilityUtils.ActivateActorAbility` _returnvalue_2 (`self.Enforce Peace Ability`) "/Game/Scenarios/Shared/Configs/ActionOrigin/DA_LeaderActionOrigin.DA_LeaderActionOrigin"))))))

(fn `Add GameplayFactorValues`
  (params (`Gameplay Factor Values1` :type "Array of PXGameplayFactorValues Structure (by ref)"))
  (return))