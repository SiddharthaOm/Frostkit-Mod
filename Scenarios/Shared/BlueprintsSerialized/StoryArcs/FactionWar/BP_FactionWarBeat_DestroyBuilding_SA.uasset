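; Faction war story arc beat that destroys a random building in the best district from the game context.
; It requires that district to have buildings, then on start adds small wear to the owning district and starts deconstruction of the chosen building without refund.
; Cancelling the deconstruction is blocked with a faction war reason, and a notification reports the building as destroyed in fighting.
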(event `self.OnStarted`
  (bind _output_get (set `self.building to destroy` (`PXRandomLibrary.PXArrayRandom` (`PXDistrictComponent.GetBuildings` (`/Game/Scenarios/Shared/BlueprintsNonSerialized/SocietyUtils/BPFL_Communication_Utils.Get Best District from Context` (`self.Game Context`))))))
  (`PXWearUtils.IncreaseWear` (`ActorComponent.GetOwner` (`PXBuildingComponent.OwningDistrict` _output_get)) (`self.Small Wear`))
  (bind _returnvalue (`ActorComponent.GetOwner` _output_get))
  (`PXDeconstructionUtils.StartDeconstruction` _returnvalue "/Game/Scenarios/Shared/Configs/ActionOrigin/DA_OtherActionOrigin.DA_OtherActionOrigin")
  (`PXBlockageUtils.SetActionBlocked` _returnvalue "/Game/Scenarios/Shared/Configs/Blockages/ActionTypes/DA_Action_CancelDeconstruction.DA_Action_CancelDeconstruction" "/Game/Scenarios/Shared/Configs/Blockages/Reasons/DA_BlockageReason_FactionWar.DA_BlockageReason_FactionWar" true)
  (`PXCommunicationChannelsUtils.AddNotification` (make `PXNotificationData` "Normal" (`|FormatText` "{BUILDING} destroyed in fighting" (`PXBuildingType.IngameName` (`PXBuildingComponent.Type` (`self.building to destroy`)))))))

(fn `CanBeStarted`
  (returns (ReturnValue :type Boolean))
  (bind _returnvalue (`parent.CanBeStarted`))
  (return _returnvalue))

(fn `CanBeStarted Core`
  (returns (ReturnValue :type Boolean))
  (return (`KismetArrayLibrary.Array_IsNotEmpty` (`PXDistrictComponent.GetBuildings` (`/Game/Scenarios/Shared/BlueprintsNonSerialized/SocietyUtils/BPFL_Communication_Utils.Get Best District from Context` (`self.Game Context`))))))