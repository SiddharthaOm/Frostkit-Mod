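; BP_FactionWar_FirstProtect is a Faction War story event where the player chooses between protecting buildings and protecting people.
; On start it sends a config message for the context's best district, previewing both main-city abilities as informational desires.
; It waits for the choice, then activates the chosen ability on the district's owner with a leader action origin.
; The gameplay factor override returns empty, leaving its guard-cost logic unreachable.
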(event `self.OnStarted`
  (bind _returnvalue (`PXNationUtils.GetPlayerMainCity`))
  (bind _returnvalue_2 (`ActorComponent.GetOwner` (`/Game/Scenarios/Shared/BlueprintsNonSerialized/SocietyUtils/BPFL_Communication_Utils.Get Best District from Context` (`self.Game Context`))))
  (bind _returnvalue_3 (`PXDesireUtils.MakeAbilityDesire` (`self.Protect Buildings`) _returnvalue))
  (`KismetArrayLibrary.Array_Add` (`self.desire array`) _returnvalue_3)
  (bind _returnvalue_4 (`PXDesireUtils.MakeAbilityDesire` (`self.Protect People`) _returnvalue))
  (`KismetArrayLibrary.Array_Add` (`self.desire array`) _returnvalue_4)
  (bind _decision (`/Game/Scenarios/Shared/BlueprintsNonSerialized/SocietyUtils/BPFL_Communication_Utils.Send Config Message` (`self.Lens Config`) (`/Game/Scenarios/Shared/BlueprintsNonSerialized/SocietyUtils/BPFL_Communication_Utils.Get Best District from Context` (`self.Game Context`)) null null (`|MakeMap` "PROTECT_BUILDINGS" (`PXAbility.IngameName` (`self.Protect Buildings`)) "PROTECT_PEOPLE" (`PXAbility.IngameName` (`self.Protect People`))) null null (`/Game/Scenarios/Shared/BlueprintsNonSerialized/SocietyUtils/BPFL_Communication_Utils.Single Desire Per Choice Helper` (`self.desire array`) true) true))
  (bind _output_get (set `self.Decision` _decision))
  (bind _choice (`PXAsyncWaitForChoice.AsyncAction_WaitForChoice` _output_get)
    (:`Completed`
      (switch `int` _choice
        (:`0`
          (`PXAbilityUtils.ActivateActorAbility` _returnvalue_2 (`self.Protect Buildings`) "/Game/Scenarios/Shared/Configs/ActionOrigin/DA_LeaderActionOrigin.DA_LeaderActionOrigin"))
        (:`1`
          (`PXAbilityUtils.ActivateActorAbility` _returnvalue_2 (`self.Protect People`) "/Game/Scenarios/Shared/Configs/ActionOrigin/DA_LeaderActionOrigin.DA_LeaderActionOrigin"))))))

(fn `Add GameplayFactorValues`
  (params (`Gameplay Factor Values1` :type "Array of PXGameplayFactorValues Structure (by ref)"))
  (return))