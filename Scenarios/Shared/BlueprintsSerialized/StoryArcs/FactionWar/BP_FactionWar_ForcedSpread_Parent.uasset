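; Parent story-arc beat for a forced faction war spread, presenting a decision naming attacker and defender that the starting ongoing action awaits.
; Start is gated by unlocks and action blocks, with a "seen" unlock held while the beat runs.
; Choice handling is an empty hook.
; On finish it requests additional wars if none was ongoing at start, then optionally blocks new action starts until the spread wait passes.
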(event `self.OnStarted`
  (`PXUnlockUtils.SetUnlockActive` (`PXNationUtils.GetPlayerNation`) (`self.HACK beat seen unlock`) true)
  (set `self.first war after break` (not (`/Game/Scenarios/Shared/BlueprintsNonSerialized/OngoingEvents/BPFL_OngoingAction_Utils.Is Any Action of type Ongoing?` "/Game/Scenarios/Shared/Configs/OngoingActions/System_Started/DA_FactionWar.DA_FactionWar")))
  (bind _output_get (set `self.District` (`/Game/Scenarios/Shared/BlueprintsNonSerialized/SocietyUtils/BPFL_Communication_Utils.Get Best District from Context` (`self.Game Context`))))
  (bind _decision (`/Game/Scenarios/Shared/BlueprintsNonSerialized/SocietyUtils/BPFL_Communication_Utils.Send Config Message` (`self.Lens Config`) _output_get (`self.Get Context Community`) null (`self.Get Defines`)))
  (bind _output_get_2 (set `self.Decision` _decision))
  (`PXOngoingActionUtils.SetOngoingActionDecisionAwaitedForStart` (`PXGameplayContextUtils.TryGetOngoingActionFromGameContext` (`self.Game Context`)) _output_get_2)
  (bind _choice (`PXAsyncWaitForChoice.AsyncAction_WaitForChoice` (`self.Decision`))
    (:`Completed`
      (set `self.Choice` _choice)
      (`self.Handle Choice` (`self.Choice`)))))

(event `self.OnFinished`
  (`parent.OnFinished`)
  (`self.Start Other Wars`)
  (`self.Add Block`)
  (`PXUnlockUtils.SetUnlockActive` (`PXNationUtils.GetPlayerNation`) (`self.HACK beat seen unlock`))
  (`PXAsyncWaitForDurationPassed.AsyncAction_WaitForDurationPassed` (`self.Spread Wait`)
    (:`Completed`
      (`self.Remove Block`))))

(fn `Add Block`
  (if (`self.Manual Block After?`)
    (`PXOngoingActionUtils.AddStartingOngoingActionBlockReason` (`self.Manual Block`))))

(fn `CanBeStarted Core`
  (returns (ReturnValue :type Boolean))
  ;[1 1 1] Must set this unlock to TRUE when force starting an OA to disable these default start lenses
  (if (not (`PXUnlockUtils.IsUnlockActive` (`PXNationUtils.GetPlayerNation`) (`self.OA Start Disabled Unlock`)))
    (if (not (`PXOngoingActionUtils.IsStartingOngoingActionBlocked`))
      (if (not (`PXUnlockUtils.IsUnlockActive` (`PXNationUtils.GetPlayerNation`) (`self.HACK beat seen unlock`)))
        (return true)
        (else
          (return false))))))

(fn `Get Context Community`
  (returns (`Faction Component` :type "PXCommunityComponent Object Reference"))
  (return (`self.Get Defender`)))

(fn `Get Defender`
  (returns (`Faction Component` :type "PXCommunityComponent Object Reference"))
  (return (`.Faction Component` (`/Game/Scenarios/Shared/BlueprintsNonSerialized/FactionEmergence/BPFL_FactionWarUtils.Get Existing Opposing Faction` (`PXCommunityComponent.GetFaction` (`/Game/Scenarios/Shared/BlueprintsNonSerialized/SocietyUtils/BPFL_SharedScenariosStorage.Get Faction War Initial Aggressor`))))))

(fn `Get Defines`
  (returns (Map :type "Map of String to Text"))
  (return (`|MakeMap` "DEFENDER" (`/Game/Scenarios/Shared/BlueprintsNonSerialized/Communities/BPFL_CommunityUtils.Get Community Name` (`self.Get Defender`)) "ATTACKER" (`/Game/Scenarios/Shared/BlueprintsNonSerialized/Communities/BPFL_CommunityUtils.Get Community Name` (`/Game/Scenarios/Shared/BlueprintsNonSerialized/SocietyUtils/BPFL_SharedScenariosStorage.Get Faction War Initial Aggressor`)))))

(fn `Get Message Defines`
  (returns (Map :type "Map of String to Text"))
  (bind _defines_map_merged (`/Game/Scenarios/Shared/BlueprintsNonSerialized/SocietyUtils/BPFL_Communication_Utils.Merge Defines` (`parent.Get Message Defines`) (`self.Get Defines`)))
  (return _defines_map_merged))

(fn `Handle Choice`
  (params (Selection :type Integer))
  (switch `int` Selection))

(fn `Readd Start Block`
  (params (changeType :type "EPXOngoingActionChangeType Enum" :default "HintsStart") (ongoingAction :type "PXOngoingActionComponent Object Reference"))
  (if (and (`|EnumEquality` changeType "Start") (`/Game/Scenarios/Shared/BlueprintsNonSerialized/OngoingEvents/BPFL_OngoingAction_Utils.OA is Faction War` ongoingAction))
    (remove `PXOngoingActionSubsystem.OngoingActionChangedEvent` (subsystem `PXOngoingActionSubsystem`) (`|CreateDelegate` :!event `Readd Start Block`))
    (`PXOngoingActionUtils.AddStartingOngoingActionBlockReason` "/Game/Scenarios/Shared/Configs/OngoingActions/StartBlockReasons/DA_FactionWars_ManualStage_OABlock.DA_FactionWars_ManualStage_OABlock")))

(fn `Remove Block`
  (`PXOngoingActionUtils.RemoveStartingOngoingActionBlockReason` (`self.Manual Block`)))

(fn `Start Other Wars`
  (bind (_faction_war_aggressor _faction_war_aggressor_type _faction_war_aggressor_name _is_valid) (`/Game/Scenarios/Shared/BlueprintsNonSerialized/SocietyUtils/BPFL_SharedScenariosStorage.Get Faction War Initial Aggressor`))
  ;[1 1 1] Fix to handle Captain speedruns, Faction Wars might be over
  (if (`PXUnlockUtils.IsUnlockActive` (`PXNationUtils.GetPlayerNation`) "/Game/Scenarios/Shared/Configs/Unlocks/FactionWarEndings/DA_FactionWarStage_Unlock.DA_FactionWarStage_Unlock")
    (if _is_valid
      (if (`self.first war after break`)
        (`PXUnlockUtils.SetUnlockActive` (`PXNationUtils.GetPlayerNation`) "/Game/Scenarios/Shared/Configs/Unlocks/DA_SuppressOAStartMessage_Unlock.DA_SuppressOAStartMessage_Unlock" true)
        (`PXOngoingActionUtils.RequestOngoingAction` :`type` "/Game/Scenarios/Shared/Configs/OngoingActions/System_Started/DA_FactionWar.DA_FactionWar" :`community` _faction_war_aggressor :`ignoreMandatoryFilterCheck` true :`additionalInstancesOnStart` (- (`/Game/Scenarios/Shared/BlueprintsNonSerialized/FactionEmergence/BPFL_FactionWarUtils.Get Additional Instances on Start`) 2))))))