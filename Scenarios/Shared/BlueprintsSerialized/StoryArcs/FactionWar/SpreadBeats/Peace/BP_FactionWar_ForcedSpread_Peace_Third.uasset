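; Story beat for the third forced peace spread in the Faction War arc, startable only after the second spread lens message is logged and parent checks pass.
; On choice 1, it waits for a duration and an immediate scenario-lane beat slot, then sends a hunt follow-up lens with the initial aggressor's community art and awaits any choice.
; Message defines extend the parent's with the quest duration as TIME.
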(event `self.OnFinished`
  (`parent.OnFinished`)
  (switch `int` (`self.Choice`)
    (:`1`
      (`PXAsyncWaitForDurationPassed.AsyncAction_WaitForDurationPassed` (struct :`ScaledTicks` 16800)
        (:`Completed`
          (`PXAsyncWaitForStoryBeat.AsyncAction_WaitForStoryBeat` "/Game/Scenarios/Shared/Configs/StoryBeat/DA_ImmediateStoryBeat.DA_ImmediateStoryBeat" "/Game/Scenarios/Shared/Configs/StoryBeat/Lanes/DA_0_Scenario_Lane.DA_0_Scenario_Lane"
            (:`Completed`
              (bind _decision (`/Game/Scenarios/Shared/BlueprintsNonSerialized/SocietyUtils/BPFL_Communication_Utils.Send Lens With Community Art` (`self.Hunt Followup Lens Config`) null (`.Faction War Aggressor Type` (`/Game/Scenarios/Shared/BlueprintsNonSerialized/SocietyUtils/BPFL_SharedScenariosStorage.Get Faction War Initial Aggressor`)) (`self.Get Message Defines`) (struct) (struct) true))
              (`PXAsyncWaitForAnyChoice.AsyncAction_WaitForAnyChoice` _decision))))))))

(fn `CanBeStarted Core`
  (returns (ReturnValue :type Boolean))
  (if (`/Game/Scenarios/Shared/BlueprintsNonSerialized/SocietyUtils/BPFL_SharedScenariosStorage.Is Message Logged?` "/Game/Scenarios/Shared/Configs/Messages/Lenses/FactionWar/DA_FactionWar_SecondSpread_Lens.DA_FactionWar_SecondSpread_Lens")
    (bind _returnvalue (`parent.CanBeStarted Core`))
    (return _returnvalue)))

(fn `Get Message Defines`
  (returns (Map :type "Map of String to Text"))
  (bind _defines_map_merged (`/Game/Scenarios/Shared/BlueprintsNonSerialized/SocietyUtils/BPFL_Communication_Utils.Merge Defines` (`parent.Get Message Defines`) (`|MakeMap` "TIME" (`PXTextUtils.GameTimeToTextMostImportant` (`self.Custom Parameters Quest Duration`)))))
  (return _defines_map_merged))