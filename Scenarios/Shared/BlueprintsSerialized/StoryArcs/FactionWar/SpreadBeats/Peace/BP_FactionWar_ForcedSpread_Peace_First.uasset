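; Faction war story beat on the forced peace path, where one choice resolves a hostage rescue with deaths on both sides.
; Choice 1 rolls random losses for the defender's hostages and the aggressor's hostage takers, capped against community size less 200, then kills and notifies each community.
; The combined toll feeds a population notification, district absence event and murder history record.
; Defines add the quest duration as TIME text.
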(fn `Get Defines`
  (returns (Map :type "Map of String to Text"))
  (bind _defines_map_merged (`/Game/Scenarios/Shared/BlueprintsNonSerialized/SocietyUtils/BPFL_Communication_Utils.Merge Defines` (`parent.Get Defines`) (`|MakeMap` "TIME" (`PXTextUtils.GameTimeToTextMostImportant` (`self.Custom Parameters Quest Duration`)))))
  (return _defines_map_merged))

(fn `Handle Choice`
  (params (Selection :type Integer))
  (locals (`hostages killed` :type Integer :default 0) (`hostage takers killed` :type Integer :default 0))
  (bind _faction_war_aggressor (`/Game/Scenarios/Shared/BlueprintsNonSerialized/SocietyUtils/BPFL_SharedScenariosStorage.Get Faction War Initial Aggressor`))
  (bind _defender (`/Game/Scenarios/Shared/BlueprintsNonSerialized/SocietyUtils/BPFL_SharedScenariosStorage.Get Faction War Initial Defender`))
  (bind _returnvalue (+ (`local.hostages killed`) (`local.hostage takers killed`)))
  (switch `int` Selection
    (:`1`
      (bind _output_get (set `local.hostages killed` (`KismetMathLibrary.Min` (`PXRandomLibrary.PXRandomIntegerInRange` (`self.Min Hostage Deaths`) (`self.Max Hostage Deaths`)) (- (`PXCommunityComponent.GetCommunitySize` (`/Game/Scenarios/Shared/BlueprintsNonSerialized/SocietyUtils/BPFL_SharedScenariosStorage.Get Faction War Initial Defender`)) 200))))
      (`/Game/Scenarios/Shared/BlueprintsNonSerialized/Communities/BPFL_CommunityUtils.Kill People in Community For Real` _defender _output_get true)
      (`/Game/Scenarios/Shared/BlueprintsNonSerialized/Communities/BPFL_CommunityUtils.DisplayCommunityNotification` _defender (`|FormatText` "{Number} hostages killed" (`local.hostages killed`)))
      (bind _output_get_2 (set `local.hostage takers killed` (`KismetMathLibrary.Min` (`PXRandomLibrary.PXRandomIntegerInRange` (* (`self.Min Hostage Deaths`) (`self.multiplier for hostage takesrs`)) (* (`self.Max Hostage Deaths`) 3)) (- (`PXCommunityComponent.GetCommunitySize` _faction_war_aggressor) 200))))
      (`/Game/Scenarios/Shared/BlueprintsNonSerialized/Communities/BPFL_CommunityUtils.Kill People in Community For Real` _faction_war_aggressor _output_get_2 true)
      (`/Game/Scenarios/Shared/BlueprintsNonSerialized/Communities/BPFL_CommunityUtils.DisplayCommunityNotification` (`/Game/Scenarios/Shared/BlueprintsNonSerialized/SocietyUtils/BPFL_SharedScenariosStorage.Get Faction War Initial Aggressor`) (`|FormatText` "{Number} hostage takers killed" (`local.hostage takers killed`)))
      (`PXCommunicationChannelsUtils.AddNotification` (make `PXNotificationData` "PopulationDeath" (`|FormatText` "{Number} killed during rescue of {DEFENDER}' hostages" _returnvalue (`.Faction War Defender Name` (`/Game/Scenarios/Shared/BlueprintsNonSerialized/SocietyUtils/BPFL_SharedScenariosStorage.Get Faction War Initial Defender`)))))
      (`PXUICustomEventsUtils.BroadcastDistrictAbsenceChangedEvent` (`self.District`) "Dead" _returnvalue "/Game/UI/Assets/Textures/AtlasedTextures/Icons/Frames/UIT_PopulationDeath.UIT_PopulationDeath" 0 null 3)
      (`PXHistoryRecordUtils.AddActorHistoryRecord` (`ActorComponent.GetOwner` (`self.District`)) "/Game/Scenarios/Shared/Configs/HistoryRecords/Types/DA_HistoryRecord_Murdered.DA_HistoryRecord_Murdered" _returnvalue))))