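; Story arc for a retroactive promise built on a failed policy desire, covering both pass and repeal quests.
; The failed desire's quest type selects the pass or repeal lens config.
; It can start only if parent checks succeed and the desire is still unmet, judged by whether any policy in the fallback group is active.
; The policy also feeds the game context and the POLICY text define.
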(fn `CanBeStarted Core`
  (returns (ReturnValue :type Boolean))
  (bind _failed_desire (`self.Failed desire`))
  (bind _returnvalue (`PXPolicyUtils.IsAnyPolicyInFallbackGroupActive` (`PXPolicyUtils.GetPlayerPolicy`) (`.Policy` (break `PXDesire` _failed_desire))))
  (bind _returnvalue_2 (`parent.CanBeStarted Core`))
  (if _returnvalue_2
    (if (select `EPXPolicyQuestObjectiveType` (`PXDesireUtils.GetPolicyQuestType` _failed_desire) :`Pass` (not _returnvalue) :`Repeal` _returnvalue)
      (return true))))

(fn `Get Defines`
  (returns (Map :type "Map of String to Text"))
  (bind _defines_map_merged (`/Game/Scenarios/Shared/BlueprintsNonSerialized/SocietyUtils/BPFL_Communication_Utils.Merge Defines` (`parent.Get Defines`) (`|MakeMap` "POLICY" (`PXPolicyType.IngameName` (`.Policy` (break `PXDesire` (`self.Failed desire`)))))))
  (return _defines_map_merged))

(fn `Get game context`
  (returns (ReturnValue :type "PXGameContext Structure"))
  (bind _failed_desire_policy (break `PXDesire` (`self.Failed desire`)))
  (return (`PXGameplayContextUtils.MakePXGameContext` null null null null null null _failed_desire_policy)))

(fn `Get Lens Config`
  (returns (ReturnValue :type "PXLens Soft Object Reference"))
  (return (select `EPXPolicyQuestObjectiveType` (`PXDesireUtils.GetPolicyQuestType` (`self.Failed desire`)) :`Pass` (`self.Retro Promise Pass Lens`) :`Repeal` (`self.Retro Promise Repeal Lens`))))