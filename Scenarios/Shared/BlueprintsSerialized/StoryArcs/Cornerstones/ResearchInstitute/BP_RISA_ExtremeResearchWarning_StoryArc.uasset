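; Research Institute story arc that warns the player while a topic from the extreme affinity bucket is being researched.
; CanBeStarted requires an assigned research community and caches it with the matching outcome.
; On start, it sends a lens message tied to the institute's district, naming the faction and unlocked building or policy, with an immediate desire for that outcome.
; After any choice, it constructs and starts the ResearcherDeath follow-up arc with the same context.
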(event `self.OnStarted`
  (bind _extreme_research_in_progress (`self.Extreme Research In Progress`))
  (bind (_found _unlocked_building) (`/Game/Scenarios/Shared/BlueprintsNonSerialized/SocietyUtils/BPFL_Cornerstone_Utils.Get building with outcome requirement` _extreme_research_in_progress))
  (if _found
    (set `self.Research Text` (`PXBuildingType.IngameName` _unlocked_building))
    (else
      (set `self.Research Text` (`PXPolicyType.IngameName` (`/Game/Scenarios/Shared/BlueprintsNonSerialized/SocietyUtils/BPFL_Cornerstone_Utils.Get policy with outcome requirement` _extreme_research_in_progress)))))
  (set `self.Defines Map` (`|MakeMap` "RESEARCH" (`self.Research Text`) "FACTION" (`/Game/Scenarios/Shared/BlueprintsNonSerialized/Communities/BPFL_CommunityUtils.Get Community Name` (`self.Research Community`))))
  (bind _decision (`/Game/Scenarios/Shared/BlueprintsNonSerialized/SocietyUtils/BPFL_Communication_Utils.Send Config Message` "/Game/Scenarios/Sandbox/Configs/Messages/Lenses/ResearchInstitute/DA_RISA_ExtremeResearchWarning_Lens.DA_RISA_ExtremeResearchWarning_Lens" (`PXBuildingComponent.OwningDistrict` (`|GetArrayItem` (`PXBuildingUtils.GetBuildingsOfTypeFromCity` (`PXNationUtils.GetPlayerMainCity`) "/Game/Scenarios/Shared/Configs/Buildings/ResearchInstitute/DA_H_ResearchInstitute.DA_H_ResearchInstitute"))) (`PXResearchUtils.GetResearchOutcomeCommunity` (`PXNationUtils.GetPlayerNation`) (`self.Extreme Research In Progress`)) null (`self.Defines Map`) null null (struct) true (make `/Game/Scenarios/Shared/BlueprintsNonSerialized/SocietyUtils/F_DesiresArray_Struct` (`|MakeArray` (`self.Get Immediate Desire`)))))
  (`PXAsyncWaitForAnyChoice.AsyncAction_WaitForAnyChoice` _decision
    (:`Completed`
      (bind _returnvalue (`|GenericCreateObject` (subsystem `PXStoryArcSubsystem`) "/Game/Scenarios/Shared/BlueprintsSerialized/StoryArcs/Cornerstones/ResearchInstitute/BP_RISA_ResearcherDeath_StoryArc.BP_RISA_ResearcherDeath_StoryArc_C" (`self.Defines Map`) (`self.Extreme Research In Progress`)))
      (`PXStoryUtils.StartParameterizedStoryArc` _returnvalue))))

(fn `CanBeStarted`
  (returns (ReturnValue :type Boolean))
  (bind _returnvalue (`PXNationUtils.GetPlayerNation`))
  (bind (_research_community _found) (`self.Get Current Research Community`))
  (bind _returnvalue_2 (`PXNationUtils.GetPlayerNation`))
  (if (`PXResearchUtils.IsAnyResearchTopicInProgress` _returnvalue)
    (if (== (`PXResearchTopic.AffinityBucket` (`PXResearchUtils.GetCurrentlyResearchedTopic` _returnvalue)) (`self.Extreme Affinity Bucket`))
      (if _found
        (bind _output_get (set `self.Research Community` _research_community))
        (set `self.Extreme Research In Progress` (`PXResearchUtils.GetMatchingOutcome` _returnvalue_2 (`PXResearchUtils.GetCurrentlyResearchedTopic` _returnvalue_2) _output_get))
        (return true)
        (else
          (return false)))
      (else
        (return false)))
    (else
      (return false))))

(fn `Get Current Research Community`
  (returns (`Research Community` :type "PXCommunityComponent Object Reference") (Found :type Boolean))
  (for _array_element (`PXResearchUtils.GetCommunitiesAvailableForResearch`)
    (if (`PXResearchUtils.IsCommunityAssignedToResearch` (`PXNationUtils.GetPlayerNation`) _array_element)
      (return _array_element true)))
  (return null false))

(fn `Get Immediate Desire`
  (returns (ReturnValue :type "PXDesire Structure"))
  (bind _returnvalue (`PXDesireUtils.MakeResearchOutcomeDesire` (`self.Extreme Research In Progress`)))
  (return _returnvalue))