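; Research Institute story arc that presents a researcher death event tied to extreme research.
; It can start when the first policy requiring the ExtremeResearchInProgress outcome is active, checking for the first such building in the main city only if no policies require it.
; On start, it sends the ghost config message with text defines, targeting the closest district, and waits for any choice with no follow-up logic.
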(event `self.OnStarted`
  (bind _decision (`/Game/Scenarios/Shared/BlueprintsNonSerialized/SocietyUtils/BPFL_Communication_Utils.Send Config Message` "/Game/Scenarios/Sandbox/Configs/Messages/Ghosts/ResearchInstituteStoryArcs/DA_RISA_ResearcherDeath_Ghost.DA_RISA_ResearcherDeath_Ghost" null null null (`self.Defines Map`) null null (struct) true))
  (`PXAsyncWaitForAnyChoice.AsyncAction_WaitForAnyChoice` _decision))

(fn `CanBeStarted`
  (returns (ReturnValue :type Boolean))
  (bind _extreme_research_in_progress (`self.Extreme Research In Progress`))
  (bind _returnvalue (`PXRequirementRelationsUtils.GetBuildingsRequiringResearchOutcome` _extreme_research_in_progress))
  (bind _returnvalue_2 (`PXRequirementRelationsUtils.GetPoliciesRequiringResearchOutcome` _extreme_research_in_progress))
  (if (`KismetArrayLibrary.Array_IsEmpty` _returnvalue_2)
    (if (`KismetArrayLibrary.Array_IsEmpty` _returnvalue)
      (return false)
      (elif (`PXBuildingUtils.HasBuildingOfTypeInCity` (`PXNationUtils.GetPlayerMainCity`) (`|GetArrayItem` _returnvalue))
        (return true)))
    (elif (`/Game/Scenarios/Shared/BlueprintsNonSerialized/Policies/BPFL_PolicyUtils.IsPolicyActive` (`|GetArrayItem` _returnvalue_2))
      (return true))))