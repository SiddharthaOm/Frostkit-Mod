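; Radicalisation ghost story variant, by its name for a refused next step, that can start only if the parent check passes and the community is not rallying.
; It extends the parent text defines with the faction's name, its first cornerstone's sentence and the opposing faction's name.
; Ghost genders come from a config-keyed map, and a removal function drops the first entry of the shared RadicalisationRefuseGhosts array.
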(fn `CanBeStarted`
  (returns (ReturnValue :type Boolean))
  (bind _returnvalue (`parent.CanBeStarted`))
  (if _returnvalue
    (if (not (`/Game/Scenarios/Shared/BlueprintsNonSerialized/OngoingEvents/BPFL_OngoingAction_Utils.Is Community Rallying?` (`self.Community`)))
      (return true))))

(fn `Get Ghost Config`
  (returns (Ghost :type "PXGhost Soft Object Reference"))
  (return null))

(fn `Ghost Defines`
  (returns (Map :type "Map of String to Text"))
  (bind _returnvalue (`PXCommunityComponent.GetFaction` (`self.Community`)))
  (bind _cornerstones1 (`/Game/Scenarios/Shared/BlueprintsNonSerialized/SocietyUtils/BPFL_Cornerstone_Utils.Get Faction Cornerstones` _returnvalue))
  (bind _output (`|GetArrayItem` _cornerstones1))
  (bind (_exists _faction_community) (`/Game/Scenarios/Shared/BlueprintsNonSerialized/SocietyUtils/BPFL_Cornerstone_Utils.Get Faction Opposed to Cornerstone` _output))
  (bind _defines_map_merged (`/Game/Scenarios/Shared/BlueprintsNonSerialized/SocietyUtils/BPFL_Communication_Utils.Merge Defines` (`parent.Ghost Defines`) (`|MakeMap` "CORNERSTONE_SENTENCE" (`BlueprintMapLibrary.Map_Find` (`self.Cornerstone Sentence`) _output) "FACTION" (`PXFactionType.IngameName` _returnvalue) "OPPOSITE_FACTION" (`PXFactionUtils.GetFactionInGameName` _faction_community))))
  (return _defines_map_merged))

(fn `Remove Ghost from Array`
  (bind _radicalisation_refuse_ghosts (`/Game/Scenarios/Shared/BlueprintsSerialized/VariableStorage/BP_SharedVariableStorage.Radicalisation Refuse Ghosts` (`/Game/Scenarios/Shared/BlueprintsNonSerialized/SocietyUtils/BPFL_SharedScenariosStorage.Get Shared Variable Storage`)))
  (`KismetArrayLibrary.Array_RemoveItem` _radicalisation_refuse_ghosts (`|GetArrayItem` _radicalisation_refuse_ghosts)))

(fn `Setup Genders for Ghosts`
  (returns (`Ghost Gender` :type "/Game/Scenarios/Shared/BlueprintsSerialized/StoryArcs/OngoingActions/RadicalProtest/ENUM_AffinityGhostGender Enum"))
  (return (`BlueprintMapLibrary.Map_Find` (`self.Ghost to Gender Map`) (`self.Get Ghost Config`))))