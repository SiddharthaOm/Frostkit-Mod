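; Radicalisation ghost story-arc child for counter-protests, startable when the parent allows it, the Community is not protesting and counter-protest ghosts remain in shared storage.
; Overrides take the first config from that shared array, look up its gender setup and provide a function to remove it.
; Text defines swap perspective: FACTION names the opposite faction and OPPOSITE_FACTION names the Community.
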(fn `CanBeStarted`
  (returns (ReturnValue :type Boolean))
  (bind _returnvalue (`parent.CanBeStarted`))
  (if _returnvalue
    (if (not (`/Game/Scenarios/Shared/BlueprintsNonSerialized/OngoingEvents/BPFL_OngoingAction_Utils.Is Community Protesting?` (`self.Community`)))
      (if (`KismetArrayLibrary.Array_IsNotEmpty` (`/Game/Scenarios/Shared/BlueprintsSerialized/VariableStorage/BP_SharedVariableStorage.Radicalisation CounterProtest Ghosts` (`/Game/Scenarios/Shared/BlueprintsNonSerialized/SocietyUtils/BPFL_SharedScenariosStorage.Get Shared Variable Storage`)))
        (return true)))))

(fn `Get Ghost Config`
  (returns (Ghost :type "PXGhost Soft Object Reference"))
  (return (`|GetArrayItem` (`/Game/Scenarios/Shared/BlueprintsSerialized/VariableStorage/BP_SharedVariableStorage.Radicalisation CounterProtest Ghosts` (`/Game/Scenarios/Shared/BlueprintsNonSerialized/SocietyUtils/BPFL_SharedScenariosStorage.Get Shared Variable Storage`)))))

(fn `Ghost Defines`
  (returns (Map :type "Map of String to Text"))
  (return (`|MakeMap` "FACTION" (`PXFactionUtils.GetFactionInGameName` (`self.Opposite Faction`)) "OPPOSITE_FACTION" (`PXFactionUtils.GetFactionInGameName` (`self.Community`)))))

(fn `Remove Ghost from Array`
  (bind _radicalisation_counterprotest_ghosts (`/Game/Scenarios/Shared/BlueprintsSerialized/VariableStorage/BP_SharedVariableStorage.Radicalisation CounterProtest Ghosts` (`/Game/Scenarios/Shared/BlueprintsNonSerialized/SocietyUtils/BPFL_SharedScenariosStorage.Get Shared Variable Storage`)))
  (`KismetArrayLibrary.Array_RemoveItem` _radicalisation_counterprotest_ghosts (`|GetArrayItem` _radicalisation_counterprotest_ghosts)))

(fn `Setup Genders for Ghosts`
  (returns (`Ghost Gender` :type "/Game/Scenarios/Shared/BlueprintsSerialized/StoryArcs/OngoingActions/RadicalProtest/ENUM_AffinityGhostGender Enum"))
  (return (`BlueprintMapLibrary.Map_Find` (`self.Ghost to Gender Map`) (`self.Get Ghost Config`))))