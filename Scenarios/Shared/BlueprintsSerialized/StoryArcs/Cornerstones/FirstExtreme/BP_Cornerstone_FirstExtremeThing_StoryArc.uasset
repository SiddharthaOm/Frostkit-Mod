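; Story arc where a faction rallies the player to embrace a Cornerstone once the City leans extreme in its affinity.
; Accepting starts a timed side quest to research the Cornerstone and hold that direction, with optional objectives generated from aligned faction desires.
; Objective and affinity event handlers track progress, push affinity to its cap and finish the quest.
; Refusal or failure escalates radicalisation through a refusal sub-arc or Fervour modifiers.
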(event `self.OnStarted`
  (bind _faction_community (`self.Faction Community`))
  (bind _promise_quest (`self.Promise Quest`))
  (bind (_desire_temp_policy _desire_temp_building _desire_temp_researchoutcome) (break `PXDesire` (`self.Desire Temp`)))
  (bind _desire_temp_policy_2 (break `PXDesire` (`self.Desire Temp`)))
  (bind (_desire_temp_policy_3 _desire_temp_building_2) (break `PXDesire` (`self.Desire Temp`)))
  (bind _faction_community_2 (`self.Faction Community`))
  (bind (_data_ingamename _data_shortdescription _data_axis) (break `PXAffinity` (`EntriesBlueprintFunctionLibrary.GetAffinityDetails` (`self.Extreme Affinity`))))
  (bind _data_ingamename_2 (break `PXAffinity` (`EntriesBlueprintFunctionLibrary.GetAffinityDetails` (`self.Extreme Affinity`))))
  (bind _ingame_name (`self.Get Extreme Stuff` (`self.Extreme Affinity`)))
  (set `self.Extreme Ingame Name` _ingame_name)
  (`PXAsyncWaitForDurationPassed.AsyncAction_WaitForDurationPassed` (struct :`ScaledTicks` 8400)
    (:`Completed`
      (set `self.Defines` (`|MakeMap` "EXTREME_THING" (`self.Extreme Ingame Name`) "SUPPORTING_FACTION" (`/Game/Scenarios/Shared/BlueprintsNonSerialized/Communities/BPFL_CommunityUtils.Get Community Name` (`self.Faction Community`)) "CORNERSTONE" (`PXCornerstone.InGameName` (`self.Cornerstone`)) "WEEKS" (`KismetTextLibrary.Conv_IntToText` (`PXTimeSubsystem.GetTotalWeeks` (`self.Quest Duration`)))))
      (bind _returnvalue (`PXDesireUtils.MakeResearchOutcomeDesire` (`|GetArrayItem` (`PXResearchTopic.Outcomes` (`BlueprintMapLibrary.Map_Find` (`self.Cornerstone Research Map`) (`self.Cornerstone`))))))
      (bind _decision (`/Game/Scenarios/Shared/BlueprintsNonSerialized/SocietyUtils/BPFL_Communication_Utils.Send Config Message` (`self.RadicalRally BigLens Config`) (`PXCityComponent.GetMainDistrict` (`PXNationUtils.GetPlayerMainCity`)) (`self.Faction Community`) null (`self.Defines`) null null (`PXCommunicationChannelsUtils.CreateDesiresPerChoiceArray` (`|MakeArray` (make `PXCommunicationChannelsDesiresPerChoice` (`|MakeArray` _returnvalue))))))
      (bind _choice (`PXAsyncWaitForChoice.AsyncAction_WaitForChoice` _decision)
        (:`Completed`
          (switch `int` _choice
            (:`0`
              (bind _returnvalue_2 (`PXQuestUtils.StartQuestInPlace` (`|FormatText` "Embrace {CORNERSTONE}" (`PXCornerstone.InGameName` (`self.Cornerstone`))) "" (`self.Quest Duration`) "SideQuest" "DebugQuestName" true))
              (set `self.Promise Quest` _returnvalue_2)
              (bind _returnvalue_3 (`PXQuest.AddQuestObjective` (`self.Promise Quest`) (`|FormatText` "Keep the current direction of the City in {AFFINITY}" _data_ingamename_2) "" 0 1 false null "DebugObjectiveName"))
              (set `self.Affinity Direction` _returnvalue_3)
              (add `PXAffinitySubsystem.AffinityChangedEvent` (subsystem `PXAffinitySubsystem`) (`|CreateDelegate` :!event `Affinity Changed`))
              (bind _returnvalue_4 (`PXQuestUtils.AddResearchQuestObjective` (`self.Promise Quest`) (`|FormatText` "Research and embrace '{CORNERSTONE}'" (`PXCornerstone.InGameName` (`self.Cornerstone`))) "" (`BlueprintMapLibrary.Map_Find` (`self.Cornerstone Research Map`) (`self.Cornerstone`)) false null null null))
              (set `self.Cornerstone Objective` _returnvalue_4)
              (bind _returnvalue_5 (`PXDesireUtils.GetBroadSpectrumDesires` (`PXCommunityComponent.GetCommunityType` (`self.Faction Community`)) (make `PXBroadSpectrumDesiresSearchParameters` 3 (`|MakeArray` "ResearchOutcomeDesire" "PolicyDesire" "BuildingDesire" "ResearchOutcomeDesire" "PolicyDesire" "BuildingDesire" "ResearchOutcomeDesire" "PolicyDesire" "BuildingDesire" :!type "EPXDesireType Enum") (struct :`BuildingTagsQuery` (struct)) _data_axis "Nonadversary" true false true)))
              (bind _output_get (set `self.Cornerstone Desires` _returnvalue_5))
              (for _array_element _output_get
                (set `self.Desire Temp` _array_element)
                (switch `EPXDesireType` (`PXDesireUtils.GetDesireType` (`self.Desire Temp`))
                  (:`PolicyDesire`
                    (`PXQuestUtils.AddPolicyQuestObjective` (make `PXObjectiveParameters` (`|FormatText` "Pass '{POLICY}'" (`PXPolicyType.IngameName` _desire_temp_policy_2)) "" true 1 null _promise_quest) (make `PXPolicyObjectiveParameters` _desire_temp_policy_2)))
                  (:`BuildingDesire`
                    (`PXQuestUtils.AddBuildingQuestObjective` (make `PXObjectiveParameters` (`|FormatText` "Construct '{BUILDING}'" (`PXBuildingType.IngameName` _desire_temp_building_2)) "" true 1 null _promise_quest) (make `PXBuildingObjectiveParameters` _desire_temp_building_2 "Build" 1 null null (`PXNationUtils.GetPlayerMainCity`) _ false)))
                  (:`ResearchOutcomeDesire`
                    (`PXQuestUtils.AddResearchOutcomeQuestObjective` (make `PXObjectiveParameters` (`|FormatText` "Research and enact '{THING}'" (`PXRequirementRelationsUtils.GetResearchOutcomeEffectIngameName` _desire_temp_researchoutcome)) "" true 1 null _promise_quest) (make `PXResearchOutcomeObjectiveParameters` _desire_temp_researchoutcome true)))))
              (`self.Define Objectives`)
              (add `PXQuestSubsystem.QuestObjectiveFinishedEvent` (subsystem `PXQuestSubsystem`) (`|CreateDelegate` :!event `Bump Affinity`))
              (bind _succeeded (`PXAsyncWaitForQuest.AsyncAction_WaitForQuest` (`self.Promise Quest`))
                (:`Completed`
                  (if (not _succeeded)
                    (`PXAsyncOpenPredefinedDialog.AsyncAction_OpenPredefinedDialog` "/Game/Scenarios/Shared/Configs/Messages/Dialogs/Quests/DA_CornerstoneEmbracementQuest_Fail.DA_CornerstoneEmbracementQuest_Fail" (`self.Defines`)
                      (:`Completed`
                        (if (`KismetArrayLibrary.Array_IsNotEmpty` (`/Game/Scenarios/Shared/BlueprintsSerialized/VariableStorage/BP_SharedVariableStorage.Radicalisation Refuse Ghosts` (`/Game/Scenarios/Shared/BlueprintsNonSerialized/SocietyUtils/BPFL_SharedScenariosStorage.Get Shared Variable Storage`)))
                          (bind _returnvalue_6 (`|GenericCreateObject` (subsystem `PXStoryArcSubsystem`) "/Game/Scenarios/Shared/BlueprintsSerialized/StoryArcs/Cornerstones/RadicalisationGhosts/Children/BP_RadicalisationGhosts_NextStepRefused.BP_RadicalisationGhosts_NextStepRefused_C" (`self.Faction Community`)))
                          (bind _returnvalue_7 (`PXStoryUtils.StartParameterizedStoryArc` _returnvalue_6))
                          (if _returnvalue_7
                            (`PXAsyncWaitForStoryArc.AsyncAction_WaitForStoryArc` _returnvalue_6
                              (:`Completed`
                                (`PXPredefinedModifierUtils.SetPredefinedModifierActiveManualTarget` (`PXNationUtils.GetPlayerNation`) "/Game/Scenarios/Shared/BlueprintsSerialized/StoryArcs/Modifiers/Radicalisation/DA_RadicalisationStrengthIncrease_PredefinedModifier.DA_RadicalisationStrengthIncrease_PredefinedModifier" (`ActorComponent.GetOwner` (`self.Faction Community`)) true)
                                (`PXPredefinedModifierUtils.SetPredefinedModifierActiveManualTarget` (`PXNationUtils.GetPlayerNation`) "/Game/Scenarios/Shared/Configs/PredefinedModifiers/DA_CornerstoneEmbrace_QuestFailed_Modifier.DA_CornerstoneEmbrace_QuestFailed_Modifier" (`ActorComponent.GetOwner` (`self.Faction Community`)) true :!label _label)))
                            (else
                              (`KismetSystemLibrary.PrintString` "Radicalisation Ghost Next Step Refused to construct")))
                          (else
                            (`/Game/Scenarios/Shared/BlueprintsNonSerialized/Communities/BPFL_CommunityUtils.DisplayCommunityNotification` _faction_community (`|FormatText` "{FACTION}' Fervour rises due to cornerstone refusal" (`PXFactionUtils.GetFactionInGameName` _faction_community)))
                            (`PXPredefinedModifierUtils.SetPredefinedModifierActiveManualTarget` (`PXNationUtils.GetPlayerNation`) "/Game/Scenarios/Shared/BlueprintsSerialized/StoryArcs/Modifiers/Radicalisation/DA_Radicalisation_GreatStrengthIncrease_PredefinedModifier.DA_Radicalisation_GreatStrengthIncrease_PredefinedModifier" (`ActorComponent.GetOwner` (`self.Faction Community`)) true)
                            (goto _label)))))))))
            (:`1`
              (if (`KismetArrayLibrary.Array_IsNotEmpty` (`/Game/Scenarios/Shared/BlueprintsSerialized/VariableStorage/BP_SharedVariableStorage.Radicalisation Refuse Ghosts` (`/Game/Scenarios/Shared/BlueprintsNonSerialized/SocietyUtils/BPFL_SharedScenariosStorage.Get Shared Variable Storage`)))
                (bind _returnvalue_8 (`|GenericCreateObject` (subsystem `PXStoryArcSubsystem`) "/Game/Scenarios/Shared/BlueprintsSerialized/StoryArcs/Cornerstones/RadicalisationGhosts/Children/BP_RadicalisationGhosts_NextStepRefused.BP_RadicalisationGhosts_NextStepRefused_C" (`self.Faction Community`)))
                (`PXStoryUtils.StartParameterizedStoryArc` _returnvalue_8)
                (else
                  (`/Game/Scenarios/Shared/BlueprintsNonSerialized/Communities/BPFL_CommunityUtils.DisplayCommunityNotification` _faction_community_2 (`|FormatText` "{FACTION}' Fervour rises due to cornerstone refusal" (`PXFactionUtils.GetFactionInGameName` _faction_community_2)))
                  (`PXPredefinedModifierUtils.SetPredefinedModifierActiveManualTarget` (`PXNationUtils.GetPlayerNation`) "/Game/Scenarios/Shared/BlueprintsSerialized/StoryArcs/Modifiers/Radicalisation/DA_RadicalisationStrengthIncrease_PredefinedModifier.DA_RadicalisationStrengthIncrease_PredefinedModifier" (`ActorComponent.GetOwner` (`self.Faction Community`)) true))))))))))

(fn `Affinity Changed`
  (params (holder :type "PXAffinityHolderComponent Object Reference") (affinityPermutation :type "PXAffinityPermutation Structure (by ref)"))
  (if (>= (`PXAffinityUtils.GetNationLeaderAffinity` (`PXNationUtils.GetPlayerNation`) (`self.Affinity to Check`)) 100)
    (`PXQuestObjective.ModifyObjectiveProgress` (`self.Affinity Direction`) 1)
    (return)
    (else
      (return))))

(fn `Building Dominant Affinity and Bucket`
  (params (`Building Component` :type "PXBuildingComponent Object Reference"))
  (returns (entry :type "PXAffinityEntry Structure") (ReturnValue :type Boolean))
  (bind _type (`PXBuildingComponent.Type` `Building Component`))
  (bind (_entry _hasaffinity) (`PXBuildingUtils.GetBuildingDominantAffinity` _type))
  (bind (_value _returnvalue) (`BlueprintMapLibrary.Map_Find` (`PXBuildingType.Affinities` _type) _entry))
  (bind (_value_2 _returnvalue_2) (`BlueprintMapLibrary.Map_Find` (`.Map` (break `PXBucketValueMap` _value)) "/Game/Scenarios/Shared/Configs/Affinity/DA_Extreme_Bucket.DA_Extreme_Bucket"))
  (if _hasaffinity
    (if _returnvalue
      (if _returnvalue_2
        (return _entry (> _value_2 0))))))

(fn `Bump Affinity`
  (params (Objective :type "PXQuestObjective Object Reference"))
  (if (and (`PXQuestObjective.IsObjectiveFinished` (`self.Promise Objective 1`)) (`PXQuestObjective.IsObjectiveFinished` (`self.Promise Objective 2`)) (`PXQuestObjective.IsObjectiveFinished` (`self.Promise Objective 3`)))
    (if (>= (`PXAffinityUtils.GetNationLeaderAffinity` (`PXNationUtils.GetPlayerNation`) (`self.Extreme Affinity`)) 100) :!label _label
      (remove `PXQuestSubsystem.QuestObjectiveFinishedEvent` (subsystem `PXQuestSubsystem`) (`|CreateDelegate` :!event `Bump Affinity`))
      (else
        (`PXCityUtils.ExecuteCityAction` (`PXNationUtils.GetPlayerMainCity`) (`BlueprintMapLibrary.Map_Find` (`self.Extreme Affinity Bump Map`) (`self.Extreme Affinity`)) "/Game/Scenarios/Shared/Configs/ActionOrigin/DA_LeaderActionOrigin.DA_LeaderActionOrigin")
        (goto _label)))))

(fn `CanBeStarted`
  (returns (ReturnValue :type Boolean))
  (bind _extreme_affinity (`self.Extreme Affinity`))
  (bind (_returnvalue _extreme_affinity_2) (`self.Player Is Extreme on Anything` (`|MakeArray` (`self.Affinity to Check`))))
  (if _returnvalue
    (set `self.Extreme Affinity` _extreme_affinity_2)
    (if (not (or (`/Game/Scenarios/Shared/BlueprintsNonSerialized/SocietyUtils/BPFL_Cornerstone_Utils.Is Cornerstone Embraced` (`PXCornerstoneUtils.GetCornerstoneFromAffinity` (`/Game/Scenarios/Shared/BlueprintsNonSerialized/SocietyUtils/BPFL_Cornerstone_Utils.Get Opposite Affinity` _extreme_affinity))) (`/Game/Scenarios/Shared/BlueprintsNonSerialized/SocietyUtils/BPFL_Cornerstone_Utils.Is Cornerstone Embraced` (`PXCornerstoneUtils.GetCornerstoneFromAffinity` _extreme_affinity))))
      (if (>= (`PXAffinityUtils.GetNationLeaderAffinity` (`PXNationUtils.GetPlayerNation`) (`self.Extreme Affinity`)) 80)
        (if (not (`/Game/Scenarios/Shared/BlueprintsNonSerialized/SocietyUtils/BPFL_Cornerstone_Utils.Is Cornerstone Embraced` (`self.Cornerstone`)))
          (bind _cornerstone (`/Game/Scenarios/Shared/BlueprintsNonSerialized/SocietyUtils/BPFL_Cornerstone_Utils.Get Cornerstone for Affinity` (`self.Extreme Affinity`)))
          (bind _output_get (set `self.Cornerstone` _cornerstone))
          (bind (_exists _faction_community) (`/Game/Scenarios/Shared/BlueprintsNonSerialized/SocietyUtils/BPFL_Cornerstone_Utils.Get Faction Supporting Cornerstone` _output_get))
          (if _exists
            (bind (_exists_2 _faction_community_2) (`/Game/Scenarios/Shared/BlueprintsNonSerialized/SocietyUtils/BPFL_Cornerstone_Utils.Get Faction Opposed to Cornerstone` _output_get))
            (if _exists_2
              (set `self.Faction Opposing` _faction_community_2)
              (set `self.Faction Community` _faction_community)
              (return true))))))))

(fn `Define Objectives`
  (bind _returnvalue (`PXQuest.GetQuestObjectives` (`self.Promise Quest`)))
  (set `self.Promise Objective 1` (`|GetArrayItem` _returnvalue 2))
  (set `self.Promise Objective 2` (`|GetArrayItem` _returnvalue 3))
  (set `self.Promise Objective 3` (`|GetArrayItem` _returnvalue 4)))

(fn `Embraced Cornerstone`
  (params (Objective :type "PXQuestObjective Object Reference"))
  (if (== Objective (`self.Cornerstone Objective`))
    (`PXQuestUtils.FinishQuest` (`self.Promise Quest`) true)
    (remove `PXQuestSubsystem.QuestObjectiveFinishedEvent` (subsystem `PXQuestSubsystem`) (`|CreateDelegate` :!event `Embraced Cornerstone`))))

(fn `Extreme Building Exists`
  (params (`Must Have Affinity` :type "PXAffinityEntry Structure"))
  (returns (ReturnValue :type Boolean) (`Extreme Building` :type "PXBuildingComponent Object Reference") (`Extreme Affinity` :type "PXAffinityEntry Structure"))
  (locals (NewLocalVar_0 :type "Array of PXBuildingComponent Object Reference"))
  (bind _output_get (set `local.NewLocalVar_0` (`PXBuildingUtils.GetBuildingsFromCity` (`PXNationUtils.GetPlayerMainCity`))))
  (for _array_element _output_get
    (bind (_entry _is_extreme) (`/Game/Scenarios/Shared/BlueprintsNonSerialized/SocietyUtils/BPFL_Quest_Utils.Building Dominant Affinity and Bucket` _array_element))
    (if _is_extreme
      (if (`PXAffinityUtils.Equal` _entry (`local.Must Have Affinity`))
        (return true _array_element))))
  (return false null))

(fn `Extreme Policy Active`
  (params (`Must Have Affinity` :type "PXAffinityEntry Structure"))
  (returns (ReturnValue :type Boolean) (`Extreme Policy` :type "PXPolicyType Object Reference") (`Extreme Affinity` :type "PXAffinityEntry Structure"))
  (locals (NewLocalVar :type "Array of PXPolicyType Object Reference"))
  (bind _values (`BlueprintMapLibrary.Map_Values` (`PXPolicyUtils.GetActivePoliciesMap` (`PXPolicyUtils.GetPlayerPolicy`))))
  (bind _output_get (set `local.NewLocalVar` _values))
  (for _array_element _output_get
    (bind (_affinity _is_extreme) (`self.Policy Dominant Affinity and Bucket` _array_element))
    (if _is_extreme
      (if (`PXAffinityUtils.Equal` _affinity (`local.Must Have Affinity`))
        (return true _array_element _affinity))))
  (return false null))

(fn `Get Extreme Stuff`
  (params (`Must Have Affinity` :type "PXAffinityEntry Structure"))
  (returns (`Ingame Name` :type Text) (`Extreme Building` :type "PXBuildingComponent Object Reference") (`Extreme Policy` :type "PXPolicyType Object Reference"))
  (bind (_returnvalue _extreme_building) (`self.Extreme Building Exists` `Must Have Affinity`))
  (if _returnvalue
    (return (`PXBuildingType.IngameName` (`PXBuildingComponent.Type` _extreme_building)) _extreme_building null)
    (else
      (bind (_returnvalue_2 _extreme_policy) (`self.Extreme Policy Active` (`local.Must Have Affinity`)))
      (if _returnvalue_2
        (return (`PXPolicyType.IngameName` _extreme_policy) null _extreme_policy)
        (else
          (return (`|FormatText` "Something Else") null null))))))

(fn `Player Is Extreme on Anything`
  (params (Array :type "Array of PXAffinityEntry Structure"))
  (returns (ReturnValue :type Boolean) (`Extreme affinity` :type "PXAffinityEntry Structure"))
  (for _array_element Array
    (if (> (`PXAffinityUtils.GetNationLeaderAffinityValueFromBucket` (`PXNationUtils.GetPlayerNation`) _array_element "/Game/Scenarios/Shared/Configs/Affinity/DA_Extreme_Bucket.DA_Extreme_Bucket") 0)
      (return true _array_element)))
  (return false))

(fn `Policy Dominant Affinity and Bucket`
  (params (Policy :type "PXPolicyType Object Reference"))
  (returns (Affinity :type "PXAffinityEntry Structure") (`Is extreme` :type Boolean))
  (bind _affinitychanges (`PXPolicyType.AffinityChanges` Policy))
  (bind _output (`|GetArrayItem` _affinitychanges))
  (if (not (`KismetArrayLibrary.Array_IsEmpty` _affinitychanges))
    (return (break `PXAffinityValue` (break `PXAffinityChange` _output)) (and (> (`.Value` (break `PXAffinityValue` (break `PXAffinityChange` _output))) 0) (== (`.AffinityBucket` (break `PXAffinityChange` _output)) "/Game/Scenarios/Shared/Configs/Affinity/DA_Extreme_Bucket.DA_Extreme_Bucket")))))