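; Story arc Blueprint that announces when the player has enacted three Cornerstones.
; It can start only when exactly three Cornerstones are embraced.
; On start it sends a Lens config message at the main city's main district, filling text placeholders with the three Cornerstone names, then waits for any choice.
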(event `self.OnStarted`
  (bind _embraced_cornerstones (`/Game/Scenarios/Shared/BlueprintsNonSerialized/SocietyUtils/BPFL_Cornerstone_Utils.Get Embraced Cornerstones`))
  (bind _decision (`/Game/Scenarios/Shared/BlueprintsNonSerialized/SocietyUtils/BPFL_Communication_Utils.Send Config Message` "/Game/Scenarios/Shared/Configs/Messages/SmallLenses/DA_ThreeCornerstones_Enacted_Lens.DA_ThreeCornerstones_Enacted_Lens" (`PXCityComponent.GetMainDistrict` (`PXNationUtils.GetPlayerMainCity`)) null null (`|MakeMap` "CORNERSTONE_1" (`PXCornerstone.InGameName` (`|GetArrayItem` _embraced_cornerstones)) "CORNERSTONE_2" (`PXCornerstone.InGameName` (`|GetArrayItem` _embraced_cornerstones 1)) "CORNERSTONE_3" (`PXCornerstone.InGameName` (`|GetArrayItem` _embraced_cornerstones 2)))))
  (`PXAsyncWaitForAnyChoice.AsyncAction_WaitForAnyChoice` _decision))

(fn `CanBeStarted`
  (returns (ReturnValue :type Boolean))
  (if (== (`KismetArrayLibrary.Array_Length` (`/Game/Scenarios/Shared/BlueprintsNonSerialized/SocietyUtils/BPFL_Cornerstone_Utils.Get Embraced Cornerstones`)) 3)
    (return true)))