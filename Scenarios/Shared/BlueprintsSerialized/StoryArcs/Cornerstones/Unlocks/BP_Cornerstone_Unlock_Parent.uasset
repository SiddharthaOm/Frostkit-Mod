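; Parent story arc Blueprint for Cornerstone unlocks, prompting the player to research a Cornerstone topic.
; On start it sends the unlock lens message with the topic's name, a desire for its first research outcome and an optional district, then waits for a choice.
; The first choice sets the research selector's subcategory, opens the Idea Tree and, if a central research node actor exists, triggers that node's click with the topic.
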(event `self.OnStarted`
  (bind _returnvalue (`PXDesireUtils.MakeResearchOutcomeDesire` (`|GetArrayItem` (`PXResearchTopic.Outcomes` (`self.Cornerstone Topic`)))))
  (bind _decision (`/Game/Scenarios/Shared/BlueprintsNonSerialized/SocietyUtils/BPFL_Communication_Utils.Send Config Message` (`self.Get Lens Config`) (`self.Get District for Tracker`) null null (`self.Get Defines`) null null (struct) true (make `/Game/Scenarios/Shared/BlueprintsNonSerialized/SocietyUtils/F_DesiresArray_Struct` (`|MakeArray` _returnvalue))))
  (bind _choice (`PXAsyncWaitForChoice.AsyncAction_WaitForChoice` _decision)
    (:`Completed`
      (switch `int` _choice
        (:`0`
          (set `/Game/UI/UiWidgets/KBM_Widgets/IdeaTree/SubcategorySelection/WBP_ResearchSubcategorySelector.CurrentSubcategory` (`BlueprintMapLibrary.Map_Find` (`self.Research Topic to Subcategory`) (`self.Cornerstone Topic`)) (`PXPanelsManagementUtils.GetPanelOfClass` "/Game/UI/UiWidgets/KBM_Widgets/IdeaTree/SubcategorySelection/WBP_ResearchSubcategorySelector.WBP_ResearchSubcategorySelector_C"))
          (`PXIdeaTreeUtils.OpenIdeaTree`)
          (bind _returnvalue_2 (`GameplayStatics.GetActorOfClass` "/Game/Scenarios/Shared/BlueprintsNonSerialized/IdeaTree/Core/ResearchNodes/BP_CentralResearchNode.BP_CentralResearchNode_C"))
          (`/Engine/EditorBlueprintResources/StandardMacros.IsValid` _returnvalue_2
            (:`Is Valid`
              (`/Game/UI/UiWidgets/KBM_Widgets/IdeaTree/ResearchNode/WBP_CentralNodeWidget.CentralResearchNodeClicked` (`/Game/UI/UiWidgets/KBM_Widgets/IdeaTree/ResearchNode/WBP_CentralResearchNodeWithReflections.CentralNode` (`PXPanelsManagementUtils.GetPanelOfClass` "/Game/UI/UiWidgets/KBM_Widgets/IdeaTree/ResearchNode/WBP_CentralResearchNodeWithReflections.WBP_CentralResearchNodeWithReflections_C")) (`self.Cornerstone Topic`)))))))))

(fn `Get Defines`
  (returns (Map :type "Map of String to Text"))
  (return (`|MakeMap` "CORNERSTONE" (`PXResearchTopic.IngameName` (`self.Cornerstone Topic`)))))

(fn `Get District for Tracker`
  (returns (`Optional District` :type "PXDistrictComponent Object Reference"))
  (return (`self.Optional District`)))

(fn `Get Lens Config`
  (returns (ReturnValue :type "PXLens Soft Object Reference"))
  (return (`self.Cornerstone Unlock Lens`)))