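; Story proposition in the People's Voice arc that reacts to the first failed vote in parliament.
; It can start when the current parliament has a failed vote and the latest one was not session-requested.
; On start it sends a message naming the council path's first policy, waits for any choice, then unlocks the Council Branch Charter for the player nation.
; An absentee threshold check is defined but never bound here.
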(event `self.OnStarted`
  (bind _decision (`/Game/Scenarios/Shared/BlueprintsNonSerialized/SocietyUtils/BPFL_Communication_Utils.Send Config Message` (`self.failed vote small lens`) null null null (`self.Get Defines`) null null (struct) true))
  (`PXAsyncWaitForAnyChoice.AsyncAction_WaitForAnyChoice` _decision
    (:`Completed`
      (`self.Unlock Council Branch Charter`))))

(fn `Any Absentees Appeared?`
  (params (absence :type "PXAbsenceComponent Object Reference"))
  (if (> (`PXAbsenceUtils.GetCurrentWorkforceAbsenceInCity` (`PXNationUtils.GetPlayerMainCity`) "/Game/Scenarios/Shared/Configs/Absences/AbsenceTypes/DA_Sickliness_Absence.DA_Sickliness_Absence") 299)
    (set `self.Absentees appeared` true)
    (remove `PXAbsenceSubsystem.AbsenceChangedEvent` (subsystem `PXAbsenceSubsystem`) (`|CreateDelegate` :!event `Any Absentees Appeared?`))))

(fn `CanBeStarted`
  (returns (ReturnValue :type Boolean))
  (bind (_allitems _hasanyitem _latestitem) (`PXParliamentUtils.GetVotingHistory` :`parliament` (`PXParliamentUtils.GetCurrentParliament`) :`passFilter` "NotPassedOnly" :`promiseFilter` "All" :`swayFilter` "All" :`recountFilter` "All"))
  (if (and _hasanyitem (not (`.SessionRequested` (break `PXVotingHistoryItem` _latestitem))))
    (return true)))

(fn `Get Defines`
  (returns (Map :type "Map of String to Text"))
  (return (`|MakeMap` "POLICY" (`PXPolicyType.IngameName` (`self.Council Path First Policy`)))))

(fn `Unlock Council Branch Charter`
  (`PXUnlockUtils.SetUnlockActive` (`PXNationUtils.GetPlayerNation`) (`self.Council Branch Charter Unlock`) true))