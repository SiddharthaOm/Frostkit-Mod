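; Story arc scenario in the People's Voice propositions set that notifies the player of a faction passive bonus.
; On start it sends a small lens with the context community's art, filling name, description and effect text from the activated imprint and shared constants maps.
; It then waits for any choice with no follow-up logic, and its start condition always passes.
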(event `self.OnStarted`
  (bind _decision (`/Game/Scenarios/Shared/BlueprintsNonSerialized/SocietyUtils/BPFL_Communication_Utils.Send Lens With Community Art` "/Game/Scenarios/Shared/Configs/Messages/Lenses/Propositions/DA_PeoplesVoice_Propositions_FactionPassiveBonus_SmallLens.DA_PeoplesVoice_Propositions_FactionPassiveBonus_SmallLens" null (`PXCommunityComponent.GetCommunityType` (`self.Context Community`)) (`|MakeMap` "FACTION_SPECIFIC" (`BlueprintMapLibrary.Map_Find` (`/Game/Scenarios/Shared/Configs/ConstantsStorage/BP_SharedConstantsStorageBaseClass.Faction Passive Bonuses Description Text` (`/Game/Scenarios/Shared/BlueprintsNonSerialized/SocietyUtils/BPFL_SharedScenariosStorage.Get Shared Constants Storage`)) (`self.Activated Imprint`)) "FACTION" (`/Game/Scenarios/Shared/BlueprintsNonSerialized/Communities/BPFL_CommunityUtils.Get Community Name` (`self.Context Community`)) "EFFECT" (`BlueprintMapLibrary.Map_Find` (`/Game/Scenarios/Shared/Configs/ConstantsStorage/BP_SharedConstantsStorageBaseClass.Faction Passive Bonuses Modifiers Text` (`/Game/Scenarios/Shared/BlueprintsNonSerialized/SocietyUtils/BPFL_SharedScenariosStorage.Get Shared Constants Storage`)) (`self.Activated Imprint`)) "BONUSNAME" (`PXImprint.IngameName` (`self.Activated Imprint`))) (struct) (struct) true))
  (`PXAsyncWaitForAnyChoice.AsyncAction_WaitForAnyChoice` _decision))

(fn `CanBeStarted`
  (returns (ReturnValue :type Boolean))
  (return true))