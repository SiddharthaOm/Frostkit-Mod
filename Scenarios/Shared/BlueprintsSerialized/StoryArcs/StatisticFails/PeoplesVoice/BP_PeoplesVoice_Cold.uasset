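; Cold variant of the People's Voice statistic-fail story arc, deciding whether a community can propose a generator upgrade desire as the solution.
; Looks up the community's desire leading to level 3 generator research and resolves its building, directly or through an unlocked research outcome.
; Communities matching one affinity value also require city oil supply; others skip that check.
; The building's Cores cost must fit the stockpile, otherwise the parent's solution applies.
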(fn `Can Afford Parts Cost`
  (params (type :type "PXBuildingType Object Reference"))
  (returns (ReturnValue :type Boolean))
  (return (<= (`PXOperationUtils.GetStockpileResourceCostFromOperationCost` (`PXBuildingUtils.GetBuildingTypeConstructionCost` (`PXNationUtils.GetPlayerNation`) type) "/Game/Scenarios/Shared/Configs/Resources/Types/DA_CoresResource.DA_CoresResource") (`PXStockpileUtils.GetCityStockpileOfResource` (`PXNationUtils.GetPlayerMainCity`) "/Game/Scenarios/Shared/Configs/Resources/Types/DA_CoresResource.DA_CoresResource"))))

(fn `City Has Oil`
  (returns (ReturnValue :type Boolean))
  (bind _returnvalue (`/Game/Scenarios/Shared/BlueprintsNonSerialized/Cities/BPFL_CityUtils.Get Current Resource Supply` (`PXNationUtils.GetPlayerMainCity`) "/Game/Scenarios/Shared/Configs/Resources/Types/DA_OilResource.DA_OilResource"))
  (return (> _returnvalue 0)))

(fn `Get Generator Addon Desire`
  (params (communityType :type "PXCommunityType Object Reference"))
  (returns (ReturnValue :type "PXDesire Structure") (Valid :type Boolean) (Output_Get :type "PXBuildingType Object Reference"))
  (locals (building :type "PXBuildingType Object Reference"))
  (bind _returnvalue (`PXDesireUtils.GetResearchDesireLeadingToTopic` communityType "/Game/Scenarios/Shared/Configs/Research/ResearchTopics/_Heating/Generator/GeneratorUpgrades/GeneratorUpgradeLvl3/DA_GeneratorUpgradeLvl3ResearchTopic.DA_GeneratorUpgradeLvl3ResearchTopic"))
  (bind (_policy _building _researchoutcome) (break `PXDesire` _returnvalue))
  (if (and (`PXDesireUtils.IsDesireValid` _returnvalue) (`PXDesireUtils.IsValidDesireForCommunity` _returnvalue communityType))
    (switch `EPXDesireType` (`PXDesireUtils.GetDesireType` _returnvalue)
      (:`BuildingDesire`
        (set `local.building` _building)
        (return _returnvalue true (`local.building`)))
      (:`ResearchOutcomeDesire`
        (if (`PXResearchUtils.IsResearchTopicUnlocked` (`PXNationUtils.GetPlayerNation`) (`PXResearchUtils.GetResearchTopicFromOutcome` (`PXNationUtils.GetPlayerNation`) _researchoutcome))
          (bind (_found _unlocked_building) (`/Game/Scenarios/Shared/BlueprintsNonSerialized/SocietyUtils/BPFL_Cornerstone_Utils.Get building with outcome requirement` _researchoutcome))
          (if _found
            (set `local.building` _unlocked_building)
            (return _returnvalue true (`local.building`))))))))

(fn `Has Solution?`
  (params (Community :type "PXCommunityComponent Object Reference"))
  (returns (`Has Solution` :type Boolean) (Desire :type "PXDesire Structure"))
  (locals (building :type "PXBuildingType Object Reference") (NewLocalVar :type "PXDesire Structure"))
  (bind (_array_element _found) (`/Game/Scenarios/Shared/BlueprintsNonSerialized/FactionEmergence/BPFL_FactionEmergenceUtils.Get Community Affinity on Axis` Community (struct :`Name` "Environment")))
  (if _found
    (if (`PXAffinityUtils.Equal` _array_element (struct :`Name` "Dominion"))
      (if (`self.City Has Oil`)
        (bind (_returnvalue _valid _output_get) (`self.Get Generator Addon Desire` (`PXCommunityComponent.GetCommunityType` (`local.Community`)) :!label _label))
        (if _valid
          (set `local.building` _output_get)
          (set `local.NewLocalVar` _returnvalue)
          (if (`self.Can Afford Parts Cost` (`local.building`))
            (return true (`local.NewLocalVar`))
            (else
              (bind (_has_solution _desire) (`parent.Has Solution?` (`local.Community`)))
              (return _has_solution _desire)))
          (else
            _)))
      (else
        (goto _label))))
  (bind (_has_solution_2 _desire_2) (`parent.Has Solution?` (`local.Community`)))
  (return _has_solution_2 _desire_2))