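; People's Voice story arc for Heatnotes shortage, triggered when the main city's stockpile and the per-community-size balance drop to thresholds.
; It picks the voicing community's desired fix: Goods policy, building or research when Possession is unmet, then currency policy or research.
; The last fallback is an action on another community, preferring opposite affinity.
; A lens presents the desire, and the first choice starts a solution quest and blocks further SNOPS arcs.
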(event `self.OnFinished`
  (`parent.OnFinished`))

(fn `Generic Lens`
  (returns (Decision :type "PXDecision Object Reference"))
  (bind _voice_community (`self.Voice Community`))
  (`PXUnlockUtils.SetUnlockActive` (`PXNationUtils.GetPlayerNation`) (`self.Hide 2nd choice Unlock Asset`) true)
  (if (`|EnumEquality` (`PXDesireUtils.GetDesireType` (`self.Desired Solution`)) "ActionDesire")
    (bind _decision (`parent.Generic Lens`))
    (return _decision)
    (else
      (bind _decision_2 (`/Game/Scenarios/Shared/BlueprintsNonSerialized/SocietyUtils/BPFL_Communication_Utils.Send Lens With Community Art` (`self.Lens for Building / Research / Policy`) null (`PXCommunityComponent.GetCommunityType` _voice_community) (`self.Lens Defines`) (`PXGameplayContextUtils.MakePXGameContext` _voice_community) (`PXCommunicationChannelsUtils.CreateDesiresPerChoiceArray` (`|MakeArray` (make `PXCommunicationChannelsDesiresPerChoice` (`|MakeArray` (`self.Desired Solution`))))) true))
      (return _decision_2))))

(fn `Get Solution Quest Name`
  (returns (`Quest Name` :type Text))
  (return (`self.quest name`)))

(fn `Goods Demand Unmet?`
  (returns (ReturnValue :type Boolean))
  (return (< (`PXNeedUtils.GetCityNeedBalance` (`PXNationUtils.GetPlayerMainCity`) "/Game/Scenarios/Shared/Configs/Needs/Needs/DA_Possession.DA_Possession") (`self.Unmet Demand Threshold`))))

(fn `Handle Choices`
  (locals (`Request Funds` :type "PXCommunityAction Object Reference" :default "/Script/Frostpunk2.PXCommunityAction'/Game/Scenarios/Shared/Configs/Communities/CommunityActions/Favours_Group/RequestFunds/DA_RequestFunds_CA.DA_RequestFunds_CA'"))
  (`PXUnlockUtils.SetUnlockActive` (`PXNationUtils.GetPlayerNation`) (`self.Hide 2nd choice Unlock Asset`))
  (switch `int` (`self.choice`)
    (:`0`
      (`self.Start Solution Quest`)
      (`PXStoryUtils.AddStoryArcBlockReason` (struct :`TagName` "StoryArcTag.Snops") "/Game/Scenarios/Shared/Configs/BlockReasons/DA_SNOPS_PeopleVoice_Block.DA_SNOPS_PeopleVoice_Block"))))

(fn `Has Currency Policy Desire?`
  (params (Community :type "PXCommunityComponent Object Reference"))
  (returns (Desire :type "PXDesire Structure") (`Has Desire` :type Boolean))
  (bind (_array_element _found) (`/Game/Scenarios/Shared/BlueprintsNonSerialized/FactionEmergence/BPFL_FactionEmergenceUtils.Get Community Affinity on Axis` Community (struct :`Name` "Economy")))
  (if _found
    (for _array_element_2 (select `bool` (`PXAffinityUtils.Equal` _array_element (struct :`Name` "Competition")) :`false` (`self.Currency Policies - Equality`) :`true` (`self.Currency Policies - Merit`))
      (if (not (`/Game/Scenarios/Shared/BlueprintsNonSerialized/Policies/BPFL_PolicyUtils.Policy or Fallback is Active` _array_element_2))
        (bind _returnvalue (`PXDesireUtils.MakePolicyDesire` _array_element_2))
        (bind _returnvalue_2 (`PXDesireUtils.IsValidDesireForCommunity` _returnvalue (`PXCommunityComponent.GetCommunityType` (`local.Community`))))
        (if _returnvalue_2
          (return _returnvalue _returnvalue_2))))
    (return (struct) false)
    (else
      (return (struct) false))))

(fn `Has Currency Research Desire?`
  (params (Community :type "PXCommunityComponent Object Reference"))
  (returns (ReturnValue :type Boolean) (Output :type "PXDesire Structure"))
  (bind _returnvalue (`PXDesireUtils.GetCommunityTypeDesiresHelpingWithStatistic` (`PXCommunityComponent.GetCommunityType` Community) (`self.Fake Currency Stat`)))
  (return (`KismetArrayLibrary.Array_IsNotEmpty` _returnvalue) (`|GetArrayItem` _returnvalue)))

(fn `Has Goods Building Desire?`
  (params (Community :type "PXCommunityComponent Object Reference"))
  (returns (Desire :type "PXDesire Structure") (`Has Desire` :type Boolean))
  (for _array_element (`self.Goods Buildings`)
    (bind _returnvalue_passed (break `PXCheckResult` (`PXBuildingUtils.HasUnlockedBuilding` (`PXNationUtils.GetPlayerMainCity`) _array_element)))
    (if _returnvalue_passed
      (bind (_entry _hasaffinity) (`PXBuildingUtils.GetBuildingDominantAffinity` _array_element))
      (if _hasaffinity
        (if (`KismetArrayLibrary.Array_Contains` (`PXCommunityUtils.GetCommunityCoreAffinities` (`local.Community`)) _entry)
          (bind _returnvalue (`PXDesireUtils.MakeBuildingDesire` _array_element 1 :!label _label))
          (if (`PXDesireUtils.IsValidDesireForCommunity` _returnvalue (`PXCommunityComponent.GetCommunityType` (`local.Community`)))
            (return _returnvalue true)))
        (elif (not (`.Found` (`/Game/Scenarios/Shared/BlueprintsNonSerialized/FactionEmergence/BPFL_FactionEmergenceUtils.Get Community Affinity on Axis` (`local.Community`) (struct :`Name` "Environment"))))
          (goto _label)))))
  (return (struct) false))

(fn `Has Goods Policy Desire?`
  (params (Community :type "PXCommunityComponent Object Reference"))
  (returns (`Has Desire?` :type Boolean) (Desire :type "PXDesire Structure"))
  (bind (_array_element _found) (`/Game/Scenarios/Shared/BlueprintsNonSerialized/FactionEmergence/BPFL_FactionEmergenceUtils.Get Community Affinity on Axis` Community (struct :`Name` "Environment")))
  (bind _value (`BlueprintMapLibrary.Map_Find` (`self.Goods Policies`) _array_element))
  (if _found
    (if (not (`/Game/Scenarios/Shared/BlueprintsNonSerialized/Policies/BPFL_PolicyUtils.Policy or Fallback is Active` _value))
      (bind _returnvalue (`PXDesireUtils.MakePolicyDesire` _value))
      (return (`PXDesireUtils.IsValidDesireForCommunity` _returnvalue (`PXCommunityComponent.GetCommunityType` Community)) _returnvalue)
      (else
        (return false)))
    (else
      (return false))))

(fn `Has Goods Research Desire?`
  (params (Community :type "PXCommunityComponent Object Reference"))
  (returns (ReturnValue :type Boolean) (Output :type "PXDesire Structure"))
  (bind _returnvalue (`PXDesireUtils.GetCommunityTypeDesiresHelpingWithStatistic` (`PXCommunityComponent.GetCommunityType` Community) (`self.Fake Goods Stat`)))
  (return (`KismetArrayLibrary.Array_IsNotEmpty` _returnvalue) (`|GetArrayItem` _returnvalue)))

(fn `Has Solution?`
  (params (Community :type "PXCommunityComponent Object Reference"))
  (returns (`Has Solution` :type Boolean) (Desire :type "PXDesire Structure"))
  (if (`self.Goods Demand Unmet?`)
    (bind (_has_desire_ _desire) (`self.Has Goods Policy Desire?` (`local.Community`)))
    (if _has_desire_
      (return true _desire)
      (else
        (bind (_desire_2 _has_desire) (`self.Has Goods Building Desire?` (`local.Community`)))
        (if _has_desire
          (return true _desire_2)
          (else
            (bind (_returnvalue _output) (`self.Has Goods Research Desire?` (`local.Community`)))
            (if _returnvalue
              (return true _output)
              (else
                _)))))))
  (bind (_desire_3 _has_desire_2) (`self.Has Currency Policy Desire?` (`local.Community`)))
  (if _has_desire_2
    (return true _desire_3)
    (else
      (bind (_returnvalue_2 _output_2) (`self.Has Currency Research Desire?` (`local.Community`)))
      (if _returnvalue_2
        (return true _output_2)
        (else
          (for _array_element (`PXCommunityUtils.GetCommunityCoreAffinities` (`local.Community`))
            (bind (_exists _community) (`/Game/Scenarios/Shared/BlueprintsNonSerialized/SocietyUtils/BPFL_Cornerstone_Utils.Get X Affinity Commenter` (`/Game/Scenarios/Shared/BlueprintsNonSerialized/SocietyUtils/BPFL_Cornerstone_Utils.Get Opposite Affinity` _array_element)))
            (if _exists
              (bind _output_get (set `self.Target Community` _community))
              (bind _returnvalue_3 (`PXDesireUtils.MakeActionDesire` (`self.Community Action`) (`PXNationUtils.GetPlayerMainCity`) (`PXCommunityComponent.GetCommunityType` _output_get)))
              (if (and (`.Passed` (break `PXCheckResult` (`PXCommunityActionUtils.IsActionPossible` (`self.Community Action`) _output_get))) (`PXDesireUtils.IsValidDesireForCommunity` _returnvalue_3 (`PXCommunityComponent.GetCommunityType` (`local.Community`))))
                (return true _returnvalue_3))))
          (return false))))))

(fn `Lens Defines`
  (returns (Map :type "Map of String to Text"))
  (locals (NewLocalVar :type "Map of String to Text"))
  (bind (_problem_exists _problem_stats _worst_stat1) (`/Game/Scenarios/Shared/BlueprintsNonSerialized/SocietyUtils/BPFL_CanBeStarted_Utils.Worst Stat from List Over Trait Threshold` (`self.Main Stats`) (`self.Min Trait Level 2nd problem`)))
  (bind _defines_map_merged (`/Game/Scenarios/Shared/BlueprintsNonSerialized/SocietyUtils/BPFL_Communication_Utils.Merge Defines` (`parent.Lens Defines`) (`|MakeMap` "SECOND_PROBLEM" (`PXStatistic.IngameName` _worst_stat1) "TARGET_COMMUNITY" (`/Game/Scenarios/Shared/BlueprintsNonSerialized/Communities/BPFL_CommunityUtils.Get Community Name` (`self.Target Community`)) "PROBLEM" "{HEATNOTES}")))
  (return _defines_map_merged))

(fn `SNOPS core stat check`
  (returns (`Conditions met` :type Boolean))
  (bind _returnvalue (`PXNationUtils.GetPlayerMainCity`))
  (if (<= (`PXStockpileUtils.GetCityStockpileOfResource` _returnvalue "/Game/Scenarios/Shared/Configs/Resources/Types/DA_Core_Heatnotes.DA_Core_Heatnotes") (`self.Heatnotes Stockpile Threshold`))
    (if (<= (/ (`KismetMathLibrary.Conv_IntToDouble` (`PXEconomyUtils.GetTargetResourceBalanceInNation` (`PXNationUtils.GetPlayerNation`) "/Game/Scenarios/Shared/Configs/Resources/Types/DA_Core_Heatnotes.DA_Core_Heatnotes")) (`KismetMathLibrary.Conv_IntToDouble` (`PXCommunityUtils.GetCityCommunitiesSize` _returnvalue))) (`self.Threshold to start`))
      (return true))))