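; Story arc that reacts when opposite extremes conflict on an affinity axis.
; CanBeStarted picks the first axis flagged in shared ConflictingExtremesOnAxis storage.
; On start it resolves an extreme thing and community commenter for each affinity, then sends that axis's LensConfig message with those names and waits for a choice.
; A helper, uncalled here, finds axes where the player nation is extreme on both sides.
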(event `self.OnStarted`
  (bind (_data _firstaffinity _secondaffinity) (`EntriesBlueprintFunctionLibrary.GetAffinityAxisDetails` (`self.extreme axis`)))
  (bind (_data_2 _firstaffinity_2 _secondaffinity_2) (`EntriesBlueprintFunctionLibrary.GetAffinityAxisDetails` (`self.extreme axis`)))
  (bind _data_ingamename (break `PXAffinity` (`EntriesBlueprintFunctionLibrary.GetAffinityDetails` _secondaffinity_2)))
  (bind _data_ingamename_2 (break `PXAffinity` (`EntriesBlueprintFunctionLibrary.GetAffinityDetails` _firstaffinity_2)))
  (bind _ingame_name (`self.Get Extreme Stuff` _firstaffinity))
  (set `self.first extreme thing` _ingame_name)
  (bind _ingame_name_2 (`self.Get Extreme Stuff` _secondaffinity))
  (set `self.second extreme thing` _ingame_name_2)
  (bind (_exists _community) (`/Game/Scenarios/Shared/BlueprintsNonSerialized/SocietyUtils/BPFL_Cornerstone_Utils.Get X Affinity Commenter` _firstaffinity_2 false))
  (bind (_exists_2 _community_2) (`/Game/Scenarios/Shared/BlueprintsNonSerialized/SocietyUtils/BPFL_Cornerstone_Utils.Get X Affinity Commenter` _secondaffinity_2 false))
  (bind _decision (`/Game/Scenarios/Shared/BlueprintsNonSerialized/SocietyUtils/BPFL_Communication_Utils.Send Config Message` (`BlueprintMapLibrary.Map_Find` (`self.Lens config`) (`self.extreme axis`)) null null null (`|MakeMap` "AXIS" (break `PXAffinityAxis` _data_2) "AFFINITY_1" _data_ingamename_2 "AFFINITY_2" _data_ingamename "THING" (`self.first extreme thing`) "OPPOSITE_THING" (`self.second extreme thing`) "THING_FACTION" (`/Game/Scenarios/Shared/BlueprintsNonSerialized/Communities/BPFL_CommunityUtils.Get Community Name` _community) "OPPOSITE_THING_FACTION" (`/Game/Scenarios/Shared/BlueprintsNonSerialized/Communities/BPFL_CommunityUtils.Get Community Name` _community_2)) null null (struct) true))
  (`PXAsyncWaitForAnyChoice.AsyncAction_WaitForAnyChoice` _decision))

(fn `CanBeStarted`
  (returns (ReturnValue :type Boolean))
  (bind _conflicting_extremes_on_axis (`/Game/Scenarios/Shared/BlueprintsSerialized/VariableStorage/BP_SharedVariableStorage.Conflicting Extremes on Axis` (`/Game/Scenarios/Shared/BlueprintsNonSerialized/SocietyUtils/BPFL_SharedScenariosStorage.Get Shared Variable Storage`)))
  (bind _keys (`BlueprintMapLibrary.Map_Keys` _conflicting_extremes_on_axis))
  (for _array_element _keys
    (if (`BlueprintMapLibrary.Map_Find` _conflicting_extremes_on_axis _array_element)
      (set `self.extreme axis` _array_element)
      (return true))))

(fn `Player is Extreme on Opposites`
  (params (Array :type "Array of PXAffinityAxisEntry Structure"))
  (returns (`Array Element` :type "PXAffinityAxisEntry Structure") (Return :type Boolean))
  (for _array_element Array
    (bind (_data _firstaffinity _secondaffinity) (`EntriesBlueprintFunctionLibrary.GetAffinityAxisDetails` _array_element))
    (if (and (> (`PXAffinityUtils.GetNationLeaderAffinityValueFromBucket` (`PXNationUtils.GetPlayerNation`) _firstaffinity "/Game/Scenarios/Shared/Configs/Affinity/DA_Extreme_Bucket.DA_Extreme_Bucket") 0) (> (`PXAffinityUtils.GetNationLeaderAffinityValueFromBucket` (`PXNationUtils.GetPlayerNation`) _secondaffinity "/Game/Scenarios/Shared/Configs/Affinity/DA_Extreme_Bucket.DA_Extreme_Bucket") 0))
      (return _array_element true))))