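; Story arc for the Cold Homes situation of a significant community, startable only while that community has the Cold Homes imprint active.
; On start it sends a ghost with affinity art for the cold district, filling text with the district and community names, and waits for any player choice.
; Its parameters hash derives from the ghost config.
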(event `self.OnStarted`
  (bind _decision (`/Game/Scenarios/Shared/BlueprintsNonSerialized/FactionEmergence/BPFL_FactionEmergenceUtils.Send Ghost with Affinity Art` (`self.Ghost`) (`self.Cold District`) (`PXCommunityComponent.GetCommunityType` (`self.Community`)) (`|MakeMap` "DISTRICT_FLUFF" (`/Game/Scenarios/Shared/BlueprintsNonSerialized/Cities/BPFL_CityUtils.GetDistrictFluffName` (`self.Cold District`)) "COMMUNITY" (`/Game/Scenarios/Shared/BlueprintsNonSerialized/Communities/BPFL_CommunityUtils.Get Community Name` (`self.Community`)))))
  (`PXAsyncWaitForAnyChoice.AsyncAction_WaitForAnyChoice` _decision))

(fn `CanBeStarted`
  (returns (ReturnValue :type Boolean))
  (return (`PXCommunityComponent.HasActiveImprint` (`self.Community`) "/Game/Scenarios/Shared/Configs/Communities/Imprints/PresenceBased/DA_ColdHomes_Imprint.DA_ColdHomes_Imprint")))

(fn `GetParametersHash`
  (returns (ReturnValue :type Integer))
  (return (`PXStoryUtils.GetHashForUObjectParameter` (`|ConvertAsset` (`self.Ghost`)))))