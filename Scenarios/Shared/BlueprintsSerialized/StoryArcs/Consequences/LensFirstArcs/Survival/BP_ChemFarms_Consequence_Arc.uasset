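; Consequence story arc in the Survival lens arcs for chem farms, able to start only when the parent check passes and the food policy is active.
; Building its message defines also sets the building type to Advanced Drum Hothouses if one is active in the player's main city, otherwise the basic Drum Hothouse.
; It merges the food policy's in-game name into the parent's defines; choice handling is empty.
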(fn `CanBeStarted`
  (returns (ReturnValue :type Boolean))
  (bind _returnvalue (`parent.CanBeStarted`))
  (if _returnvalue
    (if (`/Game/Scenarios/Shared/BlueprintsNonSerialized/Policies/BPFL_PolicyUtils.IsPolicyActive` (`self.Policy Food`))
      (return true)
      (else
        (return false)))
    (else
      (return false))))

(fn `Get message defines`
  (returns (Map :type "Map of String to Text"))
  (if (`PXBuildingUtils.HasBuildingOfTypeInCity` (`PXNationUtils.GetPlayerMainCity`) "/Game/Scenarios/Shared/Configs/Buildings/AdvancedDrumHotHouses/DA_F_AdvancedDrumHothouses_Dominion.DA_F_AdvancedDrumHothouses_Dominion" true)
    (set `self.Building Type` "/Game/Scenarios/Shared/Configs/Buildings/AdvancedDrumHotHouses/DA_F_AdvancedDrumHothouses_Dominion.DA_F_AdvancedDrumHothouses_Dominion")
    (else
      (set `self.Building Type` "/Game/Scenarios/Shared/Configs/Buildings/DrumHothouse/DA_F_DrumHothouse_Dominion.DA_F_DrumHothouse_Dominion")))
  (`BlueprintMapLibrary.Map_Add` (`self.Local Defines Map`) "POLICY_FOOD" (`PXPolicyType.IngameName` (`self.Policy Food`)))
  (bind _defines_map_merged (`/Game/Scenarios/Shared/BlueprintsNonSerialized/SocietyUtils/BPFL_Communication_Utils.Merge Defines` (`parent.Get message defines`) (`self.Local Defines Map`)))
  (return _defines_map_merged))

(fn `Handle Choice`
  (params (Selection :type Integer)))