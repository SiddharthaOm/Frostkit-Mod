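; Heat recycling consequence story arc in the Survival lens-first scenario arcs, following up on an earlier player choice.
; HandleChoice waits for a story beat of the arc's beat type and lane, then checks whether the consequence can start.
; If so, it sends a config message chosen by that choice (RepurposeGhost or SuckItUpGhost), targeting the closest district to the lens tracker's.
; It then waits for the player to make any choice on that message.
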(event `self.Handle Choice`
  (params (Selection :type Integer))
  (bind (_beat_type _lane_type) (`self.Get Story Beat Types`))
  (`PXAsyncWaitForStoryBeat.AsyncAction_WaitForStoryBeat` _beat_type _lane_type
    (:`Completed`
      (bind _returnvalue (`self.Consequence CanBeStarted Core`))
      (if _returnvalue
        (bind _decision (`/Game/Scenarios/Shared/BlueprintsNonSerialized/SocietyUtils/BPFL_Communication_Utils.Send Config Message` (select `int` (`self.Choice`) :`0` (`self.Repurpose Ghost`) :`1` (`self.Suck it up Ghost`) :!type "PXCommunicationChannelMessage Soft Object Reference") (`self.Get District for Lens Tracker`) null null (`self.Get message defines`) null null (struct) true))
        (bind _output_get (set `self.Decision_0` _decision))
        (`PXAsyncWaitForAnyChoice.AsyncAction_WaitForAnyChoice` _output_get)))))