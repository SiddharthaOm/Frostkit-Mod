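; Story arc for the Algorithm Hunger cornerstone consequence, presenting a lens decision about the Algorithm and its follow-up.
; On start it sends the lens message with the cornerstone name injected into the text, then branches on the player's choice.
; Each branch, gated by a nation unlock to play once, waits for a major story beat, shows its consequence message, then sets that unlock.
; Agreeing also kills a percentage of the main city's population by starvation.
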(event `self.OnStarted`
  (bind _defines_map_merged (`/Game/Scenarios/Shared/BlueprintsNonSerialized/SocietyUtils/BPFL_Communication_Utils.Merge Defines` (`/Game/Scenarios/Shared/BlueprintsNonSerialized/SocietyUtils/BPFL_Communication_Utils.Get Common Text Defines` null) (`|MakeMap` "CORNERSTONE" (`PXResearchOutcome.IngameName` (`self.Reason Cronerstone Outcome`)))))
  (bind _decision (`/Game/Scenarios/Shared/BlueprintsNonSerialized/SocietyUtils/BPFL_Communication_Utils.Send Config Message` (`self.The Algorithm Lens`) null null null _defines_map_merged null null (struct) true))
  (bind _output_get (set `self.Lens Decision` _decision))
  (bind _choice (`PXAsyncWaitForChoice.AsyncAction_WaitForChoice` _output_get)
    (:`Completed`
      (bind _output_get_2 (set `self.Choice` _choice))
      (switch `int` _output_get_2
        (:`0`
          (if (not (`PXUnlockUtils.IsUnlockActive` (`PXNationUtils.GetPlayerNation`) "/Game/Scenarios/Shared/Configs/Unlocks/ConsequenceArcs/CornerstoneConsequences/DA_AlgoritmConsequenceChoice1Seen.DA_AlgoritmConsequenceChoice1Seen"))
            (`PXAsyncWaitForStoryBeat.AsyncAction_WaitForStoryBeat` (`self.Major Story Beat Type`) (`self.Main Story Beat Lane`)
              (:`Completed`
                (bind _defines_map_merged_2 (`/Game/Scenarios/Shared/BlueprintsNonSerialized/SocietyUtils/BPFL_Communication_Utils.Merge Defines` (`/Game/Scenarios/Shared/BlueprintsNonSerialized/SocietyUtils/BPFL_Communication_Utils.Get Common Text Defines` null) (`|MakeMap` "CORNERSTONE" (`PXResearchOutcome.IngameName` (`self.Reason Cronerstone Outcome`)))))
                (bind _decision_2 (`/Game/Scenarios/Shared/BlueprintsNonSerialized/SocietyUtils/BPFL_Communication_Utils.Send Config Message` (`self.Agree with the Algorithm Consequence Ghost`) null null null _defines_map_merged_2 null null (struct) true))
                (`PXAsyncWaitForAnyChoice.AsyncAction_WaitForAnyChoice` _decision_2
                  (:`Completed`
                    (`PXUnlockUtils.SetUnlockActive` (`PXNationUtils.GetPlayerNation`) "/Game/Scenarios/Shared/Configs/Unlocks/ConsequenceArcs/CornerstoneConsequences/DA_AlgoritmConsequenceChoice1Seen.DA_AlgoritmConsequenceChoice1Seen" true)
                    (`/Game/Scenarios/Shared/BlueprintsNonSerialized/GameplayActions/BPFL_GameplayAction_Utils.Kill Percent Of City` (`|FormatText` "Children and elderly starved to death") (`PXNationUtils.GetPlayerMainCity`) 0.1 true true true)))))))
        (:`1`
          (if (not (`PXUnlockUtils.IsUnlockActive` (`PXNationUtils.GetPlayerNation`) "/Game/Scenarios/Shared/Configs/Unlocks/ConsequenceArcs/CornerstoneConsequences/DA_AlgoritmConsequenceChoice2Seen.DA_AlgoritmConsequenceChoice2Seen"))
            (`PXAsyncWaitForStoryBeat.AsyncAction_WaitForStoryBeat` (`self.Major Story Beat Type`) (`self.Main Story Beat Lane`)
              (:`Completed`
                (bind _defines_map_merged_3 (`/Game/Scenarios/Shared/BlueprintsNonSerialized/SocietyUtils/BPFL_Communication_Utils.Merge Defines` (`/Game/Scenarios/Shared/BlueprintsNonSerialized/SocietyUtils/BPFL_Communication_Utils.Get Common Text Defines` null) (`|MakeMap` "CORNERSTONE" (`PXResearchOutcome.IngameName` (`self.Reason Cronerstone Outcome`)))))
                (bind _decision_3 (`/Game/Scenarios/Shared/BlueprintsNonSerialized/SocietyUtils/BPFL_Communication_Utils.Send Config Message` (`self.Disagree with the Algorithm Consequence SmallLens`) null null null _defines_map_merged_3 null null (struct) true))
                (`PXAsyncWaitForAnyChoice.AsyncAction_WaitForAnyChoice` _decision_3
                  (:`Completed`
                    (`PXUnlockUtils.SetUnlockActive` (`PXNationUtils.GetPlayerNation`) "/Game/Scenarios/Shared/Configs/Unlocks/ConsequenceArcs/CornerstoneConsequences/DA_AlgoritmConsequenceChoice2Seen.DA_AlgoritmConsequenceChoice2Seen" true)))))))))))