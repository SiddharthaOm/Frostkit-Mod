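; Consequence arc for the Infection Badge starting law, turning a lens choice into either a hospital promise or a policy-unlock notification.
; With the Hospital lens, the first option starts a timed side quest to research and construct a hospital; other lenses announce the No Contagion Prevention policy.
; On arc finish, a valid quest is awaited, then its result opens a success or failure dialog and activates a promise kept or broken trust modifier.
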(event `self.Handle Choice`
  (params (Selection :type Integer))
  (bind _hospital_research_topic (`self.Hospital Research Topic`))
  (if (== (`PXCommunicationChannelsUtils.ToObject` (`self.Lens Config`)) "/Game/Scenarios/Shared/Configs/Messages/Lenses/Consequences/ConsequenceLenses/StartingLaws/DA_InfectionBadge_Hospital_Lens.DA_InfectionBadge_Hospital_Lens")
    (switch `int` Selection
      (:`0`
        (bind _returnvalue (`PXQuestUtils.StartQuestInPlace` (`|FormatText` "Hospital Quest Name") "" (`self.duration quest`) "SideQuest" "DebugQuestName" true))
        (set `self.Hospital Quest` _returnvalue)
        (`PXQuestUtils.AddBuildingWithTagsQuestObjective` (make `PXObjectiveParameters` (`|FormatText` "Construct newly researched building") "" false 1 null (`self.Hospital Quest`)) (make `PXBuildingWithTagsObjectiveParameters` (`self.Hospital Gameplay Tag`) "Build" 1 null null false))
        (`PXQuestUtils.AddResearchQuestObjective` (`self.Hospital Quest`) (`|FormatText` "Research '{TOPIC}'" (`PXResearchTopic.IngameName` _hospital_research_topic)) "" _hospital_research_topic false null null null)))
    (else
      (switch `int` 0
        (:`0`
          (`PXCentralNotificationUtils.ShowCentralNotificationOfType` "Parliament" (`|FormatText` "{POLICY_UNLOCK}" (`PXPolicyType.IngameName` (`self.No Contagion Prevention Policy`))) (`|FormatText` "New Policy Unlocked")))))))

(event `self.OnFinished`
  (`/Engine/EditorBlueprintResources/StandardMacros.IsValid` (`self.Hospital Quest`)
    (:`Is Valid`
      (bind _succeeded (`PXAsyncWaitForQuest.AsyncAction_WaitForQuest` (`self.Hospital Quest`))
        (:`Completed`
          (if _succeeded
            (`PXAsyncOpenPredefinedDialog.AsyncAction_OpenPredefinedDialog` "/Game/Scenarios/Shared/Configs/Messages/Dialogs/Quests/DA_InfectionBadgeHospital_QuestSuccess.DA_InfectionBadgeHospital_QuestSuccess"
              (:`Completed`
                (`PXPredefinedModifierUtils.SetPredefinedModifierActive` (`PXNationUtils.GetPlayerNation`) "/Game/Scenarios/Shared/BlueprintsSerialized/Quests/Demands/DA_PromiseKept_AllCommunitiesTrust.DA_PromiseKept_AllCommunitiesTrust" true)))
            (else
              (`PXAsyncOpenPredefinedDialog.AsyncAction_OpenPredefinedDialog` "/Game/Scenarios/Shared/Configs/Messages/Dialogs/Quests/DA_InfectionBadgeHospital_QuestFail.DA_InfectionBadgeHospital_QuestFail"
                (:`Completed`
                  (`PXPredefinedModifierUtils.SetPredefinedModifierActive` (`PXNationUtils.GetPlayerNation`) "/Game/Scenarios/Shared/BlueprintsSerialized/Quests/Demands/DA_PromiseBroken_AllCommunitiesTrust.DA_PromiseBroken_AllCommunitiesTrust" true))))))))))

(fn `CanBeStarted`
  (returns (ReturnValue :type Boolean))
  (bind _returnvalue (`parent.CanBeStarted`))
  (return _returnvalue))

(fn `Get message defines`
  (returns (Map :type "Map of String to Text"))
  (bind _defines_map_merged (`/Game/Scenarios/Shared/BlueprintsNonSerialized/SocietyUtils/BPFL_Communication_Utils.Merge Defines` (`parent.Get message defines`) (`|MakeMap` "POLICY_UNLOCK" (`PXPolicyType.IngameName` (`self.No Contagion Prevention Policy`)) "DURATION" (`PXTextUtils.GameTimeToText` (`self.duration quest`) true false false false))))
  (return _defines_map_merged))