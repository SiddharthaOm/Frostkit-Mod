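; Consequence story arc that announces the unlock of the No Contagion Prevention policy.
; On start it sends an Infection Badge small lens if the Quarantine Merit policy is active, otherwise a Supported Quarantine one.
; It waits for any choice on the lens, then shows a Parliament-type central notification titled with the unlocked policy's name.
; Message defines extend the parent's with in-game names for the unlocked and badge policies.
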(event `self.OnStarted`
  (if (`/Game/Scenarios/Shared/BlueprintsNonSerialized/Policies/BPFL_PolicyUtils.IsPolicyActive` "/Game/Scenarios/Shared/Configs/Policies/Survival/Quarantine/DA_Quarantine_Merit.DA_Quarantine_Merit")
    (set `self.SupportedQuarantineSmallLens` "/Game/Scenarios/Shared/Configs/Messages/SmallLenses/DA_InfectionBadge_NoQuarantineUnlock_Consequence_SmallLens.DA_InfectionBadge_NoQuarantineUnlock_Consequence_SmallLens")
    (else
      (set `self.SupportedQuarantineSmallLens` "/Game/Scenarios/Shared/Configs/Messages/SmallLenses/DA_SupportedQuarantine_NoQuarantineUnlock_Consequence_SmallLens.DA_SupportedQuarantine_NoQuarantineUnlock_Consequence_SmallLens")))
  (bind _decision (`self.Send Lens` (`self.SupportedQuarantineSmallLens`)))
  (`PXAsyncWaitForAnyChoice.AsyncAction_WaitForAnyChoice` _decision
    (:`Completed`
      (`PXCentralNotificationUtils.ShowCentralNotificationOfType` "Parliament" (`|FormatText` "{POLICY_UNLOCK}" (`PXPolicyType.IngameName` (`self.No Contagion Prevention Policy`))) (`|FormatText` "New Policy Unlocked")))))

(fn `CanBeStarted`
  (returns (ReturnValue :type Boolean))
  (bind _returnvalue (`parent.CanBeStarted`))
  (return _returnvalue))

(fn `Get message defines`
  (returns (Map :type "Map of String to Text"))
  (bind _defines_map_merged (`/Game/Scenarios/Shared/BlueprintsNonSerialized/SocietyUtils/BPFL_Communication_Utils.Merge Defines` (`parent.Get message defines`) (`|MakeMap` "POLICY_UNLOCK" (`PXPolicyType.IngameName` (`self.No Contagion Prevention Policy`)) "POLICY" (`PXPolicyType.IngameName` (`self.Badge Policy`)))))
  (return _defines_map_merged))