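; Consequence story arc that reacts to large heat disparity between housing districts in the player's main city.
; It starts outside the Nomads scenario when a Council Hall and the Chaos heat-access policy are active and enough housing is cold.
; The player can promise equal or paid heating, creating a timed policy quest whose outcome shows a dialog and adjusts affinity-matched communities' trust.
; Declining or failing sends a Ghost message after a story-beat wait.
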(event `self.Handle Choice`
  (params (Selection :type Integer))
  (bind (_beat_type _lane_type) (`self.Get Story Beat Types`))
  (switch `int` Selection
    (:`0`
      (bind _returnvalue (`PXQuestUtils.StartQuestInPlace` (`|FormatText` "Regulate {Law}" (`PXLawType.IngameName` (`self.Heating Law`))) "" (`self.Duration`) "SideQuest" "DebugQuestName" true))
      (set `self.Regulate Heating Quest` _returnvalue)
      (`PXQuestUtils.AddPolicyQuestObjective` (make `PXObjectiveParameters` (`|FormatText` "Pass {POLICY}" (`PXPolicyType.IngameName` (`self.Equal heating policy`))) "" false 1 null (`self.Regulate Heating Quest`)) (make `PXPolicyObjectiveParameters` (`self.Equal heating policy`)))
      (set `self.Equality Choice` true))
    (:`1`
      (bind _returnvalue_2 (`PXQuestUtils.StartQuestInPlace` (`|FormatText` "Regulate {Law}" (`PXLawType.IngameName` (`self.Heating Law`))) "" (`self.Duration`) "SideQuest" "DebugQuestName" true))
      (set `self.Regulate Heating Quest` _returnvalue_2)
      (`PXQuestUtils.AddPolicyQuestObjective` (make `PXObjectiveParameters` (`|FormatText` "Pass {POLICY}" (`PXPolicyType.IngameName` (`self.Paid heating policy`))) "" false 1 null (`self.Regulate Heating Quest`)) (make `PXPolicyObjectiveParameters` (`self.Paid heating policy`)))
      (set `self.Merit Choice` true))
    (:`2`
      (`PXAsyncWaitForStoryBeat.AsyncAction_WaitForStoryBeat` _beat_type _lane_type
        (:`Completed`
          (`/Game/Scenarios/Shared/BlueprintsNonSerialized/SocietyUtils/BPFL_Communication_Utils.Send Config Message` (`self.Ghost`) null null null (`/Game/Scenarios/Shared/BlueprintsNonSerialized/SocietyUtils/BPFL_Communication_Utils.Get Common Text Defines` null) null null (struct) true))))))

(event `self.OnFinished`
  (bind (_beat_type _lane_type) (`self.Get Story Beat Types`))
  (if (or (`self.Equality Choice`) (`self.Merit Choice`))
    (bind _succeeded (`PXAsyncWaitForQuest.AsyncAction_WaitForQuest` (`self.Regulate Heating Quest`))
      (:`Completed`
        (if _succeeded
          (`PXAsyncOpenPredefinedDialog.AsyncAction_OpenPredefinedDialog` (`self.Success Dialog`)
            (:`Completed`
              (`self.Add success trust modifier`)))
          (else
            (`PXAsyncOpenPredefinedDialog.AsyncAction_OpenPredefinedDialog` (`self.Failed Dialog`)
              (:`Completed`
                (`self.Add failed trust modifier`)
                (`PXAsyncWaitForStoryBeat.AsyncAction_WaitForStoryBeat` _beat_type _lane_type
                  (:`Completed`
                    (`/Game/Scenarios/Shared/BlueprintsNonSerialized/SocietyUtils/BPFL_Communication_Utils.Send Config Message` (`self.Ghost`) null null null (`/Game/Scenarios/Shared/BlueprintsNonSerialized/SocietyUtils/BPFL_Communication_Utils.Get Common Text Defines` null) null null (struct) true)))))))))))

(fn `Add failed trust modifier`
  (if (`self.Equality Choice`)
    (bind (_factions_exist _factions _member_communities _indies_exist _indy_communities) (`/Game/Scenarios/Shared/BlueprintsNonSerialized/SocietyUtils/BPFL_Cornerstone_Utils.Get Factions and Communities with Affinity` (struct :`Name` "Solidarity")))
    (if _factions_exist
      (for _array_element _factions
        (`PXPredefinedModifierUtils.SetPredefinedModifierActiveManualTarget` (`PXNationUtils.GetPlayerNation`) "/Game/Scenarios/Shared/BlueprintsSerialized/Quests/Demands/DA_PromiseBroken_CommunityTrust.DA_PromiseBroken_CommunityTrust" (`ActorComponent.GetOwner` (`.ReturnValue` (`PXFactionUtils.GetCommunityFromFaction` _array_element))) true))
      (for _array_element_2 _indy_communities :!label _label
        (`PXPredefinedModifierUtils.SetPredefinedModifierActiveManualTarget` (`PXNationUtils.GetPlayerNation`) "/Game/Scenarios/Shared/BlueprintsSerialized/Quests/Demands/DA_PromiseBroken_CommunityTrust.DA_PromiseBroken_CommunityTrust" (`ActorComponent.GetOwner` _array_element_2) true))
      (elif _indies_exist
        (goto _label)))
    (else
      (bind (_factions_exist_2 _factions_2 _member_communities_2 _indies_exist_2 _indy_communities_2) (`/Game/Scenarios/Shared/BlueprintsNonSerialized/SocietyUtils/BPFL_Cornerstone_Utils.Get Factions and Communities with Affinity` (struct :`Name` "Competition")))
      (if _factions_exist_2
        (for _array_element_3 _factions_2
          (`PXPredefinedModifierUtils.SetPredefinedModifierActiveManualTarget` (`PXNationUtils.GetPlayerNation`) "/Game/Scenarios/Shared/BlueprintsSerialized/Quests/Demands/DA_PromiseBroken_CommunityTrust.DA_PromiseBroken_CommunityTrust" (`ActorComponent.GetOwner` (`.ReturnValue` (`PXFactionUtils.GetCommunityFromFaction` _array_element_3))) true))
        (for _array_element_4 _indy_communities_2 :!label _label_2
          (`PXPredefinedModifierUtils.SetPredefinedModifierActiveManualTarget` (`PXNationUtils.GetPlayerNation`) "/Game/Scenarios/Shared/BlueprintsSerialized/Quests/Demands/DA_PromiseBroken_CommunityTrust.DA_PromiseBroken_CommunityTrust" (`ActorComponent.GetOwner` _array_element_4) true))
        (elif _indies_exist_2
          (goto _label_2))))))

(fn `Add success trust modifier`
  (if (`self.Equality Choice`)
    (bind (_factions_exist _factions _member_communities _indies_exist _indy_communities) (`/Game/Scenarios/Shared/BlueprintsNonSerialized/SocietyUtils/BPFL_Cornerstone_Utils.Get Factions and Communities with Affinity` (struct :`Name` "Solidarity")))
    (if _factions_exist
      (for _array_element _factions
        (`PXPredefinedModifierUtils.SetPredefinedModifierActiveManualTarget` (`PXNationUtils.GetPlayerNation`) "/Game/Scenarios/Shared/BlueprintsSerialized/Quests/Demands/DA_PromiseKept_CommunityTrust.DA_PromiseKept_CommunityTrust" (`ActorComponent.GetOwner` (`.ReturnValue` (`PXFactionUtils.GetCommunityFromFaction` _array_element))) true))
      (for _array_element_2 _indy_communities :!label _label
        (`PXPredefinedModifierUtils.SetPredefinedModifierActiveManualTarget` (`PXNationUtils.GetPlayerNation`) "/Game/Scenarios/Shared/BlueprintsSerialized/Quests/Demands/DA_PromiseKept_CommunityTrust.DA_PromiseKept_CommunityTrust" (`ActorComponent.GetOwner` _array_element_2) true))
      (elif _indies_exist
        (goto _label)))
    (else
      (bind (_factions_exist_2 _factions_2 _member_communities_2 _indies_exist_2 _indy_communities_2) (`/Game/Scenarios/Shared/BlueprintsNonSerialized/SocietyUtils/BPFL_Cornerstone_Utils.Get Factions and Communities with Affinity` (struct :`Name` "Competition")))
      (if _factions_exist_2
        (for _array_element_3 _factions_2
          (`PXPredefinedModifierUtils.SetPredefinedModifierActiveManualTarget` (`PXNationUtils.GetPlayerNation`) "/Game/Scenarios/Shared/BlueprintsSerialized/Quests/Demands/DA_PromiseKept_CommunityTrust.DA_PromiseKept_CommunityTrust" (`ActorComponent.GetOwner` (`.ReturnValue` (`PXFactionUtils.GetCommunityFromFaction` _array_element_3))) true))
        (for _array_element_4 _indy_communities_2 :!label _label_2
          (`PXPredefinedModifierUtils.SetPredefinedModifierActiveManualTarget` (`PXNationUtils.GetPlayerNation`) "/Game/Scenarios/Shared/BlueprintsSerialized/Quests/Demands/DA_PromiseKept_CommunityTrust.DA_PromiseKept_CommunityTrust" (`ActorComponent.GetOwner` _array_element_4) true))
        (elif _indies_exist_2
          (goto _label_2))))))

(fn `CanBeStarted`
  (returns (ReturnValue :type Boolean))
  (locals (District :type "PXDistrictComponent Object Reference") (HeatLevel :type "PXHeatLevelComponent Object Reference") (`Minimum number of housings` :type Integer :default 6) (`2 heat levels difference` :type Integer :default 40) (`Minimum number of cold housings` :type Integer :default 2))
  (bind _returnvalue (`PXNationUtils.GetPlayerMainCity`))
  (bind _returnvalue_2 (`PXDistrictUtils.GetDistrictWithTagFromCity` (`PXNationUtils.GetPlayerMainCity`) (struct :`TagDictionary` (struct :`(TagName` "District.Housing")) :`QueryTokenStream` "(0,1,1,1,0)" :`AutoDescription` " ANY( District.Housing )") true))
  (bind _returnvalue_3 (`PXDistrictUtils.GetDistrictWithTagFromCity` (`PXNationUtils.GetPlayerMainCity`) (struct :`TagDictionary` (struct :`(TagName` "District.Housing")) :`QueryTokenStream` "(0,1,1,1,0)" :`AutoDescription` " ANY( District.Housing )") true))
  (bind (_current_warmest_level _warmest_heat_balance _heat_component_warmest) (`/Game/Scenarios/Shared/BlueprintsNonSerialized/Cities/BPFL_CityUtils.Get Warmest Temperature Level District with Tag in City` _returnvalue_3))
  (bind (_current_coldest_level _coldest_heat_balance _heat_component_coldest) (`/Game/Scenarios/Shared/BlueprintsNonSerialized/Cities/BPFL_CityUtils.Get Coldest Temperature Level from District with Tag in City` _returnvalue_3))
  (if (not (`/Game/Scenarios/Main/BlueprintsNonSerialized/ScenarioFunctionLibrary/BPFL_S1_ScenarioFunctionLibrary.Is Nomads Scenario`))
    (`/Engine/EditorBlueprintResources/StandardMacros.IsValid` _returnvalue
      (:`Is Valid`
        (if (`PXBuildingUtils.HasBuildingOfTypeInCity` _returnvalue "/Game/Scenarios/Shared/Configs/Buildings/TheCouncilHall/DA_H_TheCouncilHall.DA_H_TheCouncilHall" true)
          (if (`/Game/Scenarios/Shared/BlueprintsNonSerialized/Policies/BPFL_PolicyUtils.IsPolicyActive` "/Game/Scenarios/Shared/Configs/Policies/Economy/AccessToHeat/DA_AccessToHeat_Chaos_Policy.DA_AccessToHeat_Chaos_Policy")
            (if (>= (`KismetArrayLibrary.Array_Length` _returnvalue_3) (`local.Minimum number of housings`))
              (if (and (`.ReturnValue` (`PXHeatManagementUtils.CompareHeatLevel` _heat_component_coldest "LessThanOrEqualTo" "/Game/Scenarios/Shared/Configs/Heat/HeatLevels/DA_HeatLevel_3_Cold.DA_HeatLevel_3_Cold")) (`.ReturnValue` (`PXHeatManagementUtils.CompareHeatLevel` _heat_component_warmest "GreaterThanOrEqualTo" "/Game/Scenarios/Shared/Configs/Heat/HeatLevels/DA_HeatLevel_4_Chilly.DA_HeatLevel_4_Chilly")))
                (if (and (>= (`KismetArrayLibrary.Array_Length` (`PXDistrictUtils.FilterDistrictsByHeatLevel` _returnvalue_3 null _current_coldest_level)) (`local.Minimum number of cold housings`)) (> (`KismetArrayLibrary.Array_Length` (`PXDistrictUtils.FilterDistrictsByHeatLevel` _returnvalue_3 _current_warmest_level)) 0))
                  (if (> (- _warmest_heat_balance _coldest_heat_balance) (`local.2 heat levels difference`))
                    (set `self.District for Tracker` (`KismetArrayLibrary.Array_Random` (`PXDistrictUtils.FilterDistrictsByHeatLevel` _returnvalue_2 null (`/Game/Scenarios/Shared/BlueprintsNonSerialized/Cities/BPFL_CityUtils.Get Coldest Temperature Level from District with Tag in City` _returnvalue_2))))
                    (return true))
                  (else
                    (return false)))
                (else
                  (return false)))
              (else
                (return false)))
            (else
              (return false))))))))

(fn `Get message defines`
  (returns (Map :type "Map of String to Text"))
  (bind _defines_map_merged (`/Game/Scenarios/Shared/BlueprintsNonSerialized/SocietyUtils/BPFL_Communication_Utils.Merge Defines` (`parent.Get message defines`) (`|MakeMap` "WEEKS" (`PXTextUtils.GameTimeToTextMostImportant` (`self.Duration`)) "EQUAL" (`PXPolicyType.IngameName` (`self.Equal heating policy`)) "PAID" (`PXPolicyType.IngameName` (`self.Paid heating policy`)))))
  (return _defines_map_merged))