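; Consequence story arc that follows up on the player's choice in the Equal Pay lens-first economy arc.
; HandleChoice waits on a story beat slot, then for choice 1 sends the StayFirmSmallLens lens without community art and waits for any response.
; Message defines extend the parent's with MERIT_FACTION, the community name of an affinity-selected commenter.
; Start eligibility adds no conditions beyond the parent check.
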(event `self.Handle Choice`
  (params (Selection :type Integer))
  (bind (_beat_type _lane_type) (`self.Get Story Beat Types`))
  (`PXAsyncWaitForStoryBeat.AsyncAction_WaitForStoryBeat` _beat_type _lane_type
    (:`Completed`
      (switch `int` (`self.Choice`)
        (:`1`
          (bind _decision (`self.Send Lens` (`self.StayFirm SmallLens`)))
          (`PXAsyncWaitForAnyChoice.AsyncAction_WaitForAnyChoice` _decision))))))

(fn `CanBeStarted`
  (returns (ReturnValue :type Boolean))
  (bind _returnvalue (`parent.CanBeStarted`))
  (if _returnvalue
    (return true)))

(fn `Get message defines`
  (returns (Map :type "Map of String to Text"))
  (bind (_exists _community) (`/Game/Scenarios/Shared/BlueprintsNonSerialized/SocietyUtils/BPFL_Cornerstone_Utils.Get X Affinity Commenter` (struct :`Name` "Competition") false))
  (bind _defines_map_merged (`/Game/Scenarios/Shared/BlueprintsNonSerialized/SocietyUtils/BPFL_Communication_Utils.Merge Defines` (`parent.Get message defines`) (`|MakeMap` "MERIT_FACTION" (`/Game/Scenarios/Shared/BlueprintsNonSerialized/Communities/BPFL_CommunityUtils.Get Community Name` _community))))
  (return _defines_map_merged))