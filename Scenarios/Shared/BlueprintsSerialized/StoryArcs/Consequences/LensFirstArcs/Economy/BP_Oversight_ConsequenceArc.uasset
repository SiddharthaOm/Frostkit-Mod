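; Consequence story arc for the Economy Oversight decision, following up on the player's earlier choice.
; Only choice 1 triggers a follow-up: it waits for a matching story beat and lane, then rechecks the core start conditions.
; If they pass, it sends the Compensate "Ghost" consequence message, targeting the closest district, and waits for any response.
; Start eligibility adds nothing beyond the parent check.
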(event `self.Handle Choice`
  (params (Selection :type Integer))
  (bind (_beat_type _lane_type) (`self.Get Story Beat Types`))
  (switch `int` (`PXDecision.GetSelectedChoice` (`self.Decision_0`))
    (:`1`
      (`PXAsyncWaitForStoryBeat.AsyncAction_WaitForStoryBeat` _beat_type _lane_type
        (:`Completed`
          (bind _returnvalue (`self.Consequence CanBeStarted Core`))
          (if _returnvalue
            (bind _decision (`/Game/Scenarios/Shared/BlueprintsNonSerialized/SocietyUtils/BPFL_Communication_Utils.Send Config Message` "/Game/Scenarios/Shared/Configs/Messages/Ghosts/Consequences/GhostOnly/New/DA_Oversight_Compensate_Consequence_Ghost.DA_Oversight_Compensate_Consequence_Ghost" null null null (`self.Get message defines`) null null (struct) true))
            (`PXAsyncWaitForAnyChoice.AsyncAction_WaitForAnyChoice` _decision)))))))

(fn `CanBeStarted`
  (returns (ReturnValue :type Boolean))
  (bind _returnvalue (`parent.CanBeStarted`))
  (if _returnvalue
    (return true)))