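; Economy consequence story arc for Self-Organisation, playing out escalating follow-up Lens messages after the player's initial "I see" or bribe choice.
; Each step waits for a story beat and a can-start check before messaging the closest district.
; The first two choices set flags that select the Alexei Stakhanov, Next Bribe or Slander message; Next Bribe can branch into Slander or Make Them Disappear.
; Message text reports the law as changed if either "I see" flag is set.
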(event `self.Handle Choice`
  (params (Selection :type Integer))
  (bind (_beat_type _lane_type) (`self.Get Story Beat Types`))
  (bind (_beat_type_2 _lane_type_2) (`self.Get Story Beat Types`))
  (bind (_beat_type_3 _lane_type_3) (`self.Get Story Beat Types`))
  (bind (_beat_type_4 _lane_type_4) (`self.Get Story Beat Types`))
  (switch `int` Selection
    (:`0`
      (set `self.I see A` true))
    (:`1`
      (set `self.Bribe A` true)))
  (`PXAsyncWaitForStoryBeat.AsyncAction_WaitForStoryBeat` _beat_type _lane_type
    (:`Completed`
      (bind _returnvalue (`self.Consequence CanBeStarted Core`))
      (if _returnvalue
        (bind _decision (`/Game/Scenarios/Shared/BlueprintsNonSerialized/SocietyUtils/BPFL_Communication_Utils.Send Config Message` "/Game/Scenarios/Shared/Configs/Messages/Lenses/Consequences/ConsequenceLenses/Economy/SelfOrganisation/DA_SelfOrganisation_NextDemand_ConsequenceArc_Lens.DA_SelfOrganisation_NextDemand_ConsequenceArc_Lens" null null null (`self.Get message defines`) null null (struct) true))
        (bind _output_get (set `self.Decision_0` _decision))
        (`PXAsyncWaitForAnyChoice.AsyncAction_WaitForAnyChoice` _output_get
          (:`Completed`
            (switch `int` (`PXDecision.GetSelectedChoice` (`self.Decision_0`))
              (:`0`
                (set `self.I see B` true))
              (:`1`
                (set `self.Bribe B` true)))
            (`self.Check and setup previous choices`)
            (`PXAsyncWaitForStoryBeat.AsyncAction_WaitForStoryBeat` _beat_type_2 _lane_type_2
              (:`Completed`
                (bind _returnvalue_2 (`self.Consequence CanBeStarted Core`))
                (if _returnvalue_2
                  (bind _decision_2 (`/Game/Scenarios/Shared/BlueprintsNonSerialized/SocietyUtils/BPFL_Communication_Utils.Send Config Message` (select `/Game/Scenarios/Shared/BlueprintsSerialized/StoryArcs/Consequences/LensFirstArcs/Economy/ENUM_SelfOrganisationConsequenceArc` (`self.SelfOrganisationEnum`) :`NewEnumerator0` (`self.Alexei Stakhanov Lens`) :`NewEnumerator1` (`self.NextBribe Lens`) :`NewEnumerator2` (`self.Slander Lens`) :!type "PXCommunicationChannelMessage Soft Object Reference") null null null (`self.Get message defines`) null null (struct) true))
                  (set `self.Decision_1` _decision_2)
                  (if (`|EnumEquality` (`self.SelfOrganisationEnum`) "NewEnumerator1")
                    (`PXAsyncWaitForAnyChoice.AsyncAction_WaitForAnyChoice` (`self.Decision_1`)
                      (:`Completed`
                        (switch `int` (`PXDecision.GetSelectedChoice` (`self.Decision_1`))
                          (:`1`
                            (`PXAsyncWaitForStoryBeat.AsyncAction_WaitForStoryBeat` _beat_type_3 _lane_type_3
                              (:`Completed`
                                (bind _returnvalue_3 (`self.Consequence CanBeStarted Core`))
                                (if _returnvalue_3
                                  (bind _decision_3 (`/Game/Scenarios/Shared/BlueprintsNonSerialized/SocietyUtils/BPFL_Communication_Utils.Send Config Message` (`self.Slander Lens`) null null null (`self.Get message defines`) null null (struct) true))
                                  (`PXAsyncWaitForAnyChoice.AsyncAction_WaitForAnyChoice` _decision_3)))))
                          (:`2`
                            (`PXAsyncWaitForStoryBeat.AsyncAction_WaitForStoryBeat` _beat_type_4 _lane_type_4
                              (:`Completed`
                                (bind _returnvalue_4 (`self.Consequence CanBeStarted Core`))
                                (if _returnvalue_4
                                  (bind _decision_4 (`/Game/Scenarios/Shared/BlueprintsNonSerialized/SocietyUtils/BPFL_Communication_Utils.Send Config Message` "/Game/Scenarios/Shared/Configs/Messages/Lenses/Consequences/ConsequenceLenses/Economy/SelfOrganisation/DA_SelfOrganisation_MakeThemDisappear_ConsequenceArc_Lens.DA_SelfOrganisation_MakeThemDisappear_ConsequenceArc_Lens" null null null (`self.Get message defines`) null null (struct) true))
                                  (`PXAsyncWaitForAnyChoice.AsyncAction_WaitForAnyChoice` _decision_4))))))))
                    (else
                      (`PXAsyncWaitForAnyChoice.AsyncAction_WaitForAnyChoice` (`self.Decision_1`)))))))))))))

(fn `Check and setup previous choices`
  (if (and (`self.I see A`) (`self.I see B`))
    (set `self.SelfOrganisationEnum` "NewEnumerator0")
    (return)
    (elif (or (and (`self.Bribe A`) (`self.Bribe B`)) (and (`self.I see A`) (`self.Bribe B`)))
      (set `self.SelfOrganisationEnum` "NewEnumerator1")
      (return)
      (elif (and (`self.Bribe A`) (`self.I see B`))
        (set `self.SelfOrganisationEnum` "NewEnumerator2")
        (return)))))

(fn `Get message defines`
  (returns (Map :type "Map of String to Text"))
  (locals (`local message defines` :type "Map of String to Text"))
  (`BlueprintMapLibrary.Map_Add` (`local.local message defines`) "GAMEPLAY INFO" (select `bool` (or (`self.I see A`) (`self.I see B`)) :`false` (`|FormatText` "The law was not changed") :`true` (`|FormatText` "The law was changed")))
  (bind _defines_map_merged (`/Game/Scenarios/Shared/BlueprintsNonSerialized/SocietyUtils/BPFL_Communication_Utils.Merge Defines` (`parent.Get message defines`) (`local.local message defines`)))
  (return _defines_map_merged))