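; Consequence story arc for the city's stimulants and opioids drug problem.
; A choice activates low and high death cyclical events, then starts a main quest to destroy all buildings of the stimulant type, opioid type or both.
; The quest result picks a success or fail dialog and, after a story beat, the matching small lens message.
; CanBeStarted relies only on the parent check; CheckOtherDrugsArcs is not called here.
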(event `self.Handle Choice`
  (params (Selection :type Integer))
  (bind (_beat_type _lane_type) (`self.Get Story Beat Types`))
  (set `self.Selection` Selection)
  (`PXCyclicalEventUtils.SetCyclicalEventActiveInCity` (`PXNationUtils.GetPlayerMainCity`) "/Game/Scenarios/Shared/Configs/CyclicalEvents/PoliciesEffects/DA_OpioidsAndStimulans_Low_Death_CyclicalEvent.DA_OpioidsAndStimulans_Low_Death_CyclicalEvent")
  (`PXCyclicalEventUtils.SetCyclicalEventActiveInCity` (`PXNationUtils.GetPlayerMainCity`) "/Game/Scenarios/Shared/Configs/CyclicalEvents/PoliciesEffects/DA_OpioidsAndStimulans_High_Death_CyclicalEvent.DA_OpioidsAndStimulans_High_Death_CyclicalEvent")
  (switch `int` (`self.Selection`)
    (:`0`
      _)
    (:`1`
      _)
    (:`2`
      _))
  (bind _returnvalue (`PXQuestUtils.StartQuestInPlace` "Get rid of the drug problem" "" (struct :`ScaledTicks` 84000) "MainQuest" "DebugQuestName" true))
  (set `self.Quest` _returnvalue)
  (switch `int` (`self.Selection`)
    (:`0`
      (`PXQuestUtils.AddBuildingQuestObjective` (make `PXObjectiveParameters` (`|FormatText` "Destory all {BUILDING}" (`PXBuildingType.IngameName` (`self.Building Type`))) "" false 1 null (`self.Quest`)) (make `PXBuildingObjectiveParameters` (`self.Building Type`) "Destroy" (`KismetArrayLibrary.Array_Length` (`PXBuildingUtils.GetBuildingsOfTypeFromCity` (`PXNationUtils.GetPlayerMainCity`) (`self.Building Type`))) null null null _ false)))
    (:`1`
      (`PXQuestUtils.AddBuildingQuestObjective` (make `PXObjectiveParameters` (`|FormatText` "Destory all {BUILDING}" (`PXBuildingType.IngameName` (`self.Building Type 2`))) "" false 1 null (`self.Quest`)) (make `PXBuildingObjectiveParameters` (`self.Building Type 2`) "Destroy" (`KismetArrayLibrary.Array_Length` (`PXBuildingUtils.GetBuildingsOfTypeFromCity` (`PXNationUtils.GetPlayerMainCity`) (`self.Building Type 2`))) null null null _ false)))
    (:`2`
      (`PXQuestUtils.AddBuildingQuestObjective` (make `PXObjectiveParameters` (`|FormatText` "Destory all {BUILDING}" (`PXBuildingType.IngameName` (`self.Building Type`))) "" false 1 null (`self.Quest`)) (make `PXBuildingObjectiveParameters` (`self.Building Type`) "Destroy" (`KismetArrayLibrary.Array_Length` (`PXBuildingUtils.GetBuildingsOfTypeFromCity` (`PXNationUtils.GetPlayerMainCity`) (`self.Building Type`))) null null null _ false))
      (`PXQuestUtils.AddBuildingQuestObjective` (make `PXObjectiveParameters` (`|FormatText` "Destory all {BUILDING}" (`PXBuildingType.IngameName` (`self.Building Type 2`))) "" false 1 null (`self.Quest`)) (make `PXBuildingObjectiveParameters` (`self.Building Type 2`) "Destroy" (`KismetArrayLibrary.Array_Length` (`PXBuildingUtils.GetBuildingsOfTypeFromCity` (`PXNationUtils.GetPlayerMainCity`) (`self.Building Type 2`))) null null null _ false))))
  (bind _succeeded (`PXAsyncWaitForQuest.AsyncAction_WaitForQuest` (`self.Quest`))
    (:`Completed`
      (set `self.Succeeded` _succeeded)
      (`PXAsyncOpenPredefinedDialog.AsyncAction_OpenPredefinedDialog` (select `bool` (`self.Succeeded`) :`false` (select `int` (`self.Selection`) :`0` (`self.Dialog Stimulants Fail`) :`1` (`self.Dialog Opioids Fail`) :`2` (`self.Dialog Opioids and Stimulants Fail`)) :`true` (select `int` (`self.Selection`) :`0` (`self.Dialog Stimulants Success`) :`1` (`self.Dialog Opioids Success`) :`2` (`self.Dialog Opioids and Stimulants Success`))) (`self.Get message defines`)
        (:`Completed`
          (`PXAsyncWaitForStoryBeat.AsyncAction_WaitForStoryBeat` _beat_type _lane_type
            (:`Completed`
              (bind _decision (`/Game/Scenarios/Shared/BlueprintsNonSerialized/SocietyUtils/BPFL_Communication_Utils.Send Config Message` (select `bool` (`self.Succeeded`) :`false` "/Game/Scenarios/Shared/Configs/Messages/Lenses/Consequences/ConsequenceLenses/Economy/DrugsManufactory/DA_StimulantsAndOpioids_Fail_Consequence_SmallLens.DA_StimulantsAndOpioids_Fail_Consequence_SmallLens" :`true` "/Game/Scenarios/Shared/Configs/Messages/Lenses/Consequences/ConsequenceLenses/Economy/DrugsManufactory/DA_StimulantsAndOpioids_Success_Consequence_SmallLens.DA_StimulantsAndOpioids_Success_Consequence_SmallLens" :!type "PXCommunicationChannelMessage Soft Object Reference") null null null (`self.Get message defines`) null null (struct) true))
              (`PXAsyncWaitForAnyChoice.AsyncAction_WaitForAnyChoice` _decision))))))))

(fn `CanBeStarted`
  (returns (ReturnValue :type Boolean))
  (bind _returnvalue (`parent.CanBeStarted`))
  (if _returnvalue
    (return true)
    (else
      (return false))))

(fn `Check other Drugs Arcs`
  (returns (ReturnValue :type Boolean))
  (return (or (or (`PXStoryUtils.IsAnyStoryArcOfClassInStatus` "/Game/Scenarios/Shared/BlueprintsSerialized/StoryArcs/Consequences/LensFirstArcs/Economy/BP_StimulantsManufactory_ConsequenceArc.BP_StimulantsManufactory_ConsequenceArc_C" "Active") (`PXStoryUtils.IsAnyStoryArcOfClassInStatus` "/Game/Scenarios/Shared/BlueprintsSerialized/StoryArcs/Consequences/LensFirstArcs/Economy/BP_StimulantsManufactory_ConsequenceArc.BP_StimulantsManufactory_ConsequenceArc_C" "Finished")) (or (`PXStoryUtils.IsAnyStoryArcOfClassInStatus` "/Game/Scenarios/Shared/BlueprintsSerialized/StoryArcs/Consequences/LensFirstArcs/Economy/BP_OpioidsManufactory_ConsequenceArc.BP_OpioidsManufactory_ConsequenceArc_C" "Active") (`PXStoryUtils.IsAnyStoryArcOfClassInStatus` "/Game/Scenarios/Shared/BlueprintsSerialized/StoryArcs/Consequences/LensFirstArcs/Economy/BP_OpioidsManufactory_ConsequenceArc.BP_OpioidsManufactory_ConsequenceArc_C" "Finished")))))

(fn `Get message defines`
  (returns (Map :type "Map of String to Text"))
  (`BlueprintMapLibrary.Map_Add` (`self.Local Defines Map`) "BUILDING_2" (`PXBuildingType.IngameName` (`self.Building Type 2`)))
  (bind _defines_map_merged (`/Game/Scenarios/Shared/BlueprintsNonSerialized/SocietyUtils/BPFL_Communication_Utils.Merge Defines` (`self.Local Defines Map`) (`parent.Get message defines`)))
  (return _defines_map_merged))