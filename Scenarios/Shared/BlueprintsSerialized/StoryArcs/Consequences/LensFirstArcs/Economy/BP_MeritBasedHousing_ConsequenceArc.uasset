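; Story arc Blueprint for the Merit-Based Housing consequence, filed under the Economy lens-first arcs.
; Start event and start eligibility defer to the parent class, with no extra conditions added.
; A separate check reports whether the main city's required shelter exceeds fulfilled shelter by more than a small fixed margin, though neither override calls it.
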(event `self.OnStarted`
  (`parent.OnStarted`))

(fn `CanBeStarted`
  (returns (ReturnValue :type Boolean))
  (bind _returnvalue (`parent.CanBeStarted`))
  (if _returnvalue
    (return true)))

(fn `Check Shelter Need`
  (returns (ReturnValue :type Boolean))
  (bind _returnvalue (`PXNationUtils.GetPlayerMainCity`))
  (return (> (`PXNeedUtils.GetCityNeedRequired` _returnvalue "/Game/Scenarios/Shared/Configs/Needs/Needs/DA_Shelter.DA_Shelter") (+ (`PXNeedUtils.GetCityNeedFulfilled` _returnvalue "/Game/Scenarios/Shared/Configs/Needs/Needs/DA_Shelter.DA_Shelter") 10))))