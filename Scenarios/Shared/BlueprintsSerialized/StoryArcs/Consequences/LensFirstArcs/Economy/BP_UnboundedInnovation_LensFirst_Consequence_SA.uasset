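; Consequence story arc for the Unbounded Innovation economy lens-first arc, following up on the player's choice about fines.
; After a choice it waits for a story beat, sends the StayFirm lens, then sends the FinesOrFirmGhost message using the closest district, re-checking eligibility before each send.
; The first option at either decision sets Fines, which feeds the message text defines alongside an affinity-matched faction name.
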(event `self.Handle Choice`
  (params (Selection :type Integer))
  (bind (_beat_type _lane_type) (`self.Get Story Beat Types`))
  (switch `int` Selection
    (:`1`
      (set `self.Fines?` true))
    (:`2`
      _))
  (`PXAsyncWaitForStoryBeat.AsyncAction_WaitForStoryBeat` _beat_type _lane_type
    (:`Completed`
      (bind _returnvalue (`self.Consequence CanBeStarted Core`))
      (if _returnvalue
        (bind _decision (`self.Send Lens` (`self.Stay Firm Lens`)))
        (bind _output_get (set `self.Decision_0` _decision))
        (`PXAsyncWaitForAnyChoice.AsyncAction_WaitForAnyChoice` _output_get
          (:`Completed`
            (switch `int` (`PXDecision.GetSelectedChoice` (`self.Decision_0`))
              (:`1`
                (set `self.Fines?` true))
              (:`2`
                _))
            (bind _returnvalue_2 (`self.Consequence CanBeStarted Core`))
            (if _returnvalue_2
              (bind _decision_2 (`/Game/Scenarios/Shared/BlueprintsNonSerialized/SocietyUtils/BPFL_Communication_Utils.Send Config Message` (`self.Fines or Firm Ghost`) (`self.Get District for Lens Tracker`) null null (`self.Get message defines`) null null (struct) true))
              (`PXAsyncWaitForAnyChoice.AsyncAction_WaitForAnyChoice` _decision_2))))))))

(fn `Get message defines`
  (returns (Map :type "Map of String to Text"))
  (bind _defines_map_merged (`/Game/Scenarios/Shared/BlueprintsNonSerialized/SocietyUtils/BPFL_Communication_Utils.Merge Defines` (`parent.Get message defines`) (`|MakeMap` "FINES" (select `bool` (`self.Fines?`) :`true` (`self.FINES_YES`)) "EQUALITY_FACTION" (`PXFactionType.IngameName` (`/Game/Scenarios/Shared/BlueprintsNonSerialized/SocietyUtils/BPFL_StoryArc_Utils.Get existing faction with affinity` (struct :`Name` "Solidarity"))))))
  (return _defines_map_merged))