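; Consequence story arc for Efficiency Bounties in the Economy group, delivering a ghost message that reflects the player's earlier choice.
; HandleChoice waits for a story beat, checks that the consequence can still start, then sends the tone-down or stay-firm message to the closest district and waits for any choice.
; Message defines add a SPEAKER name from an affinity-based community commenter, with fallbacks, merged with the parent's defines.
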(event `self.Handle Choice`
  (params (Selection :type Integer))
  (bind (_beat_type _lane_type) (`self.Get Story Beat Types`))
  (set `self.Selection` Selection)
  (`PXAsyncWaitForStoryBeat.AsyncAction_WaitForStoryBeat` _beat_type _lane_type
    (:`Completed`
      (bind _returnvalue (`self.Consequence CanBeStarted Core`))
      (if _returnvalue
        (bind _decision (`/Game/Scenarios/Shared/BlueprintsNonSerialized/SocietyUtils/BPFL_Communication_Utils.Send Config Message` (select `int` (`self.Selection`) :`0` (`self.Tone Down Ghost`) :`1` (`self.Stay Firm Ghost`) :!type "PXCommunicationChannelMessage Soft Object Reference") null null null (`self.Get message defines`) null null (struct) true))
        (`PXAsyncWaitForAnyChoice.AsyncAction_WaitForAnyChoice` _decision)))))

(fn `Get message defines`
  (returns (Map :type "Map of String to Text"))
  (bind (_exists _community) (`/Game/Scenarios/Shared/BlueprintsNonSerialized/SocietyUtils/BPFL_Cornerstone_Utils.Get X Affinity Commenter` (struct :`Name` "Competition") true true))
  (`BlueprintMapLibrary.Map_Add` (`self.Local Define Map`) "SPEAKER" (`.first + last1` (`/Game/Scenarios/Shared/BlueprintsNonSerialized/FactionEmergence/BPFL_FactionEmergenceUtils.Get Community Ghost Speaker` (`PXCommunityComponent.GetCommunityType` _community))))
  (bind _defines_map_merged (`/Game/Scenarios/Shared/BlueprintsNonSerialized/SocietyUtils/BPFL_Communication_Utils.Merge Defines` (`parent.Get message defines`) (`self.Local Define Map`)))
  (return _defines_map_merged))