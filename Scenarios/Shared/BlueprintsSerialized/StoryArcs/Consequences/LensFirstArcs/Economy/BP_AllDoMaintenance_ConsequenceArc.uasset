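; Consequence story arc in the Economy lens-first set, tied by name to the "All Do Maintenance" outcome, supplying citizen complaint text about children.
; GetMessageDefines picks a quote matching the children policy (no childhood policy, apprenticeship or school) and merges it as KIDS with the parent's defines.
; CanBeStarted only defers to the parent.
; An older KidsLawText lookup by active law remains disconnected.
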(fn `CanBeStarted`
  (returns (ReturnValue :type Boolean))
  (bind _returnvalue (`parent.CanBeStarted`))
  (return _returnvalue))

(fn `Get message defines`
  (returns (Map :type "Map of String to Text"))
  (bind _returnvalue (`/Game/Scenarios/Shared/BlueprintsNonSerialized/SocietyUtils/BPFL_StoryArc_Utils.Get Children Based On Policy Tag` "‘Gotta do something with ‘em kids, don’t I? Or would ya rather they muck about?’ answered a widowed mother." "‘This is in line with Family Apprenticeship,’ asserts a father of five. ‘My lads shadow me all the time. How else are they supposed to learn?’" "‘School’s fine and dandy, but what are we supposed to do with them after hours?’ complained a couple of parents."))
  (`BlueprintMapLibrary.Map_Add` (`self.Local Defines Map`) "KIDS" _returnvalue)
  (bind _defines_map_merged (`/Game/Scenarios/Shared/BlueprintsNonSerialized/SocietyUtils/BPFL_Communication_Utils.Merge Defines` (`parent.Get message defines`) (`self.Local Defines Map`)))
  (return _defines_map_merged))