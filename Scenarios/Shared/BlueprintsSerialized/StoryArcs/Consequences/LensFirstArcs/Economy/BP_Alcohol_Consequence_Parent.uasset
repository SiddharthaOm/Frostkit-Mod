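; Parent story arc for the alcohol consequence, escalating through optional lens and foreshadowing ghost to a Prohibition lens that unlocks the policy.
; One choice starts a timed quest to pass it, with pass/fail dialogs and follow-up ghosts.
; If BoozeGuysCome, parliament events trigger a pre-vote lens with predicted outcome and pay a Heatnotes bribe when the vote fails.
; Donors who paid strike back if Prohibition later passes through the quest follow-up.
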(event `MoneyIfVoteFails`
  (`PXAsyncOpenPredefinedDialog.AsyncAction_OpenPredefinedDialog` "/Game/Scenarios/Shared/Configs/Messages/Dialogs/StoryArcs/DA_Alcohol_ConsequenceBribe.DA_Alcohol_ConsequenceBribe" (`|MakeMap` "X" (`KismetTextLibrary.Conv_IntToText` (`self.Bribe Amount`)))
    (:`Completed`
      (set `self.Booze Guys Gave Money` true)
      (bind _returnvalue (`PXStockpileUtils.TryChangeNationStockpile` (`PXNationUtils.GetPlayerNation`) "/Game/Scenarios/Shared/Configs/Resources/Types/DA_Core_Heatnotes.DA_Core_Heatnotes" (`self.Bribe Amount`)))
      (if _returnvalue
        (`PXCommunicationChannelsUtils.AddNotification` (make `PXNotificationData` "Normal" (`|FormatText` "{X} Heatnotes from anonymous donors" (`self.Bribe Amount`))))))))

(event `self.OnStarted`
  (bind (_beat_type _lane_type) (`self.Get Story Beat Types`))
  (bind (_beat_type_2 _lane_type_2) (`self.Get Story Beat Types`))
  (if (`self.Start with Lens?`)
    (bind _decision (`self.Send Lens` (`self.Lens Config`)))
    (bind _output_get (set `self.first decision` _decision))
    (`PXAsyncWaitForAnyChoice.AsyncAction_WaitForAnyChoice` _output_get
      (:`Completed`
        (`PXAsyncWaitForStoryBeat.AsyncAction_WaitForStoryBeat` _beat_type _lane_type
          (:`Completed`
            (bind _returnvalue (`self.Consequence CanBeStarted Core`))
            (if _returnvalue
              (bind _decision_2 (`/Game/Scenarios/Shared/BlueprintsNonSerialized/SocietyUtils/BPFL_Communication_Utils.Send Config Message` (`self.Foreshadowing Ghost`) (`self.Get District for Lens Tracker`) null null (`self.Get message defines`) null null (struct) true :!label _label))
              (bind _output_get_2 (set `self.ghost decision` _decision_2))
              (`PXAsyncWaitForAnyChoice.AsyncAction_WaitForAnyChoice` _output_get_2
                (:`Completed`
                  (`PXAsyncWaitForStoryBeat.AsyncAction_WaitForStoryBeat` _beat_type_2 _lane_type_2
                    (:`Completed`
                      (bind _returnvalue_2 (`self.Consequence CanBeStarted Core`))
                      (if _returnvalue_2
                        (bind _decision_3 (`self.Send Lens` (`self.Prohibition Lens`)))
                        (bind _output_get_3 (set `self.Decision` _decision_3))
                        (`PXAsyncWaitForAnyChoice.AsyncAction_WaitForAnyChoice` _output_get_3
                          (:`Completed`
                            (`PXUnlockUtils.SetUnlockActive` (`PXNationUtils.GetPlayerNation`) "/Game/Scenarios/Shared/Configs/Unlocks/CL/DA_Prohibition.DA_Prohibition" true)
                            (if (`self.Booze Guys Come`)
                              (add `PXParliamentSubsystem.ParliamentAgendaAddedEvent` (subsystem `PXParliamentSubsystem`) (`|CreateDelegate` :!event `New Modal Lens When Proposed`)))
                            (switch `int` (`PXDecision.GetSelectedChoice` (`self.Decision`))
                              (:`0`
                                (bind _returnvalue_3 (`PXQuestUtils.StartQuestInPlace` (`|FormatText` "Solve Alcohol Problem") "" (`self.Duration for Prohibition Quest`) "MainQuest" "DebugQuestName" true))
                                (bind _output_get_4 (set `self.prohibition quest` _returnvalue_3))
                                (`PXQuestUtils.AddPolicyQuestObjective` (make `PXObjectiveParameters` (`|FormatText` "Pass {POLICY}" (`PXPolicyType.IngameName` (`self.Prohibition Policy`))) "" false 1 null _output_get_4) (make `PXPolicyObjectiveParameters` (`self.Prohibition Policy`)))))))))))))))))
    (else
      (goto _label))))

(event `self.OnFinished`
  (bind (_beat_type _lane_type) (`self.Get Story Beat Types`))
  (bind (_beat_type_2 _lane_type_2) (`self.Get Story Beat Types`))
  (`parent.OnFinished`)
  (bind _prohibition_quest (`self.prohibition quest`)
    (:`then`
      (bind _succeeded (`PXAsyncWaitForQuest.AsyncAction_WaitForQuest` _prohibition_quest)
        (:`Completed`
          (if _succeeded
            (`PXAsyncOpenPredefinedDialog.AsyncAction_OpenPredefinedDialog` (`self.Prohibition Quest Pass Dialog`) (`|MakeMap` "POLICY" (`PXPolicyType.IngameName` (`self.Prohibition Policy`)))
              (:`Completed`
                ;[1 1 1] Booze Guys Come Back if you ever pass Prohibition
                (if (`self.Booze Guys Gave Money`) :!label _label_2
                  (`PXAsyncWaitForStoryBeat.AsyncAction_WaitForStoryBeat` _beat_type_2 _lane_type_2
                    (:`Completed`
                      (`/Game/Scenarios/Shared/BlueprintsNonSerialized/SocietyUtils/BPFL_Communication_Utils.Send Config Message` (`self.Booze Guys strike back smallens`) (`self.Get District for Lens Tracker`) null null (`|MakeMap` "POLICY" (`PXPolicyType.IngameName` (`self.Prohibition Policy`))) null null (struct) true))))))
            (else
              (`PXAsyncOpenPredefinedDialog.AsyncAction_OpenPredefinedDialog` (`self.Prohibition Quest Fail Dialog`) (`|MakeMap` "POLICY" (`PXPolicyType.IngameName` (`self.Prohibition Policy`)))
                (:`Completed`
                  (`|ExecutionSequence`
                    (:`then_0`
                      (`PXAsyncWaitForPolicyPassed.AsyncAction_WaitForPolicyPassed` (`self.Prohibition Policy`)
                        (:`Completed`
                          (goto _label_2))))
                    (:`then_1`
                      (`PXAsyncWaitForStoryBeat.AsyncAction_WaitForStoryBeat` _beat_type _lane_type :!label _label_3
                        (:`Completed`
                          (if (not (`/Game/Scenarios/Shared/BlueprintsNonSerialized/Policies/BPFL_PolicyUtils.IsPolicyActive` (`self.Prohibition Policy`)))
                            (bind _decision (`self.Send Ghost` (`self.No Prohibition Ghost`)))
                            (`PXAsyncWaitForAnyChoice.AsyncAction_WaitForAnyChoice` _decision)))))))))))))
    (:`else`
      (`PXAsyncWaitForDurationPassed.AsyncAction_WaitForDurationPassed` (`self.Wait Before Booze Ghost`)
        (:`Completed`
          (goto _label_3))))))

(fn `CanBeStarted`
  (returns (ReturnValue :type Boolean))
  (if (`PXStoryUtils.IsAnyStoryArcOfClassInStatus` (`self.Companion Arc`) "Inactive")
    (bind _returnvalue (`parent.CanBeStarted`))
    (return _returnvalue)))

(fn `Community for Art + Defines`
  (returns (`Community for art` :type "PXCommunityType Object Reference") (`Community component` :type "PXCommunityComponent Object Reference"))
  (bind (_community_for_art _community_component) (`parent.Community for Art + Defines`))
  (return _community_for_art _community_component))

(fn `Get message defines`
  (returns (Map :type "Map of String to Text"))
  (`BlueprintMapLibrary.Map_Add` (`self.Local Defines Map`) "X" (`KismetTextLibrary.Conv_IntToText` (`PXTimeSubsystem.GetTotalWeeks` (`self.Duration for Prohibition Quest`))))
  (bind _defines_map_merged (`/Game/Scenarios/Shared/BlueprintsNonSerialized/SocietyUtils/BPFL_Communication_Utils.Merge Defines` (`parent.Get message defines`) (`self.Local Defines Map`)))
  (return _defines_map_merged))

(fn `Modal Lens When Proposed`
  (params (parliament :type "PXParliamentComponent Object Reference") (NewPhase :type "EPXSessionPhase Enum" :default "NONE"))
  (bind _returnvalue (`PXParliamentUtils.GetCurrentPolicyFromAgenda`))
  (if (and (== _returnvalue (`self.Prohibition Policy`)) (`|EnumEquality` NewPhase "Negotiations"))
    (bind (_percommunityresult _returnvalue_2) (`PXParliamentSubsystem.PredictVote` (subsystem `PXParliamentSubsystem`) parliament _returnvalue))
    (bind _defines_map_merged (`/Game/Scenarios/Shared/BlueprintsNonSerialized/SocietyUtils/BPFL_Communication_Utils.Merge Defines` (`self.Get message defines`) (`|MakeMap` "VOTE_PREDICTION" (select `bool` (> (break `PXVoteResultData` _returnvalue_2) (`.NayCount` (break `PXVoteResultData` _returnvalue_2))) :`false` (`|FormatText` "VOTE_PREDICTION: prohibition will not pass") :`true` (`|FormatText` "VOTE_PREDICTION: prohibition will pass ")))))
    (bind _decision (`/Game/Scenarios/Shared/BlueprintsNonSerialized/SocietyUtils/BPFL_Communication_Utils.Send Config Message` (`self.Before Vote ModalLens`) null null null _defines_map_merged null null (struct) true))
    (set `self.before vote decision` _decision)
    (remove `PXParliamentSubsystem.ParliamentPhaseChangedEvent` (subsystem `PXParliamentSubsystem`) (`|CreateDelegate` :!event `Modal Lens When Proposed`))
    (add `PXParliamentSubsystem.VoteFinishedEvent` (subsystem `PXParliamentSubsystem`) (`|CreateDelegate` :!event `Quest Ends When Vote Finishes`))))

(fn `New Modal Lens When Proposed`
  (params (parliament :type "PXParliamentComponent Object Reference") (policy :type "PXPolicyType Object Reference"))
  (if (== policy (`self.Prohibition Policy`))
    (bind (_percommunityresult _returnvalue) (`PXParliamentSubsystem.PredictVote` (subsystem `PXParliamentSubsystem`) parliament policy))
    (bind _defines_map_merged (`/Game/Scenarios/Shared/BlueprintsNonSerialized/SocietyUtils/BPFL_Communication_Utils.Merge Defines` (`self.Get message defines`) (`|MakeMap` "VOTE_PREDICTION" (select `bool` (> (break `PXVoteResultData` _returnvalue) (`.NayCount` (break `PXVoteResultData` _returnvalue))) :`false` (`|FormatText` "VOTE_PREDICTION: prohibition will not pass") :`true` (`|FormatText` "VOTE_PREDICTION: prohibition will pass ")))))
    (bind _decision (`/Game/Scenarios/Shared/BlueprintsNonSerialized/SocietyUtils/BPFL_Communication_Utils.Send Config Message` (`self.Before Vote ModalLens`) null null null _defines_map_merged null null (struct) true))
    (set `self.before vote decision` _decision)
    (remove `PXParliamentSubsystem.ParliamentAgendaAddedEvent` (subsystem `PXParliamentSubsystem`) (`|CreateDelegate` :!event `New Modal Lens When Proposed`))
    (add `PXParliamentSubsystem.VoteFinishedEvent` (subsystem `PXParliamentSubsystem`) (`|CreateDelegate` :!event `Quest Ends When Vote Finishes`))))

(fn `Quest Ends When Vote Finishes`
  (params (parliament :type "PXParliamentComponent Object Reference") (affectedPolicy :type "PXPolicyType Object Reference") (results :type "PXVoteResultData Structure"))
  (if (== affectedPolicy (`self.Prohibition Policy`))
    (remove `PXParliamentSubsystem.VoteFinishedEvent` (subsystem `PXParliamentSubsystem`) (`|CreateDelegate` :!event `Quest Ends When Vote Finishes`))
    (if (not (>= (`.AyeCount` (break `PXVoteResultData` results)) 51))
      (`self.MoneyIfVoteFails`))))