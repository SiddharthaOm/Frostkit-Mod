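; Story arc consequence for the lens-first Mandatory Procreation population arc, delivering follow-up messages after the player's earlier choice.
; HandleChoice sends both handled selections down one path: wait for a story beat, then send LeaveThemBe or StrikeADeal based on Choice, with community context and closest-district targeting.
; A response of 1 waits for another beat, then sends LeaveThemBe and waits for any choice.
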(event `self.Handle Choice`
  (params (Selection :type Integer))
  (bind (_beat_type _lane_type) (`self.Get Story Beat Types`))
  (bind (_beat_type_2 _lane_type_2) (`self.Get Story Beat Types`))
  (switch `int` Selection
    (:`1`
      _)
    (:`2`
      _))
  (`PXAsyncWaitForStoryBeat.AsyncAction_WaitForStoryBeat` _beat_type_2 _lane_type_2
    (:`Completed`
      (bind _decision (`/Game/Scenarios/Shared/BlueprintsNonSerialized/SocietyUtils/BPFL_Communication_Utils.Send Config Message` (select `int` (`self.Choice`) :`0` null :`1` (`self.Leave Them Be`) :`2` (`self.Strike A Deal`) :!type "PXCommunicationChannelMessage Soft Object Reference") null (`.Community component` (`self.Community for Art + Defines`)) null (`self.Get message defines`) null null (struct) true))
      (bind _choice (`PXAsyncWaitForChoice.AsyncAction_WaitForChoice` _decision)
        (:`Completed`
          (switch `int` _choice
            (:`1`
              (`PXAsyncWaitForStoryBeat.AsyncAction_WaitForStoryBeat` _beat_type _lane_type
                (:`Completed`
                  (bind _decision_2 (`/Game/Scenarios/Shared/BlueprintsNonSerialized/SocietyUtils/BPFL_Communication_Utils.Send Config Message` (`self.Leave Them Be`) null (`.Community component` (`self.Community for Art + Defines`)) null (`self.Get message defines`) null null (struct) true))
                  (`PXAsyncWaitForAnyChoice.AsyncAction_WaitForAnyChoice` _decision_2))))))))))