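; Story arc consequence of the Secret Police lens-first Charter arc, startable when exactly two factions are present in the main city.
; It casts the lowest-standing faction's community as the opposition for message text and art.
; Any choice enables a tension modifier, then either starts a city cyclical event or sends a delayed investigation Lens.
; That Lens either clears the tension and later sends a blame-militia Ghost, or starts the cyclical event.
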(event `self.OnStarted`
  (`self.Setup Factions`)
  (`parent.OnStarted`))

(event `self.Handle Choice`
  (params (Selection :type Integer))
  (bind (_beat_type _lane_type) (`self.Get Story Beat Types`))
  (bind (_beat_type_2 _lane_type_2) (`self.Get Story Beat Types`))
  (`PXPredefinedModifierUtils.SetPredefinedModifierActive` (`PXNationUtils.GetPlayerNation`) (`self.Tension modifier`) true)
  (switch `int` Selection
    (:`0`
      (`PXAsyncWaitForStoryBeat.AsyncAction_WaitForStoryBeat` _beat_type_2 _lane_type_2
        (:`Completed`
          (bind _decision (`self.Send Lens` (`self.Investigate Lens`)))
          (bind _choice (`PXAsyncWaitForChoice.AsyncAction_WaitForChoice` _decision)
            (:`Completed`
              (switch `int` _choice
                (:`0`
                  (`PXPredefinedModifierUtils.SetPredefinedModifierActive` (`PXNationUtils.GetPlayerNation`) (`self.Tension modifier`))
                  (`PXAsyncWaitForStoryBeat.AsyncAction_WaitForStoryBeat` _beat_type _lane_type
                    (:`Completed`
                      (bind _decision_2 (`self.Send Ghost` (`self.Blame militia ghost`)))
                      (`PXAsyncWaitForAnyChoice.AsyncAction_WaitForAnyChoice` _decision_2))))
                (:`1`
                  (`PXCyclicalEventUtils.SetCyclicalEventActiveInCity` (`PXNationUtils.GetPlayerMainCity`) (`self.Cyclical Event`)))))))))
    (:`1`
      (`PXCyclicalEventUtils.SetCyclicalEventActiveInCity` (`PXNationUtils.GetPlayerMainCity`) (`self.Cyclical Event`)))))

(fn `CanBeStarted`
  (returns (ReturnValue :type Boolean))
  (bind _returnvalue (`parent.CanBeStarted`))
  (if _returnvalue
    (if (== (`KismetArrayLibrary.Array_Length` (`/Game/Scenarios/Shared/BlueprintsNonSerialized/SocietyUtils/BPFL_StoryArc_Utils.Get Factions with Presence In Main City`)) 2)
      (`self.Setup Factions`)
      (return true))))

(fn `Community for Art + Defines`
  (returns (`Community for art` :type "PXCommunityType Object Reference") (`Community component` :type "PXCommunityComponent Object Reference"))
  (bind _opposition_f_action (`self.opposition f action`))
  (return (`PXCommunityComponent.GetCommunityType` _opposition_f_action) _opposition_f_action))

(fn `Get message defines`
  (returns (Map :type "Map of String to Text"))
  (bind _opposition_f_action (`self.opposition f action`))
  (bind _defines_map_merged (`/Game/Scenarios/Shared/BlueprintsNonSerialized/SocietyUtils/BPFL_Communication_Utils.Merge Defines` (`parent.Get message defines`) (`|MakeMap` "OPPOSITION_FACTION" (`/Game/Scenarios/Shared/BlueprintsNonSerialized/Communities/BPFL_CommunityUtils.Get Community Name` _opposition_f_action) "OPPOSITION_FACTION_MEMBER" (`BlueprintMapLibrary.Map_Find` (`PXCommunityType.MemberNames` (`PXCommunityComponent.GetCommunityType` _opposition_f_action)) "Masculine"))))
  (return _defines_map_merged))

(fn `Setup Factions`
  (bind _faction_with_lowest_standing (`/Game/Scenarios/Shared/BlueprintsNonSerialized/FactionEmergence/BPFL_FactionWarUtils.Get Faction with Lowest Standing`))
  (bind (_outfound _returnvalue) (`PXFactionUtils.GetCommunityFromFaction` _faction_with_lowest_standing))
  (`/Engine/EditorBlueprintResources/StandardMacros.IsValid` _faction_with_lowest_standing
    (:`Is Valid`
      (if _outfound
        (set `self.opposition f action` _returnvalue)))))