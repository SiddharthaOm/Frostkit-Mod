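; Early-game consequence story arc for waste repurposing, which plays character barks in the player's city after a choice.
; On the first choice, it picks a random building of the configured type in the main city, active or not, to supply the district.
; It then plays the arc's bark set there, with both generated speakers drawn from the community type used for art.
; The start check simply passes through the parent's result.
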(fn `CanBeStarted`
  (returns (ReturnValue :type Boolean))
  (bind _returnvalue (`parent.CanBeStarted`))
  (if _returnvalue
    (return true)
    (else
      (return false))))

(fn `Handle Choice`
  (params (Selection :type Integer))
  (bind (_outfound _returnvalue) (`PXCommunityUtils.GetCommunityOfCommunityType` (`self.Community for art`)))
  (switch `int` Selection
    (:`0`
      (bind _returnvalue_2 (`PXBuildingUtils.GetRandomBuildingOfTypeFromCity` (`PXNationUtils.GetPlayerMainCity`) (`self.Building Type`)))
      (`/Game/Scenarios/Shared/BlueprintsNonSerialized/SocietyUtils/BPFL_Communication_Utils.Pick Barks with Generated Speaker` _returnvalue _returnvalue false (`self.Get message defines`) "/Game/Scenarios/Shared/Configs/Messages/Barks/Other/WasteManagement/DA_WasteRepurposing_Consequence_BarkSet.DA_WasteRepurposing_Consequence_BarkSet" (`PXBuildingComponent.OwningDistrict` _returnvalue_2)))))