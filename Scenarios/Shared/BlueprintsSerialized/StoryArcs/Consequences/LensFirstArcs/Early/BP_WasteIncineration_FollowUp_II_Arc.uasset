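; Story arc for the second follow-up in the waste incineration consequence chain, startable only while the player's main city has a building of the given type.
; It sends a random follow-up lens message tied to the district of a random such building, with the building name as text, and waits for any choice.
; It then removes that lens from the pool and starts the third follow-up arc, passing on the building type and remaining lenses.
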(event `self.OnStarted`
  (bind _returnvalue (`PXBuildingUtils.GetRandomBuildingOfTypeFromCity` (`PXNationUtils.GetPlayerMainCity`) (`self.Building Type`)))
  (set `self.Follow Up Lens to Fire` (`PXRandomLibrary.PXArrayRandom` (`self.Follow Up Lenses`)))
  (bind _decision (`/Game/Scenarios/Shared/BlueprintsNonSerialized/SocietyUtils/BPFL_Communication_Utils.Send Config Message` (`self.Follow Up Lens to Fire`) (`PXBuildingComponent.OwningDistrict` _returnvalue) null null (`|MakeMap` "BUILDING" (`PXBuildingType.IngameName` (`self.Building Type`)))))
  (`PXAsyncWaitForAnyChoice.AsyncAction_WaitForAnyChoice` _decision
    (:`Completed`
      (`KismetArrayLibrary.Array_RemoveItem` (`self.Follow Up Lenses`) (`self.Follow Up Lens to Fire`))
      (bind _returnvalue_2 (`|GenericCreateObject` (subsystem `PXStoryArcSubsystem`) "/Game/Scenarios/Shared/BlueprintsSerialized/StoryArcs/Consequences/LensFirstArcs/Early/BP_WasteIncineration_FollowUp_III_Arc.BP_WasteIncineration_FollowUp_III_Arc_C" (`self.Building Type`) (`self.Follow Up Lenses`)))
      (`PXStoryUtils.StartParameterizedStoryArc` _returnvalue_2))))

(fn `CanBeStarted`
  (returns (ReturnValue :type Boolean))
  (return (`PXBuildingUtils.HasBuildingOfTypeInCity` (`PXNationUtils.GetPlayerMainCity`) (`self.Building Type`))))