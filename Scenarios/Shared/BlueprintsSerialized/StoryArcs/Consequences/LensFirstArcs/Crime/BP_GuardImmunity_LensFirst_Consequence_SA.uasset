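; Story arc Blueprint for a lens-first crime consequence concerning guard immunity, tied to a faction with affinity.
; It can start only when the parent check passes and such a faction exists.
; It extends the parent's message defines with a REASON_FACTION entry holding that faction's in-game name, so messages can name it as the reason.
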(fn `CanBeStarted`
  (returns (ReturnValue :type Boolean))
  (bind _returnvalue (`parent.CanBeStarted`))
  (if _returnvalue
    (if (`.Exists` (`/Game/Scenarios/Shared/BlueprintsNonSerialized/SocietyUtils/BPFL_Cornerstone_Utils.Get Faction With Affinity` (struct :`Name` "Change")))
      (return true))))

(fn `Get message defines`
  (returns (Map :type "Map of String to Text"))
  (bind _defines_map_merged (`/Game/Scenarios/Shared/BlueprintsNonSerialized/SocietyUtils/BPFL_Communication_Utils.Merge Defines` (`parent.Get message defines`) (`|MakeMap` "REASON_FACTION" (`PXFactionUtils.GetFactionInGameName` (`/Game/Scenarios/Shared/BlueprintsNonSerialized/SocietyUtils/BPFL_Cornerstone_Utils.Get Faction With Affinity` (struct :`Name` "Change"))))))
  (return _defines_map_merged))