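; Lens-first consequence story arc for the experimental treatment disease scenario, following up on a player choice.
; When the first option is chosen, it waits for a story beat of the arc's beat type and lane, then checks whether the consequence can start.
; If so, it randomly sends either a good or bad small lens without community art, stores it as the second decision and waits for any choice on it.
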(event `self.Handle Choice`
  (params (Selection :type Integer))
  (bind (_beat_type _lane_type) (`self.Get Story Beat Types`))
  (if (== Selection 0)
    (`PXAsyncWaitForStoryBeat.AsyncAction_WaitForStoryBeat` _beat_type _lane_type
      (:`Completed`
        (bind _returnvalue (`self.Consequence CanBeStarted Core`))
        (if _returnvalue
          (bind _decision (`self.Send Lens` (select `bool` (`PXRandomLibrary.PXRandomBool`) :`false` (`self.Good SmallLens`) :`true` (`self.Bad SmallLens`))))
          (bind _output_get (set `self.Decision 2` _decision))
          (`PXAsyncWaitForAnyChoice.AsyncAction_WaitForAnyChoice` _output_get))))))