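; Story consequence arc that reacts to injury absence in the player's main city when an active production district is Cold or worse, outside the Nomads scenario.
; One choice starts a timed side quest to bring workplace heat up to a desired level; the other waits for a story beat slot, then sends a Ghost message.
; The quest's outcome activates a promise kept or broken trust modifier and opens the matching dialog.
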(event `self.Handle Choice`
  (params (Selection :type Integer))
  (bind (_beat_type _lane_type) (`self.Get Story Beat Types`))
  (switch `int` Selection
    (:`0`
      (bind _returnvalue (`PXQuestUtils.StartQuestInPlace` (`|FormatText` "Warm up workplaces") "" (`self.Duration`) "SideQuest" "DebugQuestName" true))
      (set `self.Warm Up Workplaces Quest` _returnvalue)
      (`PXQuestUtils.AddHeatLevelQuestObjective` (`self.Warm Up Workplaces Quest`) (`|FormatText` "Provide at least {HEAT} in all {EXTRACTION} and {PRODUCTION} in the City" (`PXHeatLevelType.IngameName` (`self.Desired Heat Level`)) (`PXDistrictType.IngameName` (`self.Extraction`)) (`PXDistrictType.IngameName` (`self.Production`))) "" (struct :`GameplayTags` (struct :`(TagName` "District.Extraction") :`(TagName` "District.Production"))) (`self.Desired Heat Level`) "GreaterThanOrEqualTo" false false (`PXNationUtils.GetPlayerMainCity`) false null))
    (:`1`
      (`PXAsyncWaitForStoryBeat.AsyncAction_WaitForStoryBeat` _beat_type _lane_type
        (:`Completed`
          (bind _decision (`/Game/Scenarios/Shared/BlueprintsNonSerialized/SocietyUtils/BPFL_Communication_Utils.Send Config Message` (`self.Ghost`) null null null (`/Game/Scenarios/Shared/BlueprintsNonSerialized/SocietyUtils/BPFL_Communication_Utils.Get Common Text Defines` null) null null (struct) true))
          (`PXAsyncWaitForAnyChoice.AsyncAction_WaitForAnyChoice` _decision))))))

(event `/Game/Scenarios/Shared/BlueprintsSerialized/StoryArcs/Consequences/BP_ConsequenceArc_Parent.OnFinished`
  (bind _warm_up_workplaces_quest (`self.Warm Up Workplaces Quest`))
  (`/Engine/EditorBlueprintResources/StandardMacros.IsValid` _warm_up_workplaces_quest
    (:`Is Valid`
      (bind _succeeded (`PXAsyncWaitForQuest.AsyncAction_WaitForQuest` _warm_up_workplaces_quest)
        (:`Completed`
          (if _succeeded
            (`PXPredefinedModifierUtils.SetPredefinedModifierActive` (`PXNationUtils.GetPlayerNation`) "/Game/Scenarios/Shared/BlueprintsSerialized/Quests/Demands/DA_PromiseKept_AllCommunitiesTrust.DA_PromiseKept_AllCommunitiesTrust" true)
            (`PXAsyncOpenPredefinedDialog.AsyncAction_OpenPredefinedDialog` (`self.Success Dialog`))
            (else
              (`PXPredefinedModifierUtils.SetPredefinedModifierActive` (`PXNationUtils.GetPlayerNation`) "/Game/Scenarios/Shared/BlueprintsSerialized/Quests/Demands/DA_PromiseBroken_AllCommunitiesTrust.DA_PromiseBroken_AllCommunitiesTrust" true)
              (`PXAsyncOpenPredefinedDialog.AsyncAction_OpenPredefinedDialog` (`self.Failed Dialog`)))))))))

(fn `CanBeStarted`
  (returns (ReturnValue :type Boolean))
  (locals (District :type "PXDistrictComponent Object Reference") (HeatLevel :type "PXHeatLevelComponent Object Reference"))
  (bind _returnvalue (`PXNationUtils.GetPlayerMainCity`))
  (if (not (`/Game/Scenarios/Main/BlueprintsNonSerialized/ScenarioFunctionLibrary/BPFL_S1_ScenarioFunctionLibrary.Is Nomads Scenario`))
    (if (> (`PXAbsenceUtils.GetCurrentWorkforceAbsenceInCity` _returnvalue "/Game/Scenarios/Shared/Configs/Absences/AbsenceTypes/DA_Injured_Absence.DA_Injured_Absence") 0)
      (for _array_element (`PXDistrictUtils.GetDistrictWithTagFromCity` _returnvalue (struct :`TagDictionary` (struct :`(TagName` "District.Production") :`(TagName` "District.Extraction")) :`QueryTokenStream` "(0,1,1,2,0,1)" :`AutoDescription` " ANY( District.Production, District.Extraction )") true)
        (set `local.District` _array_element)
        (set `local.HeatLevel` (`Actor.GetComponentByClass` (`ActorComponent.GetOwner` (`local.District`)) "/Script/Frostpunk2.PXHeatLevelComponent"))
        (if (`.ReturnValue` (`PXHeatManagementUtils.CompareHeatLevel` (`local.HeatLevel`) "LessThanOrEqualTo" "/Game/Scenarios/Shared/Configs/Heat/HeatLevels/DA_HeatLevel_3_Cold.DA_HeatLevel_3_Cold"))
          (set `self.District for Tracker` (`local.District`))
          (return true)))
      (return false))))

(fn `Get message defines`
  (returns (Map :type "Map of String to Text"))
  (bind _defines_map_merged (`/Game/Scenarios/Shared/BlueprintsNonSerialized/SocietyUtils/BPFL_Communication_Utils.Merge Defines` (`parent.Get message defines`) (`|MakeMap` "WEEKS" (`PXTextUtils.GameTimeToTextMostImportant` (`self.Duration`)))))
  (return _defines_map_merged))