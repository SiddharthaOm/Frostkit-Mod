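; A story arc consequence for catastrophic hunger in the city, gated on deaths from starvation.
; It can start only when the shared storage hunger death counter reaches a configured minimum and the parent start check passes.
; Its message defines extend the parent's with a burials sentence, picking harvesting wording when the burials policy or its fallback is active, otherwise ceremonial or no-rules wording.
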(fn `CanBeStarted`
  (returns (ReturnValue :type Boolean))
  (if (>= (`/Game/Scenarios/Shared/BlueprintsSerialized/VariableStorage/BP_SharedVariableStorage.CatastrophicHungerDeathTimeCount` (`/Game/Scenarios/Shared/BlueprintsNonSerialized/SocietyUtils/BPFL_SharedScenariosStorage.Get Shared Variable Storage`)) (`self.Catastrophic Hunger min death count`))
    (bind _returnvalue (`parent.CanBeStarted`))
    (return _returnvalue)))

(fn `Get Message Defines`
  (returns (`Defines Map` :type "Map of String to Text"))
  (`BlueprintMapLibrary.Map_Add` (`self.Defines Map`) "BURIALS" (select `bool` (`/Game/Scenarios/Shared/BlueprintsNonSerialized/Policies/BPFL_PolicyUtils.Policy or Fallback is Active` (`self.Burials Policy`)) :`false` (`|FormatText` "Ceremonial or no common rules sentence") :`true` (`|FormatText` "Harvesting burials sentence")))
  (bind _defines_map_merged (`/Game/Scenarios/Shared/BlueprintsNonSerialized/SocietyUtils/BPFL_Communication_Utils.Merge Defines` (`parent.Get Message Defines`) (`self.Defines Map`)))
  (return _defines_map_merged))