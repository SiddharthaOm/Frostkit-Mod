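; Story arc consequence that sends a city message when a main district's heat level drops.
; CanBeStarted caches each active main district's heat level and triggers on the first one found below its cached value.
; Seeing heat auto-allocation enabled on the generator sets a flag that blocks later triggering.
; OnStarted sends the configured message for that district, with lens and text defines, then waits for a choice.
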(event `self.OnStarted`
  (bind _decision (`/Game/Scenarios/Shared/BlueprintsNonSerialized/SocietyUtils/BPFL_Communication_Utils.Send Config Message` (`self.Lens`) (`self.District for Tracker`) null null (`/Game/Scenarios/Shared/BlueprintsNonSerialized/SocietyUtils/BPFL_Communication_Utils.Get Common Text Defines` null)))
  (bind _output_get (set `self.Decision` _decision))
  (bind _choice (`PXAsyncWaitForChoice.AsyncAction_WaitForChoice` _output_get)
    (:`Completed`
      (switch `int` _choice))))

(fn `CanBeStarted`
  (returns (ReturnValue :type Boolean))
  (locals (District :type "PXDistrictComponent Object Reference") (HeatLevel :type "PXHeatLevelComponent Object Reference"))
  (if (not (`PXHeatAllocationHolderComponent.AutoAllocate` (`Actor.GetComponentByClass` (`ActorComponent.GetOwner` (`PXGeneratorUtils.GetGeneratorFromCity` (`PXNationUtils.GetPlayerMainCity`))) "/Script/Frostpunk2.PXHeatAllocationHolderComponent")))
    (if (not (`self.Auto Allocate used`))
      (for _array_element (`PXDistrictUtils.GetDistrictWithTagFromCity` (`PXNationUtils.GetPlayerMainCity`) (struct :`TagDictionary` (struct :`(TagName` "District.Main") :`(TagName` "District.Hub")) :`QueryTokenStream` "(0,1,3,2,0,1)" :`AutoDescription` " NONE( District.Main, District.Hub )") true)
        (set `local.District` _array_element)
        (set `local.HeatLevel` (`Actor.GetComponentByClass` (`ActorComponent.GetOwner` (`local.District`)) "/Script/Frostpunk2.PXHeatLevelComponent"))
        (if (`BlueprintMapLibrary.Map_Contains` (`self.DistrictsHeatLevels`) (`local.District`))
          (if (`.ReturnValue` (`PXHeatManagementUtils.CompareHeatLevel` (`local.HeatLevel`) "LessThan" (`BlueprintMapLibrary.Map_Find` (`self.DistrictsHeatLevels`) (`local.District`))))
            (set `self.District for Tracker` (`local.District`))
            (return true)
            (else
              (`BlueprintMapLibrary.Map_Add` (`self.DistrictsHeatLevels`) (`local.District`) (`PXHeatLevelComponent.CurrentHeatLevel` (`local.HeatLevel`)))))
          (else
            (`BlueprintMapLibrary.Map_Add` (`self.DistrictsHeatLevels`) (`local.District`) (`PXHeatLevelComponent.CurrentHeatLevel` (`local.HeatLevel`))))))
      (return false))
    (else
      (set `self.Auto Allocate used` true))))