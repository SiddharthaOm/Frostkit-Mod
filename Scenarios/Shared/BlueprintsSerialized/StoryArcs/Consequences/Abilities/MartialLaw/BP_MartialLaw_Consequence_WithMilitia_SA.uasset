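; Story arc for a martial law consequence variant that requires an active stewards' militia policy (or fallback).
; CanBeStartedCore also requires a community in context and a fully opposite faction's community that has executed the StewardMilitia action, then defers to the parent; CanBeStarted always returns true.
; Text defines label that opposite community FACTION and the context community OPPOSITE_FACTION.
; District and context community come from the game context.
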(fn `CanBeStarted`
  (returns (ReturnValue :type Boolean))
  (return true))

(fn `CanBeStarted Core`
  (returns (ReturnValue :type Boolean))
  (bind (_community _isvalid) (`PXGameplayContextUtils.TryGetCommunityComponentFromGameContext` (`self.Game Context`)))
  (bind (_outfound _returnvalue) (`PXFactionUtils.GetCommunityFromFaction` (`/Game/Scenarios/Shared/BlueprintsNonSerialized/FactionEmergence/BPFL_FactionWarUtils.Get Fully Opposite Faction` (`PXCommunityComponent.GetFaction` _community))))
  (if (`/Game/Scenarios/Shared/BlueprintsNonSerialized/Policies/BPFL_PolicyUtils.Policy or Fallback is Active` (`self.Stewards Militia Policy`))
    (if _isvalid
      ;[1 1 1] Opposite Faction must be found
      (if _outfound
        ;[1 1 1] Must have recruited from opposite
        (if (`PXCommunityActionUtils.WasCommunityActionEverExecuted` (`self.Steward Militia`) _returnvalue)
          (bind _returnvalue_2 (`parent.CanBeStarted Core`))
          (return _returnvalue_2))))))

(fn `Get Context Community`
  (returns (`Optional Context Community` :type "PXCommunityComponent Object Reference"))
  (return (`PXGameplayContextUtils.TryGetCommunityComponentFromGameContext` (`self.Game Context`))))

(fn `Get Defines`
  (returns (Map :type "Map of String to Text"))
  (bind _community (`PXGameplayContextUtils.TryGetCommunityComponentFromGameContext` (`self.Game Context`)))
  (set `self.additional defines` (`|MakeMap` "OPPOSITE_FACTION" (`/Game/Scenarios/Shared/BlueprintsNonSerialized/Communities/BPFL_CommunityUtils.Get Community Name` _community) "FACTION" (`/Game/Scenarios/Shared/BlueprintsNonSerialized/Communities/BPFL_CommunityUtils.Get Community Name` (`.ReturnValue` (`PXFactionUtils.GetCommunityFromFaction` (`/Game/Scenarios/Shared/BlueprintsNonSerialized/FactionEmergence/BPFL_FactionWarUtils.Get Fully Opposite Faction` (`PXCommunityComponent.GetFaction` _community)))))))
  (bind _defines_map_merged (`/Game/Scenarios/Shared/BlueprintsNonSerialized/SocietyUtils/BPFL_Communication_Utils.Merge Defines` (`parent.Get Defines`) (`self.additional defines`)))
  (return _defines_map_merged))

(fn `Get District`
  (returns (`Optional District` :type "PXDistrictComponent Object Reference"))
  (return (`PXGameplayContextUtils.TryGetDistrictFromGameContext` (`self.Game Context`))))