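; Base story-arc consequence for martial law abilities that presents the player with a decision tied to a state of emergency ability.
; On start it sends a modal or regular lens message with the context's district, community and ability name, setting a wait duration in the non-modal case.
; It then awaits the choice asynchronously and passes it to HandleChoice, which has no branch logic here.
; The parameter hash derives from the selected message config.
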(event `self.OnStarted`
  (if (not (`self.Modal Lens?`))
    (set `self.Wait for Duration` (`self.Wait for Duration`)))
  (bind _decision (`/Game/Scenarios/Shared/BlueprintsNonSerialized/SocietyUtils/BPFL_Communication_Utils.Send Config Message` (`self.Get Message Config`) (`self.Get District`) (`self.Get Context Community`) null (`self.Get Defines`) null null (struct) true))
  (bind _output_get (set `self.Decision` _decision))
  (bind _choice (`PXAsyncWaitForChoice.AsyncAction_WaitForChoice` _output_get)
    (:`Completed`
      (bind _output_get_2 (set `self.Choice` _choice))
      (`self.Handle Choice` _output_get_2))))

(fn `CanBeStarted Core`
  (returns (ReturnValue :type Boolean))
  (bind _returnvalue (`parent.CanBeStarted Core`))
  (return _returnvalue))

(fn `Get Context Community`
  (returns (`Optional Context Community` :type "PXCommunityComponent Object Reference"))
  (return (`/Game/Scenarios/Shared/BlueprintsNonSerialized/SocietyUtils/BPFL_Communication_Utils.Get Best Community from Context` (`self.Game Context`))))

(fn `Get Defines`
  (returns (Map :type "Map of String to Text"))
  (return (`|MakeMap` "ABILITY" (`PXAbility.IngameName` (`self.State of Emergency Ability`)))))

(fn `Get District`
  (returns (`Optional District` :type "PXDistrictComponent Object Reference"))
  (return (`/Game/Scenarios/Shared/BlueprintsNonSerialized/SocietyUtils/BPFL_Communication_Utils.Get Best District from Context` (`self.Game Context`))))

(fn `Get Message Config`
  (returns (ReturnValue :type "PXCommunicationChannelMessage Soft Object Reference"))
  (return (select `bool` (`self.Modal Lens?`) :`false` (`self.Lens Config`) :`true` (`self.Modal Lens Config`) :!type "PXCommunicationChannelMessage Soft Object Reference")))

(fn `GetParametersHash`
  (returns (ReturnValue :type Integer))
  (return (`PXStoryUtils.GetHashForUObjectParameter` (`PXCommunicationChannelsUtils.ToObject` (`self.Get Message Config`)))))

(fn `Handle Choice`
  (params (Selection :type Integer))
  (switch `int` Selection))