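; Story arc ability that delivers the low-standing consequence of an abuse-promise quest for the abused community.
; On start it sends the configured lens with that community's art and in-game name as the faction text, then waits for the player's choice.
; It then resolves the community from its type and adds the abuse-promise imprint to it.
; It has no start conditions of its own.
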(event `self.OnStarted`
  (bind _abused_community (`self.Abused Community`))
  (bind _decision (`/Game/Scenarios/Shared/BlueprintsNonSerialized/SocietyUtils/BPFL_Communication_Utils.Send Lens With Community Art` (`self.AbusePromiseQuest Lens`) null _abused_community (`|MakeMap` "FACTION" (`PXCommunityType.IngameName` _abused_community))))
  (bind _output_get (set `self.Decision` _decision))
  (`PXAsyncWaitForChoice.AsyncAction_WaitForChoice` _output_get
    (:`Completed`
      (`PXCommunityUtils.AddImprint` (`.ReturnValue` (`PXCommunityUtils.GetCommunityOfCommunityType` (`self.Abused Community`))) (`self.AbusePromiseQuest Imprint`)))))

(fn `CanBeStarted`
  (returns (ReturnValue :type Boolean))
  (return true))