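; Exile the Weak story arc that offers a decision to make exiling the weakest part of the population a yearly event.
; It can start when an affinity commenter exists and the previously used exile ability has stayed inactive past a timer, which restarts while the ability is active.
; If the ability's requirements are met, it shows a modal lens; the first choice activates the city's cyclical event and posts a notification.
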(event `self.OnStarted`
  (bind (_returnvalue_visibilityrequirementsmet _returnvalue_requirementsmet) (break `PXAbilityState` (`PXAbilityUtils.GetActorAbilityState` (`ActorComponent.GetOwner` (`PXNationUtils.GetPlayerMainCity`)) (`self.Exile Ability`))))
  (if _returnvalue_requirementsmet
    (set `self.ExiletheWeak Modal Lens` "/Game/Scenarios/Shared/Configs/Messages/Lenses/Consequences/ConsequenceLenses/Survival/ExileTheWeak/DA_ExileTheWeak_LastUnused_Lens.DA_ExileTheWeak_LastUnused_Lens")
    (bind _decision (`/Game/Scenarios/Shared/BlueprintsNonSerialized/SocietyUtils/BPFL_Communication_Utils.Send Config Message` (`self.ExiletheWeak Modal Lens`) null null null (`self.Get Defines`) null null (struct) true))
    (bind _output_get (set `self.Decision` _decision))
    (bind _choice (`PXAsyncWaitForChoice.AsyncAction_WaitForChoice` _output_get)
      (:`Completed`
        (bind _output_get_2 (set `self.choice` _choice))
        (`self.Handle Choice` _output_get_2)))))

(fn `CanBeStarted Core`
  (returns (ReturnValue :type Boolean))
  (bind _exists (`/Game/Scenarios/Shared/BlueprintsNonSerialized/SocietyUtils/BPFL_Cornerstone_Utils.Get X Affinity Commenter` (struct :`Name` "Symbiosis") false))
  (if _exists
    (bind _returnvalue (`parent.CanBeStarted Core`))
    (if _returnvalue
      (if (`PXAbilityUtils.WasAbilityEverUsedInCity` (`PXNationUtils.GetPlayerMainCity`) (`self.Exile Ability`))
        (`self.Set Timer`)
        (if (`PXAbilityUtils.IsActorAbilityActive` (`ActorComponent.GetOwner` (`PXNationUtils.GetPlayerMainCity`)) (`self.Exile Ability`))
          (`self.Restart Timer`)
          (elif (`self.Timer has expired?` (`self.No Ability Duration`))
            (return true)
            (else
              (return false))))
        (else
          (return false)))
      (else
        (return false)))
    (else
      (return false))))

(fn `Handle Choice`
  (params (Selection :type Integer))
  (switch `int` Selection
    (:`0`
      (`PXCentralNotificationUtils.ShowCentralNotificationOfType` "PopulationChange" (`|FormatText` "Yearly Weak Examinations Instituted") (`|FormatText` "Every 52 weeks, the weakest {PERCENT} percent of your population will be exiled" (`KismetTextLibrary.AsPercent_Float` (`self.Percent to Exile Threshold`) "HalfToEven")))
      (`PXCyclicalEventUtils.SetCyclicalEventActiveInCity` (`self.Get city`) (`self.Cyclical Event`)))))