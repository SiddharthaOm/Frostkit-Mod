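; Parent story arc for "nasty faction" consequences, presenting the player with a choice message involving their highest- and lowest-standing factions.
; On start it finds both factions, builds a condemn desire against the least-liked one's community, and sends the configured message in the most-liked one's context.
; Faction and member names fill text defines, and the desire appears as informational on one choice.
; It awaits the player's choice, then calls HandleChoice, which is empty here.
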(event `self.OnStarted`
  (`self.Setup Players`)
  (`self.Make Desires`)
  (bind _decision (`self.Send Message`))
  (bind _output_get (set `self.Decision` _decision))
  (bind _choice (`PXAsyncWaitForChoice.AsyncAction_WaitForChoice` _output_get)
    (:`Completed`
      (bind _output_get_2 (set `self.Choice` _choice))
      (`self.Handle Choice` _output_get_2))))

(fn `Defines`
  (returns (Map :type "Map of String to Text"))
  (bind _faction_with_highest_relations (`self.Faction With Highest Relations`))
  (bind _faction_with_lowest_relations (`self.Faction With Lowest Relations`))
  (return (`|MakeMap` "LIKE_FACTION" (`PXFactionType.IngameName` _faction_with_highest_relations) "DISLIKE_FACTION" (`PXFactionType.IngameName` _faction_with_lowest_relations) "LIKE_FACTION_MALE_MEMBER" (`BlueprintMapLibrary.Map_Find` (`PXCommunityType.MemberNames` (`PXFactionUtils.GetCommunityTypeFromFaction` (`PXNationUtils.GetPlayerNation`) _faction_with_highest_relations)) "Masculine") "DISLIKE_FACTION_MALE_MEMBER" (`BlueprintMapLibrary.Map_Find` (`PXCommunityType.MemberNames` (`PXFactionUtils.GetCommunityTypeFromFaction` (`PXNationUtils.GetPlayerNation`) _faction_with_lowest_relations)) "Masculine"))))

(fn `Get Affected District`
  (returns (`Optional Affected District` :type "PXDistrictComponent Object Reference"))
  (return (`self.Optional Affected District`)))

(fn `Get Context Community`
  (returns (ReturnValue :type "PXCommunityComponent Object Reference"))
  (return (`.ReturnValue` (`PXFactionUtils.GetCommunityFromFaction` (`self.Faction With Highest Relations`)))))

(fn `Get Message`
  (returns (Message :type "PXCommunicationChannelMessage Soft Object Reference"))
  (return (`self.Message`)))

(fn `Handle Choice`
  (params (Selection :type Integer))
  (switch `int` Selection))

(fn `Informational Desires`
  (returns (ReturnValue :type "PXCommunicationChannelsDesiresPerChoiceArray Structure"))
  (return (`PXCommunicationChannelsUtils.CreateDesiresPerChoiceArray` (`|MakeArray` (make `PXCommunicationChannelsDesiresPerChoice` (`|MakeArray` (`self.Condemn Desire`)) 1 true)))))

(fn `Make Desires`
  (bind _returnvalue (`PXDesireUtils.MakeActionDesire` (`self.Condemn CA`) (`PXNationUtils.GetPlayerMainCity`) (`PXFactionUtils.GetCommunityTypeFromFaction` (`PXNationUtils.GetPlayerNation`) (`self.Faction With Lowest Relations`))))
  (set `self.Condemn Desire` _returnvalue))

(fn `Send Message`
  (returns (Decision :type "PXDecision Object Reference"))
  (bind _decision (`/Game/Scenarios/Shared/BlueprintsNonSerialized/SocietyUtils/BPFL_Communication_Utils.Send Config Message` (`self.Get Message`) (`self.Get Affected District`) (`self.Get Context Community`) null (`self.Defines`) null null (`self.Informational Desires`) true))
  (return _decision))

(fn `Setup Players`
  (set `self.Faction With Highest Relations` (`/Game/Scenarios/Shared/BlueprintsNonSerialized/FactionEmergence/BPFL_FactionWarUtils.Get Faction with Highest Standing`))
  (set `self.Faction With Lowest Relations` (`/Game/Scenarios/Shared/BlueprintsNonSerialized/FactionEmergence/BPFL_FactionWarUtils.Get Faction with Lowest Standing`)))