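; Parent Blueprint for ghost-only consequence story arcs, which present a ghost message to the player.
; On start it sends the GhostConfig message with text defines and a random housing district from the player's main city, then waits for any choice.
; The message is flagged to use the closest district instead of the specific one.
; CanBeStarted adds no conditions beyond the parent check.
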(event `self.OnStarted`
  (bind _decision (`/Game/Scenarios/Shared/BlueprintsNonSerialized/SocietyUtils/BPFL_Communication_Utils.Send Config Message` (`self.Get ghost config`) (`self.Get district for ghost tracker`) null null (`self.Get message defines`) null null (struct) true))
  (`PXAsyncWaitForAnyChoice.AsyncAction_WaitForAnyChoice` _decision))

(fn `CanBeStarted`
  (returns (ReturnValue :type Boolean))
  (bind _returnvalue (`parent.CanBeStarted`))
  (if _returnvalue
    (return true)))

(fn `Get district for ghost tracker`
  (returns (OutItem :type "PXDistrictComponent Object Reference"))
  (bind _returnvalue (`PXDistrictUtils.GetDistrictWithTagFromCity` (`PXNationUtils.GetPlayerMainCity`) (struct :`TagDictionary` (struct :`(TagName` "District.Housing")) :`QueryTokenStream` "(0,1,2,1,0)" :`AutoDescription` " ALL( District.Housing )")))
  (if (not (`KismetArrayLibrary.Array_IsEmpty` _returnvalue))
    (return (`PXRandomLibrary.PXArrayRandom` _returnvalue))))

(fn `Get ghost config`
  (returns (`Ghost config` :type "PXGhost Soft Object Reference"))
  (return (`self.Ghost config`)))