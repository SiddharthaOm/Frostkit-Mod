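; Ghost-only consequence story arc for the Mandatory School law, tracked on a housing district in the player's main city.
; It can start only if a housing district exists, the Family Apprenticeship ghost arc is neither active nor finished, and parent checks pass.
; It swaps to an after-chaos ghost config once the Children Chaos warning arc has finished, otherwise using the parent's.
; The ghost tracker targets a random housing district, active or not.
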(fn `Consequence CanBeStarted Core`
  (returns (ReturnValue :type Boolean))
  (if (`KismetArrayLibrary.Array_IsNotEmpty` (`PXDistrictUtils.GetDistrictWithTagFromCity` (`PXNationUtils.GetPlayerMainCity`) (struct :`TagDictionary` (struct :`(TagName` "District.Housing")) :`QueryTokenStream` "(0,1,2,1,0)" :`AutoDescription` " ALL( District.Housing )")))
    (if (not (or (`PXStoryUtils.IsAnyStoryArcOfClassInStatus` "/Game/Scenarios/Shared/BlueprintsSerialized/StoryArcs/Consequences/GhostOnlyArcs/StartingLaws/BP_FamilyApprenticeship_GhostOnly_ConsequenceArc.BP_FamilyApprenticeship_GhostOnly_ConsequenceArc_C" "Active") (`PXStoryUtils.IsAnyStoryArcOfClassInStatus` "/Game/Scenarios/Shared/BlueprintsSerialized/StoryArcs/Consequences/GhostOnlyArcs/StartingLaws/BP_FamilyApprenticeship_GhostOnly_ConsequenceArc.BP_FamilyApprenticeship_GhostOnly_ConsequenceArc_C" "Finished")))
      (bind _returnvalue (`parent.Consequence CanBeStarted Core`))
      (return _returnvalue)
      (else
        (return false)))))

(fn `Get district for ghost tracker`
  (returns (OutItem :type "PXDistrictComponent Object Reference"))
  (return (`PXRandomLibrary.PXArrayRandom` (`PXDistrictUtils.GetDistrictWithTagFromCity` (`PXNationUtils.GetPlayerMainCity`) (struct :`TagDictionary` (struct :`(TagName` "District.Housing")) :`QueryTokenStream` "(0,1,2,1,0)" :`AutoDescription` " ALL( District.Housing )")))))

(fn `Get ghost config`
  (returns (`Ghost config` :type "PXGhost Soft Object Reference"))
  (if (`PXStoryUtils.IsAnyStoryArcOfClassInStatus` "/Game/Scenarios/Shared/BlueprintsSerialized/StoryArcs/Consequences/ChaosConsequences/Children/BP_ChildrenChaos_WarningGhost_Consequence_SA.BP_ChildrenChaos_WarningGhost_Consequence_SA_C" "Finished")
    (return (`self.After Chaos Ghost`))
    (else
      (return (`parent.Get ghost config`)))))