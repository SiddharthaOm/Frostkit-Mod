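; Ghost consequence story arc for cold work districts, defining only the condition under which it can start.
; On top of the parent check, it needs enough active efficiency-tagged districts in the player's main city at Very Cold or below.
; Active housing districts at Chilly or below must not exceed the NoColdHousings limit.
; It is also blocked while the sibling cold-housing ghost arc is active or once that arc has finished.
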(fn `CanBeStarted`
  (returns (ReturnValue :type Boolean))
  (locals (`Minimal number or work districts below temperature level` :type Integer :default 5) (`No cold Housings` :type Integer))
  (bind _returnvalue (`parent.CanBeStarted`))
  (if _returnvalue
    (if (and (>= (`KismetArrayLibrary.Array_Length` (`PXDistrictUtils.FilterDistrictsByHeatLevel` (`PXDistrictUtils.GetDistrictWithTagFromCity` (`PXNationUtils.GetPlayerMainCity`) (struct :`TagDictionary` (struct :`(TagName` "District.HasEfficiency")) :`QueryTokenStream` "(0,1,1,1,0)" :`AutoDescription` " ANY( District.HasEfficiency )") true) null "/Game/Scenarios/Shared/Configs/Heat/HeatLevels/DA_HeatLevel_2_VeryCold.DA_HeatLevel_2_VeryCold")) (`local.Minimal number or work districts below temperature level`)) (<= (`KismetArrayLibrary.Array_Length` (`PXDistrictUtils.FilterDistrictsByHeatLevel` (`PXDistrictUtils.GetDistrictWithTagFromCity` (`PXNationUtils.GetPlayerMainCity`) (struct :`TagDictionary` (struct :`(TagName` "District.Housing")) :`QueryTokenStream` "(0,1,1,1,0)" :`AutoDescription` " ANY( District.Housing )") true) null "/Game/Scenarios/Shared/Configs/Heat/HeatLevels/DA_HeatLevel_4_Chilly.DA_HeatLevel_4_Chilly")) (`local.No cold Housings`)))
      (if (and (not (`PXStoryUtils.IsAnyStoryArcOfClassInStatus` "/Game/Scenarios/Shared/BlueprintsSerialized/StoryArcs/Consequences/GhostOnlyArcs/Other/BP_Cold_HousingDistricts_Ghost_ConsequenceArc.BP_Cold_HousingDistricts_Ghost_ConsequenceArc_C" "Active")) (not (`PXStoryUtils.IsAnyStoryArcOfClassInStatus` "/Game/Scenarios/Shared/BlueprintsSerialized/StoryArcs/Consequences/GhostOnlyArcs/Other/BP_Cold_HousingDistricts_Ghost_ConsequenceArc.BP_Cold_HousingDistricts_Ghost_ConsequenceArc_C" "Finished")))
        (return true)
        (else
          (return false)))
      (else
        (return false)))))