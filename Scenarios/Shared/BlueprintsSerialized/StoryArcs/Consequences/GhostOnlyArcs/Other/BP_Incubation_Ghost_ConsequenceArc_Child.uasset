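; Ghost-only consequence arc for Incubation (child variant) that fills the story message with text reflecting the city's Parenthood policy.
; GetMessageDefines picks a PROFESSION by policy tag and a CONCLUSION from the active policy's text, with an unregulated fallback, then merges both into the parent's defines.
; GetNamesOfChildren supplies four first names from ghost speakers of random main-city communities for the conclusion.
; An older block adding those names as separate defines is left disconnected.
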(fn `Get message defines`
  (returns (Map :type "Map of String to Text"))
  (bind (_name1 _name2 _name3 _name4) (`self.Get Names of Children`))
  (bind (_value _returnvalue) (`BlueprintMapLibrary.Map_Find` (`self.Parenthood To Text`) (`/Game/Scenarios/Shared/BlueprintsNonSerialized/Policies/BPFL_PolicyUtils.Get Active Policy for Policy Law` (`self.Parenthood Policy`))))
  (bind _returnvalue_2 (`/Game/Scenarios/Shared/BlueprintsNonSerialized/SocietyUtils/BPFL_StoryArc_Utils.Get Parenthood Based On Policy Tag` "Welder" "Office Clerk" "Childbearer"))
  (`BlueprintMapLibrary.Map_Add` (`self.Local Defines Map`) "PROFESSION" _returnvalue_2)
  (if _returnvalue
    (`BlueprintMapLibrary.Map_Add` (`self.Local Defines Map`) "CONCLUSION" (`|FormatText` _value _name1 _name2 _name3 _name4))
    (else
      (`BlueprintMapLibrary.Map_Add` (`self.Local Defines Map`) "CONCLUSION" "Incubation Housed Ghost Unregulated Conclusion")))
  (bind _defines_map_merged (`/Game/Scenarios/Shared/BlueprintsNonSerialized/SocietyUtils/BPFL_Communication_Utils.Merge Defines` (`parent.Get message defines`) (`self.Local Defines Map`)))
  (return _defines_map_merged))

(fn `Get Names of Children`
  (returns (NAME1 :type Text) (NAME2 :type Text) (NAME3 :type Text) (NAME4 :type Text))
  (return (`.first name1` (`/Game/Scenarios/Shared/BlueprintsNonSerialized/FactionEmergence/BPFL_FactionEmergenceUtils.Get Community Ghost Speaker` (`PXCommunityComponent.GetCommunityType` (`PXCityUtils.GetRandomCommunityFromCity` (`PXNationUtils.GetPlayerMainCity`))))) (`.first name1` (`/Game/Scenarios/Shared/BlueprintsNonSerialized/FactionEmergence/BPFL_FactionEmergenceUtils.Get Community Ghost Speaker` (`PXCommunityComponent.GetCommunityType` (`PXCityUtils.GetRandomCommunityFromCity` (`PXNationUtils.GetPlayerMainCity`))))) (`.first name1` (`/Game/Scenarios/Shared/BlueprintsNonSerialized/FactionEmergence/BPFL_FactionEmergenceUtils.Get Community Ghost Speaker` (`PXCommunityComponent.GetCommunityType` (`PXCityUtils.GetRandomCommunityFromCity` (`PXNationUtils.GetPlayerMainCity`))))) (`.first name1` (`/Game/Scenarios/Shared/BlueprintsNonSerialized/FactionEmergence/BPFL_FactionEmergenceUtils.Get Community Ghost Speaker` (`PXCommunityComponent.GetCommunityType` (`PXCityUtils.GetRandomCommunityFromCity` (`PXNationUtils.GetPlayerMainCity`)))))))