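; Story arc that confronts the player with a faction community's reaction to research abuse, as a lens with community art and three choices.
; It starts only if the AbuseResearch scenario script finds affinity bad enough and the recent research actionable, latching off once research is not actionable.
; It builds follow-up research and condemn desires for the lens.
; Choices disable the community's research relations boost, promise the research, or reset the faction-member removal cooldown.
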(event `self.OnStarted`
  (bind _researchcommunity (`self.ResearchCommunity`))
  (`self.Make Desires`)
  (bind _decision (`/Game/Scenarios/Shared/BlueprintsNonSerialized/SocietyUtils/BPFL_Communication_Utils.Send Lens With Community Art` (`self.AbuseResearchLens`) null (`PXCommunityComponent.GetCommunityType` _researchcommunity) (`|MakeMap` "{COMMUNITY}" (`/Game/Scenarios/Shared/BlueprintsNonSerialized/Communities/BPFL_CommunityUtils.Get Community Name` _researchcommunity)) (struct) (`self.Make Desires per choice`)))
  (bind _choice (`PXAsyncWaitForChoice.AsyncAction_WaitForChoice` _decision)
    (:`Completed`
      (set `self.Choice` _choice)
      (switch `int` (`self.Choice`)
        (:`0`
          (bind _returnvalue (`PXScenarioScriptSubsystem.FindScenarioScript` (subsystem `PXScenarioScriptSubsystem`) (`self.Abuse Research Script`))
            (:`Found`
              (`BlueprintMapLibrary.Map_Add` (`/Game/Scenarios/Shared/BlueprintsSerialized/ScenarioScripts/BP_AbuseResearch_Script.Research Relations Boost Disabled` _returnvalue) (`self.ResearchCommunity`) true))))
        (:`1`
          (`PXDesireUtils.MakePromise` (`PXCommunityComponent.GetCommunityType` (`self.ResearchCommunity`)) (`self.Research Desire`) (make `PXPromiseQuestParameters` false (struct :`ScaledTicks` 84000))))
        (:`2`
          (`PXCommunityActionUtils.ResetCooldown` "/Game/Scenarios/Shared/Configs/Communities/CommunityActions/Relations_Group/RemoveFactionMembers/DA_RemoveFactionMembers_CA.DA_RemoveFactionMembers_CA" (`self.ResearchCommunity`)))))))

(fn `CanBeStarted`
  (returns (ReturnValue :type Boolean))
  (if (not (`self.Research Was Ever Not Actionable?`))
    (bind _returnvalue (`PXScenarioScriptSubsystem.FindScenarioScript` (subsystem `PXScenarioScriptSubsystem`) (`self.Abuse Research Script`))
      (:`Found`
        (if (`/Game/Scenarios/Shared/BlueprintsSerialized/ScenarioScripts/BP_AbuseResearch_Script.Is Affinity Bad Enough` _returnvalue (`self.ResearchCommunity`))
          (if (`/Game/Scenarios/Shared/BlueprintsSerialized/ScenarioScripts/BP_AbuseResearch_Script.Actionable Research` _returnvalue (`self.MostRecentResearch`))
            (return true)
            (else
              (set `self.Research Was Ever Not Actionable?` true)
              (return false)))
          (else
            (return false))))
      (:`NotFound`
        (return false)))))

(fn `GetParametersHash`
  (returns (ReturnValue :type Integer))
  (return (`PXStoryUtils.GetHashForUObjectParameter` (`|ConvertAsset` (`self.AbuseResearchLens`)))))

(fn `Make Desires`
  (bind _researchcommunity (`self.ResearchCommunity`))
  (bind _returnvalue (`PXDesireUtils.MakeResearchOutcomeDesire` (`self.MostRecentResearch`) true))
  (set `self.Research Desire` (`PXDesireUtils.GetFollowupDesire` _returnvalue))
  (set `/Game/Scenarios/Shared/BlueprintsSerialized/VariableStorage/BP_SharedVariableStorage.AbuseResearchDesire` (`self.Research Desire`) (`/Game/Scenarios/Shared/BlueprintsNonSerialized/SocietyUtils/BPFL_SharedScenariosStorage.Get Shared Variable Storage`))
  (bind _returnvalue_2 (`PXDesireUtils.MakeActionDesire` "/Game/Scenarios/Shared/Configs/Communities/CommunityActions/Relations_Group/RemoveFactionMembers/DA_RemoveFactionMembers_CA.DA_RemoveFactionMembers_CA" (`PXCommunityComponent.ParentCity` _researchcommunity) (`PXCommunityComponent.GetCommunityType` _researchcommunity)))
  (set `self.Condemn Desire` _returnvalue_2))

(fn `Make Desires per choice`
  (returns (PXCommunicationChannelsDesiresPerChoiceArray :type "PXCommunicationChannelsDesiresPerChoiceArray Structure"))
  (return (make `PXCommunicationChannelsDesiresPerChoiceArray` (`|MakeArray` (make `PXCommunicationChannelsDesiresPerChoice` (`|MakeArray` (`self.Research Desire`)) 1) (make `PXCommunicationChannelsDesiresPerChoice` (`|MakeArray` (`self.Condemn Desire`)) 2)))))