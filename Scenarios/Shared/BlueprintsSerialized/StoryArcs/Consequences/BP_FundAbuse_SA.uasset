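; Story arc consequence in which a repeatedly funded community presents the player with a three-choice lens, keyed to show once per community.
; It finds an opposing faction or affinity community for the lens text and context, and builds action desires.
; Choices promise the community's desires, promise increased funding with a cooldown reset, or promise nothing.
; The funding imprint is added beforehand for the choice's economic layout, then removed unless funding is chosen.
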(event `self.OnStarted`
  (bind (_result _result2) (`self.Funding Increase Success Modal Text`))
  (bind (_result_2 _result2_2) (`self.Funding Increase Fail Modal Text`))
  (bind _funded_community (`self.Funded Community`))
  (bind _output (`self.Get Opposite Community`))
  (set `self.opposite community` _output)
  (`self.Setup Desires`)
  ;[1 1 1] Adding imprint now so choice 1 economic layout will work
  (`PXCommunityUtils.AddImprint` (`self.Funded Community`) "/Game/Scenarios/Shared/Configs/Communities/Imprints/NarrativeBased/DA_FundAbuse_IncreaseFunding_Imprint.DA_FundAbuse_IncreaseFunding_Imprint")
  (bind _decision (`/Game/Scenarios/Shared/BlueprintsNonSerialized/SocietyUtils/BPFL_Communication_Utils.Send Lens With Community Art` (`self.Lens Config`) null (`PXCommunityComponent.GetCommunityType` _funded_community) (`self.Get Defines`) (`PXGameplayContextUtils.MakePXGameContext` _funded_community (`self.opposite community`)) (`self.Get Desires per Choice`)))
  (bind _choice (`PXAsyncWaitForChoice.AsyncAction_WaitForChoice` _decision)
    (:`Completed`
      (switch `int` _choice
        (:`0`
          (`PXCommunityUtils.RemoveImprint` (`self.Funded Community`) "/Game/Scenarios/Shared/Configs/Communities/Imprints/NarrativeBased/DA_FundAbuse_IncreaseFunding_Imprint.DA_FundAbuse_IncreaseFunding_Imprint")
          (`PXDesireUtils.MakeMultipleDesirePromise` (`PXCommunityComponent.GetCommunityType` (`self.Funded Community`)) (`self.Desires`) (make `PXPromiseQuestParameters` false (`self.Custom Parameters Quest Duration`) "/Game/Scenarios/Shared/BlueprintsSerialized/Quests/Demands/BP_DefaultMultipleDesiresPromise_Quest.BP_DefaultMultipleDesiresPromise_Quest_C")))
        (:`1`
          (`PXDesireUtils.MakePromise` (`PXCommunityComponent.GetCommunityType` (`self.Funded Community`)) (`self.Fund Projects Desire`) (make `PXPromiseQuestParameters` false (`self.Custom Parameters Quest Duration`) "/Script/Frostpunk2.PXPromiseQuest" (`|FormatText` "Double {COMMUNITY}' Funding" (`/Game/Scenarios/Shared/BlueprintsNonSerialized/Communities/BPFL_CommunityUtils.Get Community Name` (`self.Funded Community`))) _result _result2 _result_2 _result2_2))
          (`PXCommunityActionUtils.ResetCooldown` (`self.Fund Projects CA`) (`self.Funded Community`)))
        (:`2`
          (`PXCommunityUtils.RemoveImprint` (`self.Funded Community`) "/Game/Scenarios/Shared/Configs/Communities/Imprints/NarrativeBased/DA_FundAbuse_IncreaseFunding_Imprint.DA_FundAbuse_IncreaseFunding_Imprint"))))))

(fn `CanBeStarted`
  (returns (ReturnValue :type Boolean))
  (return true))

(fn `Funding Increase Fail Modal Text`
  (returns (Result :type Text) (Result2 :type Text))
  (bind _ingame_name (`/Game/Scenarios/Shared/BlueprintsNonSerialized/Communities/BPFL_CommunityUtils.Get Community Name` (`self.Funded Community`)))
  (return (`|FormatText` "{COMMUNITY} Miffed at Delay in Funding" _ingame_name) (`|FormatText` "The {COMMUNITY} are very upset you have not carried through on your vow to provide them with significantly increased fundings. \n \nHaving already drawn up plans on how to spend the funds, they will accept nothing less than the promised amount in the future." _ingame_name)))

(fn `Funding Increase Success Modal Text`
  (returns (Result :type Text) (Result2 :type Text))
  (bind _ingame_name (`/Game/Scenarios/Shared/BlueprintsNonSerialized/Communities/BPFL_CommunityUtils.Get Community Name` (`self.Funded Community`)))
  (return (`|FormatText` "{COMMUNITY} Accept Generous Donation" _ingame_name) (`|FormatText` "The {COMMUNITY} are very pleased you carried through on your vow to provide them with significantly increased fundings. \n \nThey are already cooking up new uses for the even greater levels of funding they expect to receive in the future." _ingame_name)))

(fn `Get Defines`
  (returns (Map :type "Map of String to Text"))
  (return (`|MakeMap` "COMMUNITY" (`/Game/Scenarios/Shared/BlueprintsNonSerialized/Communities/BPFL_CommunityUtils.Get Community Name` (`self.Funded Community`)) "THINGS" (`/Game/Scenarios/Shared/BlueprintsNonSerialized/SocietyUtils/BPFL_Quest_Utils.Desires Things Combined Text` (`self.Desires`)) "CUSTOM_PROJECTS_LINE" (`BlueprintMapLibrary.Map_Find` (`/Game/Scenarios/Shared/Configs/ConstantsStorage/BP_SharedConstantsStorageBaseClass.Custom Projects Line` (`/Game/Scenarios/Shared/BlueprintsNonSerialized/SocietyUtils/BPFL_SharedScenariosStorage.Get Current Scenario Constants Storage`)) (`PXCommunityComponent.GetCommunityType` (`self.Funded Community`))) "FUND_TIMES" (`KismetTextLibrary.Conv_IntToText` (`self.Times funded`)) "WEEKS" (`PXTextUtils.GameTimeToTextMostImportant` (`self.Custom Parameters Quest Duration`)) "OPPOSITE_COMMUNITY" (`/Game/Scenarios/Shared/BlueprintsNonSerialized/Communities/BPFL_CommunityUtils.Get Community Name` (`self.opposite community`)))))

(fn `Get Desires per Choice`
  (returns (PXCommunicationChannelsDesiresPerChoiceArray :type "PXCommunicationChannelsDesiresPerChoiceArray Structure"))
  (return (make `PXCommunicationChannelsDesiresPerChoiceArray` (`|MakeArray` (make `PXCommunicationChannelsDesiresPerChoice` (`self.Desires`)) (make `PXCommunicationChannelsDesiresPerChoice` (`|MakeArray` (`self.Fund Projects Desire`)) 1) :!type "PXCommunicationChannelsDesiresPerChoice Structure"))))

(fn `Get Opposite Community`
  (returns (Output :type "PXCommunityComponent Object Reference"))
  (bind _funded_community (`self.Funded Community`))
  (if (`PXCommunityComponent.IsFactionMember` _funded_community)
    (bind _community (`PXFactionUtils.FindExistingOpposingFaction` (`PXCommunityComponent.GetFaction` _funded_community) (`PXNationUtils.GetPlayerMainCity`)))
    (return _community)
    (else
      (bind _communities_with_affinity (`/Game/Scenarios/Shared/BlueprintsNonSerialized/SocietyUtils/BPFL_Cornerstone_Utils.Get Communites With Opposite Affinity` (`PXNationUtils.GetPlayerMainCity`) (`PXCommunityUtils.GetCommunityCoreAffinities` (`self.Funded Community`))))
      (if (`KismetArrayLibrary.Array_IsNotEmpty` _communities_with_affinity)
        (return (`|GetArrayItem` _communities_with_affinity))
        (else
          (bind _communities_with_affinity_2 (`/Game/Scenarios/Shared/BlueprintsNonSerialized/SocietyUtils/BPFL_Cornerstone_Utils.Get Communites Without Affinity` (`PXNationUtils.GetPlayerMainCity`) (`PXCommunityUtils.GetCommunityCoreAffinities` (`self.Funded Community`))))
          (return (`|GetArrayItem` _communities_with_affinity_2)))))))

(fn `GetParametersHash`
  (returns (ReturnValue :type Integer))
  (return (`PXStoryUtils.GetHashForUObjectParameter` (`self.Funded Community`))))

(fn `Setup Desires`
  (bind _funded_community (`self.Funded Community`))
  (bind _funded_community_2 (`self.Funded Community`))
  (bind _returnvalue (`PXDesireUtils.MakeActionDesire` (`self.Condemn CA`) (`PXCommunityComponent.ParentCity` _funded_community) (`PXCommunityComponent.GetCommunityType` _funded_community)))
  (set `self.Condemn Desire` _returnvalue)
  (bind _returnvalue_2 (`PXDesireUtils.MakeActionDesire` (`self.Fund Projects CA`) (`PXCommunityComponent.ParentCity` _funded_community_2) (`PXCommunityComponent.GetCommunityType` _funded_community_2)))
  (set `self.Fund Projects Desire` _returnvalue_2)
  (bind _returnvalue_3 (`PXDesireUtils.MakeActionDesire` (`self.Fund Projects CA`) (`PXNationUtils.GetPlayerMainCity`) (`PXCommunityComponent.GetCommunityType` (`self.opposite community`))))
  (set `self.fund opposite projects desire` _returnvalue_3))