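; Parent Blueprint for warning-ghost consequences in the unregulated chaos story arcs.
; On finish, it sets a follow-up policy in the player's fallback group and records the current week as the last warning ghost shown in shared storage.
; It then waits, ten weeks per its comment, before resetting the highest-priority arc to release priority.
; Its start check defers to the parent's condition.
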(event `self.OnFinished`
  (`parent.OnFinished`)
  (`PXPolicyUtils.SetCurrentPolicyInFallbackGroup` (`PXPolicyUtils.GetPlayerPolicy`) (`self.policy after ghost`))
  (set `/Game/Scenarios/Shared/BlueprintsSerialized/VariableStorage/BP_SharedVariableStorage.WeekLastChaosWarningGhostShown` (`PXTimeSubsystem.GetTotalWeeks` (`PXTimeUtils.GetCurrentGameTime`)) (`/Game/Scenarios/Shared/BlueprintsNonSerialized/SocietyUtils/BPFL_SharedScenariosStorage.Get Shared Variable Storage`))
  ;[1 1 1] Only release prio after 10 weeks
  (`PXAsyncWaitForDurationPassed.AsyncAction_WaitForDurationPassed` (struct :`ScaledTicks` 16800)
    (:`Completed`
      (set `/Game/Scenarios/Shared/BlueprintsSerialized/VariableStorage/BP_SharedVariableStorage.HighestPrioArc` -1 (`/Game/Scenarios/Shared/BlueprintsNonSerialized/SocietyUtils/BPFL_SharedScenariosStorage.Get Shared Variable Storage`)))))

(fn `CanBeStarted`
  (returns (ReturnValue :type Boolean))
  (bind _returnvalue (`parent.CanBeStarted`))
  (if _returnvalue
    (return true)))