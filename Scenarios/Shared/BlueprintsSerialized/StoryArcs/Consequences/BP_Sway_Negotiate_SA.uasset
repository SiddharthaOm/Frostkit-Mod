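; Story arc consequence where a community with granted agenda reacts to the player passing a law through negotiation or sway, ending in improved relations.
; CanBeStarted reads the latest filtered vote, requires a promise on a passed, requested session and non-positive community relations, then caches the result, law and community.
; OnStarted sends a ghost message worded by the tactics used, waits for any choice, then activates a relations modifier and notifies.
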(event `self.OnStarted`
  (bind (_outfound _returnvalue) (`PXCommunityUtils.GetCommunityOfCommunityType` (`self.Grant Agenda Community`)))
  (bind _decision (`/Game/Scenarios/Shared/BlueprintsNonSerialized/FactionEmergence/BPFL_FactionEmergenceUtils.Send Ghost with Affinity Art` (`self.Ghost to send`) null (`self.Grant Agenda Community`) (`|MakeMap` "COMMUNITY" (`PXCommunityType.IngameName` (`self.Grant Agenda Community`)) "REASON" (select `bool` (and (`self.Sway used`) (`self.Negotiate used`)) :`false` (select `bool` (`self.Sway used`) :`false` (`|FormatText` "making promises to convince some people") :`true` (`|FormatText` "using his authority to push others")) :`true` (`|FormatText` "making promises to convince some people and using his authority to push others")) "LAW" (`PXPolicyType.IngameName` (`self.Trigger Policy`))) "NewEnumerator0" true))
  (`PXAsyncWaitForAnyChoice.AsyncAction_WaitForAnyChoice` _decision
    (:`Completed`
      (`PXPredefinedModifierUtils.SetPredefinedModifierActiveManualTarget` (`PXNationUtils.GetPlayerNation`) "/Game/Scenarios/Shared/Configs/PredefinedModifiers/Consequences/DA_SwayNegotiate_Relations_PredefinedModifier.DA_SwayNegotiate_Relations_PredefinedModifier" (`ActorComponent.GetOwner` _returnvalue) true)
      (`/Game/Scenarios/Shared/BlueprintsNonSerialized/Communities/BPFL_CommunityUtils.DisplayCommunityNotification` _returnvalue "Relations Rises"))))

(fn `CanBeStarted`
  (returns (ReturnValue :type Boolean))
  (bind (_allitems _hasanyitem _latestitem) (`PXParliamentUtils.GetVotingHistory` :`parliament` (`PXParliamentUtils.GetCurrentParliament`) :`passFilter` "PassedOnly" :`promiseFilter` "PromiseForMadeOnly" :`swayFilter` "SwayForUsedOnly" :`recountFilter` "All"))
  (bind _grant_agenda_community (`/Game/Scenarios/Shared/BlueprintsSerialized/VariableStorage/BP_SharedVariableStorage.Grant Agenda Community` (`/Game/Scenarios/Shared/BlueprintsNonSerialized/SocietyUtils/BPFL_SharedScenariosStorage.Get Shared Variable Storage`)))
  (if (not (`self.Check passed`))
    (if (`.SwayUsed` (break `PXVotingHistoryItem` _latestitem))
      (set `self.Sway used` true))
    (if (`.AyePromiseMade` (break `PXVotingHistoryItem` _latestitem))
      (set `self.Negotiate used` true)
      (if (and (`.Passed` (break `PXVotingHistoryItem` _latestitem)) (`.SessionRequested` (break `PXVotingHistoryItem` _latestitem)) (or (`.SwayUsed` (break `PXVotingHistoryItem` _latestitem)) (`.AyePromiseMade` (break `PXVotingHistoryItem` _latestitem))))
        (if (`KismetSystemLibrary.IsValid` _grant_agenda_community)
          (switch `/Game/Scenarios/Shared/BlueprintsNonSerialized/SocietyUtils/E_CommunityRelationsZone` (`/Game/Scenarios/Shared/BlueprintsNonSerialized/SocietyUtils/BPFL_Trust_Utils.Get Community Relations Zone` (`.ReturnValue` (`PXCommunityUtils.GetCommunityOfCommunityType` _grant_agenda_community)))
            (:`NewEnumerator0`
              _)
            (:`NewEnumerator1`
              _)
            (:`NewEnumerator2`
              (return false)))
          (set `self.Check passed` true)
          (set `self.Trigger Policy` (`.Policy` (break `PXVotingHistoryItem` _latestitem)))
          (set `self.Grant Agenda Community` _grant_agenda_community)
          (else
            (return false)))
        (else
          (return false)))
      (else
        (return false))))
  (return true))