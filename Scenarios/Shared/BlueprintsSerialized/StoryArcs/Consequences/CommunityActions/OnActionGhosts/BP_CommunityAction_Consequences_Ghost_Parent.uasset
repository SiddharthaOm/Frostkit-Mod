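; Parent story arc for community consequence "ghosts": after a wait timer expires, it sends a configured message to a community and district.
; On start it resolves the community if unset, sends the message, waits for any choice, then removes an optional imprint and modifier.
; An empty SpecialEffects hook and config/define getters support child variants.
; Parameter comparison and hashing use the ghost config to identify equivalent arcs.
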(event `self.OnStarted`
  (bind _optional_imprint_to_remove (`self.Optional Imprint To Remove`))
  (bind _optional_modifier_to_remove (`self.Optional Modifier To Remove`))
  ;[1 1 1] Allow manual override of community
  (`/Engine/EditorBlueprintResources/StandardMacros.IsValid` (`self.Community Component`)
    (:`Is Valid`
      _)
    (:`Is Not Valid`
      (set `self.Community Component` (`PXGameplayContextUtils.TryGetCommunityComponentFromGameContext` (`self.Game Context`)))))
  (bind _decision (`/Game/Scenarios/Shared/BlueprintsNonSerialized/SocietyUtils/BPFL_Communication_Utils.Send Config Message` (`self.Get Ghost Config`) (`self.Optional District`) (`self.Community Component`) null (`self.Get Defines`) null null (struct) true))
  (`PXAsyncWaitForAnyChoice.AsyncAction_WaitForAnyChoice` _decision
    (:`Completed`
      (if (`KismetSystemLibrary.IsValid` _optional_imprint_to_remove)
        (`PXCommunityUtils.RemoveImprint` (`self.Community Component`) _optional_imprint_to_remove))
      (if (`KismetSystemLibrary.IsValid` _optional_modifier_to_remove)
        (`/Game/Scenarios/Shared/BlueprintsNonSerialized/SocietyUtils/BPFL_StoryArc_Utils.Remove Modifier` _optional_modifier_to_remove))
      (`self.Special Effects`))))

(fn `CanBeStarted_0`
  (returns (ReturnValue :type Boolean))
  (`self.Set Timer`)
  (if true
    (return (`self.Timer has expired?` (`self.Wait before Ghost`)))))

(fn `Get Defines`
  (returns (`Ghost Defines` :type "Map of String to Text"))
  (return (`self.Ghost Defines`)))

(fn `Get Ghost Config`
  (returns (Ghost :type "PXGhost Soft Object Reference"))
  (return (`self.Ghost`)))

(fn `GetParametersHash`
  (returns (ReturnValue :type Integer))
  (return (`PXStoryUtils.GetHashForUObjectParameter` (`PXCommunicationChannelsUtils.ToObject` (`self.Get Ghost Config`)))))

(fn `HasThisSameParameters`
  (params (selfPtr :type "PXParameterizedStoryArc Object Reference") (otherStoryArc :type "PXParameterizedStoryArc Object Reference"))
  (returns (ReturnValue :type Boolean))
  (bind _asbp_community_action_consequences_ghost_parent (cast `/Scenarios/Shared/BlueprintsSerialized/StoryArcs/Consequences/CommunityActions/OnActionGhosts/BP_CommunityAction_Consequences_Ghost_Parent` selfPtr))
  (bind _asbp_community_action_consequences_ghost_parent_2 (cast `/Scenarios/Shared/BlueprintsSerialized/StoryArcs/Consequences/CommunityActions/OnActionGhosts/BP_CommunityAction_Consequences_Ghost_Parent` otherStoryArc))
  (return (== (`self.Get Ghost Config` _asbp_community_action_consequences_ghost_parent) (`self.Get Ghost Config` _asbp_community_action_consequences_ghost_parent_2))))

(fn `Special Effects`)