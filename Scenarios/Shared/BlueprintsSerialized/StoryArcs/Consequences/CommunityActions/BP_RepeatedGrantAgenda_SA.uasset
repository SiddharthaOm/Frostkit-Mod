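; Story arc that follows a community's repeatedly failed Grant Agenda, provided that community still has a policy it wants.
; A lens offers a choice: promise a passed session vote as a timed quest, or activate the no-negotiation unlock.
; The promise enables a quest-tracking unlock and binds to parliament's vote-finished event.
; That community's granted vote decides the quest by Aye majority, with fallback success when the granted community has no policy left to table.
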(event `self.OnStarted`
  (bind _output_get (set `self.Community Grant Agenda Failed` (`/Game/Scenarios/Shared/BlueprintsSerialized/VariableStorage/BP_SharedVariableStorage.Community Grant Agenda Failed` (`/Game/Scenarios/Shared/BlueprintsNonSerialized/SocietyUtils/BPFL_SharedScenariosStorage.Get Shared Variable Storage`))))
  ;[1 1 1] Kill the arc if they have nothing they want. Putting it here and not in CBS to not kil perfo
  (bind (_policy_cache1 _has_valid_policy) (`/Game/Scenarios/Shared/BlueprintsNonSerialized/Policies/BPFL_PolicyUtils.Get Community Policy to Put On Agenda` _output_get))
  (if (or _has_valid_policy (`self.Has Valid Requested Policy` _output_get))
    (bind _returnvalue (`PXDesireUtils.MakeActionDesire` (`self.Grant Agenda CA`) (`PXNationUtils.GetPlayerMainCity`) (`self.Community Grant Agenda Failed`)))
    (set `self.Grant Agenda Desire` _returnvalue)
    (bind _decision (`/Game/Scenarios/Shared/BlueprintsNonSerialized/SocietyUtils/BPFL_Communication_Utils.Send Lens With Community Art` "/Game/Scenarios/Shared/Configs/Messages/Lenses/Consequences/ConsequenceLenses/Reactivity/DA_GranAgenedaRepeatedFail_Lens.DA_GranAgenedaRepeatedFail_Lens" null (`self.Community Grant Agenda Failed`) (`|MakeMap` "FACTION" (`PXCommunityType.IngameName` (`self.Community Grant Agenda Failed`)) "X" (`PXTextUtils.GameTimeToText` (`self.Quest Duration`) true false false false)) (struct) (`PXCommunicationChannelsUtils.CreateDesiresPerChoiceArray` (`|MakeArray` (make `PXCommunicationChannelsDesiresPerChoice` (`|MakeArray` (`self.Grant Agenda Desire`)) 0 true))) true))
    (bind _output_get_2 (set `self.Decision` _decision))
    (bind _choice (`PXAsyncWaitForChoice.AsyncAction_WaitForChoice` _output_get_2)
      (:`Completed`
        (set `self.Choice` _choice)
        (switch `int` (`self.Choice`)
          (:`0`
            (`PXUnlockUtils.SetUnlockActive` (`PXNationUtils.GetPlayerNation`) "/Game/Scenarios/Shared/Configs/Unlocks/ConsequenceArcs/DA_GrantAgendaQuestTrackingBlock_Unlock.DA_GrantAgendaQuestTrackingBlock_Unlock" true)
            (bind _returnvalue_2 (`PXDesireUtils.MakePromise` (`self.Community Grant Agenda Failed`) (`self.Grant Agenda Desire`) (make `PXPromiseQuestParameters` false (`self.Quest Duration`) "/Script/Frostpunk2.PXPromiseQuest" (`|FormatText` "Pass Granted Session Vote"))))
            (set `self.Quest` _returnvalue_2)
            (bind _returnvalue_3 (`PXQuest.AddQuestObjective` (`self.Quest`) (`|FormatText` "Make sure the vote passes") "" 0 1 false null "DebugObjectiveName"))
            (set `self.Law Objective` _returnvalue_3)
            (add `PXParliamentSubsystem.VoteFinishedEvent` (subsystem `PXParliamentSubsystem`) (`|CreateDelegate` :!event `Vote Finished Event`)))
          (:`1`
            (`PXUnlockUtils.SetUnlockActive` (`PXNationUtils.GetPlayerNation`) "/Game/Scenarios/Shared/Configs/Unlocks/ConsequenceArcs/DA_GrantAgendaNoNegotiation_Unlock.DA_GrantAgendaNoNegotiation_Unlock" true)))))))

(event `self.OnFinished`
  (`PXAsyncWaitForQuest.AsyncAction_WaitForQuest` (`self.Quest`)
    (:`Completed`
      (`PXUnlockUtils.SetUnlockActive` (`PXNationUtils.GetPlayerNation`) "/Game/Scenarios/Shared/Configs/Unlocks/ConsequenceArcs/DA_GrantAgendaQuestTrackingBlock_Unlock.DA_GrantAgendaQuestTrackingBlock_Unlock"))))

(fn `CanBeStarted`
  (returns (ReturnValue :type Boolean))
  (`/Engine/EditorBlueprintResources/StandardMacros.IsValid` (`/Game/Scenarios/Shared/BlueprintsSerialized/VariableStorage/BP_SharedVariableStorage.Community Grant Agenda Failed` (`/Game/Scenarios/Shared/BlueprintsNonSerialized/SocietyUtils/BPFL_SharedScenariosStorage.Get Shared Variable Storage`))
    (:`Is Valid`
      (return true))))

(fn `Has Valid Requested Policy`
  (params (Key :type "PXCommunityType Object Reference (by ref)"))
  (returns (ReturnValue :type Boolean))
  (bind (_value _returnvalue) (`BlueprintMapLibrary.Map_Find` (`/Game/Scenarios/Shared/BlueprintsSerialized/VariableStorage/BP_SharedVariableStorage.Community Preferred Policy` (`/Game/Scenarios/Shared/BlueprintsNonSerialized/SocietyUtils/BPFL_SharedScenariosStorage.Get Shared Variable Storage`)) Key))
  (if _returnvalue
    (return (not (`/Game/Scenarios/Shared/BlueprintsNonSerialized/Policies/BPFL_PolicyUtils.Policy or Fallback is Active` _value)))))

(fn `Vote Finished Event`
  (params (parliament :type "PXParliamentComponent Object Reference") (affectedPolicy :type "PXPolicyType Object Reference") (results :type "PXVoteResultData Structure"))
  (if (`/Game/Scenarios/Shared/BlueprintsSerialized/VariableStorage/BP_SharedVariableStorage.Grant Agenda Session` (`/Game/Scenarios/Shared/BlueprintsNonSerialized/SocietyUtils/BPFL_SharedScenariosStorage.Get Shared Variable Storage`))
    (if (== (`/Game/Scenarios/Shared/BlueprintsSerialized/VariableStorage/BP_SharedVariableStorage.Grant Agenda Community` (`/Game/Scenarios/Shared/BlueprintsNonSerialized/SocietyUtils/BPFL_SharedScenariosStorage.Get Shared Variable Storage`)) (`self.Community Grant Agenda Failed`))
      (if (>= results_AyeCount 51)
        (`PXQuestUtils.FinishQuest` (`self.Quest`) true)
        (else
          (`PXQuestUtils.FinishQuest` (`self.Quest`))))
      (set `/Game/Scenarios/Shared/BlueprintsSerialized/VariableStorage/BP_SharedVariableStorage.Grant Agenda Session` false (`/Game/Scenarios/Shared/BlueprintsNonSerialized/SocietyUtils/BPFL_SharedScenariosStorage.Get Shared Variable Storage`))
      (remove `PXParliamentSubsystem.VoteFinishedEvent` (subsystem `PXParliamentSubsystem`) (`|CreateDelegate` :!event `Vote Finished Event`))
      (else
        ;[1 1 1] Fallback to suceed quest if player manages to pass everything they want some other way
        (bind (_policy_cache1 _has_valid_policy) (`/Game/Scenarios/Shared/BlueprintsNonSerialized/Policies/BPFL_PolicyUtils.Get Community Policy to Put On Agenda` (`/Game/Scenarios/Shared/BlueprintsSerialized/VariableStorage/BP_SharedVariableStorage.Grant Agenda Community` (`/Game/Scenarios/Shared/BlueprintsNonSerialized/SocietyUtils/BPFL_SharedScenariosStorage.Get Shared Variable Storage`)) :!label _label))
        (if (not _has_valid_policy)
          (`PXQuestUtils.FinishQuest` (`self.Quest`) true))))
    (else
      (goto _label))))